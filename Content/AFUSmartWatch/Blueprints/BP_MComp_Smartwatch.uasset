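; BP_MComp_Smartwatch is a VR smartwatch component that spawns smart screens from widget commands and flips its handle for the left side.
; While attached, a spawn command creates the requested screen and snaps it to CompAnchor, first deleting any connected one; requesting the same class only removes it.
; Attach, detach and screen replacement swap the Huella fingerprint material to show state.
; An optional Tick interpolation keeps the actor upright.
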(event WidgetCommandServer(Comp_Widget)
  (params (Command :type Name :default "None") (Payload :type Struct%20Generic%20Payload%20Structure))
  (bind _output (Utilities|Array|Get(acopy) (.classes Payload)))
  (bind _comp_anchor (Variables|Default|GetComp_Anchor))
  (bind _connectedconnector (Variables|/Game/AFCore/Blueprints/Components/Snapping/Comp_Anchor.Comp_Anchor_C|GetConnectedConnector _comp_anchor))
  (bind _returnvalue (Components|GetOwner _connectedconnector))
  (if (Variables|Default|Getattached)
    (switch name Command
      (:SpawnSmartScreen
        (Utilities|IsValid _connectedconnector
          (:Is%20Valid
            (bind _out (CallFunction|SaveBool (== _output (Utilities|GetClass _returnvalue))))
            (CallFunction|DeleteActor _returnvalue "NewEnumerator1" false)
            (Utilities|FlowControl|Delay 1.0)
            (Rendering|Material|SetMaterial (Variables|Default|Gethuella) 0 "/Game/AFCore/Pawns/huellas1_verde.huellas1_verde")
            (Variables|Default|Setattached true)
            (if (not _out)
              (bind _asbp_smart_screen (Utilities|Casting|CastToBP_SmartScreenClass _output :!label _label))
              (bind _returnvalue_2 (Game|SpawnActorfromClass _asbp_smart_screen (Transformation|GetWorldTransform (Variables|Default|GetSmartScreenSpawnLocation)) "Undefined" "SelectDefaultAtRuntime" 0 (Variables|Default|GetVRPawn) 0))
              (Default|SnapConnectortoAnchor (Variables|Default|GetComp_Anchor) (Variables|/Game/AFUSmartWatch/Blueprints/BP_SmartScreen.BP_SmartScreen_C|GetComp_Connector_Anchor_Smartwatch _returnvalue_2))))
          (:Is%20Not%20Valid
            (goto _label)))))))

(event ActorGotDetached(Comp_Anchor)
  (params (Anchor :type Comp%20Anchor%20Object%20Reference) (Actor :type Actor%20Object%20Reference) (Connector :type Comp%20Connector%20Anchor%20Object%20Reference))
  (Variables|Default|Setattached false)
  (Rendering|Material|SetMaterial (Variables|Default|Gethuella) 0 "/Game/AFCore/Pawns/huellas1_roja.huellas1_roja"))

(event ActorGotAttached(Comp_Anchor)
  (params (Anchor :type Comp%20Anchor%20Object%20Reference) (Actor :type Actor%20Object%20Reference) (Connector :type Comp%20Connector%20Anchor%20Object%20Reference))
  (Variables|Default|Setattached true)
  (Rendering|Material|SetMaterial (Variables|Default|Gethuella) 0 "/Game/AFCore/Pawns/huellas.huellas"))

(event EventBeginPlay
  (|CallParentFunction) ; This node is disabled and will not be called.\nDrag off pins to build functionality.
)

(event Collision|EventActorBeginOverlap
  (params (OtherActor :type Actor%20Object%20Reference))
  (|CallParentFunction OtherActor) ; This node is disabled and will not be called.\nDrag off pins to build functionality.
)

(event EventTick
  (params (DeltaSeconds :type Float%20%28single-precision%29))
  (bind _returnvalue (Transformation|GetActorRotation))
  (|CallParentFunction DeltaSeconds)
  (if (Variables|Settings|GetShouldKeepUpright)
    (Transformation|SetActorRotation (Math|Interpolation|RInterpTo (Transformation|GetActorRotation) (Math|Rotator|MakeRotator 1.8e+02 (.pitch _returnvalue) (.yaw _returnvalue)) DeltaSeconds 1e+01))))

(event EventSetupMComp
  (switch Utilities|FlowControl|Switch|SwitchonEnum_Side (Variables|Default|GetSide)
    (:NewEnumerator0
      (Utilities|SetRelativeRotationZ (Variables|Default|GetHandle) 1.8e+02 false false))))

(fn ConstructionScript
  (|CallParentFunction))