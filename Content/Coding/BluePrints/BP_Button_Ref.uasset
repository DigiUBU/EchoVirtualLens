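; Reference button that spawns linked copies of the cube, sphere or cone attached to BP_PlatformRefValue onto an unoccupied BP_PlatformSpawn, up to a spawn limit.
; BeginPlay caches each shape's original as owner; copies get cables to a shape actor, and cube and cone copies also register with BP_Button_Copy.
; Tick mirrors the owner's scale, color and color-button visibility onto copies.
; ClearArrayCopy resets the count and hides non-owner shapes, disabling their collision.
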(event OnStateChanged(Comp_Switch)
  (params (SourceInfo :type Struct%20Component%20Source%20Info%20Structure) (Value :type Boolean))
  (bind _output_get (Variables|Default|Setpressed Value))
  (CallFunction|ColorActivation _output_get)
  (if _output_get
    (bind _returnvalue (Actor|GetActorOfClass "/Game/Coding/BluePrints/BP_PlatformSpawn.BP_PlatformSpawn_C"))
    (Utilities|FlowControl|Sequence
      (:then_0
        (if (Variables|Default|GetcanSpawn)
          (bind _returnvalue_2 (Actor|GetActorOfClass "/Game/Coding/BluePrints/BP_PlatformSpawn.BP_PlatformSpawn_C"))
          (bind _returnvalue_3 (Actor|GetActorOfClass "/Game/Coding/BluePrints/BP_PlatformRefValue.BP_PlatformRefValue_C"))
          (for _array_element (Actor|GetAttachedActors _returnvalue_3 true false)
            (switch string (Utilities|GetDisplayName _array_element)
              (:BP_CubeSynchro_1
                (if (not (Variables|/Game/Coding/BluePrints/BP_PlatformSpawn.BP_PlatformSpawn_C|Getoccupied _returnvalue))
                  (Utilities|FlowControl|DoOnce false
                    (:Completed
                      (Actor|GetActorOfClass "/Game/Coding/BluePrints/BP_CubeSynchro_1.BP_CubeSynchro_1_C")
                      (bind _returnvalue_4 (Game|SpawnActorfromClass "/Game/Coding/BluePrints/BP_CubeSynchro_1.BP_CubeSynchro_1_C" (Math|Transform|MakeTransform (Math|Vector|MakeVector (.x (Transformation|GetWorldLocation (Variables|/Game/Coding/BluePrints/BP_PlatformSpawn.BP_PlatformSpawn_C|GetArrow _returnvalue_2))) (.y (Transformation|GetWorldLocation (Variables|/Game/Coding/BluePrints/BP_PlatformSpawn.BP_PlatformSpawn_C|GetArrow _returnvalue_2))) (+ (.z (Transformation|GetWorldLocation (Variables|/Game/Coding/BluePrints/BP_PlatformSpawn.BP_PlatformSpawn_C|GetArrow _returnvalue_2))) 1e+01)) (Transformation|GetWorldRotation (Variables|/Game/Coding/BluePrints/BP_PlatformSpawn.BP_PlatformSpawn_C|GetArrow _returnvalue_2)) "1.000000,1.000000,1.000000") "Undefined" "MultiplyWithRoot" 0 0))
                      (Actor|SetOwner _returnvalue_4 (Variables|Default|GetownerCube))
                      (Variables|/Game/Coding/BluePrints/BP_CubeSynchro_1.BP_CubeSynchro_1_C|SetisReference _returnvalue_4 true)
                      (Utilities|Array|Add (Variables|Default|GetcubeSynchroRef) _returnvalue_4)
                      (CallFunction|SameasRefCube _returnvalue_4)
                      (bind _returnvalue_5 (Actor|GetActorOfClass "/Game/Coding/BluePrints/BP_Button_Copy.BP_Button_Copy_C"))
                      (Utilities|Array|Add (Variables|/Game/Coding/BluePrints/BP_Button_Copy.BP_Button_Copy_C|GetcubeSynchroCopy _returnvalue_5) _returnvalue_4)
                      (Math|Integer|IncrementInt (Variables|Default|GetcounterSpawn)
                        (:%20%20
                          (CallFunction|ReferenceCable (Utilities|GetDisplayName _array_element))))))))
              (:BP_SphereSynchro_1
                (if (not (Variables|/Game/Coding/BluePrints/BP_PlatformSpawn.BP_PlatformSpawn_C|Getoccupied _returnvalue))
                  (Utilities|FlowControl|DoOnce false
                    (:Completed
                      (bind _returnvalue_6 (Game|SpawnActorfromClass "/Game/Coding/BluePrints/BP_SphereSynchro_1.BP_SphereSynchro_1_C" (Math|Transform|MakeTransform (Math|Vector|MakeVector (.x (Transformation|GetWorldLocation (Variables|/Game/Coding/BluePrints/BP_PlatformSpawn.BP_PlatformSpawn_C|GetArrow _returnvalue_2))) (.y (Transformation|GetWorldLocation (Variables|/Game/Coding/BluePrints/BP_PlatformSpawn.BP_PlatformSpawn_C|GetArrow _returnvalue_2))) (+ (.z (Transformation|GetWorldLocation (Variables|/Game/Coding/BluePrints/BP_PlatformSpawn.BP_PlatformSpawn_C|GetArrow _returnvalue_2))) 1e+01)) (Transformation|GetWorldRotation (Variables|/Game/Coding/BluePrints/BP_PlatformSpawn.BP_PlatformSpawn_C|GetArrow _returnvalue_2)) "1.000000,1.000000,1.000000") "Undefined" "MultiplyWithRoot" 0 0))
                      (Actor|SetOwner _returnvalue_6 (Variables|Default|GetownerSphere))
                      (Variables|/Game/Coding/BluePrints/BP_SphereSynchro_1.BP_SphereSynchro_1_C|SetisReference _returnvalue_6 true)
                      (Utilities|Array|Add (Variables|Default|GetsphereSynchroRef) _returnvalue_6)
                      (CallFunction|SameasRefSphere _returnvalue_6)
                      (Math|Integer|IncrementInt (Variables|Default|GetcounterSpawn)
                        (:%20%20
                          (CallFunction|ReferenceCable (Utilities|GetDisplayName _array_element))))))))
              (:BP_ConeSynchro_1
                (if (not (Variables|/Game/Coding/BluePrints/BP_PlatformSpawn.BP_PlatformSpawn_C|Getoccupied _returnvalue))
                  (Utilities|FlowControl|DoOnce false
                    (:Completed
                      (bind _returnvalue_7 (Game|SpawnActorfromClass "/Game/Coding/BluePrints/BP_ConeSynchro_1.BP_ConeSynchro_1_C" (Math|Transform|MakeTransform (Math|Vector|MakeVector (.x (Transformation|GetWorldLocation (Variables|/Game/Coding/BluePrints/BP_PlatformSpawn.BP_PlatformSpawn_C|GetArrow _returnvalue_2))) (.y (Transformation|GetWorldLocation (Variables|/Game/Coding/BluePrints/BP_PlatformSpawn.BP_PlatformSpawn_C|GetArrow _returnvalue_2))) (+ (.z (Transformation|GetWorldLocation (Variables|/Game/Coding/BluePrints/BP_PlatformSpawn.BP_PlatformSpawn_C|GetArrow _returnvalue_2))) 1e+01)) (Transformation|GetWorldRotation (Variables|/Game/Coding/BluePrints/BP_PlatformSpawn.BP_PlatformSpawn_C|GetArrow _returnvalue_2)) "1.000000,1.000000,1.000000") "Undefined" "MultiplyWithRoot" 0 0))
                      (Actor|SetOwner _returnvalue_7 (Variables|Default|GetownerCone))
                      (Variables|/Game/Coding/BluePrints/BP_ConeSynchro_1.BP_ConeSynchro_1_C|SetisReference _returnvalue_7 true)
                      (Utilities|Array|Add (Variables|Default|GetconeSynchroRef) _returnvalue_7)
                      (CallFunction|SameasRefCone _returnvalue_7)
                      (bind _returnvalue_8 (Actor|GetActorOfClass "/Game/Coding/BluePrints/BP_Button_Copy.BP_Button_Copy_C"))
                      (Utilities|Array|Add (Variables|/Game/Coding/BluePrints/BP_Button_Copy.BP_Button_Copy_C|GetconeSynchroCopy _returnvalue_8) _returnvalue_7)
                      (Math|Integer|IncrementInt (Variables|Default|GetcounterSpawn)
                        (:%20%20
                          (CallFunction|ReferenceCable (Utilities|GetDisplayName _array_element))))))))))
          (Utilities|FlowControl|Sequence
            (:then_0
              (Utilities|FlowControl|DoOnce false) ; enters at Reset
            )
            (:then_1
              (Utilities|FlowControl|DoOnce false) ; enters at Reset
            )
            (:then_2
              (Utilities|FlowControl|DoOnce false) ; enters at Reset
            ))))
      (:then_1
        (Utilities|FlowControl|Delay 1.0)
        (Default|Toggle (Variables|Default|GetComp_Switch))))))

(event Custom|ColorActivation
  (params (activate :type Boolean))
  (bind _mesh_button_frame (Variables|Default|GetMesh_Button_Frame))
  (bind _returnvalue (Rendering|Material|CreateDynamicMaterialInstance _mesh_button_frame 0 (Rendering|Material|GetMaterial _mesh_button_frame 0) "None" :!class /Script/Engine.PrimitiveComponent))
  (if activate
    (Rendering|Material|SetScalarParameterValue _returnvalue "Bright" 1.0 :!class /Script/Engine.MaterialInstanceDynamic)
    (else
      (Rendering|Material|SetScalarParameterValue _returnvalue "Bright" 0.0 :!class /Script/Engine.MaterialInstanceDynamic))))

(event Custom|ClearArrayCopy
  (bind _ownercube (Variables|Default|GetownerCube))
  (bind _ownercone (Variables|Default|GetownerCone))
  (bind _ownersphere (Variables|Default|GetownerSphere))
  (Variables|Default|SetcounterSpawn 0)
  (Utilities|FlowControl|Sequence
    (:then_0
      (for _array_element (Variables|Default|GetcubeSynchroRef)
        (if (!= _array_element _ownercube)
          _))
      (Variables|Default|SetcanSpawn true)
      (bind _outactors (Actor|GetAllActorsOfClass "/Game/Coding/BluePrints/BP_CubeSynchro_1.BP_CubeSynchro_1_C"))
      (for _array_element_2 _outactors
        (if (!= _array_element_2 _ownercube)
          (Collision|SetActorEnableCollision _array_element_2 false)
          (Rendering|SetActorHiddenInGame _array_element_2 true))))
    (:then_1
      (for _array_element_3 (Variables|Default|GetsphereSynchroRef)
        (if (!= _array_element_3 _ownersphere)
          _))
      (bind _outactors_2 (Actor|GetAllActorsOfClass "/Game/Coding/BluePrints/BP_SphereSynchro_1.BP_SphereSynchro_1_C"))
      (for _array_element_4 _outactors_2
        (if (!= _array_element_4 _ownersphere)
          (Collision|SetActorEnableCollision _array_element_4 false)
          (Rendering|SetActorHiddenInGame _array_element_4 true))))
    (:then_2
      (for _array_element_5 (Variables|Default|GetconeSynchroRef)
        (if (!= _array_element_5 _ownercone)
          _))
      (bind _outactors_3 (Actor|GetAllActorsOfClass "/Game/Coding/BluePrints/BP_ConeSynchro_1.BP_ConeSynchro_1_C"))
      (for _array_element_6 _outactors_3
        (if (!= _array_element_6 _ownercone)
          (Collision|SetActorEnableCollision _array_element_6 false)
          (Rendering|SetActorHiddenInGame _array_element_6 true))))))

(event EventTick
  (params (DeltaSeconds :type Float%20%28single-precision%29))
  (Utilities|FlowControl|Sequence
    (:then_0
      (if (>= (Variables|Default|GetcounterSpawn) (Variables|Default|GetlimitSpawn))
        (Variables|Default|SetcanSpawn false)))
    (:then_1
      (for _array_element (Variables|Default|GetcubeSynchroRef)
        (CallFunction|SameasRefCube _array_element)))
    (:then_2
      (for _array_element_2 (Variables|Default|GetconeSynchroRef)
        (CallFunction|SameasRefCone _array_element_2)))
    (:then_3
      (for _array_element_3 (Variables|Default|GetsphereSynchroRef)
        (CallFunction|SameasRefSphere _array_element_3)))))

(event EventBeginPlay
  (Utilities|FlowControl|Sequence
    (:then_0
      (bind _returnvalue (Actor|GetActorOfClass "/Game/Coding/BluePrints/BP_CubeSynchro_1.BP_CubeSynchro_1_C"))
      (Variables|Default|SetownerCube _returnvalue)
      (Utilities|Array|Add (Variables|Default|GetcubeSynchroRef) _returnvalue))
    (:then_1
      (bind _returnvalue_2 (Actor|GetActorOfClass "/Game/Coding/BluePrints/BP_ConeSynchro_1.BP_ConeSynchro_1_C"))
      (Variables|Default|SetownerCone _returnvalue_2)
      (Utilities|Array|Add (Variables|Default|GetconeSynchroRef) _returnvalue_2))
    (:then_2
      (bind _returnvalue_3 (Actor|GetActorOfClass "/Game/Coding/BluePrints/BP_SphereSynchro_1.BP_SphereSynchro_1_C"))
      (bind _output_get (Variables|Default|SetownerSphere _returnvalue_3))
      (Utilities|Array|Add (Variables|Default|GetsphereSynchroRef) _output_get))))

(fn ConstructionScript
  (|CallParentFunction))

(fn ReferenceCable
  (params (displayName :type String))
  (switch string displayName
    (:BP_CubeSynchro_1
      (for _array_element (Variables|Default|GetcubeSynchroRef)
        (bind _returnvalue (Actor|GetActorOfClass "/Game/Coding/BluePrints/BP_CubeSynchro_1.BP_CubeSynchro_1_C"))
        (Class|CableComponent|SetAttachEndto (Variables|/Game/Coding/BluePrints/BP_CubeSynchro_1.BP_CubeSynchro_1_C|GetCable _array_element) _returnvalue "None" "None")))
    (:BP_SphereSynchro_1
      (for _array_element_2 (Variables|Default|GetsphereSynchroRef)
        (bind _returnvalue_2 (Actor|GetActorOfClass "/Game/Coding/BluePrints/BP_SphereSynchro_1.BP_SphereSynchro_1_C"))
        (Class|CableComponent|SetAttachEndto (Variables|/Game/Coding/BluePrints/BP_SphereSynchro_1.BP_SphereSynchro_1_C|GetCable _array_element_2) _returnvalue_2 "None" "None")))
    (:BP_ConeSynchro_1
      (for _array_element_3 (Variables|Default|GetconeSynchroRef)
        (bind _returnvalue_3 (Actor|GetActorOfClass "/Game/Coding/BluePrints/BP_ConeSynchro_1.BP_ConeSynchro_1_C"))
        (Class|CableComponent|SetAttachEndto (Variables|/Game/Coding/BluePrints/BP_ConeSynchro_1.BP_ConeSynchro_1_C|GetCable _array_element_3) _returnvalue_3 "None" "None")))))

(fn SetButtonColor
  (params (Alpha :type Float%20%28double-precision%29))
  (bind _material (CallFunction|GetButtonMaterial))
  (Rendering|Material|SetVectorParameterValue _material "Colot" (Math|Color|Lerp(LinearColor) "(R=0.043461,G=0.000000,B=1.000000,A=1.000000)" "(R=1.000000,G=0.962442,B=0.997690,A=1.000000)" 0.0) :!class /Script/Engine.MaterialInstanceDynamic)
  (Rendering|Material|SetScalarParameterValue _material "FresnelExponent" (Math|Float|Lerp 0.3 3.0 0.0) :!class /Script/Engine.MaterialInstanceDynamic))

(fn GetButtonMaterial
  (Variables|Default|GetButtonMaterial
    (:then
      _)
    (:else
      (bind _returnvalue (Rendering|Material|CreateDynamicMaterialInstance (Variables|Default|GetMesh_Button_Button) 0 "/Game/Coding/Mesh/Objects/MaterialTextureObject/M_Button_Ref_Inst.M_Button_Ref_Inst" "None" :!class /Script/Engine.PrimitiveComponent))
      (bind _output_get (Variables|Default|SetButtonMaterial _returnvalue))))
  (return _output_get))

(fn SameasRefCube
  (params (cube :type BP%20Cube%20Synchro%201%20Object%20Reference))
  (bind _ownercube (Variables|Default|GetownerCube))
  (bind _widget (Variables|/Game/Coding/BluePrints/BP_CubeSynchro_1.BP_CubeSynchro_1_C|GetWidget cube))
  (bind _returnvalue (UserInterface|GetWidget _widget))
  (bind _color_1 (Variables|/Game/Coding/BluePrints/BP_CubeSynchro_1.BP_CubeSynchro_1_C|GetColor_1 _ownercube))
  (bind _color_0 (Variables|/Game/Coding/BluePrints/BP_CubeSynchro_1.BP_CubeSynchro_1_C|GetColor_0 _ownercube))
  (bind _color_2 (Variables|/Game/Coding/BluePrints/BP_CubeSynchro_1.BP_CubeSynchro_1_C|GetColor_2 _ownercube))
  (bind _color_3 (Variables|/Game/Coding/BluePrints/BP_CubeSynchro_1.BP_CubeSynchro_1_C|GetColor_3 _ownercube))
  (bind _color_4 (Variables|/Game/Coding/BluePrints/BP_CubeSynchro_1.BP_CubeSynchro_1_C|GetColor_4 _ownercube))
  (bind _color_5 (Variables|/Game/Coding/BluePrints/BP_CubeSynchro_1.BP_CubeSynchro_1_C|GetColor_5 _ownercube))
  (bind _scale_1 (Variables|/Game/Coding/BluePrints/BP_CubeSynchro_1.BP_CubeSynchro_1_C|Getscale_1 _ownercube))
  (bind _scale_2 (Variables|/Game/Coding/BluePrints/BP_CubeSynchro_1.BP_CubeSynchro_1_C|Getscale_2 _ownercube))
  (bind _scale_3 (Variables|/Game/Coding/BluePrints/BP_CubeSynchro_1.BP_CubeSynchro_1_C|Getscale_3 _ownercube))
  (bind _scale_4 (Variables|/Game/Coding/BluePrints/BP_CubeSynchro_1.BP_CubeSynchro_1_C|Getscale_4 _ownercube))
  (bind _scale_5 (Variables|/Game/Coding/BluePrints/BP_CubeSynchro_1.BP_CubeSynchro_1_C|Getscale_5 _ownercube))
  (bind _scale_0 (Variables|/Game/Coding/BluePrints/BP_CubeSynchro_1.BP_CubeSynchro_1_C|Getscale_0 _ownercube))
  (Utilities|FlowControl|Sequence
    (:then_0
      (if (Class|KismetMathLibrary|NotEqualExactlyVectorVector (Variables|/Game/Coding/BluePrints/BP_CubeSynchro_1.BP_CubeSynchro_1_C|GetcurrentScale cube) (Variables|/Game/Coding/BluePrints/BP_CubeSynchro_1.BP_CubeSynchro_1_C|GetcurrentScale _ownercube))
        (while (Class|KismetMathLibrary|NotEqualExactlyVectorVector (Variables|/Game/Coding/BluePrints/BP_CubeSynchro_1.BP_CubeSynchro_1_C|GetcurrentScale cube) (Variables|/Game/Coding/BluePrints/BP_CubeSynchro_1.BP_CubeSynchro_1_C|GetcurrentScale _ownercube))
          (if (Class|KismetMathLibrary|EqualExactlyVectorVector (Variables|/Game/Coding/BluePrints/BP_CubeSynchro_1.BP_CubeSynchro_1_C|GetcurrentScale _ownercube) _scale_0)
            (Variables|/Game/Coding/BluePrints/BP_CubeSynchro_1.BP_CubeSynchro_1_C|SetcurrentScale cube _scale_5)
            (Default|ToChangeSize cube :!label _label)
            (elif (Class|KismetMathLibrary|EqualExactlyVectorVector (Variables|/Game/Coding/BluePrints/BP_CubeSynchro_1.BP_CubeSynchro_1_C|GetcurrentScale _ownercube) _scale_1)
              (Variables|/Game/Coding/BluePrints/BP_CubeSynchro_1.BP_CubeSynchro_1_C|SetcurrentScale cube _scale_0)
              (goto _label)
              (elif (Class|KismetMathLibrary|EqualExactlyVectorVector (Variables|/Game/Coding/BluePrints/BP_CubeSynchro_1.BP_CubeSynchro_1_C|GetcurrentScale _ownercube) _scale_2)
                (Variables|/Game/Coding/BluePrints/BP_CubeSynchro_1.BP_CubeSynchro_1_C|SetcurrentScale cube _scale_1)
                (goto _label)
                (elif (Class|KismetMathLibrary|EqualExactlyVectorVector (Variables|/Game/Coding/BluePrints/BP_CubeSynchro_1.BP_CubeSynchro_1_C|GetcurrentScale _ownercube) _scale_3)
                  (Variables|/Game/Coding/BluePrints/BP_CubeSynchro_1.BP_CubeSynchro_1_C|SetcurrentScale cube _scale_2)
                  (goto _label)
                  (elif (Class|KismetMathLibrary|EqualExactlyVectorVector (Variables|/Game/Coding/BluePrints/BP_CubeSynchro_1.BP_CubeSynchro_1_C|GetcurrentScale _ownercube) _scale_4)
                    (Variables|/Game/Coding/BluePrints/BP_CubeSynchro_1.BP_CubeSynchro_1_C|SetcurrentScale cube _scale_3)
                    (goto _label)
                    (elif (Class|KismetMathLibrary|EqualExactlyVectorVector (Variables|/Game/Coding/BluePrints/BP_CubeSynchro_1.BP_CubeSynchro_1_C|GetcurrentScale _ownercube) _scale_5)
                      (Variables|/Game/Coding/BluePrints/BP_CubeSynchro_1.BP_CubeSynchro_1_C|SetcurrentScale cube _scale_4)
                      (goto _label))))))))))
    (:then_1
      (if (!= (Variables|/Game/Coding/BluePrints/BP_CubeSynchro_1.BP_CubeSynchro_1_C|GetcurrentColor cube) (Variables|/Game/Coding/BluePrints/BP_CubeSynchro_1.BP_CubeSynchro_1_C|GetcurrentColor _ownercube))
        (while (!= (Variables|/Game/Coding/BluePrints/BP_CubeSynchro_1.BP_CubeSynchro_1_C|GetcurrentColor cube) (Variables|/Game/Coding/BluePrints/BP_CubeSynchro_1.BP_CubeSynchro_1_C|GetcurrentColor _ownercube))
          (if (Class|KismetMathLibrary|LinearColorIsNearEqual (Variables|/Game/Coding/BluePrints/BP_CubeSynchro_1.BP_CubeSynchro_1_C|GetcurrentColor cube) _color_0 0.0001)
            (Variables|/Game/Coding/BluePrints/BP_CubeSynchro_1.BP_CubeSynchro_1_C|SetcurrentColor cube _color_5)
            (Default|ToChangeColor cube :!label _label_2)
            (elif (Class|KismetMathLibrary|LinearColorIsNearEqual (Variables|/Game/Coding/BluePrints/BP_CubeSynchro_1.BP_CubeSynchro_1_C|GetcurrentColor cube) _color_1 0.0001)
              (Variables|/Game/Coding/BluePrints/BP_CubeSynchro_1.BP_CubeSynchro_1_C|SetcurrentColor cube _color_0)
              (goto _label_2)
              (elif (Class|KismetMathLibrary|LinearColorIsNearEqual (Variables|/Game/Coding/BluePrints/BP_CubeSynchro_1.BP_CubeSynchro_1_C|GetcurrentColor cube) _color_2 0.0001)
                (Variables|/Game/Coding/BluePrints/BP_CubeSynchro_1.BP_CubeSynchro_1_C|SetcurrentColor cube _color_1)
                (goto _label_2)
                (elif (Class|KismetMathLibrary|LinearColorIsNearEqual (Variables|/Game/Coding/BluePrints/BP_CubeSynchro_1.BP_CubeSynchro_1_C|GetcurrentColor cube) _color_3 0.0001)
                  (Variables|/Game/Coding/BluePrints/BP_CubeSynchro_1.BP_CubeSynchro_1_C|SetcurrentColor cube _color_2)
                  (goto _label_2)
                  (elif (Class|KismetMathLibrary|LinearColorIsNearEqual (Variables|/Game/Coding/BluePrints/BP_CubeSynchro_1.BP_CubeSynchro_1_C|GetcurrentColor cube) _color_4 0.0001)
                    (Variables|/Game/Coding/BluePrints/BP_CubeSynchro_1.BP_CubeSynchro_1_C|SetcurrentColor cube _color_3)
                    (goto _label_2)
                    (elif (Class|KismetMathLibrary|LinearColorIsNearEqual (Variables|/Game/Coding/BluePrints/BP_CubeSynchro_1.BP_CubeSynchro_1_C|GetcurrentColor cube) _color_5 0.0001)
                      (Variables|/Game/Coding/BluePrints/BP_CubeSynchro_1.BP_CubeSynchro_1_C|SetcurrentColor cube _color_4)
                      (goto _label_2))))))))))
    (:then_2
      (bind _asui_synchro_menu (Utilities|Casting|CastToUI_Synchro_Menu (UserInterface|GetWidget (Variables|/Game/Coding/BluePrints/BP_CubeSynchro_1.BP_CubeSynchro_1_C|GetWidget _ownercube))))
      (if (Widget|IsVisible (Variables|/Game/Coding/Widgets/Synchro/UI_Synchro_Menu.UI_Synchro_Menu_C|GetButton_Color _asui_synchro_menu))
        (bind _asui_synchro_menu_2 (Utilities|Casting|CastToUI_Synchro_Menu _returnvalue))
        (Widget|SetIsEnabled (Variables|/Game/Coding/Widgets/Synchro/UI_Synchro_Menu.UI_Synchro_Menu_C|GetButton_Color _asui_synchro_menu_2) true)
        (Widget|SetVisibility (Variables|/Game/Coding/Widgets/Synchro/UI_Synchro_Menu.UI_Synchro_Menu_C|GetButton_Color _asui_synchro_menu_2) "Visible")
        (else
          (bind _asui_synchro_menu_3 (Utilities|Casting|CastToUI_Synchro_Menu _returnvalue))
          (Widget|SetIsEnabled (Variables|/Game/Coding/Widgets/Synchro/UI_Synchro_Menu.UI_Synchro_Menu_C|GetButton_Color _asui_synchro_menu_3) false)
          (Widget|SetVisibility (Variables|/Game/Coding/Widgets/Synchro/UI_Synchro_Menu.UI_Synchro_Menu_C|GetButton_Color _asui_synchro_menu_3) "Hidden"))))))

(fn SameasRefSphere
  (params (sphere :type BP%20Sphere%20Synchro%201%20Object%20Reference))
  (bind _ownersphere (Variables|Default|GetownerSphere))
  (bind _widget (Variables|/Game/Coding/BluePrints/BP_SphereSynchro_1.BP_SphereSynchro_1_C|GetWidget sphere))
  (bind _returnvalue (UserInterface|GetWidget _widget))
  (bind _scale_1 (Variables|/Game/Coding/BluePrints/BP_SphereSynchro_1.BP_SphereSynchro_1_C|Getscale_1 _ownersphere))
  (bind _scale_0 (Variables|/Game/Coding/BluePrints/BP_SphereSynchro_1.BP_SphereSynchro_1_C|Getscale_0 _ownersphere))
  (bind _scale_2 (Variables|/Game/Coding/BluePrints/BP_SphereSynchro_1.BP_SphereSynchro_1_C|Getscale_2 _ownersphere))
  (bind _scale_3 (Variables|/Game/Coding/BluePrints/BP_SphereSynchro_1.BP_SphereSynchro_1_C|Getscale_3 _ownersphere))
  (bind _scale_4 (Variables|/Game/Coding/BluePrints/BP_SphereSynchro_1.BP_SphereSynchro_1_C|Getscale_4 _ownersphere))
  (bind _scale_5 (Variables|/Game/Coding/BluePrints/BP_SphereSynchro_1.BP_SphereSynchro_1_C|Getscale_5 _ownersphere))
  (bind _color_1 (Variables|/Game/Coding/BluePrints/BP_SphereSynchro_1.BP_SphereSynchro_1_C|GetColor_1 _ownersphere))
  (bind _color_0 (Variables|/Game/Coding/BluePrints/BP_SphereSynchro_1.BP_SphereSynchro_1_C|GetColor_0 _ownersphere))
  (bind _color_5 (Variables|/Game/Coding/BluePrints/BP_SphereSynchro_1.BP_SphereSynchro_1_C|GetColor_5 _ownersphere))
  (bind _color_3 (Variables|/Game/Coding/BluePrints/BP_SphereSynchro_1.BP_SphereSynchro_1_C|GetColor_3 _ownersphere))
  (bind _color_2 (Variables|/Game/Coding/BluePrints/BP_SphereSynchro_1.BP_SphereSynchro_1_C|GetColor_2 _ownersphere))
  (bind _color_4 (Variables|/Game/Coding/BluePrints/BP_SphereSynchro_1.BP_SphereSynchro_1_C|GetColor_4 _ownersphere))
  (Utilities|FlowControl|Sequence
    (:then_0
      (if (Class|KismetMathLibrary|NotEqualExactlyVectorVector (Variables|/Game/Coding/BluePrints/BP_SphereSynchro_1.BP_SphereSynchro_1_C|GetcurrentScale sphere) (Variables|/Game/Coding/BluePrints/BP_SphereSynchro_1.BP_SphereSynchro_1_C|GetcurrentScale _ownersphere))
        (while (Class|KismetMathLibrary|NotEqualExactlyVectorVector (Variables|/Game/Coding/BluePrints/BP_SphereSynchro_1.BP_SphereSynchro_1_C|GetcurrentScale sphere) (Variables|/Game/Coding/BluePrints/BP_SphereSynchro_1.BP_SphereSynchro_1_C|GetcurrentScale _ownersphere))
          (if (Class|KismetMathLibrary|EqualExactlyVectorVector (Variables|/Game/Coding/BluePrints/BP_SphereSynchro_1.BP_SphereSynchro_1_C|GetcurrentScale _ownersphere) _scale_0)
            (Variables|/Game/Coding/BluePrints/BP_SphereSynchro_1.BP_SphereSynchro_1_C|SetcurrentScale sphere _scale_5)
            (Default|ToChangeSize sphere :!label _label)
            (elif (Class|KismetMathLibrary|EqualExactlyVectorVector (Variables|/Game/Coding/BluePrints/BP_SphereSynchro_1.BP_SphereSynchro_1_C|GetcurrentScale _ownersphere) _scale_1)
              (Variables|/Game/Coding/BluePrints/BP_SphereSynchro_1.BP_SphereSynchro_1_C|SetcurrentScale sphere _scale_0)
              (goto _label)
              (elif (Class|KismetMathLibrary|EqualExactlyVectorVector (Variables|/Game/Coding/BluePrints/BP_SphereSynchro_1.BP_SphereSynchro_1_C|GetcurrentScale _ownersphere) _scale_2)
                (Variables|/Game/Coding/BluePrints/BP_SphereSynchro_1.BP_SphereSynchro_1_C|SetcurrentScale sphere _scale_1)
                (goto _label)
                (elif (Class|KismetMathLibrary|EqualExactlyVectorVector (Variables|/Game/Coding/BluePrints/BP_SphereSynchro_1.BP_SphereSynchro_1_C|GetcurrentScale _ownersphere) _scale_3)
                  (Variables|/Game/Coding/BluePrints/BP_SphereSynchro_1.BP_SphereSynchro_1_C|SetcurrentScale sphere _scale_2)
                  (goto _label)
                  (elif (Class|KismetMathLibrary|EqualExactlyVectorVector (Variables|/Game/Coding/BluePrints/BP_SphereSynchro_1.BP_SphereSynchro_1_C|GetcurrentScale _ownersphere) _scale_4)
                    (Variables|/Game/Coding/BluePrints/BP_SphereSynchro_1.BP_SphereSynchro_1_C|SetcurrentScale sphere _scale_3)
                    (goto _label)
                    (elif (Class|KismetMathLibrary|EqualExactlyVectorVector (Variables|/Game/Coding/BluePrints/BP_SphereSynchro_1.BP_SphereSynchro_1_C|GetcurrentScale _ownersphere) _scale_5)
                      (Variables|/Game/Coding/BluePrints/BP_SphereSynchro_1.BP_SphereSynchro_1_C|SetcurrentScale sphere _scale_4)
                      (goto _label))))))))))
    (:then_1
      (if (!= (Variables|/Game/Coding/BluePrints/BP_SphereSynchro_1.BP_SphereSynchro_1_C|GetcurrentColor sphere) (Variables|/Game/Coding/BluePrints/BP_SphereSynchro_1.BP_SphereSynchro_1_C|GetcurrentColor _ownersphere))
        (while (!= (Variables|/Game/Coding/BluePrints/BP_SphereSynchro_1.BP_SphereSynchro_1_C|GetcurrentColor sphere) (Variables|/Game/Coding/BluePrints/BP_SphereSynchro_1.BP_SphereSynchro_1_C|GetcurrentColor _ownersphere))
          (if (Class|KismetMathLibrary|LinearColorIsNearEqual (Variables|/Game/Coding/BluePrints/BP_SphereSynchro_1.BP_SphereSynchro_1_C|GetcurrentColor sphere) _color_0 0.0001)
            (Variables|/Game/Coding/BluePrints/BP_SphereSynchro_1.BP_SphereSynchro_1_C|SetcurrentColor sphere _color_5)
            (Default|ToChangeColor sphere :!label _label_2)
            (elif (Class|KismetMathLibrary|LinearColorIsNearEqual (Variables|/Game/Coding/BluePrints/BP_SphereSynchro_1.BP_SphereSynchro_1_C|GetcurrentColor sphere) _color_1 0.0001)
              (Variables|/Game/Coding/BluePrints/BP_SphereSynchro_1.BP_SphereSynchro_1_C|SetcurrentColor sphere _color_0)
              (goto _label_2)
              (elif (Class|KismetMathLibrary|LinearColorIsNearEqual (Variables|/Game/Coding/BluePrints/BP_SphereSynchro_1.BP_SphereSynchro_1_C|GetcurrentColor sphere) _color_2 0.0001)
                (Variables|/Game/Coding/BluePrints/BP_SphereSynchro_1.BP_SphereSynchro_1_C|SetcurrentColor sphere _color_1)
                (goto _label_2)
                (elif (Class|KismetMathLibrary|LinearColorIsNearEqual (Variables|/Game/Coding/BluePrints/BP_SphereSynchro_1.BP_SphereSynchro_1_C|GetcurrentColor sphere) _color_3 0.0001)
                  (Variables|/Game/Coding/BluePrints/BP_SphereSynchro_1.BP_SphereSynchro_1_C|SetcurrentColor sphere _color_2)
                  (goto _label_2)
                  (elif (Class|KismetMathLibrary|LinearColorIsNearEqual (Variables|/Game/Coding/BluePrints/BP_SphereSynchro_1.BP_SphereSynchro_1_C|GetcurrentColor sphere) _color_4 0.0001)
                    (Variables|/Game/Coding/BluePrints/BP_SphereSynchro_1.BP_SphereSynchro_1_C|SetcurrentColor sphere _color_3)
                    (goto _label_2)
                    (elif (Class|KismetMathLibrary|LinearColorIsNearEqual (Variables|/Game/Coding/BluePrints/BP_SphereSynchro_1.BP_SphereSynchro_1_C|GetcurrentColor sphere) _color_5 0.0001)
                      (Variables|/Game/Coding/BluePrints/BP_SphereSynchro_1.BP_SphereSynchro_1_C|SetcurrentColor sphere _color_4)
                      (goto _label_2))))))))))
    (:then_2
      (bind _asui_synchro_menu (Utilities|Casting|CastToUI_Synchro_Menu (UserInterface|GetWidget (Variables|/Game/Coding/BluePrints/BP_SphereSynchro_1.BP_SphereSynchro_1_C|GetWidget _ownersphere))))
      (if (Widget|IsVisible (Variables|/Game/Coding/Widgets/Synchro/UI_Synchro_Menu.UI_Synchro_Menu_C|GetButton_Color _asui_synchro_menu))
        (bind _asui_synchro_menu_2 (Utilities|Casting|CastToUI_Synchro_Menu _returnvalue))
        (Widget|SetIsEnabled (Variables|/Game/Coding/Widgets/Synchro/UI_Synchro_Menu.UI_Synchro_Menu_C|GetButton_Color _asui_synchro_menu_2) true)
        (Widget|SetVisibility (Variables|/Game/Coding/Widgets/Synchro/UI_Synchro_Menu.UI_Synchro_Menu_C|GetButton_Color _asui_synchro_menu_2) "Visible")
        (else
          (bind _asui_synchro_menu_3 (Utilities|Casting|CastToUI_Synchro_Menu _returnvalue))
          (Widget|SetIsEnabled (Variables|/Game/Coding/Widgets/Synchro/UI_Synchro_Menu.UI_Synchro_Menu_C|GetButton_Color _asui_synchro_menu_3) false)
          (Widget|SetVisibility (Variables|/Game/Coding/Widgets/Synchro/UI_Synchro_Menu.UI_Synchro_Menu_C|GetButton_Color _asui_synchro_menu_3) "Hidden"))))))

(fn SameasRefCone
  (params (cone :type BP%20Cone%20Synchro%201%20Object%20Reference))
  (bind _ownercone (Variables|Default|GetownerCone))
  (bind _widget (Variables|/Game/Coding/BluePrints/BP_ConeSynchro_1.BP_ConeSynchro_1_C|GetWidget cone))
  (bind _returnvalue (UserInterface|GetWidget _widget))
  (bind _color_1 (Variables|/Game/Coding/BluePrints/BP_ConeSynchro_1.BP_ConeSynchro_1_C|GetColor_1 _ownercone))
  (bind _color_2 (Variables|/Game/Coding/BluePrints/BP_ConeSynchro_1.BP_ConeSynchro_1_C|GetColor_2 _ownercone))
  (bind _color_5 (Variables|/Game/Coding/BluePrints/BP_ConeSynchro_1.BP_ConeSynchro_1_C|GetColor_5 _ownercone))
  (bind _color_0 (Variables|/Game/Coding/BluePrints/BP_ConeSynchro_1.BP_ConeSynchro_1_C|GetColor_0 _ownercone))
  (bind _color_3 (Variables|/Game/Coding/BluePrints/BP_ConeSynchro_1.BP_ConeSynchro_1_C|GetColor_3 _ownercone))
  (bind _color_4 (Variables|/Game/Coding/BluePrints/BP_ConeSynchro_1.BP_ConeSynchro_1_C|GetColor_4 _ownercone))
  (bind _scale_5 (Variables|/Game/Coding/BluePrints/BP_ConeSynchro_1.BP_ConeSynchro_1_C|Getscale_5 _ownercone))
  (bind _scale_0 (Variables|/Game/Coding/BluePrints/BP_ConeSynchro_1.BP_ConeSynchro_1_C|Getscale_0 _ownercone))
  (bind _scale_1 (Variables|/Game/Coding/BluePrints/BP_ConeSynchro_1.BP_ConeSynchro_1_C|Getscale_1 _ownercone))
  (bind _scale_2 (Variables|/Game/Coding/BluePrints/BP_ConeSynchro_1.BP_ConeSynchro_1_C|Getscale_2 _ownercone))
  (bind _scale_3 (Variables|/Game/Coding/BluePrints/BP_ConeSynchro_1.BP_ConeSynchro_1_C|Getscale_3 _ownercone))
  (bind _scale_4 (Variables|/Game/Coding/BluePrints/BP_ConeSynchro_1.BP_ConeSynchro_1_C|Getscale_4 _ownercone))
  (Utilities|FlowControl|Sequence
    (:then_0
      (if (Class|KismetMathLibrary|NotEqualExactlyVectorVector (Variables|/Game/Coding/BluePrints/BP_ConeSynchro_1.BP_ConeSynchro_1_C|GetcurrentScale cone) (Variables|/Game/Coding/BluePrints/BP_ConeSynchro_1.BP_ConeSynchro_1_C|GetcurrentScale _ownercone))
        (while (Class|KismetMathLibrary|NotEqualExactlyVectorVector (Variables|/Game/Coding/BluePrints/BP_ConeSynchro_1.BP_ConeSynchro_1_C|GetcurrentScale cone) (Variables|/Game/Coding/BluePrints/BP_ConeSynchro_1.BP_ConeSynchro_1_C|GetcurrentScale _ownercone))
          (if (Class|KismetMathLibrary|EqualExactlyVectorVector (Variables|/Game/Coding/BluePrints/BP_ConeSynchro_1.BP_ConeSynchro_1_C|GetcurrentScale _ownercone) _scale_0)
            (Variables|/Game/Coding/BluePrints/BP_ConeSynchro_1.BP_ConeSynchro_1_C|SetcurrentScale cone _scale_5)
            (Default|ToChangeSize cone :!label _label)
            (elif (Class|KismetMathLibrary|EqualExactlyVectorVector (Variables|/Game/Coding/BluePrints/BP_ConeSynchro_1.BP_ConeSynchro_1_C|GetcurrentScale _ownercone) _scale_1)
              (Variables|/Game/Coding/BluePrints/BP_ConeSynchro_1.BP_ConeSynchro_1_C|SetcurrentScale cone _scale_0)
              (goto _label)
              (elif (Class|KismetMathLibrary|EqualExactlyVectorVector (Variables|/Game/Coding/BluePrints/BP_ConeSynchro_1.BP_ConeSynchro_1_C|GetcurrentScale _ownercone) _scale_2)
                (Variables|/Game/Coding/BluePrints/BP_ConeSynchro_1.BP_ConeSynchro_1_C|SetcurrentScale cone _scale_1)
                (goto _label)
                (elif (Class|KismetMathLibrary|EqualExactlyVectorVector (Variables|/Game/Coding/BluePrints/BP_ConeSynchro_1.BP_ConeSynchro_1_C|GetcurrentScale _ownercone) _scale_3)
                  (Variables|/Game/Coding/BluePrints/BP_ConeSynchro_1.BP_ConeSynchro_1_C|SetcurrentScale cone _scale_2)
                  (goto _label)
                  (elif (Class|KismetMathLibrary|EqualExactlyVectorVector (Variables|/Game/Coding/BluePrints/BP_ConeSynchro_1.BP_ConeSynchro_1_C|GetcurrentScale _ownercone) _scale_4)
                    (Variables|/Game/Coding/BluePrints/BP_ConeSynchro_1.BP_ConeSynchro_1_C|SetcurrentScale cone _scale_3)
                    (goto _label)
                    (elif (Class|KismetMathLibrary|EqualExactlyVectorVector (Variables|/Game/Coding/BluePrints/BP_ConeSynchro_1.BP_ConeSynchro_1_C|GetcurrentScale _ownercone) _scale_5)
                      (Variables|/Game/Coding/BluePrints/BP_ConeSynchro_1.BP_ConeSynchro_1_C|SetcurrentScale cone _scale_4)
                      (goto _label))))))))))
    (:then_1
      (if (!= (Variables|/Game/Coding/BluePrints/BP_ConeSynchro_1.BP_ConeSynchro_1_C|GetcurrentColor cone) (Variables|/Game/Coding/BluePrints/BP_ConeSynchro_1.BP_ConeSynchro_1_C|GetcurrentColor _ownercone))
        (while (!= (Variables|/Game/Coding/BluePrints/BP_ConeSynchro_1.BP_ConeSynchro_1_C|GetcurrentColor cone) (Variables|/Game/Coding/BluePrints/BP_ConeSynchro_1.BP_ConeSynchro_1_C|GetcurrentColor _ownercone))
          (if (Class|KismetMathLibrary|LinearColorIsNearEqual (Variables|/Game/Coding/BluePrints/BP_ConeSynchro_1.BP_ConeSynchro_1_C|GetcurrentColor cone) _color_0 0.0001)
            (Variables|/Game/Coding/BluePrints/BP_ConeSynchro_1.BP_ConeSynchro_1_C|SetcurrentColor cone _color_5)
            (Default|ToChangeColor cone :!label _label_2)
            (elif (Class|KismetMathLibrary|LinearColorIsNearEqual (Variables|/Game/Coding/BluePrints/BP_ConeSynchro_1.BP_ConeSynchro_1_C|GetcurrentColor cone) _color_1 0.0001)
              (Variables|/Game/Coding/BluePrints/BP_ConeSynchro_1.BP_ConeSynchro_1_C|SetcurrentColor cone _color_0)
              (goto _label_2)
              (elif (Class|KismetMathLibrary|LinearColorIsNearEqual (Variables|/Game/Coding/BluePrints/BP_ConeSynchro_1.BP_ConeSynchro_1_C|GetcurrentColor cone) _color_2 0.0001)
                (Variables|/Game/Coding/BluePrints/BP_ConeSynchro_1.BP_ConeSynchro_1_C|SetcurrentColor cone _color_1)
                (goto _label_2)
                (elif (Class|KismetMathLibrary|LinearColorIsNearEqual (Variables|/Game/Coding/BluePrints/BP_ConeSynchro_1.BP_ConeSynchro_1_C|GetcurrentColor cone) _color_3 0.0001)
                  (Variables|/Game/Coding/BluePrints/BP_ConeSynchro_1.BP_ConeSynchro_1_C|SetcurrentColor cone _color_2)
                  (goto _label_2)
                  (elif (Class|KismetMathLibrary|LinearColorIsNearEqual (Variables|/Game/Coding/BluePrints/BP_ConeSynchro_1.BP_ConeSynchro_1_C|GetcurrentColor cone) _color_4 0.0001)
                    (Variables|/Game/Coding/BluePrints/BP_ConeSynchro_1.BP_ConeSynchro_1_C|SetcurrentColor cone _color_3)
                    (goto _label_2)
                    (elif (Class|KismetMathLibrary|LinearColorIsNearEqual (Variables|/Game/Coding/BluePrints/BP_ConeSynchro_1.BP_ConeSynchro_1_C|GetcurrentColor cone) _color_5 0.0001)
                      (Variables|/Game/Coding/BluePrints/BP_ConeSynchro_1.BP_ConeSynchro_1_C|SetcurrentColor cone _color_4)
                      (goto _label_2))))))))))
    (:then_2
      (bind _asui_synchro_menu (Utilities|Casting|CastToUI_Synchro_Menu (UserInterface|GetWidget (Variables|/Game/Coding/BluePrints/BP_ConeSynchro_1.BP_ConeSynchro_1_C|GetWidget _ownercone))))
      (if (Widget|IsVisible (Variables|/Game/Coding/Widgets/Synchro/UI_Synchro_Menu.UI_Synchro_Menu_C|GetButton_Color _asui_synchro_menu))
        (bind _asui_synchro_menu_2 (Utilities|Casting|CastToUI_Synchro_Menu _returnvalue))
        (Widget|SetIsEnabled (Variables|/Game/Coding/Widgets/Synchro/UI_Synchro_Menu.UI_Synchro_Menu_C|GetButton_Color _asui_synchro_menu_2) true)
        (Widget|SetVisibility (Variables|/Game/Coding/Widgets/Synchro/UI_Synchro_Menu.UI_Synchro_Menu_C|GetButton_Color _asui_synchro_menu_2) "Visible")
        (else
          (bind _asui_synchro_menu_3 (Utilities|Casting|CastToUI_Synchro_Menu _returnvalue))
          (Widget|SetIsEnabled (Variables|/Game/Coding/Widgets/Synchro/UI_Synchro_Menu.UI_Synchro_Menu_C|GetButton_Color _asui_synchro_menu_3) false)
          (Widget|SetVisibility (Variables|/Game/Coding/Widgets/Synchro/UI_Synchro_Menu.UI_Synchro_Menu_C|GetButton_Color _asui_synchro_menu_3) "Hidden"))))))