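; Synchro cube actor that steps through six preset colors and six preset sizes, with a UI_Synchro_Menu widget attached.
; BeginPlay stores the starting color and scale and registers the cube as the menu's owner.
; ToChangeColor reads the material's ColorParam and ChangeColor applies the next color through a new dynamic material instance.
; ToChangeSize advances the scale, repositioning the widget to suit each size.
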(event Custom|ToChangeColor
  (bind _cube (Variables|Default|GetCube))
  (bind _returnvalue (Rendering|Material|CreateDynamicMaterialInstance _cube 0 (Rendering|Material|GetMaterial _cube 0) "None" :!class /Script/Engine.PrimitiveComponent))
  (bind _returnvalue_2 (Rendering|Material|GetVectorParameterValue _returnvalue "ColorParam" :!class /Script/Engine.MaterialInstanceDynamic))
  (CallFunction|ChangeColor _returnvalue_2))

(event Custom|ToChangeSize
  (CallFunction|ChangeSize (Variables|Default|GetcurrentScale)))

(event EventTick
  (params (DeltaSeconds :type Float%20%28single-precision%29)))

(event EventBeginPlay
  (bind _color_0 (Variables|Default|GetColor_0))
  (bind _returnvalue (Rendering|Material|CreateDynamicMaterialInstance (Variables|Default|GetCube) 0 "/Game/Coding/Mesh/Objects/MaterialTextureObject/Synchro_1.Synchro_1" "None" :!class /Script/Engine.PrimitiveComponent))
  (Rendering|Material|SetVectorParameterValue _returnvalue "None" _color_0 :!class /Script/Engine.MaterialInstanceDynamic)
  (Variables|Default|SetcurrentColor _color_0)
  (bind _output_get (Variables|Default|SetcurrentScale (Transformation|GetWorldScale (Variables|Default|GetCube))))
  (Variables|Default|Setscale_0 _output_get)
  (bind _asui_synchro_menu (Utilities|Casting|CastToUI_Synchro_Menu (UserInterface|GetWidget (Variables|Default|GetWidget))))
  (Variables|/Game/Coding/Widgets/Synchro/UI_Synchro_Menu.UI_Synchro_Menu_C|SetownerCube _asui_synchro_menu self)
  (Variables|/Game/Coding/Widgets/Synchro/UI_Synchro_Menu.UI_Synchro_Menu_C|SetcubeOwner _asui_synchro_menu true))

(fn ConstructionScript)

(fn ChangeColor
  (params (currentColor :type Linear%20Color%20Structure))
  (bind _color_2 (Variables|Default|GetColor_2))
  (bind _color_3 (Variables|Default|GetColor_3))
  (bind _color_4 (Variables|Default|GetColor_4))
  (bind _color_5 (Variables|Default|GetColor_5))
  (bind _color_0 (Variables|Default|GetColor_0))
  (bind _color_1 (Variables|Default|GetColor_1))
  (Utilities|FlowControl|Sequence
    (:then_0
      (if (== currentColor (Variables|Default|GetColor_0))
        (bind _returnvalue (Rendering|Material|CreateDynamicMaterialInstance (Variables|Default|GetCube) 0 "/Game/Coding/Mesh/Objects/MaterialTextureObject/Synchro_1.Synchro_1" "None" :!class /Script/Engine.PrimitiveComponent))
        (Rendering|Material|SetVectorParameterValue _returnvalue "ColorParam" _color_1 :!class /Script/Engine.MaterialInstanceDynamic)
        (Variables|Default|SetcurrentColor _color_1)))
    (:then_1
      (if (== currentColor (Variables|Default|GetColor_1))
        (bind _returnvalue_2 (Rendering|Material|CreateDynamicMaterialInstance (Variables|Default|GetCube) 0 "/Game/Coding/Mesh/Objects/MaterialTextureObject/Synchro_1.Synchro_1" "None" :!class /Script/Engine.PrimitiveComponent))
        (Rendering|Material|SetVectorParameterValue _returnvalue_2 "ColorParam" _color_2 :!class /Script/Engine.MaterialInstanceDynamic)
        (Variables|Default|SetcurrentColor _color_2)))
    (:then_2
      (if (== currentColor (Variables|Default|GetColor_2))
        (bind _returnvalue_3 (Rendering|Material|CreateDynamicMaterialInstance (Variables|Default|GetCube) 0 "/Game/Coding/Mesh/Objects/MaterialTextureObject/Synchro_1.Synchro_1" "None" :!class /Script/Engine.PrimitiveComponent))
        (Rendering|Material|SetVectorParameterValue _returnvalue_3 "ColorParam" _color_3 :!class /Script/Engine.MaterialInstanceDynamic)
        (Variables|Default|SetcurrentColor _color_3)))
    (:then_3
      (if (== currentColor (Variables|Default|GetColor_3))
        (bind _returnvalue_4 (Rendering|Material|CreateDynamicMaterialInstance (Variables|Default|GetCube) 0 "/Game/Coding/Mesh/Objects/MaterialTextureObject/Synchro_1.Synchro_1" "None" :!class /Script/Engine.PrimitiveComponent))
        (Rendering|Material|SetVectorParameterValue _returnvalue_4 "ColorParam" _color_4 :!class /Script/Engine.MaterialInstanceDynamic)
        (Variables|Default|SetcurrentColor _color_4)))
    (:then_4
      (if (== currentColor (Variables|Default|GetColor_4))
        (bind _returnvalue_5 (Rendering|Material|CreateDynamicMaterialInstance (Variables|Default|GetCube) 0 "/Game/Coding/Mesh/Objects/MaterialTextureObject/Synchro_1.Synchro_1" "None" :!class /Script/Engine.PrimitiveComponent))
        (Rendering|Material|SetVectorParameterValue _returnvalue_5 "ColorParam" _color_5 :!class /Script/Engine.MaterialInstanceDynamic)
        (Variables|Default|SetcurrentColor _color_5)))
    (:then_5
      (if (== currentColor (Variables|Default|GetColor_5))
        (bind _returnvalue_6 (Rendering|Material|CreateDynamicMaterialInstance (Variables|Default|GetCube) 0 "/Game/Coding/Mesh/Objects/MaterialTextureObject/Synchro_1.Synchro_1" "None" :!class /Script/Engine.PrimitiveComponent))
        (Rendering|Material|SetVectorParameterValue _returnvalue_6 "ColorParam" _color_0 :!class /Script/Engine.MaterialInstanceDynamic)
        (Variables|Default|SetcurrentColor _color_0)))))

(fn ChangeSize
  (params (currentScale :type Vector))
  (bind _scale_0 (Variables|Default|Getscale_0))
  (bind _scale_5 (Variables|Default|Getscale_5))
  (bind _scale_4 (Variables|Default|Getscale_4))
  (bind _scale_3 (Variables|Default|Getscale_3))
  (bind _scale_2 (Variables|Default|Getscale_2))
  (bind _scale_1 (Variables|Default|Getscale_1))
  (bind _widget (Variables|Default|GetWidget))
  (if (Class|KismetMathLibrary|EqualExactlyVectorVector currentScale (Variables|Default|Getscale_0))
    (Transformation|SetRelativeScale3D (Variables|Default|GetCube) _scale_1)
    (Variables|Default|SetcurrentScale _scale_1)
    (Transformation|SetRelativeLocation _widget "8.278097,-1.559170,-5.624530" false false)
    (elif (Class|KismetMathLibrary|EqualExactlyVectorVector currentScale (Variables|Default|Getscale_1))
      (Transformation|SetRelativeScale3D (Variables|Default|GetCube) _scale_2)
      (Variables|Default|SetcurrentScale _scale_2)
      (Transformation|SetRelativeLocation _widget "22.364323,-1.559170,-16.000000" false false)
      (elif (Class|KismetMathLibrary|EqualExactlyVectorVector currentScale (Variables|Default|Getscale_2))
        (Transformation|SetRelativeScale3D (Variables|Default|GetCube) _scale_3)
        (Variables|Default|SetcurrentScale _scale_3)
        (Transformation|SetRelativeLocation _widget "31.242591,-1.559170,-20.000000" false false)
        (elif (Class|KismetMathLibrary|EqualExactlyVectorVector currentScale (Variables|Default|Getscale_3))
          (Transformation|SetRelativeScale3D (Variables|Default|GetCube) _scale_4)
          (Variables|Default|SetcurrentScale _scale_4)
          (Transformation|SetRelativeLocation _widget "49.479058,-1.559170,-27.000000" false false)
          (elif (Class|KismetMathLibrary|EqualExactlyVectorVector currentScale (Variables|Default|Getscale_4))
            (Transformation|SetRelativeScale3D (Variables|Default|GetCube) _scale_5)
            (Variables|Default|SetcurrentScale _scale_5)
            (Transformation|SetRelativeLocation _widget "62.450659,-1.559170,-32.000000" false false)
            (elif (Class|KismetMathLibrary|EqualExactlyVectorVector currentScale (Variables|Default|Getscale_5))
              (Transformation|SetRelativeScale3D (Variables|Default|GetCube) _scale_0)
              (Variables|Default|SetcurrentScale _scale_0)
              (Transformation|SetRelativeLocation _widget "12.345809,-1.559170,-6.724200" false false))))))))