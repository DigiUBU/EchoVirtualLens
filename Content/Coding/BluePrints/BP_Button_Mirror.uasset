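; Mirror button Blueprint that alters mirror-related shape actors when its switch component turns on.
; BeginPlay waits briefly, then clears the pressed flag, shows the spheres and resets the cube's scale.
; Each press hides the spheres, shifts the cone further along Y, calls UpdatePositionNoGrab on both, then toggles the switch after a delay.
; Targets are found by class lookup, and an unconnected branch holds unused cube-enlarging logic.
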(event OnStateChanged(Comp_Switch)
  (params (SourceInfo :type Struct%20Component%20Source%20Info%20Structure) (Value :type Boolean))
  (bind _output_get (Variables|Default|Setpressed Value))
  (if _output_get
    (Utilities|FlowControl|Sequence
      (:then_0
        (bind _returnvalue (Actor|GetActorOfClass "/Game/Coding/BluePrints/BP_Mirror_Spheres.BP_Mirror_Spheres_C"))
        (Rendering|SetActorHiddenInGame _returnvalue true)
        (Default|UpdatePositionNoGrab _returnvalue))
      (:then_1
        (bind _returnvalue_2 (Actor|GetActorOfClass "/Game/Coding/BluePrints/BP_Mirror_Cone.BP_Mirror_Cone_C"))
        (Transformation|SetActorLocation _returnvalue_2 (Math|Vector|MakeVector (.x (Transformation|GetWorldLocation (Variables|/Game/Coding/BluePrints/BP_Mirror.BP_Mirror_C|GetDefaultSceneRoot _returnvalue_2))) (+ (.y (Transformation|GetWorldLocation (Variables|/Game/Coding/BluePrints/BP_Mirror.BP_Mirror_C|GetDefaultSceneRoot _returnvalue_2))) 1.5e+02) (.z (Transformation|GetWorldLocation (Variables|/Game/Coding/BluePrints/BP_Mirror.BP_Mirror_C|GetDefaultSceneRoot _returnvalue_2)))) false false)
        (Default|UpdatePositionNoGrab _returnvalue_2))
      (:then_2
        (Utilities|FlowControl|Delay 1.0)
        (Default|Toggle (Variables|Default|GetComp_Switch))))))

(event EventBeginPlay
  (Utilities|FlowControl|Delay 0.2)
  (Variables|Default|Setpressed false)
  (bind _returnvalue (Actor|GetActorOfClass "/Game/Coding/BluePrints/BP_Mirror_Spheres.BP_Mirror_Spheres_C"))
  (Rendering|SetActorHiddenInGame _returnvalue false)
  (bind _returnvalue_2 (Actor|GetActorOfClass "/Game/Coding/BluePrints/BP_Mirror_Cube.BP_Mirror_Cube_C"))
  (Transformation|SetActorScale3D _returnvalue_2 "1.000000,1.000000,1.000000"))

(fn ConstructionScript
  (|CallParentFunction))