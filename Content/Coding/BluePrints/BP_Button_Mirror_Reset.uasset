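; Button Blueprint, named for a mirror reset, that behaves as a momentary switch by releasing itself after being pressed.
; Its switch component's state change drives the Pressed flag, and a press toggles the switch again after a one-second delay.
; BeginPlay clears Pressed after a brief delay, and the construction script defers to its parent.
; No mirror reset logic appears in these graphs.
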(event OnStateChanged(Comp_Switch)
  (params (SourceInfo :type Struct%20Component%20Source%20Info%20Structure) (Value :type Boolean))
  (bind _output_get (Variables|Default|Setpressed Value))
  (if _output_get
    (Utilities|FlowControl|Sequence
      (:then_2
        (Utilities|FlowControl|Delay 1.0)
        (Default|Toggle (Variables|Default|GetComp_Switch))))))

(event EventBeginPlay
  (Utilities|FlowControl|Delay 0.2)
  (Variables|Default|Setpressed false))

(fn ConstructionScript
  (|CallParentFunction))