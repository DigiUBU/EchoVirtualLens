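; BP_Mirror is a grabbable actor that can have a duplicate in a mirrored space, offset a fixed distance along X.
; MirrorObject spawns and records a same-class copy, hidden and without collision when flagged as a Reference.
; For references, releasing the grab or calling UpdatePositionNoGrab syncs the copy's transform and visibility through UpdatePosition, without flipping any axis.
; BeginPlay creates a dynamic material and caches initial color and transform.
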(event GrabActorReleased(Comp_Grab)
  (params (ReleasingPawn :type BP%20Pawn%20Base%20Object%20Reference) (ReleasingActor :type Actor%20Object%20Reference) (LastRelease :type Boolean))
  (bind _reference (Variables|Default|Getreference))
  (if _reference
    (CallFunction|UpdatePosition _reference (Variables|Default|GetmirroredObject) self)))

(event Custom|UpdatePositionNoGrab
  (bind _reference (Variables|Default|Getreference))
  (if _reference
    (CallFunction|UpdatePosition _reference (Variables|Default|GetmirroredObject) self)))

(event EventBeginPlay
  (bind _staticmesh (Variables|Default|GetStaticMesh))
  (bind _returnvalue (Rendering|Material|CreateDynamicMaterialInstance _staticmesh 0 (Rendering|Material|GetMaterial _staticmesh 0) "None" :!class /Script/Engine.PrimitiveComponent))
  (bind _returnvalue_2 (Rendering|Material|GetVectorParameterValue _returnvalue (Variables|Default|GetparameterNameColor) :!class /Script/Engine.MaterialInstanceDynamic))
  (Variables|Default|SetinitialColor _returnvalue_2)
  (Variables|Default|SetinitialTransform (Transformation|GetActorTransform)))

(fn ConstructionScript)

(fn MirrorObject
  (params (actorMirror :type Actor%20Object%20Reference) (reference :type Boolean))
  (bind _returnvalue (Transformation|GetActorTransform actorMirror))
  (Variables|Default|Setreference reference)
  (bind _returnvalue_2 (Game|SpawnActorfromClass (Utilities|GetClass actorMirror) (Math|Transform|MakeTransform (Math|Vector|MakeVector (- (.x (.location _returnvalue)) 1e+03) (.y (.location _returnvalue)) (.z (.location _returnvalue))) (.rotation _returnvalue) (.scale _returnvalue)) "Undefined" "MultiplyWithRoot" actorMirror 0))
  (bind _output_get (Variables|Default|SetmirroredObject _returnvalue_2))
  (Utilities|Array|Add (Variables|Default|GetarrayObjects) _output_get)
  (if reference
    (Collision|SetActorEnableCollision _output_get false)
    (Rendering|SetActorHiddenInGame _output_get true))
  (return true _output_get reference))

(fn UpdatePosition
  (params (mirrorActivated :type Boolean) (mirroredObject :type Actor%20Object%20Reference) (objectToMirror :type Actor%20Object%20Reference))
  (bind _returnvalue (Transformation|GetActorTransform objectToMirror))
  (if mirrorActivated
    (Transformation|SetActorTransform mirroredObject (Math|Transform|MakeTransform (Math|Vector|MakeVector (- (.x (.location _returnvalue)) 1e+03) (.y (.location _returnvalue)) (.z (.location _returnvalue))) (.rotation _returnvalue) (.scale _returnvalue)))
    (Rendering|SetActorHiddenInGame mirroredObject (Variables|/Script/Engine.Actor|GetbHidden objectToMirror))
    (Transformation|SetActorScale3D mirroredObject (Transformation|GetActorScale3D objectToMirror))))