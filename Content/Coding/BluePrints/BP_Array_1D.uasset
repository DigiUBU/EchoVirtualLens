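; BP_Array_1D is a 1D array placement puzzle that checks whether eight numbered cubes sit on their matching anchors.
; Anchor attach and detach events set a flag per slot, except slot 0, whose detach reset is unwired.
; When Tick finds all flags true, it sets Array1Dcollocated and, after a delay, changes cube materials, hides their labels and disables their collision.
; A DoOnce then moves the BP_Tablet_1D interactive tablet to a fixed location.
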(event ActorGotAttached(Comp_Anchor3)
  (params (Anchor :type Comp%20Anchor%20Object%20Reference) (Actor :type Actor%20Object%20Reference) (Connector :type Comp%20Connector%20Anchor%20Object%20Reference))
  (Utilities|Casting|CastToBP_Array_Cube_1D_3 Actor)
  (Variables|Default|Setok_3 true))

(event ActorGotDetached(Comp_Anchor3)
  (params (Anchor :type Comp%20Anchor%20Object%20Reference) (Actor :type Actor%20Object%20Reference) (Connector :type Comp%20Connector%20Anchor%20Object%20Reference))
  (Utilities|Casting|CastToBP_Array_Cube_1D_3 Actor)
  (Variables|Default|Setok_3 false))

(event ActorGotDetached(Comp_Anchor4)
  (params (Anchor :type Comp%20Anchor%20Object%20Reference) (Actor :type Actor%20Object%20Reference) (Connector :type Comp%20Connector%20Anchor%20Object%20Reference))
  (Utilities|Casting|CastToBP_Array_Cube_1D_4 Actor)
  (Variables|Default|Setok_4 false))

(event ActorGotAttached(Comp_Anchor4)
  (params (Anchor :type Comp%20Anchor%20Object%20Reference) (Actor :type Actor%20Object%20Reference) (Connector :type Comp%20Connector%20Anchor%20Object%20Reference))
  (Utilities|Casting|CastToBP_Array_Cube_1D_4 Actor)
  (Variables|Default|Setok_4 true))

(event ActorGotDetached(Comp_Anchor6)
  (params (Anchor :type Comp%20Anchor%20Object%20Reference) (Actor :type Actor%20Object%20Reference) (Connector :type Comp%20Connector%20Anchor%20Object%20Reference))
  (Utilities|Casting|CastToBP_Array_Cube_1D_6 Actor)
  (Variables|Default|Setok_6 false))

(event ActorGotAttached(Comp_Anchor6)
  (params (Anchor :type Comp%20Anchor%20Object%20Reference) (Actor :type Actor%20Object%20Reference) (Connector :type Comp%20Connector%20Anchor%20Object%20Reference))
  (Utilities|Casting|CastToBP_Array_Cube_1D_6 Actor)
  (Variables|Default|Setok_6 true))

(event ActorGotDetached(Comp_Anchor5)
  (params (Anchor :type Comp%20Anchor%20Object%20Reference) (Actor :type Actor%20Object%20Reference) (Connector :type Comp%20Connector%20Anchor%20Object%20Reference))
  (Utilities|Casting|CastToBP_Array_Cube_1D_5 Actor)
  (Variables|Default|Setok_5 false))

(event ActorGotAttached(Comp_Anchor5)
  (params (Anchor :type Comp%20Anchor%20Object%20Reference) (Actor :type Actor%20Object%20Reference) (Connector :type Comp%20Connector%20Anchor%20Object%20Reference))
  (Utilities|Casting|CastToBP_Array_Cube_1D_5 Actor)
  (Variables|Default|Setok_5 true))

(event ActorGotDetached(Comp_Anchor2)
  (params (Anchor :type Comp%20Anchor%20Object%20Reference) (Actor :type Actor%20Object%20Reference) (Connector :type Comp%20Connector%20Anchor%20Object%20Reference))
  (Utilities|Casting|CastToBP_Array_Cube_1D_2 Actor)
  (Variables|Default|Setok_2 false))

(event ActorGotAttached(Comp_Anchor2)
  (params (Anchor :type Comp%20Anchor%20Object%20Reference) (Actor :type Actor%20Object%20Reference) (Connector :type Comp%20Connector%20Anchor%20Object%20Reference))
  (Utilities|Casting|CastToBP_Array_Cube_1D_2 Actor)
  (Variables|Default|Setok_2 true))

(event ActorGotDetached(Comp_Anchor0)
  (params (Anchor :type Comp%20Anchor%20Object%20Reference) (Actor :type Actor%20Object%20Reference) (Connector :type Comp%20Connector%20Anchor%20Object%20Reference)))

(event ActorGotAttached(Comp_Anchor0)
  (params (Anchor :type Comp%20Anchor%20Object%20Reference) (Actor :type Actor%20Object%20Reference) (Connector :type Comp%20Connector%20Anchor%20Object%20Reference))
  (Utilities|Casting|CastToBP_Array_Cube_1D_0 Actor)
  (Variables|Default|Setok_0 true))

(event ActorGotDetached(Comp_Anchor1)
  (params (Anchor :type Comp%20Anchor%20Object%20Reference) (Actor :type Actor%20Object%20Reference) (Connector :type Comp%20Connector%20Anchor%20Object%20Reference))
  (Utilities|Casting|CastToBP_Array_Cube_1D_1 Actor)
  (Variables|Default|Setok_1 false))

(event ActorGotAttached(Comp_Anchor1)
  (params (Anchor :type Comp%20Anchor%20Object%20Reference) (Actor :type Actor%20Object%20Reference) (Connector :type Comp%20Connector%20Anchor%20Object%20Reference))
  (Utilities|Casting|CastToBP_Array_Cube_1D_1 Actor)
  (Variables|Default|Setok_1 true))

(event ActorGotDetached(Comp_Anchor7)
  (params (Anchor :type Comp%20Anchor%20Object%20Reference) (Actor :type Actor%20Object%20Reference) (Connector :type Comp%20Connector%20Anchor%20Object%20Reference))
  (Utilities|Casting|CastToBP_Array_Cube_1D_7 Actor)
  (Variables|Default|Setok_7 false))

(event ActorGotAttached(Comp_Anchor7)
  (params (Anchor :type Comp%20Anchor%20Object%20Reference) (Actor :type Actor%20Object%20Reference) (Connector :type Comp%20Connector%20Anchor%20Object%20Reference))
  (Utilities|Casting|CastToBP_Array_Cube_1D_7 Actor)
  (Variables|Default|Setok_7 true))

(event EventTick
  (params (DeltaSeconds :type Float%20%28single-precision%29))
  (if (Math|Boolean|ANDBoolean (Variables|Default|Getok_0) (Variables|Default|Getok_1) (Variables|Default|Getok_2) (Variables|Default|Getok_3) (Variables|Default|Getok_4) (Variables|Default|Getok_5) (Variables|Default|Getok_6) (Variables|Default|Getok_7))
    (Utilities|FlowControl|Sequence
      (:then_0
        (Variables|Default|Setarray1Dcollocated true))
      (:then_1
        (Utilities|FlowControl|Delay 2.0)
        (bind _returnvalue (Actor|GetActorOfClass "/Game/Coding/BluePrints/BP_Array_Cube_1D_0.BP_Array_Cube_1D_0_C"))
        (Rendering|Material|SetMaterial (Variables|/Game/Coding/BluePrints/BP_Array_Cube_1D_0.BP_Array_Cube_1D_0_C|Getboard_array_cube _returnvalue) 0 "/Game/Coding/Mesh/Objects/MaterialTextureObject/Mat_Cube_1D_Show.Mat_Cube_1D_Show")
        (bind _returnvalue_2 (Actor|GetActorOfClass "/Game/Coding/BluePrints/BP_Array_Cube_1D_1.BP_Array_Cube_1D_1_C"))
        (Rendering|Material|SetMaterial (Variables|/Game/Coding/BluePrints/BP_Array_Cube_1D_1.BP_Array_Cube_1D_1_C|Getboard_array_cube _returnvalue_2) 0 "/Game/Coding/Mesh/Objects/MaterialTextureObject/Mat_Cube_1D_Show.Mat_Cube_1D_Show")
        (bind _returnvalue_3 (Actor|GetActorOfClass "/Game/Coding/BluePrints/BP_Array_Cube_1D_2.BP_Array_Cube_1D_2_C"))
        (Rendering|Material|SetMaterial (Variables|/Game/Coding/BluePrints/BP_Array_Cube_1D_2.BP_Array_Cube_1D_2_C|Getboard_array_cube _returnvalue_3) 0 "/Game/Coding/Mesh/Objects/MaterialTextureObject/Mat_Cube_1D_Show.Mat_Cube_1D_Show")
        (bind _returnvalue_4 (Actor|GetActorOfClass "/Game/Coding/BluePrints/BP_Array_Cube_1D_3.BP_Array_Cube_1D_3_C"))
        (Rendering|Material|SetMaterial (Variables|/Game/Coding/BluePrints/BP_Array_Cube_1D_3.BP_Array_Cube_1D_3_C|Getboard_array_cube _returnvalue_4) 0 "/Game/Coding/Mesh/Objects/MaterialTextureObject/Mat_Cube_1D_Show.Mat_Cube_1D_Show")
        (bind _returnvalue_5 (Actor|GetActorOfClass "/Game/Coding/BluePrints/BP_Array_Cube_1D_4.BP_Array_Cube_1D_4_C"))
        (Rendering|Material|SetMaterial (Variables|/Game/Coding/BluePrints/BP_Array_Cube_1D_4.BP_Array_Cube_1D_4_C|Getboard_array_cube _returnvalue_5) 0 "/Game/Coding/Mesh/Objects/MaterialTextureObject/Mat_Cube_1D_Show.Mat_Cube_1D_Show")
        (bind _returnvalue_6 (Actor|GetActorOfClass "/Game/Coding/BluePrints/BP_Array_Cube_1D_5.BP_Array_Cube_1D_5_C"))
        (Rendering|Material|SetMaterial (Variables|/Game/Coding/BluePrints/BP_Array_Cube_1D_5.BP_Array_Cube_1D_5_C|Getboard_array_cube _returnvalue_6) 0 "/Game/Coding/Mesh/Objects/MaterialTextureObject/Mat_Cube_1D_Show.Mat_Cube_1D_Show")
        (bind _returnvalue_7 (Actor|GetActorOfClass "/Game/Coding/BluePrints/BP_Array_Cube_1D_6.BP_Array_Cube_1D_6_C"))
        (Rendering|Material|SetMaterial (Variables|/Game/Coding/BluePrints/BP_Array_Cube_1D_6.BP_Array_Cube_1D_6_C|Getboard_array_cube _returnvalue_7) 0 "/Game/Coding/Mesh/Objects/MaterialTextureObject/Mat_Cube_1D_Show.Mat_Cube_1D_Show")
        (bind _returnvalue_8 (Actor|GetActorOfClass "/Game/Coding/BluePrints/BP_Array_Cube_1D_7.BP_Array_Cube_1D_7_C"))
        (Rendering|Material|SetMaterial (Variables|/Game/Coding/BluePrints/BP_Array_Cube_1D_7.BP_Array_Cube_1D_7_C|Getboard_array_cube _returnvalue_8) 0 "/Game/Coding/Mesh/Objects/MaterialTextureObject/Mat_Cube_1D_Show.Mat_Cube_1D_Show")
        (bind _asw_array_1d_0 (Utilities|Casting|CastToW_Array_1D_0 (UserInterface|GetWidget (Variables|/Game/Coding/BluePrints/BP_Array_Cube_1D_0.BP_Array_Cube_1D_0_C|GetWidget _returnvalue))))
        (Variables|/Script/UMG.Widget|SetVisibility (Variables|/Game/Coding/Widgets/UI_Array/1D/W_Array_1D_0.W_Array_1D_0_C|GetTextBlock_0 _asw_array_1d_0) "Hidden")
        (bind _asw_array_1d_1 (Utilities|Casting|CastToW_Array_1D_1 (UserInterface|GetWidget (Variables|/Game/Coding/BluePrints/BP_Array_Cube_1D_1.BP_Array_Cube_1D_1_C|GetWidget _returnvalue_2))))
        (Variables|/Script/UMG.Widget|SetVisibility (Variables|/Game/Coding/Widgets/UI_Array/1D/W_Array_1D_1.W_Array_1D_1_C|GetTextBlock_0 _asw_array_1d_1) "Hidden")
        (bind _asw_array_1d_2 (Utilities|Casting|CastToW_Array_1D_2 (UserInterface|GetWidget (Variables|/Game/Coding/BluePrints/BP_Array_Cube_1D_2.BP_Array_Cube_1D_2_C|GetWidget _returnvalue_3))))
        (Variables|/Script/UMG.Widget|SetVisibility (Variables|/Game/Coding/Widgets/UI_Array/1D/W_Array_1D_2.W_Array_1D_2_C|GetTextBlock_0 _asw_array_1d_2) "Hidden")
        (bind _asw_array_1d_3 (Utilities|Casting|CastToW_Array_1D_3 (UserInterface|GetWidget (Variables|/Game/Coding/BluePrints/BP_Array_Cube_1D_3.BP_Array_Cube_1D_3_C|GetWidget _returnvalue_4))))
        (Variables|/Script/UMG.Widget|SetVisibility (Variables|/Game/Coding/Widgets/UI_Array/1D/W_Array_1D_3.W_Array_1D_3_C|GetTextBlock_0 _asw_array_1d_3) "Hidden")
        (bind _asw_array_1d_4 (Utilities|Casting|CastToW_Array_1D_4 (UserInterface|GetWidget (Variables|/Game/Coding/BluePrints/BP_Array_Cube_1D_4.BP_Array_Cube_1D_4_C|GetWidget _returnvalue_5))))
        (Variables|/Script/UMG.Widget|SetVisibility (Variables|/Game/Coding/Widgets/UI_Array/1D/W_Array_1D_4.W_Array_1D_4_C|GetTextBlock_0 _asw_array_1d_4) "Hidden")
        (bind _asw_array_1d_5 (Utilities|Casting|CastToW_Array_1D_5 (UserInterface|GetWidget (Variables|/Game/Coding/BluePrints/BP_Array_Cube_1D_5.BP_Array_Cube_1D_5_C|GetWidget _returnvalue_6))))
        (Variables|/Script/UMG.Widget|SetVisibility (Variables|/Game/Coding/Widgets/UI_Array/1D/W_Array_1D_5.W_Array_1D_5_C|GetTextBlock_0 _asw_array_1d_5) "Hidden")
        (bind _asw_array_1d_6 (Utilities|Casting|CastToW_Array_1D_6 (UserInterface|GetWidget (Variables|/Game/Coding/BluePrints/BP_Array_Cube_1D_6.BP_Array_Cube_1D_6_C|GetWidget _returnvalue_7))))
        (Variables|/Script/UMG.Widget|SetVisibility (Variables|/Game/Coding/Widgets/UI_Array/1D/W_Array_1D_6.W_Array_1D_6_C|GetTextBlock_0 _asw_array_1d_6) "Hidden")
        (bind _asw_array_1d_7 (Utilities|Casting|CastToW_Array_1D_7 (UserInterface|GetWidget (Variables|/Game/Coding/BluePrints/BP_Array_Cube_1D_7.BP_Array_Cube_1D_7_C|GetWidget _returnvalue_8))))
        (Variables|/Script/UMG.Widget|SetVisibility (Variables|/Game/Coding/Widgets/UI_Array/1D/W_Array_1D_7.W_Array_1D_7_C|GetTextBlock_0 _asw_array_1d_7) "Hidden")
        (Collision|SetCollisionEnabled (Variables|/Game/Coding/BluePrints/BP_Array_Cube_1D_0.BP_Array_Cube_1D_0_C|Getboard_array_cube _returnvalue) "NoCollision")
        (Collision|SetCollisionEnabled (Variables|/Game/Coding/BluePrints/BP_Array_Cube_1D_1.BP_Array_Cube_1D_1_C|Getboard_array_cube _returnvalue_2) "NoCollision")
        (Collision|SetCollisionEnabled (Variables|/Game/Coding/BluePrints/BP_Array_Cube_1D_2.BP_Array_Cube_1D_2_C|Getboard_array_cube _returnvalue_3) "NoCollision")
        (Collision|SetCollisionEnabled (Variables|/Game/Coding/BluePrints/BP_Array_Cube_1D_3.BP_Array_Cube_1D_3_C|Getboard_array_cube _returnvalue_4) "NoCollision")
        (Collision|SetCollisionEnabled (Variables|/Game/Coding/BluePrints/BP_Array_Cube_1D_4.BP_Array_Cube_1D_4_C|Getboard_array_cube _returnvalue_5) "NoCollision")
        (Collision|SetCollisionEnabled (Variables|/Game/Coding/BluePrints/BP_Array_Cube_1D_5.BP_Array_Cube_1D_5_C|Getboard_array_cube _returnvalue_6) "NoCollision")
        (Collision|SetCollisionEnabled (Variables|/Game/Coding/BluePrints/BP_Array_Cube_1D_6.BP_Array_Cube_1D_6_C|Getboard_array_cube _returnvalue_7) "NoCollision")
        (Collision|SetCollisionEnabled (Variables|/Game/Coding/BluePrints/BP_Array_Cube_1D_7.BP_Array_Cube_1D_7_C|Getboard_array_cube _returnvalue_8) "NoCollision")
        (Utilities|FlowControl|DoOnce false
          (:Completed
            (bind _returnvalue_9 (Actor|GetActorOfClass "/Game/Coding/BluePrints/BP_Tablet_1D.BP_Tablet_1D_C"))
            (Transformation|SetWorldLocation (Variables|/Game/Coding/BluePrints/BP_Tablet_1D.BP_Tablet_1D_C|Getinteractive_tablet _returnvalue_9) "-67.000000,-14.000000,15.000000" false false)))))))

(fn ConstructionScript)