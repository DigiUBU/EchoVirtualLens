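; Cone actor that cycles through six preset colors and six preset sizes, wrapping back to the first.
; On BeginPlay it stores the starting color and scale and registers itself as owner of its UI_Synchro_Menu widget.
; ToChangeColor matches the material's ColorParam against the presets and applies the next through a new Synchro_2 dynamic instance.
; ToChangeSize steps the cone's scale and repositions the widget to a fixed offset for each size.
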(event Custom|ToChangeColor
  (bind _cone (Variables|Default|GetCone))
  (bind _returnvalue (Rendering|Material|CreateDynamicMaterialInstance _cone 0 (Rendering|Material|GetMaterial _cone 0) "None" :!class /Script/Engine.PrimitiveComponent))
  (bind _returnvalue_2 (Rendering|Material|GetVectorParameterValue _returnvalue "ColorParam" :!class /Script/Engine.MaterialInstanceDynamic))
  (CallFunction|ChangeColor _returnvalue_2))

(event Custom|ToChangeSize
  (CallFunction|ChangeScale (Variables|Default|GetcurrentScale)))

(event EventBeginPlay
  (bind _cone (Variables|Default|GetCone))
  (bind _color_0 (Variables|Default|GetColor_0))
  (bind _returnvalue (Rendering|Material|CreateDynamicMaterialInstance _cone 0 (Rendering|Material|GetMaterial _cone 0) "None" :!class /Script/Engine.PrimitiveComponent))
  (Rendering|Material|SetVectorParameterValue _returnvalue "None" _color_0 :!class /Script/Engine.MaterialInstanceDynamic)
  (Variables|Default|SetcurrentColor _color_0)
  (bind _output_get (Variables|Default|SetcurrentScale (Variables|/Script/Engine.SceneComponent|GetRelativeScale3D (Variables|Default|GetCone))))
  (Variables|Default|Setscale_0 _output_get)
  (bind _asui_synchro_menu (Utilities|Casting|CastToUI_Synchro_Menu (UserInterface|GetWidget (Variables|Default|GetWidget))))
  (Variables|/Game/Coding/Widgets/Synchro/UI_Synchro_Menu.UI_Synchro_Menu_C|SetownerCone _asui_synchro_menu self)
  (Variables|/Game/Coding/Widgets/Synchro/UI_Synchro_Menu.UI_Synchro_Menu_C|SetconeOwner _asui_synchro_menu true))

(event EventTick
  (params (DeltaSeconds :type Float%20%28single-precision%29)))

(fn ConstructionScript)

(fn ChangeColor
  (params (currentColor :type Linear%20Color%20Structure :default "(R=0.000000,G=0.000000,B=0.000000,A=1.000000)"))
  (bind _color_2 (Variables|Default|GetColor_2))
  (bind _color_3 (Variables|Default|GetColor_3))
  (bind _color_4 (Variables|Default|GetColor_4))
  (bind _color_5 (Variables|Default|GetColor_5))
  (bind _color_0 (Variables|Default|GetColor_0))
  (bind _cone (Variables|Default|GetCone))
  (bind _color_1 (Variables|Default|GetColor_1))
  (if (Class|KismetMathLibrary|LinearColorIsNearEqual currentColor (Variables|Default|GetColor_0) 0.0001)
    (bind _returnvalue (Rendering|Material|CreateDynamicMaterialInstance _cone 0 "/Game/Coding/Mesh/Objects/MaterialTextureObject/Synchro_2.Synchro_2" "None" :!class /Script/Engine.PrimitiveComponent))
    (Rendering|Material|SetVectorParameterValue _returnvalue "ColorParam" _color_1 :!class /Script/Engine.MaterialInstanceDynamic)
    (Variables|Default|SetcurrentColor _color_1)
    (elif (Class|KismetMathLibrary|LinearColorIsNearEqual currentColor (Variables|Default|GetColor_1) 0.0001)
      (bind _returnvalue_2 (Rendering|Material|CreateDynamicMaterialInstance _cone 0 "/Game/Coding/Mesh/Objects/MaterialTextureObject/Synchro_2.Synchro_2" "None" :!class /Script/Engine.PrimitiveComponent))
      (Rendering|Material|SetVectorParameterValue _returnvalue_2 "ColorParam" _color_2 :!class /Script/Engine.MaterialInstanceDynamic)
      (Variables|Default|SetcurrentColor _color_2)
      (elif (Class|KismetMathLibrary|LinearColorIsNearEqual currentColor (Variables|Default|GetColor_2) 0.0001)
        (bind _returnvalue_3 (Rendering|Material|CreateDynamicMaterialInstance _cone 0 "/Game/Coding/Mesh/Objects/MaterialTextureObject/Synchro_2.Synchro_2" "None" :!class /Script/Engine.PrimitiveComponent))
        (Rendering|Material|SetVectorParameterValue _returnvalue_3 "ColorParam" _color_3 :!class /Script/Engine.MaterialInstanceDynamic)
        (Variables|Default|SetcurrentColor _color_3)
        (elif (Class|KismetMathLibrary|LinearColorIsNearEqual currentColor (Variables|Default|GetColor_3) 0.0001)
          (bind _returnvalue_4 (Rendering|Material|CreateDynamicMaterialInstance _cone 0 "/Game/Coding/Mesh/Objects/MaterialTextureObject/Synchro_2.Synchro_2" "None" :!class /Script/Engine.PrimitiveComponent))
          (Rendering|Material|SetVectorParameterValue _returnvalue_4 "ColorParam" _color_4 :!class /Script/Engine.MaterialInstanceDynamic)
          (Variables|Default|SetcurrentColor _color_4)
          (elif (Class|KismetMathLibrary|LinearColorIsNearEqual currentColor (Variables|Default|GetColor_4) 0.0001)
            (bind _returnvalue_5 (Rendering|Material|CreateDynamicMaterialInstance _cone 0 "/Game/Coding/Mesh/Objects/MaterialTextureObject/Synchro_2.Synchro_2" "None" :!class /Script/Engine.PrimitiveComponent))
            (Rendering|Material|SetVectorParameterValue _returnvalue_5 "ColorParam" _color_5 :!class /Script/Engine.MaterialInstanceDynamic)
            (Variables|Default|SetcurrentColor _color_5)
            (elif (Class|KismetMathLibrary|LinearColorIsNearEqual currentColor (Variables|Default|GetColor_5) 0.0001)
              (bind _returnvalue_6 (Rendering|Material|CreateDynamicMaterialInstance _cone 0 "/Game/Coding/Mesh/Objects/MaterialTextureObject/Synchro_2.Synchro_2" "None" :!class /Script/Engine.PrimitiveComponent))
              (Rendering|Material|SetVectorParameterValue _returnvalue_6 "ColorParam" _color_0 :!class /Script/Engine.MaterialInstanceDynamic)
              (Variables|Default|SetcurrentColor _color_0))))))))

(fn ChangeScale
  (params (currentScale :type Vector))
  (bind _scale_0 (Variables|Default|Getscale_0))
  (bind _scale_5 (Variables|Default|Getscale_5))
  (bind _scale_4 (Variables|Default|Getscale_4))
  (bind _scale_3 (Variables|Default|Getscale_3))
  (bind _scale_2 (Variables|Default|Getscale_2))
  (bind _scale_1 (Variables|Default|Getscale_1))
  (bind _widget (Variables|Default|GetWidget))
  (if (Class|KismetMathLibrary|EqualExactlyVectorVector currentScale (Variables|Default|Getscale_0))
    (Transformation|SetRelativeScale3D (Variables|Default|GetCone) _scale_1)
    (Variables|Default|SetcurrentScale _scale_1)
    (Transformation|SetRelativeLocation _widget "8.278097,-1.559170,-5.624530" false false)
    (elif (Class|KismetMathLibrary|EqualExactlyVectorVector currentScale (Variables|Default|Getscale_1))
      (Transformation|SetRelativeScale3D (Variables|Default|GetCone) _scale_2)
      (Variables|Default|SetcurrentScale _scale_2)
      (Transformation|SetRelativeLocation _widget "22.364323,-1.559170,-16.000000" false false)
      (elif (Class|KismetMathLibrary|EqualExactlyVectorVector currentScale (Variables|Default|Getscale_2))
        (Transformation|SetRelativeScale3D (Variables|Default|GetCone) _scale_3)
        (Variables|Default|SetcurrentScale _scale_3)
        (Transformation|SetRelativeLocation _widget "31.242591,-1.559170,-20.000000" false false)
        (elif (Class|KismetMathLibrary|EqualExactlyVectorVector currentScale (Variables|Default|Getscale_3))
          (Transformation|SetRelativeScale3D (Variables|Default|GetCone) _scale_4)
          (Variables|Default|SetcurrentScale _scale_4)
          (Transformation|SetRelativeLocation _widget "49.479058,-1.559170,-27.000000" false false)
          (elif (Class|KismetMathLibrary|EqualExactlyVectorVector currentScale (Variables|Default|Getscale_4))
            (Transformation|SetRelativeScale3D (Variables|Default|GetCone) _scale_5)
            (Variables|Default|SetcurrentScale _scale_5)
            (Transformation|SetRelativeLocation _widget "62.450659,-1.559170,-32.000000" false false)
            (elif (Class|KismetMathLibrary|EqualExactlyVectorVector currentScale (Variables|Default|Getscale_5))
              (Transformation|SetRelativeScale3D (Variables|Default|GetCone) _scale_0)
              (Variables|Default|SetcurrentScale _scale_0)
              (Transformation|SetRelativeLocation _widget "12.345809,-1.559170,-6.724200" false false))))))))