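; BP_Tablet_2D is a tablet actor that visualises 2D array loop output by lighting up matching cubes in the level.
; While Ready, Tick reads IndexToPrint from its W_loop_2D widget and pairs each BP_Array_Cube_2D_Loop_00 with its displayed index.
; A bubble-style pass attempts to order these pairs.
; A DoOnce-gated delayed loop recolours matches at a quickening pace, then restores their materials, resets BP_Button and re-arms.
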(event Custom|BrightCubes
  (params (cube :type BP%20Array%20Cube%202D%20Loop%2000%20Object%20Reference))
  (Utilities|Array|Add (Variables|Default|GetcubesBright) cube)
  (CallFunction|SortStruct))

(event Custom|CustomEvent
  ;[1 1 1] debug
  (bind _asw_loop_2d (Utilities|Casting|CastToW_loop_2D (UserInterface|GetWidget (Variables|Default|GetWidget))))
  (for _array_element (Variables|/Game/Coding/Widgets/UI_Array/2D_Loop/W_loop_2D.W_loop_2D_C|GetindexToPrint _asw_loop_2d)
    (Development|PrintString (Utilities|String|ToString(Text) _array_element))))

(event Custom|SortStruct
  (bind _structindex (Variables|Default|GetstructIndex))
  (bind _returnvalue (Utilities|Array|Length _structindex))
  (Utilities|ForLoopwithDelay 0 (- _returnvalue 2) 0.0
    (:LoopBody
      (bind _index (Utilities|ForLoopwithDelay 0 (- _returnvalue 2) 0.0)
        (:LoopBody
          (if (> (.index (Utilities|Array|Get(acopy) _structindex _index)) (.index (Utilities|Array|Get(acopy) _structindex (+ _index 1))))
            (Utilities|Array|Swap _structindex (.index (Utilities|Array|Get(acopy) _structindex _index)) (.index (Utilities|Array|Get(acopy) _structindex (+ _index 1))))))))))

(event EventTick
  (params (DeltaSeconds :type Float%20%28single-precision%29))
  (if (Variables|Default|Getready)
    (bind _asw_loop_2d (Utilities|Casting|CastToW_loop_2D (UserInterface|GetUserWidgetObject (Variables|Default|GetWidget))))
    (for _array_element (Variables|/Game/Coding/Widgets/UI_Array/2D_Loop/W_loop_2D.W_loop_2D_C|GetindexToPrint _asw_loop_2d)
      (bind _returnvalue (Utilities|Array|Add (Variables|Default|Gettest) (Class|VictoryBPFunctionLibrary|TexttoInt _array_element)))
      (bind _returnvalue_2 (Actor|GetActorOfClass "/Game/Coding/BluePrints/BP_Array_Cube_2D_Loop_00.BP_Array_Cube_2D_Loop_00_C"))
      (if (Utilities|Array|ContainsItem (Variables|/Game/Coding/BluePrints/BP_Array_Cube_2D_Loop_00.BP_Array_Cube_2D_Loop_00_C|Getarray2Dindex _returnvalue_2) _returnvalue)
        (bind _outactors (Actor|GetAllActorsOfClass "/Game/Coding/BluePrints/BP_Array_Cube_2D_Loop_00.BP_Array_Cube_2D_Loop_00_C"))
        (for _array_element_2 _outactors
          (bind _asw_array_2d_loop_00 (Utilities|Casting|CastToW_Array_2D_Loop_00 (UserInterface|GetWidget (Variables|/Game/Coding/BluePrints/BP_Array_Cube_2D_Loop_00.BP_Array_Cube_2D_Loop_00_C|GetWidget _array_element_2))))
          (Utilities|Array|Add (Variables|Default|GetstructIndex) (Utilities|Struct|Makearray2D _array_element_2 (Math|Conversions|ToInteger(Byte) (Utilities|String|ToString(Text) (Variables|/Script/UMG.TextBlock|GetText (Variables|/Game/Coding/Widgets/UI_Array/2D/W_Array_2D_Loop_00.W_Array_2D_Loop_00_C|Getindex_2D _asw_array_2d_loop_00))))))
          (if (Utilities|Enum|Equal(Enum) _array_element (Variables|/Script/UMG.TextBlock|GetText (Variables|/Game/Coding/Widgets/UI_Array/2D/W_Array_2D_Loop_00.W_Array_2D_Loop_00_C|Getindex_2D _asw_array_2d_loop_00)))
            (CallFunction|BrightCubes _array_element_2)))))
    (Utilities|FlowControl|Sequence
      (:then_0
        (Utilities|FlowControl|DoOnce false :!label _label
          (:Completed
            (Variables|Default|Setrestart false)
            (bind _index (Utilities|ForLoopwithDelay 0 21 (Variables|Default|Getdelay))
              (:LoopBody
                (for _array_element_3 (Variables|Default|Gettest)
                  (if (== _array_element_3 (.index (Utilities|Array|Get(acopy) (Variables|Default|GetstructIndex) _index)))
                    (Rendering|Material|SetMaterial (Variables|/Game/Coding/BluePrints/BP_Array_Cube_2D_Loop_00.BP_Array_Cube_2D_Loop_00_C|Getboard_array_cube (.cube (Utilities|Array|Get(acopy) (Variables|Default|GetstructIndex) _index))) 0 "/Game/Coding/BluePrints/MAT_2darray.MAT_2darray")
                    (Rendering|Material|SetMaterial (Variables|/Game/Coding/BluePrints/BP_Array_Cube_2D_Loop_00.BP_Array_Cube_2D_Loop_00_C|Getboard_array_cube (.cube (Utilities|Array|Get(acopy) (Variables|Default|GetstructIndex) _index))) 1 "/Game/Coding/BluePrints/MAT_2darray.MAT_2darray")
                    (Variables|Default|Setdelay (- (Variables|Default|Getdelay) 0.05)))))
              (:Completed
                ;[1 1 1] connect to completed if we want to un-color cubes
                (Utilities|FlowControl|Delay 3.0)
                (bind _index_2 (Utilities|ForLoopwithDelay 0 21 0.1)
                  (:LoopBody
                    (Rendering|Material|SetMaterial (Variables|/Game/Coding/BluePrints/BP_Array_Cube_2D_Loop_00.BP_Array_Cube_2D_Loop_00_C|Getboard_array_cube (.cube (Utilities|Array|Get(acopy) (Variables|Default|GetstructIndex) _index_2))) 1 "/Game/Coding/Mesh/Objects/MaterialTextureObject/column.column")
                    (Rendering|Material|SetMaterial (Variables|/Game/Coding/BluePrints/BP_Array_Cube_2D_Loop_00.BP_Array_Cube_2D_Loop_00_C|Getboard_array_cube (.cube (Utilities|Array|Get(acopy) (Variables|Default|GetstructIndex) _index_2))) 0 "/Game/Coding/Mesh/Objects/MaterialTextureObject/row.row"))
                  (:Completed
                    (Variables|Default|Setrestart true)
                    (Variables|Default|Setdelay 1.0)
                    (bind _returnvalue_3 (Actor|GetActorOfClass "/Game/Coding/BluePrints/BP_Button.BP_Button_C"))
                    (Default|Reset _returnvalue_3))))))))
      (:then_1
        (if (Variables|Default|Getrestart)
          (goto _label Reset))))))

(fn ConstructionScript)