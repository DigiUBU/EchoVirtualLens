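; CE_DataRegistration tracks time spent in each CE level and handles progression to the next level.
; On BeginPlay it stores the level name, moves the player pawn to a fixed transform and starts RecordTime.
; RecordTime re-calls itself after short delays, incrementing that level's GameInstance_CE timer, except Level 03's, which is overwritten rather than accumulated.
; OpenNextLevel opens the hard-coded successor, routing Level 02 through the Level 03 intro.
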(event Custom|RecordTime
  (bind _asgame_instance_ce (Utilities|Casting|CastToGameInstance_CE (Game|GetGameInstance)))
  (switch string (Variables|Default|GetcurrentLevel)
    (:CE_Level_00
      (Utilities|FlowControl|Delay 0.1)
      (Variables|/Game/Coding/BluePrints/GameInstance_CE.GameInstance_CE_C|Settime_00 _asgame_instance_ce (+ (Variables|/Game/Coding/BluePrints/GameInstance_CE.GameInstance_CE_C|Gettime_00 _asgame_instance_ce) 0.1))
      (CallFunction|RecordTime))
    (:CE_Level_01
      (Utilities|FlowControl|Delay 0.1)
      (Variables|/Game/Coding/BluePrints/GameInstance_CE.GameInstance_CE_C|Settime_01 _asgame_instance_ce (+ (Variables|/Game/Coding/BluePrints/GameInstance_CE.GameInstance_CE_C|Gettime_01 _asgame_instance_ce) 0.1))
      (CallFunction|RecordTime))
    (:CE_Level_02
      (Utilities|FlowControl|Delay 0.1)
      (Variables|/Game/Coding/BluePrints/GameInstance_CE.GameInstance_CE_C|Settime_02 _asgame_instance_ce (+ (Variables|/Game/Coding/BluePrints/GameInstance_CE.GameInstance_CE_C|Gettime_02 _asgame_instance_ce) 0.1))
      (CallFunction|RecordTime))
    (:CE_Level_03
      (Utilities|FlowControl|Delay 0.1)
      (Variables|/Game/Coding/BluePrints/GameInstance_CE.GameInstance_CE_C|Settime_03 _asgame_instance_ce (+ 0.0 0.1))
      (CallFunction|RecordTime))
    (:CE_Level_04
      (Utilities|FlowControl|Delay 0.1)
      (Variables|/Game/Coding/BluePrints/GameInstance_CE.GameInstance_CE_C|Settime_04 _asgame_instance_ce (+ (Variables|/Game/Coding/BluePrints/GameInstance_CE.GameInstance_CE_C|Gettime_04 _asgame_instance_ce) 0.1))
      (CallFunction|RecordTime))
    (:CE_Level_05
      (Utilities|FlowControl|Delay 0.1)
      (Variables|/Game/Coding/BluePrints/GameInstance_CE.GameInstance_CE_C|Settime_05 _asgame_instance_ce (+ (Variables|/Game/Coding/BluePrints/GameInstance_CE.GameInstance_CE_C|Gettime_05 _asgame_instance_ce) 0.1))
      (CallFunction|RecordTime))
    (:CE_Level_03_Intro
      (Utilities|FlowControl|Delay 0.1)
      (Variables|/Game/Coding/BluePrints/GameInstance_CE.GameInstance_CE_C|Settime_03_1 _asgame_instance_ce (+ (Variables|/Game/Coding/BluePrints/GameInstance_CE.GameInstance_CE_C|Gettime_03_1 _asgame_instance_ce) 0.1))
      (CallFunction|RecordTime))))

(event EventBeginPlay
  (bind _returnvalue (Game|GetCurrentLevelName true))
  (Variables|Default|SetcurrentLevel _returnvalue)
  (Transformation|SetActorLocationAndRotation (Game|Player|GetPlayerPawn 0) "-658.975752,287.443141,10.982586" "0.000000,-90.000000,0.000000")
  (CallFunction|RecordTime))

(fn ConstructionScript)

(fn OpenNextLevel
  (switch string (Variables|Default|GetcurrentLevel)
    (:CE_Level_00
      (Game|OpenLevel(byName) "CE_Level_01"))
    (:CE_Level_01
      (Game|OpenLevel(byName) "CE_Level_02"))
    (:CE_Level_02
      (Game|OpenLevel(byName) "CE_Level_03_Intro"))
    (:CE_Level_03
      (Game|OpenLevel(byName) "CE_Level_04"))
    (:CE_Level_04
      (Game|OpenLevel(byName) "CE_Level_05"))
    (:CE_Level_05
      (Game|OpenLevel(byName) "CE_Level_06"))
    (:CE_Level_03_Intro
      (Game|OpenLevel(byName) "CE_Level_03"))))