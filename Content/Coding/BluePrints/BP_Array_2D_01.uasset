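; BP_Array_2D_01 is a placement puzzle board with an 8x8 grid of anchor components that track cubes attached to designated cells.
; Twelve anchors cast the attached or detached actor to their matching BP_Array_Cube_2D class and set or clear an Ok flag; the other anchors' handlers are empty.
; Tick tests whether all twelve flags are true, but nothing follows that check, so completing the pattern currently triggers nothing.
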(event ActorGotDetached(Comp_Anchor_2_7)
  (params (Anchor :type Comp%20Anchor%20Object%20Reference) (Actor :type Actor%20Object%20Reference) (Connector :type Comp%20Connector%20Anchor%20Object%20Reference)))

(event ActorGotAttached(Comp_Anchor_2_7)
  (params (Anchor :type Comp%20Anchor%20Object%20Reference) (Actor :type Actor%20Object%20Reference) (Connector :type Comp%20Connector%20Anchor%20Object%20Reference)))

(event ActorGotDetached(Comp_Anchor_2_5)
  (params (Anchor :type Comp%20Anchor%20Object%20Reference) (Actor :type Actor%20Object%20Reference) (Connector :type Comp%20Connector%20Anchor%20Object%20Reference)))

(event ActorGotAttached(Comp_Anchor_4_0)
  (params (Anchor :type Comp%20Anchor%20Object%20Reference) (Actor :type Actor%20Object%20Reference) (Connector :type Comp%20Connector%20Anchor%20Object%20Reference)))

(event ActorGotDetached(Comp_Anchor_4_7)
  (params (Anchor :type Comp%20Anchor%20Object%20Reference) (Actor :type Actor%20Object%20Reference) (Connector :type Comp%20Connector%20Anchor%20Object%20Reference)))

(event ActorGotAttached(Comp_Anchor_4_7)
  (params (Anchor :type Comp%20Anchor%20Object%20Reference) (Actor :type Actor%20Object%20Reference) (Connector :type Comp%20Connector%20Anchor%20Object%20Reference)))

(event ActorGotDetached(Comp_Anchor_4_2)
  (params (Anchor :type Comp%20Anchor%20Object%20Reference) (Actor :type Actor%20Object%20Reference) (Connector :type Comp%20Connector%20Anchor%20Object%20Reference))
  (Utilities|Casting|CastToBP_Array_Cube_2D_42 Actor)
  (Variables|Default|Setok_42 false))

(event ActorGotAttached(Comp_Anchor_4_2)
  (params (Anchor :type Comp%20Anchor%20Object%20Reference) (Actor :type Actor%20Object%20Reference) (Connector :type Comp%20Connector%20Anchor%20Object%20Reference))
  (Utilities|Casting|CastToBP_Array_Cube_2D_42 Actor)
  (Variables|Default|Setok_42 true))

(event ActorGotDetached(Comp_Anchor_4_6)
  (params (Anchor :type Comp%20Anchor%20Object%20Reference) (Actor :type Actor%20Object%20Reference) (Connector :type Comp%20Connector%20Anchor%20Object%20Reference)))

(event ActorGotAttached(Comp_Anchor_4_6)
  (params (Anchor :type Comp%20Anchor%20Object%20Reference) (Actor :type Actor%20Object%20Reference) (Connector :type Comp%20Connector%20Anchor%20Object%20Reference)))

(event ActorGotDetached(Comp_Anchor_4_5)
  (params (Anchor :type Comp%20Anchor%20Object%20Reference) (Actor :type Actor%20Object%20Reference) (Connector :type Comp%20Connector%20Anchor%20Object%20Reference))
  (Utilities|Casting|CastToBP_Array_Cube_2D_45 Actor)
  (Variables|Default|Setok_45 false))

(event ActorGotAttached(Comp_Anchor_4_5)
  (params (Anchor :type Comp%20Anchor%20Object%20Reference) (Actor :type Actor%20Object%20Reference) (Connector :type Comp%20Connector%20Anchor%20Object%20Reference))
  (Utilities|Casting|CastToBP_Array_Cube_2D_45 Actor)
  (Variables|Default|Setok_45 true))

(event ActorGotDetached(Comp_Anchor_4_4)
  (params (Anchor :type Comp%20Anchor%20Object%20Reference) (Actor :type Actor%20Object%20Reference) (Connector :type Comp%20Connector%20Anchor%20Object%20Reference)))

(event ActorGotAttached(Comp_Anchor_2_5)
  (params (Anchor :type Comp%20Anchor%20Object%20Reference) (Actor :type Actor%20Object%20Reference) (Connector :type Comp%20Connector%20Anchor%20Object%20Reference)))

(event ActorGotAttached(Comp_Anchor_4_4)
  (params (Anchor :type Comp%20Anchor%20Object%20Reference) (Actor :type Actor%20Object%20Reference) (Connector :type Comp%20Connector%20Anchor%20Object%20Reference)))

(event ActorGotDetached(Comp_Anchor_4_3)
  (params (Anchor :type Comp%20Anchor%20Object%20Reference) (Actor :type Actor%20Object%20Reference) (Connector :type Comp%20Connector%20Anchor%20Object%20Reference)))

(event ActorGotAttached(Comp_Anchor_4_3)
  (params (Anchor :type Comp%20Anchor%20Object%20Reference) (Actor :type Actor%20Object%20Reference) (Connector :type Comp%20Connector%20Anchor%20Object%20Reference)))

(event ActorGotDetached(Comp_Anchor_5_5)
  (params (Anchor :type Comp%20Anchor%20Object%20Reference) (Actor :type Actor%20Object%20Reference) (Connector :type Comp%20Connector%20Anchor%20Object%20Reference))
  (Utilities|Casting|CastToBP_Array_Cube_2D_55 Actor)
  (Variables|Default|Setok_55 false))

(event ActorGotAttached(Comp_Anchor_5_5)
  (params (Anchor :type Comp%20Anchor%20Object%20Reference) (Actor :type Actor%20Object%20Reference) (Connector :type Comp%20Connector%20Anchor%20Object%20Reference))
  (Utilities|Casting|CastToBP_Array_Cube_2D_55 Actor)
  (Variables|Default|Setok_55 true))

(event ActorGotDetached(Comp_Anchor_5_7)
  (params (Anchor :type Comp%20Anchor%20Object%20Reference) (Actor :type Actor%20Object%20Reference) (Connector :type Comp%20Connector%20Anchor%20Object%20Reference)))

(event ActorGotAttached(Comp_Anchor_5_7)
  (params (Anchor :type Comp%20Anchor%20Object%20Reference) (Actor :type Actor%20Object%20Reference) (Connector :type Comp%20Connector%20Anchor%20Object%20Reference)))

(event ActorGotDetached(Comp_Anchor_5_0)
  (params (Anchor :type Comp%20Anchor%20Object%20Reference) (Actor :type Actor%20Object%20Reference) (Connector :type Comp%20Connector%20Anchor%20Object%20Reference))
  (Utilities|Casting|CastToBP_Array_Cube_2D_50 Actor)
  (Variables|Default|Setok_50 false))

(event ActorGotAttached(Comp_Anchor_5_0)
  (params (Anchor :type Comp%20Anchor%20Object%20Reference) (Actor :type Actor%20Object%20Reference) (Connector :type Comp%20Connector%20Anchor%20Object%20Reference))
  (Utilities|Casting|CastToBP_Array_Cube_2D_50 Actor)
  (Variables|Default|Setok_50 true))

(event ActorGotDetached(Comp_Anchor_5_1)
  (params (Anchor :type Comp%20Anchor%20Object%20Reference) (Actor :type Actor%20Object%20Reference) (Connector :type Comp%20Connector%20Anchor%20Object%20Reference)))

(event ActorGotAttached(Comp_Anchor_5_1)
  (params (Anchor :type Comp%20Anchor%20Object%20Reference) (Actor :type Actor%20Object%20Reference) (Connector :type Comp%20Connector%20Anchor%20Object%20Reference)))

(event ActorGotDetached(Comp_Anchor_5_4)
  (params (Anchor :type Comp%20Anchor%20Object%20Reference) (Actor :type Actor%20Object%20Reference) (Connector :type Comp%20Connector%20Anchor%20Object%20Reference)))

(event ActorGotAttached(Comp_Anchor_5_4)
  (params (Anchor :type Comp%20Anchor%20Object%20Reference) (Actor :type Actor%20Object%20Reference) (Connector :type Comp%20Connector%20Anchor%20Object%20Reference)))

(event ActorGotDetached(Comp_Anchor_5_2)
  (params (Anchor :type Comp%20Anchor%20Object%20Reference) (Actor :type Actor%20Object%20Reference) (Connector :type Comp%20Connector%20Anchor%20Object%20Reference)))

(event ActorGotAttached(Comp_Anchor_5_2)
  (params (Anchor :type Comp%20Anchor%20Object%20Reference) (Actor :type Actor%20Object%20Reference) (Connector :type Comp%20Connector%20Anchor%20Object%20Reference)))

(event ActorGotDetached(Comp_Anchor_5_6)
  (params (Anchor :type Comp%20Anchor%20Object%20Reference) (Actor :type Actor%20Object%20Reference) (Connector :type Comp%20Connector%20Anchor%20Object%20Reference)))

(event ActorGotAttached(Comp_Anchor_5_6)
  (params (Anchor :type Comp%20Anchor%20Object%20Reference) (Actor :type Actor%20Object%20Reference) (Connector :type Comp%20Connector%20Anchor%20Object%20Reference)))

(event ActorGotDetached(Comp_Anchor_5_3)
  (params (Anchor :type Comp%20Anchor%20Object%20Reference) (Actor :type Actor%20Object%20Reference) (Connector :type Comp%20Connector%20Anchor%20Object%20Reference)))

(event ActorGotAttached(Comp_Anchor_5_3)
  (params (Anchor :type Comp%20Anchor%20Object%20Reference) (Actor :type Actor%20Object%20Reference) (Connector :type Comp%20Connector%20Anchor%20Object%20Reference)))

(event ActorGotDetached(Comp_Anchor_2_4)
  (params (Anchor :type Comp%20Anchor%20Object%20Reference) (Actor :type Actor%20Object%20Reference) (Connector :type Comp%20Connector%20Anchor%20Object%20Reference))
  (Utilities|Casting|CastToBP_Array_Cube_2D_24 Actor)
  (Variables|Default|Setok_24 false))

(event ActorGotAttached(Comp_Anchor_2_4)
  (params (Anchor :type Comp%20Anchor%20Object%20Reference) (Actor :type Actor%20Object%20Reference) (Connector :type Comp%20Connector%20Anchor%20Object%20Reference))
  (Utilities|Casting|CastToBP_Array_Cube_2D_24 Actor)
  (Variables|Default|Setok_24 true))

(event ActorGotDetached(Comp_Anchor_2_6)
  (params (Anchor :type Comp%20Anchor%20Object%20Reference) (Actor :type Actor%20Object%20Reference) (Connector :type Comp%20Connector%20Anchor%20Object%20Reference)))

(event ActorGotAttached(Comp_Anchor_2_6)
  (params (Anchor :type Comp%20Anchor%20Object%20Reference) (Actor :type Actor%20Object%20Reference) (Connector :type Comp%20Connector%20Anchor%20Object%20Reference)))

(event ActorGotDetached(Comp_Anchor_3_7)
  (params (Anchor :type Comp%20Anchor%20Object%20Reference) (Actor :type Actor%20Object%20Reference) (Connector :type Comp%20Connector%20Anchor%20Object%20Reference))
  (Utilities|Casting|CastToBP_Array_Cube_2D_37 Actor)
  (Variables|Default|Setok_37 false))

(event ActorGotAttached(Comp_Anchor_3_7)
  (params (Anchor :type Comp%20Anchor%20Object%20Reference) (Actor :type Actor%20Object%20Reference) (Connector :type Comp%20Connector%20Anchor%20Object%20Reference))
  (Utilities|Casting|CastToBP_Array_Cube_2D_37 Actor)
  (Variables|Default|Setok_37 true))

(event ActorGotDetached(Comp_Anchor_3_6)
  (params (Anchor :type Comp%20Anchor%20Object%20Reference) (Actor :type Actor%20Object%20Reference) (Connector :type Comp%20Connector%20Anchor%20Object%20Reference)))

(event ActorGotDetached(Comp_Anchor_2_1)
  (params (Anchor :type Comp%20Anchor%20Object%20Reference) (Actor :type Actor%20Object%20Reference) (Connector :type Comp%20Connector%20Anchor%20Object%20Reference)))

(event ActorGotAttached(Comp_Anchor_3_6)
  (params (Anchor :type Comp%20Anchor%20Object%20Reference) (Actor :type Actor%20Object%20Reference) (Connector :type Comp%20Connector%20Anchor%20Object%20Reference)))

(event ActorGotDetached(Comp_Anchor_3_5)
  (params (Anchor :type Comp%20Anchor%20Object%20Reference) (Actor :type Actor%20Object%20Reference) (Connector :type Comp%20Connector%20Anchor%20Object%20Reference))
  (Utilities|Casting|CastToBP_Array_Cube_2D_35 Actor)
  (Variables|Default|Setok_35 false))

(event ActorGotAttached(Comp_Anchor_3_5)
  (params (Anchor :type Comp%20Anchor%20Object%20Reference) (Actor :type Actor%20Object%20Reference) (Connector :type Comp%20Connector%20Anchor%20Object%20Reference))
  (Utilities|Casting|CastToBP_Array_Cube_2D_35 Actor)
  (Variables|Default|Setok_35 true))

(event ActorGotDetached(Comp_Anchor_3_4)
  (params (Anchor :type Comp%20Anchor%20Object%20Reference) (Actor :type Actor%20Object%20Reference) (Connector :type Comp%20Connector%20Anchor%20Object%20Reference)))

(event ActorGotAttached(Comp_Anchor_3_4)
  (params (Anchor :type Comp%20Anchor%20Object%20Reference) (Actor :type Actor%20Object%20Reference) (Connector :type Comp%20Connector%20Anchor%20Object%20Reference)))

(event ActorGotDetached(Comp_Anchor_3_3)
  (params (Anchor :type Comp%20Anchor%20Object%20Reference) (Actor :type Actor%20Object%20Reference) (Connector :type Comp%20Connector%20Anchor%20Object%20Reference)))

(event ActorGotAttached(Comp_Anchor_3_3)
  (params (Anchor :type Comp%20Anchor%20Object%20Reference) (Actor :type Actor%20Object%20Reference) (Connector :type Comp%20Connector%20Anchor%20Object%20Reference)))

(event ActorGotDetached(Comp_Anchor_3_2)
  (params (Anchor :type Comp%20Anchor%20Object%20Reference) (Actor :type Actor%20Object%20Reference) (Connector :type Comp%20Connector%20Anchor%20Object%20Reference))
  (Utilities|Casting|CastToBP_Array_Cube_2D_32 Actor)
  (Variables|Default|Setok_32 false))

(event ActorGotAttached(Comp_Anchor_3_2)
  (params (Anchor :type Comp%20Anchor%20Object%20Reference) (Actor :type Actor%20Object%20Reference) (Connector :type Comp%20Connector%20Anchor%20Object%20Reference))
  (Utilities|Casting|CastToBP_Array_Cube_2D_32 Actor)
  (Variables|Default|Setok_32 true))

(event ActorGotDetached(Comp_Anchor_3_1)
  (params (Anchor :type Comp%20Anchor%20Object%20Reference) (Actor :type Actor%20Object%20Reference) (Connector :type Comp%20Connector%20Anchor%20Object%20Reference)))

(event ActorGotAttached(Comp_Anchor_2_1)
  (params (Anchor :type Comp%20Anchor%20Object%20Reference) (Actor :type Actor%20Object%20Reference) (Connector :type Comp%20Connector%20Anchor%20Object%20Reference)))

(event ActorGotAttached(Comp_Anchor_3_1)
  (params (Anchor :type Comp%20Anchor%20Object%20Reference) (Actor :type Actor%20Object%20Reference) (Connector :type Comp%20Connector%20Anchor%20Object%20Reference)))

(event ActorGotDetached(Comp_Anchor_1_1)
  (params (Anchor :type Comp%20Anchor%20Object%20Reference) (Actor :type Actor%20Object%20Reference) (Connector :type Comp%20Connector%20Anchor%20Object%20Reference)))

(event ActorGotAttached(Comp_Anchor_1_1)
  (params (Anchor :type Comp%20Anchor%20Object%20Reference) (Actor :type Actor%20Object%20Reference) (Connector :type Comp%20Connector%20Anchor%20Object%20Reference)))

(event ActorGotDetached(Comp_Anchor_0_5)
  (params (Anchor :type Comp%20Anchor%20Object%20Reference) (Actor :type Actor%20Object%20Reference) (Connector :type Comp%20Connector%20Anchor%20Object%20Reference)))

(event ActorGotAttached(Comp_Anchor_0_5)
  (params (Anchor :type Comp%20Anchor%20Object%20Reference) (Actor :type Actor%20Object%20Reference) (Connector :type Comp%20Connector%20Anchor%20Object%20Reference)))

(event ActorGotDetached(Comp_Anchor_0_4)
  (params (Anchor :type Comp%20Anchor%20Object%20Reference) (Actor :type Actor%20Object%20Reference) (Connector :type Comp%20Connector%20Anchor%20Object%20Reference)))

(event ActorGotAttached(Comp_Anchor_0_4)
  (params (Anchor :type Comp%20Anchor%20Object%20Reference) (Actor :type Actor%20Object%20Reference) (Connector :type Comp%20Connector%20Anchor%20Object%20Reference)))

(event ActorGotDetached(Comp_Anchor_0_3)
  (params (Anchor :type Comp%20Anchor%20Object%20Reference) (Actor :type Actor%20Object%20Reference) (Connector :type Comp%20Connector%20Anchor%20Object%20Reference)))

(event ActorGotAttached(Comp_Anchor_0_3)
  (params (Anchor :type Comp%20Anchor%20Object%20Reference) (Actor :type Actor%20Object%20Reference) (Connector :type Comp%20Connector%20Anchor%20Object%20Reference)))

(event ActorGotDetached(Comp_Anchor_0_2)
  (params (Anchor :type Comp%20Anchor%20Object%20Reference) (Actor :type Actor%20Object%20Reference) (Connector :type Comp%20Connector%20Anchor%20Object%20Reference)))

(event ActorGotDetached(Comp_Anchor_2_0)
  (params (Anchor :type Comp%20Anchor%20Object%20Reference) (Actor :type Actor%20Object%20Reference) (Connector :type Comp%20Connector%20Anchor%20Object%20Reference))
  (Utilities|Casting|CastToBP_Array_Cube_2D_20 Actor)
  (Variables|Default|Setok_20 false))

(event ActorGotAttached(Comp_Anchor_0_2)
  (params (Anchor :type Comp%20Anchor%20Object%20Reference) (Actor :type Actor%20Object%20Reference) (Connector :type Comp%20Connector%20Anchor%20Object%20Reference)))

(event ActorGotDetached(Comp_Anchor_0_1)
  (params (Anchor :type Comp%20Anchor%20Object%20Reference) (Actor :type Actor%20Object%20Reference) (Connector :type Comp%20Connector%20Anchor%20Object%20Reference)))

(event ActorGotAttached(Comp_Anchor_0_1)
  (params (Anchor :type Comp%20Anchor%20Object%20Reference) (Actor :type Actor%20Object%20Reference) (Connector :type Comp%20Connector%20Anchor%20Object%20Reference)))

(event ActorGotDetached(Comp_Anchor_0_0)
  (params (Anchor :type Comp%20Anchor%20Object%20Reference) (Actor :type Actor%20Object%20Reference) (Connector :type Comp%20Connector%20Anchor%20Object%20Reference)))

(event ActorGotAttached(Comp_Anchor_0_0)
  (params (Anchor :type Comp%20Anchor%20Object%20Reference) (Actor :type Actor%20Object%20Reference) (Connector :type Comp%20Connector%20Anchor%20Object%20Reference)))

(event ActorGotDetached(Comp_Anchor_0_6)
  (params (Anchor :type Comp%20Anchor%20Object%20Reference) (Actor :type Actor%20Object%20Reference) (Connector :type Comp%20Connector%20Anchor%20Object%20Reference)))

(event ActorGotAttached(Comp_Anchor_0_6)
  (params (Anchor :type Comp%20Anchor%20Object%20Reference) (Actor :type Actor%20Object%20Reference) (Connector :type Comp%20Connector%20Anchor%20Object%20Reference)))

(event ActorGotDetached(Comp_Anchor_1_7)
  (params (Anchor :type Comp%20Anchor%20Object%20Reference) (Actor :type Actor%20Object%20Reference) (Connector :type Comp%20Connector%20Anchor%20Object%20Reference)))

(event ActorGotAttached(Comp_Anchor_1_7)
  (params (Anchor :type Comp%20Anchor%20Object%20Reference) (Actor :type Actor%20Object%20Reference) (Connector :type Comp%20Connector%20Anchor%20Object%20Reference)))

(event ActorGotDetached(Comp_Anchor_1_6)
  (params (Anchor :type Comp%20Anchor%20Object%20Reference) (Actor :type Actor%20Object%20Reference) (Connector :type Comp%20Connector%20Anchor%20Object%20Reference)))

(event ActorGotAttached(Comp_Anchor_2_0)
  (params (Anchor :type Comp%20Anchor%20Object%20Reference) (Actor :type Actor%20Object%20Reference) (Connector :type Comp%20Connector%20Anchor%20Object%20Reference))
  (Utilities|Casting|CastToBP_Array_Cube_2D_20 Actor)
  (Variables|Default|Setok_20 true))

(event ActorGotAttached(Comp_Anchor_1_6)
  (params (Anchor :type Comp%20Anchor%20Object%20Reference) (Actor :type Actor%20Object%20Reference) (Connector :type Comp%20Connector%20Anchor%20Object%20Reference)))

(event ActorGotDetached(Comp_Anchor_1_4)
  (params (Anchor :type Comp%20Anchor%20Object%20Reference) (Actor :type Actor%20Object%20Reference) (Connector :type Comp%20Connector%20Anchor%20Object%20Reference)))

(event ActorGotAttached(Comp_Anchor_1_4)
  (params (Anchor :type Comp%20Anchor%20Object%20Reference) (Actor :type Actor%20Object%20Reference) (Connector :type Comp%20Connector%20Anchor%20Object%20Reference)))

(event ActorGotDetached(Comp_Anchor_1_5)
  (params (Anchor :type Comp%20Anchor%20Object%20Reference) (Actor :type Actor%20Object%20Reference) (Connector :type Comp%20Connector%20Anchor%20Object%20Reference)))

(event ActorGotAttached(Comp_Anchor_1_5)
  (params (Anchor :type Comp%20Anchor%20Object%20Reference) (Actor :type Actor%20Object%20Reference) (Connector :type Comp%20Connector%20Anchor%20Object%20Reference)))

(event ActorGotDetached(Comp_Anchor_1_3)
  (params (Anchor :type Comp%20Anchor%20Object%20Reference) (Actor :type Actor%20Object%20Reference) (Connector :type Comp%20Connector%20Anchor%20Object%20Reference)))

(event ActorGotAttached(Comp_Anchor_1_3)
  (params (Anchor :type Comp%20Anchor%20Object%20Reference) (Actor :type Actor%20Object%20Reference) (Connector :type Comp%20Connector%20Anchor%20Object%20Reference)))

(event ActorGotDetached(Comp_Anchor_1_2)
  (params (Anchor :type Comp%20Anchor%20Object%20Reference) (Actor :type Actor%20Object%20Reference) (Connector :type Comp%20Connector%20Anchor%20Object%20Reference)))

(event ActorGotAttached(Comp_Anchor_1_2)
  (params (Anchor :type Comp%20Anchor%20Object%20Reference) (Actor :type Actor%20Object%20Reference) (Connector :type Comp%20Connector%20Anchor%20Object%20Reference)))

(event ActorGotDetached(Comp_Anchor_1_0)
  (params (Anchor :type Comp%20Anchor%20Object%20Reference) (Actor :type Actor%20Object%20Reference) (Connector :type Comp%20Connector%20Anchor%20Object%20Reference)))

(event ActorGotDetached(Comp_Anchor_2_2)
  (params (Anchor :type Comp%20Anchor%20Object%20Reference) (Actor :type Actor%20Object%20Reference) (Connector :type Comp%20Connector%20Anchor%20Object%20Reference)))

(event ActorGotAttached(Comp_Anchor_1_0)
  (params (Anchor :type Comp%20Anchor%20Object%20Reference) (Actor :type Actor%20Object%20Reference) (Connector :type Comp%20Connector%20Anchor%20Object%20Reference)))

(event ActorGotDetached(Comp_Anchor_0_7)
  (params (Anchor :type Comp%20Anchor%20Object%20Reference) (Actor :type Actor%20Object%20Reference) (Connector :type Comp%20Connector%20Anchor%20Object%20Reference)))

(event ActorGotAttached(Comp_Anchor_0_7)
  (params (Anchor :type Comp%20Anchor%20Object%20Reference) (Actor :type Actor%20Object%20Reference) (Connector :type Comp%20Connector%20Anchor%20Object%20Reference)))

(event ActorGotDetached(Comp_Anchor_3_0)
  (params (Anchor :type Comp%20Anchor%20Object%20Reference) (Actor :type Actor%20Object%20Reference) (Connector :type Comp%20Connector%20Anchor%20Object%20Reference)))

(event ActorGotAttached(Comp_Anchor_3_0)
  (params (Anchor :type Comp%20Anchor%20Object%20Reference) (Actor :type Actor%20Object%20Reference) (Connector :type Comp%20Connector%20Anchor%20Object%20Reference)))

(event ActorGotDetached(Comp_Anchor_6_3)
  (params (Anchor :type Comp%20Anchor%20Object%20Reference) (Actor :type Actor%20Object%20Reference) (Connector :type Comp%20Connector%20Anchor%20Object%20Reference)))

(event ActorGotAttached(Comp_Anchor_6_3)
  (params (Anchor :type Comp%20Anchor%20Object%20Reference) (Actor :type Actor%20Object%20Reference) (Connector :type Comp%20Connector%20Anchor%20Object%20Reference)))

(event ActorGotDetached(Comp_Anchor_6_2)
  (params (Anchor :type Comp%20Anchor%20Object%20Reference) (Actor :type Actor%20Object%20Reference) (Connector :type Comp%20Connector%20Anchor%20Object%20Reference)))

(event ActorGotAttached(Comp_Anchor_6_2)
  (params (Anchor :type Comp%20Anchor%20Object%20Reference) (Actor :type Actor%20Object%20Reference) (Connector :type Comp%20Connector%20Anchor%20Object%20Reference)))

(event ActorGotDetached(Comp_Anchor_6_1)
  (params (Anchor :type Comp%20Anchor%20Object%20Reference) (Actor :type Actor%20Object%20Reference) (Connector :type Comp%20Connector%20Anchor%20Object%20Reference)))

(event ActorGotAttached(Comp_Anchor_2_2)
  (params (Anchor :type Comp%20Anchor%20Object%20Reference) (Actor :type Actor%20Object%20Reference) (Connector :type Comp%20Connector%20Anchor%20Object%20Reference)))

(event ActorGotAttached(Comp_Anchor_6_1)
  (params (Anchor :type Comp%20Anchor%20Object%20Reference) (Actor :type Actor%20Object%20Reference) (Connector :type Comp%20Connector%20Anchor%20Object%20Reference)))

(event ActorGotDetached(Comp_Anchor_6_0)
  (params (Anchor :type Comp%20Anchor%20Object%20Reference) (Actor :type Actor%20Object%20Reference) (Connector :type Comp%20Connector%20Anchor%20Object%20Reference))
  (Utilities|Casting|CastToBP_Array_Cube_2D_60 Actor)
  (Variables|Default|Setok_60 false))

(event ActorGotAttached(Comp_Anchor_6_0)
  (params (Anchor :type Comp%20Anchor%20Object%20Reference) (Actor :type Actor%20Object%20Reference) (Connector :type Comp%20Connector%20Anchor%20Object%20Reference))
  (Utilities|Casting|CastToBP_Array_Cube_2D_60 Actor)
  (Variables|Default|Setok_60 true))

(event ActorGotDetached(Comp_Anchor_6_7)
  (params (Anchor :type Comp%20Anchor%20Object%20Reference) (Actor :type Actor%20Object%20Reference) (Connector :type Comp%20Connector%20Anchor%20Object%20Reference)))

(event ActorGotAttached(Comp_Anchor_6_7)
  (params (Anchor :type Comp%20Anchor%20Object%20Reference) (Actor :type Actor%20Object%20Reference) (Connector :type Comp%20Connector%20Anchor%20Object%20Reference)))

(event ActorGotDetached(Comp_Anchor_6_5)
  (params (Anchor :type Comp%20Anchor%20Object%20Reference) (Actor :type Actor%20Object%20Reference) (Connector :type Comp%20Connector%20Anchor%20Object%20Reference)))

(event ActorGotAttached(Comp_Anchor_6_5)
  (params (Anchor :type Comp%20Anchor%20Object%20Reference) (Actor :type Actor%20Object%20Reference) (Connector :type Comp%20Connector%20Anchor%20Object%20Reference)))

(event ActorGotDetached(Comp_Anchor_6_6)
  (params (Anchor :type Comp%20Anchor%20Object%20Reference) (Actor :type Actor%20Object%20Reference) (Connector :type Comp%20Connector%20Anchor%20Object%20Reference)))

(event ActorGotAttached(Comp_Anchor_6_6)
  (params (Anchor :type Comp%20Anchor%20Object%20Reference) (Actor :type Actor%20Object%20Reference) (Connector :type Comp%20Connector%20Anchor%20Object%20Reference)))

(event ActorGotDetached(Comp_Anchor_7_6)
  (params (Anchor :type Comp%20Anchor%20Object%20Reference) (Actor :type Actor%20Object%20Reference) (Connector :type Comp%20Connector%20Anchor%20Object%20Reference))
  (Utilities|Casting|CastToBP_Array_Cube_2D_76 Actor)
  (Variables|Default|Setok_76 false))

(event ActorGotDetached(Comp_Anchor_2_3)
  (params (Anchor :type Comp%20Anchor%20Object%20Reference) (Actor :type Actor%20Object%20Reference) (Connector :type Comp%20Connector%20Anchor%20Object%20Reference)))

(event ActorGotAttached(Comp_Anchor_7_6)
  (params (Anchor :type Comp%20Anchor%20Object%20Reference) (Actor :type Actor%20Object%20Reference) (Connector :type Comp%20Connector%20Anchor%20Object%20Reference))
  (Utilities|Casting|CastToBP_Array_Cube_2D_76 Actor)
  (Variables|Default|Setok_76 true))

(event ActorGotDetached(Comp_Anchor_7_4)
  (params (Anchor :type Comp%20Anchor%20Object%20Reference) (Actor :type Actor%20Object%20Reference) (Connector :type Comp%20Connector%20Anchor%20Object%20Reference)))

(event ActorGotAttached(Comp_Anchor_7_4)
  (params (Anchor :type Comp%20Anchor%20Object%20Reference) (Actor :type Actor%20Object%20Reference) (Connector :type Comp%20Connector%20Anchor%20Object%20Reference)))

(event ActorGotDetached(Comp_Anchor_7_5)
  (params (Anchor :type Comp%20Anchor%20Object%20Reference) (Actor :type Actor%20Object%20Reference) (Connector :type Comp%20Connector%20Anchor%20Object%20Reference)))

(event ActorGotAttached(Comp_Anchor_7_5)
  (params (Anchor :type Comp%20Anchor%20Object%20Reference) (Actor :type Actor%20Object%20Reference) (Connector :type Comp%20Connector%20Anchor%20Object%20Reference)))

(event ActorGotDetached(Comp_Anchor_7_7)
  (params (Anchor :type Comp%20Anchor%20Object%20Reference) (Actor :type Actor%20Object%20Reference) (Connector :type Comp%20Connector%20Anchor%20Object%20Reference)))

(event ActorGotAttached(Comp_Anchor_7_7)
  (params (Anchor :type Comp%20Anchor%20Object%20Reference) (Actor :type Actor%20Object%20Reference) (Connector :type Comp%20Connector%20Anchor%20Object%20Reference)))

(event ActorGotDetached(Comp_Anchor_7_0)
  (params (Anchor :type Comp%20Anchor%20Object%20Reference) (Actor :type Actor%20Object%20Reference) (Connector :type Comp%20Connector%20Anchor%20Object%20Reference)))

(event ActorGotAttached(Comp_Anchor_7_0)
  (params (Anchor :type Comp%20Anchor%20Object%20Reference) (Actor :type Actor%20Object%20Reference) (Connector :type Comp%20Connector%20Anchor%20Object%20Reference)))

(event ActorGotDetached(Comp_Anchor_7_1)
  (params (Anchor :type Comp%20Anchor%20Object%20Reference) (Actor :type Actor%20Object%20Reference) (Connector :type Comp%20Connector%20Anchor%20Object%20Reference)))

(event ActorGotAttached(Comp_Anchor_2_3)
  (params (Anchor :type Comp%20Anchor%20Object%20Reference) (Actor :type Actor%20Object%20Reference) (Connector :type Comp%20Connector%20Anchor%20Object%20Reference)))

(event ActorGotAttached(Comp_Anchor_7_1)
  (params (Anchor :type Comp%20Anchor%20Object%20Reference) (Actor :type Actor%20Object%20Reference) (Connector :type Comp%20Connector%20Anchor%20Object%20Reference)))

(event ActorGotDetached(Comp_Anchor_7_2)
  (params (Anchor :type Comp%20Anchor%20Object%20Reference) (Actor :type Actor%20Object%20Reference) (Connector :type Comp%20Connector%20Anchor%20Object%20Reference))
  (Utilities|Casting|CastToBP_Array_Cube_2D_72 Actor)
  (Variables|Default|Setok_72 false))

(event ActorGotAttached(Comp_Anchor_7_2)
  (params (Anchor :type Comp%20Anchor%20Object%20Reference) (Actor :type Actor%20Object%20Reference) (Connector :type Comp%20Connector%20Anchor%20Object%20Reference))
  (Utilities|Casting|CastToBP_Array_Cube_2D_72 Actor)
  (Variables|Default|Setok_72 true))

(event ActorGotDetached(Comp_Anchor_7_3)
  (params (Anchor :type Comp%20Anchor%20Object%20Reference) (Actor :type Actor%20Object%20Reference) (Connector :type Comp%20Connector%20Anchor%20Object%20Reference)))

(event ActorGotAttached(Comp_Anchor_7_3)
  (params (Anchor :type Comp%20Anchor%20Object%20Reference) (Actor :type Actor%20Object%20Reference) (Connector :type Comp%20Connector%20Anchor%20Object%20Reference)))

(event ActorGotDetached(Comp_Anchor_6_4)
  (params (Anchor :type Comp%20Anchor%20Object%20Reference) (Actor :type Actor%20Object%20Reference) (Connector :type Comp%20Connector%20Anchor%20Object%20Reference)))

(event ActorGotAttached(Comp_Anchor_6_4)
  (params (Anchor :type Comp%20Anchor%20Object%20Reference) (Actor :type Actor%20Object%20Reference) (Connector :type Comp%20Connector%20Anchor%20Object%20Reference)))

(event ActorGotDetached(Comp_Anchor_4_1)
  (params (Anchor :type Comp%20Anchor%20Object%20Reference) (Actor :type Actor%20Object%20Reference) (Connector :type Comp%20Connector%20Anchor%20Object%20Reference)))

(event ActorGotAttached(Comp_Anchor_4_1)
  (params (Anchor :type Comp%20Anchor%20Object%20Reference) (Actor :type Actor%20Object%20Reference) (Connector :type Comp%20Connector%20Anchor%20Object%20Reference)))

(event ActorGotDetached(Comp_Anchor_4_0)
  (params (Anchor :type Comp%20Anchor%20Object%20Reference) (Actor :type Actor%20Object%20Reference) (Connector :type Comp%20Connector%20Anchor%20Object%20Reference)))

(event EventTick
  (params (DeltaSeconds :type Float%20%28single-precision%29))
  (if (Math|Boolean|ANDBoolean (Variables|Default|Getok_60) (Variables|Default|Getok_45) (Variables|Default|Getok_42) (Variables|Default|Getok_55) (Variables|Default|Getok_37) (Variables|Default|Getok_24) (Variables|Default|Getok_20) (Variables|Default|Getok_50) (Variables|Default|Getok_35) (Variables|Default|Getok_76) (Variables|Default|Getok_72) (Variables|Default|Getok_32))
    _))

(fn ConstructionScript)