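; Timed button that starts a 30-second countdown phase for the Synchro cube, cone and sphere actors.
; When pressed, it blocks pickup for snapping on every shape, shows their color buttons and starts the BP_Time_Synchro widget timer.
; It disables its own collision and toggles the switch back after a delay.
; Tick polls the widget and, once time runs out, unblocks pickup, hides the color buttons and restores collision.
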(event OnStateChanged(Comp_Switch)
  (params (SourceInfo :type Struct%20Component%20Source%20Info%20Structure) (Value :type Boolean))
  (bind _output_get (Variables|Default|Setpressed Value))
  (if _output_get
    (Variables|Default|SetfinishTime true)
    (Utilities|FlowControl|Sequence
      (:then_0
        (bind _outactors (Actor|GetAllActorsOfClass "/Game/Coding/BluePrints/BP_CubeSynchro_1.BP_CubeSynchro_1_C"))
        (for _array_element _outactors
          (Default|SetBlockPickupforSnapping (Variables|/Game/Coding/BluePrints/BP_CubeSynchro_1.BP_CubeSynchro_1_C|GetComp_Grab _array_element) true)))
      (:then_1
        (bind _outactors_2 (Actor|GetAllActorsOfClass "/Game/Coding/BluePrints/BP_ConeSynchro_1.BP_ConeSynchro_1_C"))
        (for _array_element_2 _outactors_2
          (Default|SetBlockPickupforSnapping (Variables|/Game/Coding/BluePrints/BP_ConeSynchro_1.BP_ConeSynchro_1_C|GetComp_Grab _array_element_2) true)))
      (:then_2
        (bind _outactors_3 (Actor|GetAllActorsOfClass "/Game/Coding/BluePrints/BP_SphereSynchro_1.BP_SphereSynchro_1_C"))
        (for _array_element_3 _outactors_3
          (Default|SetBlockPickupforSnapping (Variables|/Game/Coding/BluePrints/BP_SphereSynchro_1.BP_SphereSynchro_1_C|GetComp_Grab _array_element_3) true)))
      (:then_3
        (bind _returnvalue (Actor|GetActorOfClass "/Game/Coding/Widgets/Synchro/BP_Time_Synchro.BP_Time_Synchro_C"))
        (bind _asui_time_synchro (Utilities|Casting|CastToUI_Time_Synchro (UserInterface|GetWidget (Variables|/Game/Coding/Widgets/Synchro/BP_Time_Synchro.BP_Time_Synchro_C|GetWidget _returnvalue))))
        (Widget|SetVisibility (Variables|/Game/Coding/Widgets/Synchro/UI_Time_Synchro.UI_Time_Synchro_C|GetcountDown_Text _asui_time_synchro) "Visible")
        (bind _output_get_2 (Variables|/Game/Coding/Widgets/Synchro/UI_Time_Synchro.UI_Time_Synchro_C|SettimeLimit _asui_time_synchro 30))
        (Variables|/Game/Coding/Widgets/Synchro/UI_Time_Synchro.UI_Time_Synchro_C|SetcountDownOn _asui_time_synchro true))
      (:then_4
        (bind _outactors_4 (Actor|GetAllActorsOfClass "/Game/Coding/BluePrints/BP_CubeSynchro_1.BP_CubeSynchro_1_C"))
        (for _array_element_4 _outactors_4
          (bind _asui_synchro_menu (Utilities|Casting|CastToUI_Synchro_Menu (UserInterface|GetWidget (Variables|/Game/Coding/BluePrints/BP_CubeSynchro_1.BP_CubeSynchro_1_C|GetWidget _array_element_4))))
          (Widget|SetIsEnabled (Variables|/Game/Coding/Widgets/Synchro/UI_Synchro_Menu.UI_Synchro_Menu_C|GetButton_Color _asui_synchro_menu) true)
          (Widget|SetVisibility (Variables|/Game/Coding/Widgets/Synchro/UI_Synchro_Menu.UI_Synchro_Menu_C|GetButton_Color _asui_synchro_menu) "Visible"))
        (bind _outactors_5 (Actor|GetAllActorsOfClass "/Game/Coding/BluePrints/BP_SphereSynchro_1.BP_SphereSynchro_1_C"))
        (for _array_element_5 _outactors_5
          (bind _asui_synchro_menu_2 (Utilities|Casting|CastToUI_Synchro_Menu (UserInterface|GetWidget (Variables|/Game/Coding/BluePrints/BP_SphereSynchro_1.BP_SphereSynchro_1_C|GetWidget _array_element_5))))
          (Widget|SetIsEnabled (Variables|/Game/Coding/Widgets/Synchro/UI_Synchro_Menu.UI_Synchro_Menu_C|GetButton_Color _asui_synchro_menu_2) true)
          (Widget|SetVisibility (Variables|/Game/Coding/Widgets/Synchro/UI_Synchro_Menu.UI_Synchro_Menu_C|GetButton_Color _asui_synchro_menu_2) "Visible"))
        (bind _outactors_6 (Actor|GetAllActorsOfClass "/Game/Coding/BluePrints/BP_ConeSynchro_1.BP_ConeSynchro_1_C"))
        (for _array_element_6 _outactors_6
          (bind _asui_synchro_menu_3 (Utilities|Casting|CastToUI_Synchro_Menu (UserInterface|GetWidget (Variables|/Game/Coding/BluePrints/BP_ConeSynchro_1.BP_ConeSynchro_1_C|GetWidget _array_element_6))))
          (Widget|SetIsEnabled (Variables|/Game/Coding/Widgets/Synchro/UI_Synchro_Menu.UI_Synchro_Menu_C|GetButton_Color _asui_synchro_menu_3) true)
          (Widget|SetVisibility (Variables|/Game/Coding/Widgets/Synchro/UI_Synchro_Menu.UI_Synchro_Menu_C|GetButton_Color _asui_synchro_menu_3) "Visible")))
      (:then_5
        (Collision|SetActorEnableCollision self false)
        (Utilities|FlowControl|Delay (Math|Conversions|ToFloat(Integer) _output_get_2))
        (Default|Toggle (Variables|Default|GetComp_Switch))
        (Variables|Default|SetfinishTime false)))))

(event EventTick
  (params (DeltaSeconds :type Float%20%28single-precision%29))
  (bind _returnvalue (Actor|GetActorOfClass "/Game/Coding/Widgets/Synchro/BP_Time_Synchro.BP_Time_Synchro_C"))
  (bind _asui_time_synchro (Utilities|Casting|CastToUI_Time_Synchro (UserInterface|GetWidget (Variables|/Game/Coding/Widgets/Synchro/BP_Time_Synchro.BP_Time_Synchro_C|GetWidget _returnvalue))))
  (if (Variables|/Game/Coding/Widgets/Synchro/UI_Time_Synchro.UI_Time_Synchro_C|GetcountDownOn _asui_time_synchro)
    (if (<= (Variables|/Game/Coding/Widgets/Synchro/UI_Time_Synchro.UI_Time_Synchro_C|GettimeLimit _asui_time_synchro) 0)
      (Utilities|FlowControl|Sequence
        (:then_0
          (bind _outactors (Actor|GetAllActorsOfClass "/Game/Coding/BluePrints/BP_CubeSynchro_1.BP_CubeSynchro_1_C"))
          (for _array_element _outactors
            (Default|SetBlockPickupforSnapping (Variables|/Game/Coding/BluePrints/BP_CubeSynchro_1.BP_CubeSynchro_1_C|GetComp_Grab _array_element) false)))
        (:then_1
          (bind _outactors_2 (Actor|GetAllActorsOfClass "/Game/Coding/BluePrints/BP_ConeSynchro_1.BP_ConeSynchro_1_C"))
          (for _array_element_2 _outactors_2
            (Default|SetBlockPickupforSnapping (Variables|/Game/Coding/BluePrints/BP_ConeSynchro_1.BP_ConeSynchro_1_C|GetComp_Grab _array_element_2) false)))
        (:then_2
          (bind _outactors_3 (Actor|GetAllActorsOfClass "/Game/Coding/BluePrints/BP_SphereSynchro_1.BP_SphereSynchro_1_C"))
          (for _array_element_3 _outactors_3
            (Default|SetBlockPickupforSnapping (Variables|/Game/Coding/BluePrints/BP_SphereSynchro_1.BP_SphereSynchro_1_C|GetComp_Grab _array_element_3) false)))
        (:then_3
          (bind _outactors_4 (Actor|GetAllActorsOfClass "/Game/Coding/BluePrints/BP_CubeSynchro_1.BP_CubeSynchro_1_C"))
          (for _array_element_4 _outactors_4
            (bind _asui_synchro_menu (Utilities|Casting|CastToUI_Synchro_Menu (UserInterface|GetWidget (Variables|/Game/Coding/BluePrints/BP_CubeSynchro_1.BP_CubeSynchro_1_C|GetWidget _array_element_4))))
            (Widget|SetIsEnabled (Variables|/Game/Coding/Widgets/Synchro/UI_Synchro_Menu.UI_Synchro_Menu_C|GetButton_Color _asui_synchro_menu) false)
            (Widget|SetVisibility (Variables|/Game/Coding/Widgets/Synchro/UI_Synchro_Menu.UI_Synchro_Menu_C|GetButton_Color _asui_synchro_menu) "Hidden"))
          (bind _outactors_5 (Actor|GetAllActorsOfClass "/Game/Coding/BluePrints/BP_SphereSynchro_1.BP_SphereSynchro_1_C"))
          (for _array_element_5 _outactors_5
            (bind _asui_synchro_menu_2 (Utilities|Casting|CastToUI_Synchro_Menu (UserInterface|GetWidget (Variables|/Game/Coding/BluePrints/BP_SphereSynchro_1.BP_SphereSynchro_1_C|GetWidget _array_element_5))))
            (Widget|SetIsEnabled (Variables|/Game/Coding/Widgets/Synchro/UI_Synchro_Menu.UI_Synchro_Menu_C|GetButton_Color _asui_synchro_menu_2) false)
            (Widget|SetVisibility (Variables|/Game/Coding/Widgets/Synchro/UI_Synchro_Menu.UI_Synchro_Menu_C|GetButton_Color _asui_synchro_menu_2) "Hidden"))
          (bind _outactors_6 (Actor|GetAllActorsOfClass "/Game/Coding/BluePrints/BP_ConeSynchro_1.BP_ConeSynchro_1_C"))
          (for _array_element_6 _outactors_6
            (bind _asui_synchro_menu_3 (Utilities|Casting|CastToUI_Synchro_Menu (UserInterface|GetWidget (Variables|/Game/Coding/BluePrints/BP_ConeSynchro_1.BP_ConeSynchro_1_C|GetWidget _array_element_6))))
            (Widget|SetIsEnabled (Variables|/Game/Coding/Widgets/Synchro/UI_Synchro_Menu.UI_Synchro_Menu_C|GetButton_Color _asui_synchro_menu_3) false)
            (Widget|SetVisibility (Variables|/Game/Coding/Widgets/Synchro/UI_Synchro_Menu.UI_Synchro_Menu_C|GetButton_Color _asui_synchro_menu_3) "Hidden")))
        (:then_4
          (Collision|SetActorEnableCollision self true)
          (Variables|Default|SetfinishTime false))))))

(fn ConstructionScript
  (|CallParentFunction))