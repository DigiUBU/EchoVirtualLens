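; BP_Chess is a 3x3 board actor that tracks whether specific mirror pieces sit on their designated squares, apparently for a placement puzzle.
; Overlap boxes at 02, 10 and 21 set a flag while a mirror cube, sphere or cone, respectively, is inside and clear it on exit.
; BeginPlay gathers the nine plane components into ArrayChess; neither the array nor the flags are read here.
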(event OnComponentBeginOverlap(Box_10)
  (params (OverlappedComponent :type Primitive%20Component%20Object%20Reference) (OtherActor :type Actor%20Object%20Reference) (OtherComp :type Primitive%20Component%20Object%20Reference) (OtherBodyIndex :type Integer) (bFromSweep :type Boolean) (SweepResult :type Hit%20Result%20Structure%20%28by%20ref%29))
  (Utilities|Casting|CastToBP_Mirror_Spheres OtherActor)
  (Variables|Default|Setsphere10_ok true))

(event OnComponentBeginOverlap(Box_21)
  (params (OverlappedComponent :type Primitive%20Component%20Object%20Reference) (OtherActor :type Actor%20Object%20Reference) (OtherComp :type Primitive%20Component%20Object%20Reference) (OtherBodyIndex :type Integer) (bFromSweep :type Boolean) (SweepResult :type Hit%20Result%20Structure%20%28by%20ref%29))
  (Utilities|Casting|CastToBP_Mirror_Cone OtherActor)
  (Variables|Default|Setcone21_ok true))

(event OnComponentEndOverlap(Box_10)
  (params (OverlappedComponent :type Primitive%20Component%20Object%20Reference) (OtherActor :type Actor%20Object%20Reference) (OtherComp :type Primitive%20Component%20Object%20Reference) (OtherBodyIndex :type Integer))
  (Utilities|Casting|CastToBP_Mirror_Spheres OtherActor)
  (Variables|Default|Setsphere10_ok false))

(event OnComponentEndOverlap(Box_21)
  (params (OverlappedComponent :type Primitive%20Component%20Object%20Reference) (OtherActor :type Actor%20Object%20Reference) (OtherComp :type Primitive%20Component%20Object%20Reference) (OtherBodyIndex :type Integer))
  (Utilities|Casting|CastToBP_Mirror_Cone OtherActor)
  (Variables|Default|Setcone21_ok false))

(event OnComponentBeginOverlap(Box_02)
  (params (OverlappedComponent :type Primitive%20Component%20Object%20Reference) (OtherActor :type Actor%20Object%20Reference) (OtherComp :type Primitive%20Component%20Object%20Reference) (OtherBodyIndex :type Integer) (bFromSweep :type Boolean) (SweepResult :type Hit%20Result%20Structure%20%28by%20ref%29))
  (Utilities|Casting|CastToBP_Mirror_Cube OtherActor)
  (Variables|Default|Setcube02_ok true))

(event OnComponentEndOverlap(Box_02)
  (params (OverlappedComponent :type Primitive%20Component%20Object%20Reference) (OtherActor :type Actor%20Object%20Reference) (OtherComp :type Primitive%20Component%20Object%20Reference) (OtherBodyIndex :type Integer))
  (Utilities|Casting|CastToBP_Mirror_Cube OtherActor)
  (Variables|Default|Setcube02_ok false))

(event EventBeginPlay
  (Variables|Default|SetArray_Chess (Utilities|Array|MakeArray (Variables|Default|GetPlane_00) (Variables|Default|GetPlane_01) (Variables|Default|GetPlane_02) (Variables|Default|GetPlane_10) (Variables|Default|GetPlane_11) (Variables|Default|GetPlane_12) (Variables|Default|GetPlane_20) (Variables|Default|GetPlane_21) (Variables|Default|GetPlane_22))))

(fn ConstructionScript)