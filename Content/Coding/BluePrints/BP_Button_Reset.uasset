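; Reset button for a 2D-array loop exhibit that toggles its pressed state, moving the button mesh, whenever something begins overlapping its Box.
; When pressed, it clears CubesBright on the W_loop_2D widget of BP_Tablet_2D and sets the tablet's Ready to false.
; It then spawns a 4x5 grid of BP_Array_Cube_2D_Loop_00 offset from an existing one, labels each with its row-column index and appends it to the tablet's FirstCubes.
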(event OnComponentBeginOverlap(Box)
  (params (OverlappedComponent :type Primitive%20Component%20Object%20Reference) (OtherActor :type Actor%20Object%20Reference) (OtherComp :type Primitive%20Component%20Object%20Reference) (OtherBodyIndex :type Integer) (bFromSweep :type Boolean) (SweepResult :type Hit%20Result%20Structure%20%28by%20ref%29))
  (CallFunction|Press)
  (if (Variables|Default|GetisPressed)
    (bind _returnvalue (Actor|GetActorOfClass "/Game/Coding/BluePrints/BP_Tablet_2D.BP_Tablet_2D_C"))
    (bind _asw_loop_2d (Utilities|Casting|CastToW_loop_2D (UserInterface|GetWidget (Variables|/Game/Coding/BluePrints/BP_Tablet_2D.BP_Tablet_2D_C|GetWidget _returnvalue))))
    (Utilities|Array|Clear (Variables|/Game/Coding/Widgets/UI_Array/2D_Loop/W_loop_2D.W_loop_2D_C|GetcubesBright _asw_loop_2d))
    (Variables|/Game/Coding/BluePrints/BP_Tablet_2D.BP_Tablet_2D_C|Setready _returnvalue false)
    (bind _returnvalue_2 (Actor|GetActorOfClass "/Game/Coding/BluePrints/BP_Array_Cube_2D_Loop_00.BP_Array_Cube_2D_Loop_00_C"))
    (for _index (range 0 4)
      (bind _returnvalue_3 (Game|SpawnActorfromClass "/Game/Coding/BluePrints/BP_Array_Cube_2D_Loop_00.BP_Array_Cube_2D_Loop_00_C" (Math|Transform|MakeTransform (+ (Transformation|GetActorLocation _returnvalue_2) (Math|Vector|MakeVector (Math|Conversions|ToFloat(Integer) (* _index 10)) 0.0 0.0)) "0.000000,90.000000,0.000000" "1.000000,1.000000,1.000000") "Undefined" "MultiplyWithRoot" 0 0))
      (bind _asw_array_2d_loop_00 (Utilities|Casting|CastToW_Array_2D_Loop_00 (UserInterface|GetWidget (Variables|/Game/Coding/BluePrints/BP_Array_Cube_2D_Loop_00.BP_Array_Cube_2D_Loop_00_C|GetWidget _returnvalue_3))))
      (switch int _index
        (:0
          (Variables|/Script/UMG.TextBlock|SetText (Variables|/Game/Coding/Widgets/UI_Array/2D/W_Array_2D_Loop_00.W_Array_2D_Loop_00_C|Getindex_2D _asw_array_2d_loop_00) "00"))
        (:1
          (Variables|/Script/UMG.TextBlock|SetText (Variables|/Game/Coding/Widgets/UI_Array/2D/W_Array_2D_Loop_00.W_Array_2D_Loop_00_C|Getindex_2D _asw_array_2d_loop_00) "01"))
        (:2
          (Variables|/Script/UMG.TextBlock|SetText (Variables|/Game/Coding/Widgets/UI_Array/2D/W_Array_2D_Loop_00.W_Array_2D_Loop_00_C|Getindex_2D _asw_array_2d_loop_00) "02"))
        (:3
          (Variables|/Script/UMG.TextBlock|SetText (Variables|/Game/Coding/Widgets/UI_Array/2D/W_Array_2D_Loop_00.W_Array_2D_Loop_00_C|Getindex_2D _asw_array_2d_loop_00) "03"))
        (:4
          (Variables|/Script/UMG.TextBlock|SetText (Variables|/Game/Coding/Widgets/UI_Array/2D/W_Array_2D_Loop_00.W_Array_2D_Loop_00_C|Getindex_2D _asw_array_2d_loop_00) "04")))
      (Utilities|Array|Add (Variables|/Game/Coding/BluePrints/BP_Tablet_2D.BP_Tablet_2D_C|GetfirstCubes _returnvalue) _returnvalue_3))
    (for _index_2 (range 0 4)
      (bind _returnvalue_4 (Game|SpawnActorfromClass "/Game/Coding/BluePrints/BP_Array_Cube_2D_Loop_00.BP_Array_Cube_2D_Loop_00_C" (Math|Transform|MakeTransform (+ (Transformation|GetActorLocation _returnvalue_2) (Math|Vector|MakeVector (Math|Conversions|ToFloat(Integer) (* _index_2 10)) -1e+01 0.0)) "0.000000,90.000000,0.000000" "1.000000,1.000000,1.000000") "Undefined" "MultiplyWithRoot" 0 0))
      (bind _asw_array_2d_loop_00_2 (Utilities|Casting|CastToW_Array_2D_Loop_00 (UserInterface|GetWidget (Variables|/Game/Coding/BluePrints/BP_Array_Cube_2D_Loop_00.BP_Array_Cube_2D_Loop_00_C|GetWidget _returnvalue_4))))
      (switch int _index_2
        (:0
          (Variables|/Script/UMG.TextBlock|SetText (Variables|/Game/Coding/Widgets/UI_Array/2D/W_Array_2D_Loop_00.W_Array_2D_Loop_00_C|Getindex_2D _asw_array_2d_loop_00_2) "10"))
        (:1
          (Variables|/Script/UMG.TextBlock|SetText (Variables|/Game/Coding/Widgets/UI_Array/2D/W_Array_2D_Loop_00.W_Array_2D_Loop_00_C|Getindex_2D _asw_array_2d_loop_00_2) "11"))
        (:2
          (Variables|/Script/UMG.TextBlock|SetText (Variables|/Game/Coding/Widgets/UI_Array/2D/W_Array_2D_Loop_00.W_Array_2D_Loop_00_C|Getindex_2D _asw_array_2d_loop_00_2) "12"))
        (:3
          (Variables|/Script/UMG.TextBlock|SetText (Variables|/Game/Coding/Widgets/UI_Array/2D/W_Array_2D_Loop_00.W_Array_2D_Loop_00_C|Getindex_2D _asw_array_2d_loop_00_2) "13"))
        (:4
          (Variables|/Script/UMG.TextBlock|SetText (Variables|/Game/Coding/Widgets/UI_Array/2D/W_Array_2D_Loop_00.W_Array_2D_Loop_00_C|Getindex_2D _asw_array_2d_loop_00_2) "14")))
      (Utilities|Array|Add (Variables|/Game/Coding/BluePrints/BP_Tablet_2D.BP_Tablet_2D_C|GetfirstCubes _returnvalue) _returnvalue_4))
    (for _index_3 (range 0 4)
      (bind _returnvalue_5 (Game|SpawnActorfromClass "/Game/Coding/BluePrints/BP_Array_Cube_2D_Loop_00.BP_Array_Cube_2D_Loop_00_C" (Math|Transform|MakeTransform (+ (Transformation|GetActorLocation _returnvalue_2) (Math|Vector|MakeVector (Math|Conversions|ToFloat(Integer) (* _index_3 10)) -2e+01 0.0)) "0.000000,90.000000,0.000000" "1.000000,1.000000,1.000000") "Undefined" "MultiplyWithRoot" 0 0))
      (bind _asw_array_2d_loop_00_3 (Utilities|Casting|CastToW_Array_2D_Loop_00 (UserInterface|GetWidget (Variables|/Game/Coding/BluePrints/BP_Array_Cube_2D_Loop_00.BP_Array_Cube_2D_Loop_00_C|GetWidget _returnvalue_5))))
      (switch int _index_3
        (:0
          (Variables|/Script/UMG.TextBlock|SetText (Variables|/Game/Coding/Widgets/UI_Array/2D/W_Array_2D_Loop_00.W_Array_2D_Loop_00_C|Getindex_2D _asw_array_2d_loop_00_3) "20"))
        (:1
          (Variables|/Script/UMG.TextBlock|SetText (Variables|/Game/Coding/Widgets/UI_Array/2D/W_Array_2D_Loop_00.W_Array_2D_Loop_00_C|Getindex_2D _asw_array_2d_loop_00_3) "21"))
        (:2
          (Variables|/Script/UMG.TextBlock|SetText (Variables|/Game/Coding/Widgets/UI_Array/2D/W_Array_2D_Loop_00.W_Array_2D_Loop_00_C|Getindex_2D _asw_array_2d_loop_00_3) "22"))
        (:3
          (Variables|/Script/UMG.TextBlock|SetText (Variables|/Game/Coding/Widgets/UI_Array/2D/W_Array_2D_Loop_00.W_Array_2D_Loop_00_C|Getindex_2D _asw_array_2d_loop_00_3) "23"))
        (:4
          (Variables|/Script/UMG.TextBlock|SetText (Variables|/Game/Coding/Widgets/UI_Array/2D/W_Array_2D_Loop_00.W_Array_2D_Loop_00_C|Getindex_2D _asw_array_2d_loop_00_3) "24")))
      (Utilities|Array|Add (Variables|/Game/Coding/BluePrints/BP_Tablet_2D.BP_Tablet_2D_C|GetfirstCubes _returnvalue) _returnvalue_5))
    (for _index_4 (range 0 4)
      (bind _returnvalue_6 (Game|SpawnActorfromClass "/Game/Coding/BluePrints/BP_Array_Cube_2D_Loop_00.BP_Array_Cube_2D_Loop_00_C" (Math|Transform|MakeTransform (+ (Transformation|GetActorLocation _returnvalue_2) (Math|Vector|MakeVector (Math|Conversions|ToFloat(Integer) (* _index_4 10)) -3e+01 0.0)) "0.000000,90.000000,0.000000" "1.000000,1.000000,1.000000") "Undefined" "MultiplyWithRoot" 0 0))
      (bind _asw_array_2d_loop_00_4 (Utilities|Casting|CastToW_Array_2D_Loop_00 (UserInterface|GetWidget (Variables|/Game/Coding/BluePrints/BP_Array_Cube_2D_Loop_00.BP_Array_Cube_2D_Loop_00_C|GetWidget _returnvalue_6))))
      (switch int _index_4
        (:0
          (Variables|/Script/UMG.TextBlock|SetText (Variables|/Game/Coding/Widgets/UI_Array/2D/W_Array_2D_Loop_00.W_Array_2D_Loop_00_C|Getindex_2D _asw_array_2d_loop_00_4) "30"))
        (:1
          (Variables|/Script/UMG.TextBlock|SetText (Variables|/Game/Coding/Widgets/UI_Array/2D/W_Array_2D_Loop_00.W_Array_2D_Loop_00_C|Getindex_2D _asw_array_2d_loop_00_4) "31"))
        (:2
          (Variables|/Script/UMG.TextBlock|SetText (Variables|/Game/Coding/Widgets/UI_Array/2D/W_Array_2D_Loop_00.W_Array_2D_Loop_00_C|Getindex_2D _asw_array_2d_loop_00_4) "32"))
        (:3
          (Variables|/Script/UMG.TextBlock|SetText (Variables|/Game/Coding/Widgets/UI_Array/2D/W_Array_2D_Loop_00.W_Array_2D_Loop_00_C|Getindex_2D _asw_array_2d_loop_00_4) "33"))
        (:4
          (Variables|/Script/UMG.TextBlock|SetText (Variables|/Game/Coding/Widgets/UI_Array/2D/W_Array_2D_Loop_00.W_Array_2D_Loop_00_C|Getindex_2D _asw_array_2d_loop_00_4) "34")))
      (Utilities|Array|Add (Variables|/Game/Coding/BluePrints/BP_Tablet_2D.BP_Tablet_2D_C|GetfirstCubes _returnvalue) _returnvalue_6))))

(fn ConstructionScript)

(fn Press
  (bind _button_circle_002 (Variables|Default|Getbutton_Circle_002))
  (bind _button_circle_002_2 (Variables|Default|Getbutton_Circle_002))
  (bind _relativelocation (Variables|/Script/Engine.SceneComponent|GetRelativeLocation _button_circle_002))
  (bind _relativelocation_2 (Variables|/Script/Engine.SceneComponent|GetRelativeLocation _button_circle_002_2))
  (if (Variables|Default|GetisPressed)
    (Variables|Default|SetisPressed false)
    (Transformation|SetRelativeLocation _button_circle_002 (Math|Vector|MakeVector (.x _relativelocation) (.y _relativelocation) 0.0) false false)
    (else
      (Variables|Default|SetisPressed true)
      (Transformation|SetRelativeLocation _button_circle_002_2 (Math|Vector|MakeVector (.x _relativelocation_2) (.y _relativelocation_2) -1.5) false false)
      (Rendering|Material|SetScalarParameterValueonMaterials (Variables|Default|Getbutton_Circle_002) "bright" 1.0))))