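; BP_Button is a switch button that resets a 2D array loop exercise when pressed.
; Reset clears the tablet and W_loop_2D data, flags a restart, hides a loop cube and clears the array actor's Hidden flags, then toggles the switch after a delay.
; SetButtonColor drives the mesh's brightness through dynamic materials.
; Unconnected leftover logic spawns a labelled 4x5 cube grid and attaches cubes to anchors.
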(event OnStateChanged(Comp_Switch)
  (params (SourceInfo :type Struct%20Component%20Source%20Info%20Structure) (Value :type Boolean))
  (bind _output_get (Variables|Default|Setpressed Value))
  (if _output_get
    (CallFunction|Reset)))

(event Custom|Reset
  (bind _returnvalue (Actor|GetActorOfClass "/Game/Coding/BluePrints/BP_Tablet_2D.BP_Tablet_2D_C"))
  (Utilities|FlowControl|Sequence
    (:then_0
      (bind _asw_loop_2d (Utilities|Casting|CastToW_loop_2D (UserInterface|GetWidget (Variables|/Game/Coding/BluePrints/BP_Tablet_2D.BP_Tablet_2D_C|GetWidget _returnvalue))))
      (Utilities|Array|Clear (Variables|/Game/Coding/Widgets/UI_Array/2D_Loop/W_loop_2D.W_loop_2D_C|GetcubesBright _asw_loop_2d))
      (Utilities|Array|Clear (Variables|/Game/Coding/Widgets/UI_Array/2D_Loop/W_loop_2D.W_loop_2D_C|GetindexToPrint _asw_loop_2d))
      (Variables|/Game/Coding/BluePrints/BP_Tablet_2D.BP_Tablet_2D_C|Setready _returnvalue false)
      (bind _returnvalue_2 (Actor|GetActorOfClass "/Game/Coding/BluePrints/BP_Array_Cube_2D_Loop_00.BP_Array_Cube_2D_Loop_00_C"))
      (Rendering|SetActorHiddenInGame _returnvalue_2 true)
      (Utilities|FlowControl|Sequence
        (:then_0
          (Utilities|FlowControl|Delay 1.0)
          (Default|Toggle (Variables|Default|GetComp_Switch)))
        (:then_1
          (bind _returnvalue_3 (Actor|GetActorOfClass "/Game/Coding/BluePrints/BP_Array_2D_02.BP_Array_2D_02_C"))
          (Variables|/Game/Coding/BluePrints/BP_Array_2D_02.BP_Array_2D_02_C|Sethidden_00 _returnvalue_3 false)
          (Variables|/Game/Coding/BluePrints/BP_Array_2D_02.BP_Array_2D_02_C|Sethidden_01 _returnvalue_3 false)
          (Variables|/Game/Coding/BluePrints/BP_Array_2D_02.BP_Array_2D_02_C|Sethidden_02 _returnvalue_3 false)
          (Variables|/Game/Coding/BluePrints/BP_Array_2D_02.BP_Array_2D_02_C|Sethidden_03 _returnvalue_3 false)
          (Variables|/Game/Coding/BluePrints/BP_Array_2D_02.BP_Array_2D_02_C|Sethidden_04 _returnvalue_3 false)
          (Variables|/Game/Coding/BluePrints/BP_Array_2D_02.BP_Array_2D_02_C|Sethidden_10 _returnvalue_3 false)
          (Variables|/Game/Coding/BluePrints/BP_Array_2D_02.BP_Array_2D_02_C|Sethidden_11 _returnvalue_3 false)
          (Variables|/Game/Coding/BluePrints/BP_Array_2D_02.BP_Array_2D_02_C|Sethidden_12 _returnvalue_3 false)
          (Variables|/Game/Coding/BluePrints/BP_Array_2D_02.BP_Array_2D_02_C|Sethidden_13 _returnvalue_3 false)
          (Variables|/Game/Coding/BluePrints/BP_Array_2D_02.BP_Array_2D_02_C|Sethidden_14 _returnvalue_3 false)
          (Variables|/Game/Coding/BluePrints/BP_Array_2D_02.BP_Array_2D_02_C|Sethidden_20 _returnvalue_3 false)
          (Variables|/Game/Coding/BluePrints/BP_Array_2D_02.BP_Array_2D_02_C|Sethidden_21 _returnvalue_3 false)
          (Variables|/Game/Coding/BluePrints/BP_Array_2D_02.BP_Array_2D_02_C|Sethidden_22 _returnvalue_3 false)
          (Variables|/Game/Coding/BluePrints/BP_Array_2D_02.BP_Array_2D_02_C|Sethidden_23 _returnvalue_3 false)
          (Variables|/Game/Coding/BluePrints/BP_Array_2D_02.BP_Array_2D_02_C|Sethidden_24 _returnvalue_3 false)
          (Variables|/Game/Coding/BluePrints/BP_Array_2D_02.BP_Array_2D_02_C|Sethidden_30 _returnvalue_3 false)
          (Variables|/Game/Coding/BluePrints/BP_Array_2D_02.BP_Array_2D_02_C|Sethidden_31 _returnvalue_3 false)
          (Variables|/Game/Coding/BluePrints/BP_Array_2D_02.BP_Array_2D_02_C|Sethidden_32 _returnvalue_3 false)
          (Variables|/Game/Coding/BluePrints/BP_Array_2D_02.BP_Array_2D_02_C|Sethidden_33 _returnvalue_3 false)
          (Variables|/Game/Coding/BluePrints/BP_Array_2D_02.BP_Array_2D_02_C|Sethidden_34 _returnvalue_3 false))))
    (:then_1
      (Variables|/Game/Coding/BluePrints/BP_Tablet_2D.BP_Tablet_2D_C|Setrestart _returnvalue true)
      (Utilities|Array|Clear (Variables|/Game/Coding/BluePrints/BP_Tablet_2D.BP_Tablet_2D_C|GetstructIndex _returnvalue))
      (Variables|/Game/Coding/BluePrints/BP_Tablet_2D.BP_Tablet_2D_C|Setdelay _returnvalue 1.0)
      (Utilities|Array|Clear (Variables|/Game/Coding/BluePrints/BP_Tablet_2D.BP_Tablet_2D_C|GetcubesBright _returnvalue))
      (Utilities|Array|Clear (Variables|/Game/Coding/BluePrints/BP_Tablet_2D.BP_Tablet_2D_C|Gettest _returnvalue)))))

(fn ConstructionScript
  (|CallParentFunction))

(fn SetButtonColor
  (params (Alpha :type Float%20%28double-precision%29))
  (if (Variables|Default|Getpressed)
    (bind _returnvalue (Rendering|Material|CreateDynamicMaterialInstance (Variables|Default|GetMesh_Button_Button) 0 (Rendering|Material|GetMaterial (Variables|Default|GetMesh_Button_Button) 0) "None" :!class /Script/Engine.PrimitiveComponent))
    (Rendering|Material|SetScalarParameterValue _returnvalue "bright" 3.0 :!class /Script/Engine.MaterialInstanceDynamic)
    (else
      (bind _returnvalue_2 (Rendering|Material|CreateDynamicMaterialInstance (Variables|Default|GetMesh_Button_Button) 0 (Rendering|Material|GetMaterial (Variables|Default|GetMesh_Button_Button) 0) "None" :!class /Script/Engine.PrimitiveComponent))
      (Rendering|Material|SetScalarParameterValue _returnvalue_2 "bright" 0.0 :!class /Script/Engine.MaterialInstanceDynamic))))