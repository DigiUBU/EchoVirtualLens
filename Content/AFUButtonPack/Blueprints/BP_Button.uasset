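; BP_Button is an interactable button actor that toggles a switch state and forwards it to a list of controlled actors.
; Selecting it moves the drag component to the Pressed section, which on authority toggles the switch component.
; Switch changes set binary-interface components on referenced actors and fire trigger-interface ones only when turned on, then play or reverse the button's timeline.
; The construction script optionally hides the socket base.
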(event InEditorStateChanged(Comp_Switch)
  (params (Value :type Boolean))
  ;[1 1 1] ButtonStateChange
  (Utilities|ManipulateTimeline (Variables|Default|GetTimeline) Value))

(event OnStateChanged(Comp_Switch)
  (params (SourceInfo :type Struct%20Component%20Source%20Info%20Structure) (Value :type Boolean))
  ;[1 1 1] ButtonStateChange
  (|ForwardButtonState_2_2 Value SourceInfo
    (:Completed
      (if Value
        (Timeline|Timeline Play)
        (else
          (Timeline|Timeline Reverse))))))

(event PressedSelect(Comp_Select)
  (params (Pawn :type BP%20Pawn%20Base%20Object%20Reference) (SourceActor :type Actor%20Object%20Reference) (ImpactLocation :type Vector :default "0, 0, 0") (ImpactComponent :type Actor%20Component%20Object%20Reference))
  ;[1 1 1] On Selected
  (Default|MovetoSection (Variables|Default|GetComp_Drag) Pawn SourceActor "Button" "Pressed"))

(event DragStateChangedSingle(Comp_Drag)
  (params (SourceInfo :type Struct%20Component%20Source%20Info%20Structure) (Identifier :type Name :default "None") (Section :type Name :default "None") (Set :type Boolean))
  ;[1 1 1] On Pressed
  (Utilities|HasAuthorityOnlyifReplicates
    (:Authority
      (switch name Section
        (:Pressed
          (if Set
            (Class|InterfaceStateComponentBinary|ComponentBoolToggle(Message) (Variables|Default|GetComp_Switch) SourceInfo)))))))

(fn ConstructionScript
  (Rendering|SetVisibility (Variables|Default|GetSocket) (Variables|Setup|GetShowBase) false))