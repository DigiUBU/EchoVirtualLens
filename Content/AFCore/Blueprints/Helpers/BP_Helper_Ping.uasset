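; BP_Helper_Ping is a one-shot helper actor that shows an animated spherical ping with a sound at its location, then destroys itself.
; The construction script builds a dynamic M_Ping material from the Color and Thickness variables and applies it to the inner and outer spheres.
; On BeginPlay, a timeline scales the outer sphere by Size and drives the shared material's opacity, destroying the actor when finished.
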(event EventBeginPlay
  ;[1 1 1] Begin Play
  (Audio|PlaySoundatLocation (Variables|Private|GetSound) (Transformation|GetActorLocation) "0, 0, 0" 1.0 1.0 0.0 0 0 0 0)
  (bind (_direction _scale _opacity) (Timeline|PingAnimation PlayFromStart)
    (:Update
      (Transformation|SetWorldScale3D (Variables|Default|GetOuterSphere) (Math|Conversions|ToVector(Float) (* _scale (Variables|Parameters|GetSize))))
      (Rendering|Material|SetScalarParameterValue (Variables|Private|GetMaterial) "AnimatedOpacity" _opacity :!class /Script/Engine.MaterialInstanceDynamic))
    (:Finished
      (Actor|DestroyActor))))

(fn ConstructionScript
  (bind _returnvalue (Rendering|Material|CreateDynamicMaterialInstance "/Game/AFCore/Materials/Ping/M_Ping.M_Ping" "None" "None" :!class /Script/Engine.KismetMaterialLibrary))
  (bind _output_get (Variables|Private|SetMaterial _returnvalue))
  (Rendering|Material|SetMaterial (Variables|Default|GetOuterSphere) 0 _output_get)
  (Rendering|Material|SetScalarParameterValue (Variables|Private|GetMaterial) "Thickness" (Variables|Parameters|GetThickness) :!class /Script/Engine.MaterialInstanceDynamic)
  (Rendering|Material|SetVectorParameterValue (Variables|Private|GetMaterial) "Color" (Variables|Parameters|GetColor) :!class /Script/Engine.MaterialInstanceDynamic))