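; Toggle button that switches binary and trigger state components on the actors it references.
; Selecting it drags the button to its Pressed section, where the authority (if replicated) toggles the switch component.
; Switch changes forward the state through interfaces, firing triggers only when turning on.
; A timeline then blends a dynamic material from red to green with a fresnel shift, also previewed on editor state changes.
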(event InEditorStateChanged(Comp_Switch)
  (params (Value :type Boolean))
  ;[1 1 1] ButtonStateChange
  (Utilities|ManipulateTimeline (Variables|Default|GetStateTimeline) Value)
  (CallFunction|SetButtonColor (stale OnStateChanged(Comp_Switch) _procent)))

(event OnStateChanged(Comp_Switch)
  (params (SourceInfo :type Struct%20Component%20Source%20Info%20Structure) (Value :type Boolean))
  ;[1 1 1] ButtonStateChange
  (|ForwardButtonState Value SourceInfo
    (:Completed
      (if Value
        (bind _procent (Timeline|StateTimeline Play)
          (:Update
            (CallFunction|SetButtonColor _procent)))
        (else
          (Timeline|StateTimeline Reverse))))))

(event PressedSelect(Comp_Select)
  (params (Pawn :type BP%20Pawn%20Base%20Object%20Reference) (SourceActor :type Actor%20Object%20Reference) (ImpactLocation :type Vector :default "0, 0, 0") (ImpactComponent :type Actor%20Component%20Object%20Reference))
  ;[1 1 1] On Selected
  (Default|MovetoSection (Variables|Default|GetComp_Drag) Pawn SourceActor "Button" "Pressed"))

(event DragStateChangedSingle(Comp_Drag)
  (params (SourceInfo :type Struct%20Component%20Source%20Info%20Structure) (Identifier :type Name :default "None") (Section :type Name :default "None") (Set :type Boolean))
  ;[1 1 1] On Pressed
  (Utilities|HasAuthorityOnlyifReplicates
    (:Authority
      (switch name Section
        (:Pressed
          (if Set
            (Class|InterfaceStateComponentBinary|ComponentBoolToggle(Message) (Variables|Default|GetComp_Switch) SourceInfo)
            (Default|CallPress)))))))

(fn ConstructionScript)

(fn SetButtonColor
  (params (Alpha :type Float%20%28double-precision%29))
  (bind _material (CallFunction|GetButtonMaterial))
  (Rendering|Material|SetVectorParameterValue _material "Color" (Math|Color|Lerp(LinearColor) "(R=1.000000,G=0.000000,B=0.000000,A=1.000000)" "(R=0.000000,G=1.000000,B=0.000000,A=1.000000)" Alpha) :!class /Script/Engine.MaterialInstanceDynamic)
  (Rendering|Material|SetScalarParameterValue _material "FresnelExponent" (Math|Float|Lerp 0.3 2.0 Alpha) :!class /Script/Engine.MaterialInstanceDynamic))

(fn GetButtonMaterial
  (Variables|Default|GetButtonMaterial
    (:then
      _)
    (:else
      (bind _returnvalue (Rendering|Material|CreateDynamicMaterialInstance (Variables|Default|GetMesh_Button_Button) 0 "/Game/AFCore/Meshes/UI/UnrealButton/MI_Button_Logo_Door.MI_Button_Logo_Door" "None" :!class /Script/Engine.PrimitiveComponent))
      (Variables|Default|SetButtonMaterial _returnvalue)))
  (return (Variables|Default|GetButtonMaterial)))