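; Spectator camera utility actor that toggles its spectator component from a keyboard key.
; An any-key press handler compares the pressed key with a Key value and calls ToggleSpectator on CompSpectator when they match.
; The construction script copies the Name value into the component's Key and displays it on a text render as a label.
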(event Input|KeyboardEvents|AnyKey
  (params (Key :type Key%20Structure :default "None"))
  ;[1 1 1] Toggle Spectator on KeyPress
  (:Pressed
    (if (== Key (Variables|Default|GetKey))
      (Default|ToggleSpectator (Variables|Default|GetComp_Spectator)))))

(fn ConstructionScript
  (Variables|/Game/AFCore/Blueprints/Components/Misc/Comp_Spectator.Comp_Spectator_C|SetKey (Variables|Default|GetComp_Spectator) (Variables|Default|GetName))
  (Rendering|Components|TextRender|SetText (Variables|Default|GetTextRender) (Utilities|Text|ToText(Name) (Variables|Default|GetName))))