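; BP_Manager_TeleportLocation is a manager that keeps a registry of teleport locations and switches them all on or off together.
; Add and remove functions maintain the array without duplicates, and a getter exposes it.
; Activate and deactivate loop over the array, calling ActivateTeleportLocation on each valid entry.
; Any invalid entry found flags a cleanup pass that rebuilds the array from valid entries through a temporary array.
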(fn ConstructionScript)

(fn GetTeleportLocations
  (return (Variables|Manage|GetTeleportLocations)))

(fn ActivateTeleportLocations
  (for _array_element (Variables|Manage|GetTeleportLocations)
    (Utilities|IsValid _array_element
      (:Is%20Valid
        (Default|ActivateTeleportLocation _array_element true))
      (:Is%20Not%20Valid
        (LocalVariables|SetCheckArray true))))
  (if (LocalVariables|GetCheckArray)
    (Manage|CheckTeleportLocationArray)))

(fn DeactivateTeleportLocations
  (for _array_element (Variables|Manage|GetTeleportLocations)
    (Utilities|IsValid _array_element
      (:Is%20Valid
        (Default|ActivateTeleportLocation _array_element false))
      (:Is%20Not%20Valid
        (LocalVariables|SetCheckArray true))))
  (if (LocalVariables|GetCheckArray)
    (Manage|CheckTeleportLocationArray)))

(fn AddTeleportLocation
  (params (TeleportLocation :type Comp%20Teleport%20Object%20Reference))
  (Utilities|Array|AddUnique (Variables|Manage|GetTeleportLocations) TeleportLocation))

(fn RemoveTeleportLocation
  (params (TeleportLocation :type Comp%20Teleport%20Object%20Reference))
  (Utilities|Array|RemoveItem (Variables|Manage|GetTeleportLocations) TeleportLocation))

(fn CheckTeleportLocationArray
  (for _array_element (Variables|Manage|GetTeleportLocations)
    (Utilities|IsValid _array_element
      (:Is%20Valid
        (Utilities|Array|AddUnique (LocalVariables|GetTemporaryArray) _array_element))))
  (Variables|Manage|SetTeleportLocations (LocalVariables|GetTemporaryArray)))