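; Asymmetric character pawn in AFCore that adds a torso mesh that follows the head's facing.
; Each tick runs the parent logic, then smoothly interpolates the framework torso mesh's world rotation toward the head's yaw only.
; The slow interpolation makes the body trail head turns without copying pitch or roll; construction just calls the parent.
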(event EventTick
  (params (DeltaSeconds :type Float%20%28single-precision%29))
  ;[1 1 1] Event Tick
  (|CallParentFunction DeltaSeconds)
  (|MoveTorsoAccordingToHead DeltaSeconds))

(fn ConstructionScript
  (|CallParentFunction))