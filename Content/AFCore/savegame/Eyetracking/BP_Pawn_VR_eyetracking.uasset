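; VR pawn that uses Oculus eye tracking to show a marker where the player looks.
; It requests eye-tracking permission on BeginPlay, then each Tick moves GazeDir to the camera and rotates it by each eye's gaze orientation.
; A short Visibility trace along GazeDir places or hides GazeHitPoint, so the last eye processed sets the final result.
; An alternative generic eye-tracker path with debug prints is left unconnected and never runs.
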(event EventBeginPlay
  (Class|AndroidPermissionFunctionLibrary|AcquirePermissions (Utilities|Array|MakeArray "com.oculus.permission.EYE_TRACKING")))

(event EventTick
  (params (DeltaSeconds :type Float%20%28single-precision%29))
  (bind _gazedir (Variables|Default|GetGazeDir))
  (bind _returnvalue (Transformation|GetWorldLocation _gazedir))
  (Transformation|SetWorldLocation (Variables|Default|GetGazeDir) (Transformation|GetWorldLocation (Variables|Default|GetMainCamera)) false false)
  (bind _outeyegazesstate (Class|OculusXRMovementFunctionLibrary|TryGetEyeGazesState 1e+02))
  (for _array_element (.eyegazes _outeyegazesstate)
    (Transformation|SetRelativeRotation _gazedir (.orientation _array_element) false false)
    (bind (_outhit _returnvalue_2) (Collision|LineTraceByChannel _returnvalue (+ _returnvalue (* (Math|Vector|GetForwardVector _gazedir) (Math|Conversions|ToVector(Float) 1000))) "TraceTypeQuery1" false 0 "None"))
    (Rendering|SetVisibility (Variables|Default|GetGazeHitPoint) _returnvalue_2 false)
    (if _returnvalue_2
      (Transformation|SetWorldLocation (Variables|Default|GetGazeHitPoint) (.impactpoint _outhit) false false))))

(fn ConstructionScript
  (|CallParentFunction))