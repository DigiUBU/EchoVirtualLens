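; Mobile pawn Blueprint that handles server-side commands sent from its HUD component's user interface widgets.
; On a "Change Level" widget command, it casts the first payload object to a level data asset and asks the main game instance to switch to it with a fade and server travel.
; All other default events are disabled and the construction script only calls its parent.
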(event WidgetCommandServer(Comp_HUD)
  (params (Command :type Name :default "None") (Payload :type Struct%20Generic%20Payload%20Structure))
  (switch name Command
    (:ChangeLevel
      (bind _gameinstance (CallFunction|GetMainGameInstance self))
      (bind _aspda_level (Utilities|Casting|CastToPDA_Level (Utilities|Array|Get(acopy) (.objects Payload))))
      (Default|SwitchLevel _gameinstance _aspda_level true true))))

(event EventBeginPlay
  (|CallParentFunction) ; This node is disabled and will not be called.\nDrag off pins to build functionality.
)

(event Collision|EventActorBeginOverlap
  (params (OtherActor :type Actor%20Object%20Reference))
  (|CallParentFunction OtherActor) ; This node is disabled and will not be called.\nDrag off pins to build functionality.
)

(event EventTick
  (params (DeltaSeconds :type Float%20%28single-precision%29))
  (|CallParentFunction DeltaSeconds) ; This node is disabled and will not be called.\nDrag off pins to build functionality.
)

(fn ConstructionScript
  (|CallParentFunction))