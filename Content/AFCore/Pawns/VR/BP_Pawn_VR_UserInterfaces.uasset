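; VR pawn Blueprint that adds a toggleable menu widget to the player's pawn.
; It extends the parent's ExecuteControlFunction, calling the parent first and then handling the Pawn UI function.
; When that function is set, the BPCompPawnUI component toggles Widget_Menu at a preset distance with no rotation offset.
; All other behavior comes from the parent class.
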(event EventBeginPlay
  (|CallParentFunction) ; This node is disabled and will not be called.\nDrag off pins to build functionality.
)

(event Collision|EventActorBeginOverlap
  (params (OtherActor :type Actor%20Object%20Reference))
  (|CallParentFunction OtherActor) ; This node is disabled and will not be called.\nDrag off pins to build functionality.
)

(event EventTick
  (params (DeltaSeconds :type Float%20%28single-precision%29))
  (|CallParentFunction DeltaSeconds) ; This node is disabled and will not be called.\nDrag off pins to build functionality.
)

(event EventExecuteControlFunction
  (params (Function :type Name :default "None") (Set :type Boolean))
  (|CallParentFunction Function Set)
  (switch name Function
    (:PawnUI
      (if Set
        (Default|ToggleElement (Variables|Default|GetBP_Comp_PawnUI) "/Game/AFCore/Blueprints/Widgets/Menu/Widget_Menu.Widget_Menu_C" "NewEnumerator1" 0.0)))))

(fn ConstructionScript
  (|CallParentFunction))