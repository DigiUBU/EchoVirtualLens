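; Lightbulb actor that can be switched on and off, dimmed and recolored through switch, percent and named-color components.
; A timeline fades material brightness and point light intensity, with the percent component scaling only the intensity.
; A second timeline blends to colors looked up by name in ColorMap, applied to both light and lazily created dynamic material.
; In-editor state handlers preview switch and color changes.
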(event InEditorStateChanged(Comp_Switch)
  (params (Value :type Boolean))
  (Utilities|ManipulateTimeline (Variables|Default|GetLightTimeline) Value)
  (Rendering|Material|SetScalarParameterValue (CallFunction|GetLightbulbMaterial) "Brightness" (Math|Float|Lerp 0.0 42.0 (stale OnStateChanged(Comp_Switch) _percent)) :!class /Script/Engine.MaterialInstanceDynamic)
  (Rendering|Components|Light|SetIntensity (Variables|BP_Light_Bulb|GetPointLight) (Math|Float|Lerp 0.0 (Math|Float|Lerp 0.0 5e+04 (.value (Variables|/Game/AFCore/Blueprints/Components/State/Comp_Percent.Comp_Percent_C|GetPercent (Variables|Default|GetComp_Percent)))) (stale OnStateChanged(Comp_Switch) _percent))))

(event OnFloatChanged(Comp_Percent)
  (params (SourceInfo :type Struct%20Component%20Source%20Info%20Structure) (Value :type Float%20%28double-precision%29))
  (Rendering|Material|SetScalarParameterValue (CallFunction|GetLightbulbMaterial) "Brightness" (Math|Float|Lerp 0.0 42.0 (stale OnStateChanged(Comp_Switch) _percent)) :!class /Script/Engine.MaterialInstanceDynamic)
  (Rendering|Components|Light|SetIntensity (Variables|BP_Light_Bulb|GetPointLight) (Math|Float|Lerp 0.0 (Math|Float|Lerp 0.0 5e+04 (.value (Variables|/Game/AFCore/Blueprints/Components/State/Comp_Percent.Comp_Percent_C|GetPercent (Variables|Default|GetComp_Percent)))) (stale OnStateChanged(Comp_Switch) _percent))))

(event OnStateChanged(Comp_Switch)
  (params (SourceInfo :type Struct%20Component%20Source%20Info%20Structure) (Value :type Boolean))
  (if Value
    (bind _percent (Timeline|LightTimeline Play)
      (:Update
        (Rendering|Material|SetScalarParameterValue (CallFunction|GetLightbulbMaterial) "Brightness" (Math|Float|Lerp 0.0 42.0 _percent) :!class /Script/Engine.MaterialInstanceDynamic)
        (Rendering|Components|Light|SetIntensity (Variables|BP_Light_Bulb|GetPointLight) (Math|Float|Lerp 0.0 (Math|Float|Lerp 0.0 5e+04 (.value (Variables|/Game/AFCore/Blueprints/Components/State/Comp_Percent.Comp_Percent_C|GetPercent (Variables|Default|GetComp_Percent)))) _percent))))
    (else
      (Timeline|LightTimeline Reverse))))

(event InEditorNameStateChanged(Comp_Name_Color)
  (params (Active :type Name :default "None"))
  (Utilities|ManipulateTimeline (Variables|Default|GetLightColorTimeline) true)
  (CallFunction|SetLightValue (.Value (Utilities|Map|Find (Variables|Default|GetColorMap) Active))))

(event NameStateChanged(Comp_Name_Color)
  (params (SourceInfo :type Struct%20Component%20Source%20Info%20Structure) (Name :type Name :default "None"))
  (bind _out (CallFunction|SaveLinearColor (.Value (Utilities|Map|Find (Variables|Default|GetColorMap) Name))))
  (bind _out_2 (CallFunction|SaveLinearColor (Rendering|Components|Light|GetLightColor (Variables|BP_Light_Bulb|GetPointLight))))
  (bind _percent (Timeline|LightColorTimeline PlayFromStart)
    (:Update
      (CallFunction|SetLightValue (Math|Color|Lerp(LinearColor) _out_2 _out _percent)))))

(event Custom|SetLightValue
  (params (NewLightColor :type Linear%20Color%20Structure))
  (Rendering|Material|SetVectorParameterValue (CallFunction|GetLightbulbMaterial) "Color" NewLightColor :!class /Script/Engine.MaterialInstanceDynamic)
  (Rendering|Components|Light|SetLightColor (Variables|BP_Light_Bulb|GetPointLight) NewLightColor true))

(fn ConstructionScript
  (|CallParentFunction))

(fn GetLightbulbMaterial
  (bind _dynmaterial (Variables|Default|GetDynMaterial)
    (:then
      (return _dynmaterial))
    (:else
      (bind _returnvalue (Rendering|Material|CreateDynamicMaterialInstance (Variables|Default|GetStaticMesh) 1 "/Game/AFCore/Meshes/UI/Lightbulb/M_Light_Bulb_Base.M_Light_Bulb_Base" "None" :!class /Script/Engine.PrimitiveComponent))
      (bind _output_get (Variables|Default|SetDynMaterial _returnvalue))
      (return _output_get))))