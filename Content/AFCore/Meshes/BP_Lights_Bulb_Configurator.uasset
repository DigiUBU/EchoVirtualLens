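; BP_Lights_Bulb_Configurator is a configurable child actor that toggles a UI widget on selection and swaps its battery mesh by size.
; A press on its select component toggles visibility through the widget component of a referenced WidgetActor.
; A size-name component broadcasts state changes that set the battery static mesh to the small, medium or big variant.
; The construction script only runs the parent's logic.
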(event PressedSelect(Comp_Select)
  (params (Pawn :type BP%20Pawn%20Base%20Object%20Reference) (SourceActor :type Actor%20Object%20Reference) (ImpactLocation :type Vector :default "0, 0, 0") (ImpactComponent :type Actor%20Component%20Object%20Reference))
  ;[1 1 1] Spawns the widget upon select
  (Default|ToggleWidgetVisibility (Actor|GetComponentbyClass (Variables|Default|GetWidgetActor) "/Game/AFCore/Blueprints/Components/UI/Comp_Widget.Comp_Widget_C")))

(event NameStateChanged(Comp_Name_Size)
  (params (SourceInfo :type Struct%20Component%20Source%20Info%20Structure) (Name :type Name :default "None"))
  (bind _sm_battery (Variables|Default|GetSM_Battery))
  ;[1 1 1] Updates the battery mesh
  (switch name Name
    (:Small
      (Components|StaticMesh|SetStaticMesh _sm_battery "/Game/AFCore/Meshes/UI/Battery/SM_Battery_Small.SM_Battery_Small"))
    (:Medium
      (Components|StaticMesh|SetStaticMesh _sm_battery "/Game/AFCore/Meshes/UI/Battery/SM_Battery_Medium.SM_Battery_Medium"))
    (:Large
      (Components|StaticMesh|SetStaticMesh _sm_battery "/Game/AFCore/Meshes/UI/Battery/SM_Battery_Big.SM_Battery_Big"))))

(fn ConstructionScript
  (|CallParentFunction))