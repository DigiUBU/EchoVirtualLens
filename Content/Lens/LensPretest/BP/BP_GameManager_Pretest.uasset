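; Game manager for the Lens pretest, a timed series of image-based multiple-choice items shown before the first Lens level.
; It fills the options and blackboard prompt widgets from an Options array, switching instruction text at section changes.
; A looping timer records an empty "0" answer on timeout; each answer logs correctness and duration, then advances.
; After the last item it saves a per-player text file, sends it through HttpSenderActor and switches level.
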(event Custom|LoadItem
  (bind _item (Variables|Default|Getitem))
  (bind _as_ui_lens_pretest (Variables|Default|GetAs%20UI%20Lens%20Pretest))
  (bind _options (Variables|Default|Getoptions))
  (bind _returnvalue (- _item 1))
  (bind _output (Utilities|Array|Get(acopy) _options _returnvalue))
  ;[1 1 1] changes the images for the next item
  (Class|Image|SetBrush (Variables|/Game/Lens/LensPretest/Widget/UI_Lens_Pretest.UI_Lens_Pretest_C|GetImage_A _as_ui_lens_pretest) (Utilities|Struct|MakeSlateBrush "Image" "NoTile" "NoMirror" (Utilities|Struct|MakeDeprecateSlateVector2D 5e+02 3e+02) "(Left=0.000000,Top=0.000000,Right=0.000000,Bottom=0.000000)" "(SpecifiedColor=(R=1.000000,G=1.000000,B=1.000000,A=1.000000),ColorUseRule=UseColor_Specified)" "(CornerRadii=(X=0.000000,Y=0.000000,Z=0.000000,W=1.000000),Color=(SpecifiedColor=(R=0.000000,G=0.000000,B=0.000000,A=0.000000),ColorUseRule=UseColor_Specified),Width=0.000000,RoundingType=HalfHeightRadius,bUseBrushTransparency=False)" (.optiona _output)))
  (Class|Image|SetBrush (Variables|/Game/Lens/LensPretest/Widget/UI_Lens_Pretest.UI_Lens_Pretest_C|GetImage_B _as_ui_lens_pretest) (Utilities|Struct|MakeSlateBrush "Image" "NoTile" "NoMirror" (Utilities|Struct|MakeDeprecateSlateVector2D 5e+02 3e+02) "(Left=0.000000,Top=0.000000,Right=0.000000,Bottom=0.000000)" "(SpecifiedColor=(R=1.000000,G=1.000000,B=1.000000,A=1.000000),ColorUseRule=UseColor_Specified)" "(CornerRadii=(X=0.000000,Y=0.000000,Z=0.000000,W=1.000000),Color=(SpecifiedColor=(R=0.000000,G=0.000000,B=0.000000,A=0.000000),ColorUseRule=UseColor_Specified),Width=0.000000,RoundingType=HalfHeightRadius,bUseBrushTransparency=False)" (.optionb _output)))
  (Class|Image|SetBrush (Variables|/Game/Lens/LensPretest/Widget/UI_Lens_Pretest.UI_Lens_Pretest_C|GetImage_D _as_ui_lens_pretest) (Utilities|Struct|MakeSlateBrush "Image" "NoTile" "NoMirror" (Utilities|Struct|MakeDeprecateSlateVector2D 5e+02 3e+02) "(Left=0.000000,Top=0.000000,Right=0.000000,Bottom=0.000000)" "(SpecifiedColor=(R=1.000000,G=1.000000,B=1.000000,A=1.000000),ColorUseRule=UseColor_Specified)" "(CornerRadii=(X=0.000000,Y=0.000000,Z=0.000000,W=1.000000),Color=(SpecifiedColor=(R=0.000000,G=0.000000,B=0.000000,A=0.000000),ColorUseRule=UseColor_Specified),Width=0.000000,RoundingType=HalfHeightRadius,bUseBrushTransparency=False)" (.optiond _output)))
  (Class|Image|SetBrush (Variables|/Game/Lens/LensPretest/Widget/UI_Lens_Pretest.UI_Lens_Pretest_C|GetImage_C _as_ui_lens_pretest) (Utilities|Struct|MakeSlateBrush "Image" "NoTile" "NoMirror" (Utilities|Struct|MakeDeprecateSlateVector2D 5e+02 3e+02) "(Left=0.000000,Top=0.000000,Right=0.000000,Bottom=0.000000)" "(SpecifiedColor=(R=1.000000,G=1.000000,B=1.000000,A=1.000000),ColorUseRule=UseColor_Specified)" "(CornerRadii=(X=0.000000,Y=0.000000,Z=0.000000,W=1.000000),Color=(SpecifiedColor=(R=0.000000,G=0.000000,B=0.000000,A=0.000000),ColorUseRule=UseColor_Specified),Width=0.000000,RoundingType=HalfHeightRadius,bUseBrushTransparency=False)" (.optionc _output)))
  (Class|Image|SetBrush (Variables|/Game/Lens/LensPretest/Widget/UI_Lens_Pretest_Ref.UI_Lens_Pretest_Ref_C|GetImage_0 (Variables|Default|GetAs%20UI%20Lens%20Pretest%20Ref)) (Utilities|Struct|MakeSlateBrush "Image" "NoTile" "NoMirror" "(X=32.000000,Y=32.000000)" "(Left=0.000000,Top=0.000000,Right=0.000000,Bottom=0.000000)" "(SpecifiedColor=(R=1.000000,G=1.000000,B=1.000000,A=1.000000),ColorUseRule=UseColor_Specified)" "(CornerRadii=(X=0.000000,Y=0.000000,Z=0.000000,W=1.000000),Color=(SpecifiedColor=(R=0.000000,G=0.000000,B=0.000000,A=0.000000),ColorUseRule=UseColor_Specified),Width=0.000000,RoundingType=HalfHeightRadius,bUseBrushTransparency=False)" (.promptimage _output)))
  (CallFunction|StartTimer))

(event Custom|StartTimer
  ;[1 1 1] limit time management
  (Variables|Default|SetcurrentTime 0.0)
  (bind _returnvalue (Utilities|Time|SetTimerbyEvent (delegate Custom|CurrentTiming) 0.01 true)))

(event Custom|AnswerGiven
  (params (optionChosen :type String))
  (bind _istiming (Variables|Default|GetisTiming))
  (bind _options (Variables|Default|Getoptions))
  (bind _item (Variables|Default|Getitem))
  (bind _currenttime (Variables|Default|GetcurrentTime))
  (bind _returnvalue (- _item 1))
  (bind _output (Utilities|Array|Get(acopy) _options _returnvalue))
  ;[1 1 1] the answer is given and the next round is called
  (CallFunction|StopTimer)
  (bind _output_get (Variables|Default|SetwasCorrect (Utilities|Enum|Equal(Enum) optionChosen (.correctoption _output))))
  (bind _asbp_game_instance_main (Utilities|Casting|CastToBP_GameInstance_Main (Game|GetGameInstance)))
  (Utilities|Array|Add (Variables|Default|Getresults) (Utilities|Struct|MakeStr_Lens_Pretest_Results (Variables|/Game/AFCore/Blueprints/Game/BP_GameInstance_Main.BP_GameInstance_Main_C|GetplayerName _asbp_game_instance_main) (Variables|Default|Getitem) (.correctoption _output) optionChosen _output_get _currenttime _istiming))
  (Utilities|Array|Add (Variables|Default|Getdata) (Utilities|String|Append (Utilities|String|Append "ITEM: " (Utilities|String|ToString(Integer) (Variables|Default|Getitem))) " 
" (Utilities|String|Append "User answer: " optionChosen) " 
" (Utilities|String|Append "Correct: " (Utilities|String|ToString(Boolean) _output_get)) " 
" (Utilities|String|Append "Duration: " (Utilities|String|ToString(Float) _currenttime)) " 
" (Utilities|String|Append "In time: " (Utilities|String|ToString(Boolean) _istiming)) " 
"))
  (Utilities|FlowControl|Delay 2.0)
  (CallFunction|NextItem))

(event Custom|NextItem
  (bind _item (Variables|Default|Getitem))
  ;[1 1 1] continue with another item or we have finished
  (Variables|Default|SetwasCorrect false)
  (Variables|Default|SetisTiming true)
  (Math|Integer|IncrementInt _item
    (:%20%20
      (if (< (- (Variables|Default|Getitem) 1) (Utilities|Array|Length (Variables|Default|Getoptions)))
        (if (== _item 4)
          (Variables|/Script/UMG.TextBlock|SetText (Variables|/Game/Lens/LensPretest/Widget/UI_Lens_Pretest_Ref.UI_Lens_Pretest_Ref_C|Getexplanation (Variables|Default|GetAs%20UI%20Lens%20Pretest%20Ref)) "Choose the correct puzzle solution")
          (Widget|SetVisibility (Variables|Default|GetAs%20UI%20Lens%20Pretest) "Hidden" :!label _label)
          (Utilities|FlowControl|Delay 15.0)
          (Widget|SetVisibility (Variables|/Game/Lens/LensPretest/Widget/UI_Lens_Pretest_Ref.UI_Lens_Pretest_Ref_C|GetImage_0 (Variables|Default|GetAs%20UI%20Lens%20Pretest%20Ref)) "Visible")
          (elif (== _item 7)
            (Variables|/Script/UMG.TextBlock|SetText (Variables|/Game/Lens/LensPretest/Widget/UI_Lens_Pretest_Ref.UI_Lens_Pretest_Ref_C|Getexplanation (Variables|Default|GetAs%20UI%20Lens%20Pretest%20Ref)) "Guide the truck to get to the target")
            (goto _label)
            (else
              _)))
        (CallFunction|LoadItem)
        (else
          ;[1 1 1] next level once finished the pretest
          (CallFunction|SaveData)
          (Utilities|FlowControl|Delay 2.0)
          (bind _asbp_game_instance_main (Utilities|Casting|CastToBP_GameInstance_Main (Game|GetGameInstance)))
          (Default|SwitchLevel _asbp_game_instance_main "/Game/Lens/DA_Lens_001.DA_Lens_001" false false))))))

(event Custom|CurrentTiming
  ;[1 1 1] limit time management
  (bind _output_get (Variables|Default|SetcurrentTime (+ (Variables|Default|GetcurrentTime) (Utilities|Time|GetWorldDeltaSeconds))))
  ;[1 1 1] if the time is surpassed
  (if (>= _output_get (.timelimit (Utilities|Array|Get(acopy) (Variables|Default|Getoptions) (- (Variables|Default|Getitem) 1))))
    (Variables|Default|SetisTiming false)
    (CallFunction|AnswerGiven "0")))

(event Custom|StopTimer
  ;[1 1 1] limit time management
  (Utilities|Time|ClearandInvalidateTimerbyHandle (stale Custom|StartTimer _returnvalue)))

(event Custom|WeStart
  ;[1 1 1] start the pretest
  (bind _returnvalue (Actor|GetActorOfClass "/Game/Lens/LensPretest/BP/BP_ShowingPretest.BP_ShowingPretest_C"))
  (bind _returnvalue_2 (Actor|GetActorOfClass "/Game/Lens/LensPretest/BP/BP_Showing_Pretest_Blackboard.BP_Showing_Pretest_Blackboard_C"))
  (Rendering|SetActorHiddenInGame _returnvalue false)
  (Collision|SetActorEnableCollision _returnvalue true)
  (CallFunction|LoadItem)
  (CallFunction|StartTimer))

(event EventBeginPlay
  ;[1 1 1] reference to the widget of options
  (Variables|Default|Setitem 1)
  (bind _returnvalue (Actor|GetActorOfClass "/Game/Lens/LensPretest/BP/BP_ShowingPretest.BP_ShowingPretest_C"))
  (bind _returnvalue_2 (Actor|GetActorOfClass "/Game/Lens/LensPretest/BP/BP_Showing_Pretest_Blackboard.BP_Showing_Pretest_Blackboard_C"))
  (Rendering|SetActorHiddenInGame _returnvalue true)
  (Collision|SetActorEnableCollision _returnvalue false)
  (bind _returnvalue_3 (Actor|GetActorOfClass "/Game/Lens/LensPretest/BP/BP_ShowingPretest.BP_ShowingPretest_C"))
  (bind _asui_lens_pretest (Utilities|Casting|CastToUI_Lens_Pretest (UserInterface|GetWidget (Variables|/Game/Lens/LensPretest/BP/BP_ShowingPretest.BP_ShowingPretest_C|GetWidget _returnvalue_3))))
  (Variables|Default|SetAs%20UI%20Lens%20Pretest _asui_lens_pretest)
  (bind _returnvalue_4 (Actor|GetActorOfClass "/Game/Lens/LensPretest/BP/BP_Showing_Pretest_Blackboard.BP_Showing_Pretest_Blackboard_C"))
  (bind _asui_lens_pretest_ref (Utilities|Casting|CastToUI_Lens_Pretest_Ref (UserInterface|GetWidget (Variables|/Game/Lens/LensPretest/BP/BP_Showing_Pretest_Blackboard.BP_Showing_Pretest_Blackboard_C|GetWidget _returnvalue_4))))
  (Variables|Default|SetAs%20UI%20Lens%20Pretest%20Ref _asui_lens_pretest_ref))

(fn ConstructionScript)

(fn SaveData
  (bind _returnvalue (Class|KismetSystemLibrary|GetProjectSavedDirectory))
  (bind _returnvalue_2 (Math|DateTime|Now))
  (bind _returnvalue_3 (Utilities|String|Append _returnvalue "/Data"))
  ;[1 1 1] save the data of the test
  (bind _asbp_game_instance_main (Utilities|Casting|CastToBP_GameInstance_Main (Game|GetGameInstance)))
  (Class|VictoryBPFunctionLibrary|FileIOSaveStringArraytoFile _returnvalue_3 (Utilities|String|Append "EVL_" (Utilities|String|ToString(Integer) (.year _returnvalue_2)) (Utilities|String|ToString(Integer) (.month _returnvalue_2)) (Utilities|String|ToString(Integer) (.day _returnvalue_2)) (Utilities|String|ToString(Integer) (.hour _returnvalue_2)) (Utilities|String|ToString(Integer) (.minute _returnvalue_2)) (Utilities|String|ToString(Integer) (.second _returnvalue_2)) "_Pretest_" (Variables|/Game/AFCore/Blueprints/Game/BP_GameInstance_Main.BP_GameInstance_Main_C|GetplayerName _asbp_game_instance_main) ".txt") (Variables|Default|Getdata) false false)
  (bind _returnvalue_4 (Actor|GetActorOfClass "/Script/TheVirtualCode.HttpSenderActor"))
  (Class|HttpSenderActor|SendTxtFile _returnvalue_4 (Utilities|String|Append _returnvalue_3 "/" (Utilities|String|Append "EVL_" (Utilities|String|ToString(Integer) (.year _returnvalue_2)) (Utilities|String|ToString(Integer) (.month _returnvalue_2)) (Utilities|String|ToString(Integer) (.day _returnvalue_2)) (Utilities|String|ToString(Integer) (.hour _returnvalue_2)) (Utilities|String|ToString(Integer) (.minute _returnvalue_2)) (Utilities|String|ToString(Integer) (.second _returnvalue_2)) "_Pretest_" (Variables|/Game/AFCore/Blueprints/Game/BP_GameInstance_Main.BP_GameInstance_Main_C|GetplayerName _asbp_game_instance_main) ".txt"))))