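; Selectable figure 7 for round 5 of Lens01, picked by attaching its anchor connector.
; Attaching sets Selected, and after a short delay the figure, if still selected, submits itself to BP_GameManager_01 for validation; detaching clears the flag.
; SelectedOverlayColor toggles cube opacity through dynamic material instances, but its only calls are in unreachable code, alongside old logic that deselected sibling figures.
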(event PressedSelect(Comp_Select)
  (params (Pawn :type BP%20Pawn%20Base%20Object%20Reference) (SourceActor :type Actor%20Object%20Reference) (ImpactLocation :type Vector :default "0, 0, 0") (ImpactComponent :type Actor%20Component%20Object%20Reference))
  ;[1 1 1] OLD
)

(event ConnectorAttached(Comp_Connector_Anchor)
  (params (Connector :type Comp%20Connector%20Object%20Reference) (AttachedToActor :type Actor%20Object%20Reference) (AttachedToComponent :type Scene%20Component%20Object%20Reference))
  ;[1 1 1] if it is ready to validate selection
  (Variables|Default|Setselected true)
  (bind _returnvalue (Actor|GetActorOfClass "/Game/Lens/Lens01/BP/BP_GameManager_01.BP_GameManager_01_C"))
  (Utilities|FlowControl|Delay 2.0)
  (if (Variables|Default|Getselected)
    (Default|ValidateSelection _returnvalue self 5)))

(event ConnectorDetached(Comp_Connector_Anchor)
  ;[1 1 1] if it is ready to validate selection
  (Variables|Default|Setselected false))

(fn ConstructionScript)

(fn SelectedOverlayColor
  (params (select :type Boolean))
  (bind _figures_5_7_cube_369 (Variables|Default|Getfigures_5_7_Cube_369))
  (bind _figures_5_7_cube_365 (Variables|Default|Getfigures_5_7_Cube_365))
  (bind _figures_5_7_cube_362 (Variables|Default|Getfigures_5_7_Cube_362))
  (bind _figures_5_7_cube_364 (Variables|Default|Getfigures_5_7_Cube_364))
  (bind _figures_5_7_cube_378 (Variables|Default|Getfigures_5_7_Cube_378))
  (bind _figures_5_7_cube_379 (Variables|Default|Getfigures_5_7_Cube_379))
  (bind _figures_5_7_cube_380 (Variables|Default|Getfigures_5_7_Cube_380))
  (bind _figures_5_7_cube_381 (Variables|Default|Getfigures_5_7_Cube_381))
  (bind _figures_5_7_cube_377 (Variables|Default|Getfigures_5_7_Cube_377))
  (bind _figures_5_7_cube_370 (Variables|Default|Getfigures_5_7_Cube_370))
  (bind _figures_5_7_cube_371 (Variables|Default|Getfigures_5_7_Cube_371))
  (bind _figures_5_7_cube_372 (Variables|Default|Getfigures_5_7_Cube_372))
  (bind _figures_5_7_cube_366 (Variables|Default|Getfigures_5_7_Cube_366))
  (bind _figures_5_7_cube_373 (Variables|Default|Getfigures_5_7_Cube_373))
  (bind _figures_5_7_cube_374 (Variables|Default|Getfigures_5_7_Cube_374))
  (bind _figures_5_7_cube_376 (Variables|Default|Getfigures_5_7_Cube_376))
  (bind _figures_5_7_cube_369_2 (Variables|Default|Getfigures_5_7_Cube_369))
  (bind _figures_5_7_cube_365_2 (Variables|Default|Getfigures_5_7_Cube_365))
  (bind _figures_5_7_cube_366_2 (Variables|Default|Getfigures_5_7_Cube_366))
  (bind _figures_5_7_cube_367 (Variables|Default|Getfigures_5_7_Cube_367))
  (bind _figures_5_7_cube_368 (Variables|Default|Getfigures_5_7_Cube_368))
  (bind _figures_5_7_cube_358 (Variables|Default|Getfigures_5_7_Cube_358))
  (bind _figures_5_7_cube_359 (Variables|Default|Getfigures_5_7_Cube_359))
  (bind _figures_5_7_cube_367_2 (Variables|Default|Getfigures_5_7_Cube_367))
  (bind _figures_5_7_cube_360 (Variables|Default|Getfigures_5_7_Cube_360))
  (bind _figures_5_7_cube_363 (Variables|Default|Getfigures_5_7_Cube_363))
  (bind _figures_5_7_cube_361 (Variables|Default|Getfigures_5_7_Cube_361))
  (bind _figures_5_7_cube_362_2 (Variables|Default|Getfigures_5_7_Cube_362))
  (bind _figures_5_7_cube_364_2 (Variables|Default|Getfigures_5_7_Cube_364))
  (bind _figures_5_7_cube_378_2 (Variables|Default|Getfigures_5_7_Cube_378))
  (bind _figures_5_7_cube_379_2 (Variables|Default|Getfigures_5_7_Cube_379))
  (bind _figures_5_7_cube_380_2 (Variables|Default|Getfigures_5_7_Cube_380))
  (bind _figures_5_7_cube_381_2 (Variables|Default|Getfigures_5_7_Cube_381))
  (bind _figures_5_7_cube_377_2 (Variables|Default|Getfigures_5_7_Cube_377))
  (bind _figures_5_7_cube_368_2 (Variables|Default|Getfigures_5_7_Cube_368))
  (bind _figures_5_7_cube_370_2 (Variables|Default|Getfigures_5_7_Cube_370))
  (bind _figures_5_7_cube_371_2 (Variables|Default|Getfigures_5_7_Cube_371))
  (bind _figures_5_7_cube_372_2 (Variables|Default|Getfigures_5_7_Cube_372))
  (bind _figures_5_7_cube_373_2 (Variables|Default|Getfigures_5_7_Cube_373))
  (bind _figures_5_7_cube_374_2 (Variables|Default|Getfigures_5_7_Cube_374))
  (bind _figures_5_7_cube_376_2 (Variables|Default|Getfigures_5_7_Cube_376))
  (bind _figures_5_7_cube_358_2 (Variables|Default|Getfigures_5_7_Cube_358))
  (bind _figures_5_7_cube_359_2 (Variables|Default|Getfigures_5_7_Cube_359))
  (bind _figures_5_7_cube_360_2 (Variables|Default|Getfigures_5_7_Cube_360))
  (bind _figures_5_7_cube_363_2 (Variables|Default|Getfigures_5_7_Cube_363))
  (bind _figures_5_7_cube_361_2 (Variables|Default|Getfigures_5_7_Cube_361))
  (if select
    (Utilities|FlowControl|Sequence
      (:then_0
        (bind _returnvalue (Rendering|Material|CreateDynamicMaterialInstance _figures_5_7_cube_358 0 (Rendering|Material|GetMaterial _figures_5_7_cube_358 0) "opacity" :!class /Script/Engine.PrimitiveComponent))
        (Rendering|Material|SetScalarParameterValue _returnvalue "opacity" 0.25 :!class /Script/Engine.MaterialInstanceDynamic))
      (:then_1
        (bind _returnvalue_2 (Rendering|Material|CreateDynamicMaterialInstance _figures_5_7_cube_369_2 0 (Rendering|Material|GetMaterial _figures_5_7_cube_369_2 0) "opacity" :!class /Script/Engine.PrimitiveComponent))
        (Rendering|Material|SetScalarParameterValue _returnvalue_2 "opacity" 0.25 :!class /Script/Engine.MaterialInstanceDynamic))
      (:then_2
        (bind _returnvalue_3 (Rendering|Material|CreateDynamicMaterialInstance _figures_5_7_cube_365_2 0 (Rendering|Material|GetMaterial _figures_5_7_cube_365_2 0) "opacity" :!class /Script/Engine.PrimitiveComponent))
        (Rendering|Material|SetScalarParameterValue _returnvalue_3 "opacity" 0.25 :!class /Script/Engine.MaterialInstanceDynamic))
      (:then_3
        (bind _returnvalue_4 (Rendering|Material|CreateDynamicMaterialInstance _figures_5_7_cube_366_2 0 (Rendering|Material|GetMaterial _figures_5_7_cube_366_2 0) "opacity" :!class /Script/Engine.PrimitiveComponent))
        (Rendering|Material|SetScalarParameterValue _returnvalue_4 "opacity" 0.25 :!class /Script/Engine.MaterialInstanceDynamic))
      (:then_4
        (bind _returnvalue_5 (Rendering|Material|CreateDynamicMaterialInstance _figures_5_7_cube_367 0 (Rendering|Material|GetMaterial _figures_5_7_cube_367 0) "opacity" :!class /Script/Engine.PrimitiveComponent))
        (Rendering|Material|SetScalarParameterValue _returnvalue_5 "opacity" 0.25 :!class /Script/Engine.MaterialInstanceDynamic))
      (:then_5
        (bind _returnvalue_6 (Rendering|Material|CreateDynamicMaterialInstance _figures_5_7_cube_368 0 (Rendering|Material|GetMaterial _figures_5_7_cube_368 0) "opacity" :!class /Script/Engine.PrimitiveComponent))
        (Rendering|Material|SetScalarParameterValue _returnvalue_6 "opacity" 0.25 :!class /Script/Engine.MaterialInstanceDynamic))
      (:then_6
        (bind _returnvalue_7 (Rendering|Material|CreateDynamicMaterialInstance _figures_5_7_cube_359 0 (Rendering|Material|GetMaterial _figures_5_7_cube_359 0) "opacity" :!class /Script/Engine.PrimitiveComponent))
        (Rendering|Material|SetScalarParameterValue _returnvalue_7 "opacity" 0.25 :!class /Script/Engine.MaterialInstanceDynamic))
      (:then_7
        (bind _returnvalue_8 (Rendering|Material|CreateDynamicMaterialInstance _figures_5_7_cube_360 0 (Rendering|Material|GetMaterial _figures_5_7_cube_360 0) "opacity" :!class /Script/Engine.PrimitiveComponent))
        (Rendering|Material|SetScalarParameterValue _returnvalue_8 "opacity" 0.25 :!class /Script/Engine.MaterialInstanceDynamic))
      (:then_8
        (bind _returnvalue_9 (Rendering|Material|CreateDynamicMaterialInstance _figures_5_7_cube_363 0 (Rendering|Material|GetMaterial _figures_5_7_cube_363 0) "opacity" :!class /Script/Engine.PrimitiveComponent))
        (Rendering|Material|SetScalarParameterValue _returnvalue_9 "opacity" 0.25 :!class /Script/Engine.MaterialInstanceDynamic))
      (:then_9
        (bind _returnvalue_10 (Rendering|Material|CreateDynamicMaterialInstance _figures_5_7_cube_361 0 (Rendering|Material|GetMaterial _figures_5_7_cube_361 0) "opacity" :!class /Script/Engine.PrimitiveComponent))
        (Rendering|Material|SetScalarParameterValue _returnvalue_10 "opacity" 0.25 :!class /Script/Engine.MaterialInstanceDynamic))
      (:then_10
        (bind _returnvalue_11 (Rendering|Material|CreateDynamicMaterialInstance _figures_5_7_cube_362_2 0 (Rendering|Material|GetMaterial _figures_5_7_cube_362_2 0) "opacity" :!class /Script/Engine.PrimitiveComponent))
        (Rendering|Material|SetScalarParameterValue _returnvalue_11 "opacity" 0.25 :!class /Script/Engine.MaterialInstanceDynamic))
      (:then_11
        (bind _returnvalue_12 (Rendering|Material|CreateDynamicMaterialInstance _figures_5_7_cube_364_2 0 (Rendering|Material|GetMaterial _figures_5_7_cube_364_2 0) "opacity" :!class /Script/Engine.PrimitiveComponent))
        (Rendering|Material|SetScalarParameterValue _returnvalue_12 "opacity" 0.25 :!class /Script/Engine.MaterialInstanceDynamic))
      (:then_12
        (bind _returnvalue_13 (Rendering|Material|CreateDynamicMaterialInstance _figures_5_7_cube_378_2 0 (Rendering|Material|GetMaterial _figures_5_7_cube_378_2 0) "opacity" :!class /Script/Engine.PrimitiveComponent))
        (Rendering|Material|SetScalarParameterValue _returnvalue_13 "opacity" 0.25 :!class /Script/Engine.MaterialInstanceDynamic))
      (:then_13
        (bind _returnvalue_14 (Rendering|Material|CreateDynamicMaterialInstance _figures_5_7_cube_379_2 0 (Rendering|Material|GetMaterial _figures_5_7_cube_379_2 0) "opacity" :!class /Script/Engine.PrimitiveComponent))
        (Rendering|Material|SetScalarParameterValue _returnvalue_14 "opacity" 0.25 :!class /Script/Engine.MaterialInstanceDynamic))
      (:then_14
        (bind _returnvalue_15 (Rendering|Material|CreateDynamicMaterialInstance _figures_5_7_cube_380_2 0 (Rendering|Material|GetMaterial _figures_5_7_cube_380_2 0) "opacity" :!class /Script/Engine.PrimitiveComponent))
        (Rendering|Material|SetScalarParameterValue _returnvalue_15 "opacity" 0.25 :!class /Script/Engine.MaterialInstanceDynamic))
      (:then_15
        (bind _returnvalue_16 (Rendering|Material|CreateDynamicMaterialInstance _figures_5_7_cube_381_2 0 (Rendering|Material|GetMaterial _figures_5_7_cube_381_2 0) "opacity" :!class /Script/Engine.PrimitiveComponent))
        (Rendering|Material|SetScalarParameterValue _returnvalue_16 "opacity" 0.25 :!class /Script/Engine.MaterialInstanceDynamic))
      (:then_16
        (bind _returnvalue_17 (Rendering|Material|CreateDynamicMaterialInstance _figures_5_7_cube_377_2 0 (Rendering|Material|GetMaterial _figures_5_7_cube_377_2 0) "opacity" :!class /Script/Engine.PrimitiveComponent))
        (Rendering|Material|SetScalarParameterValue _returnvalue_17 "opacity" 0.25 :!class /Script/Engine.MaterialInstanceDynamic))
      (:then_17
        (bind _returnvalue_18 (Rendering|Material|CreateDynamicMaterialInstance _figures_5_7_cube_370_2 0 (Rendering|Material|GetMaterial _figures_5_7_cube_370_2 0) "opacity" :!class /Script/Engine.PrimitiveComponent))
        (Rendering|Material|SetScalarParameterValue _returnvalue_18 "opacity" 0.25 :!class /Script/Engine.MaterialInstanceDynamic))
      (:then_18
        (bind _returnvalue_19 (Rendering|Material|CreateDynamicMaterialInstance _figures_5_7_cube_371_2 0 (Rendering|Material|GetMaterial _figures_5_7_cube_371_2 0) "opacity" :!class /Script/Engine.PrimitiveComponent))
        (Rendering|Material|SetScalarParameterValue _returnvalue_19 "opacity" 0.25 :!class /Script/Engine.MaterialInstanceDynamic))
      (:then_19
        (bind _returnvalue_20 (Rendering|Material|CreateDynamicMaterialInstance _figures_5_7_cube_372_2 0 (Rendering|Material|GetMaterial _figures_5_7_cube_372_2 0) "opacity" :!class /Script/Engine.PrimitiveComponent))
        (Rendering|Material|SetScalarParameterValue _returnvalue_20 "opacity" 0.25 :!class /Script/Engine.MaterialInstanceDynamic))
      (:then_20
        (bind _returnvalue_21 (Rendering|Material|CreateDynamicMaterialInstance _figures_5_7_cube_373_2 0 (Rendering|Material|GetMaterial _figures_5_7_cube_373_2 0) "opacity" :!class /Script/Engine.PrimitiveComponent))
        (Rendering|Material|SetScalarParameterValue _returnvalue_21 "opacity" 0.25 :!class /Script/Engine.MaterialInstanceDynamic))
      (:then_21
        (bind _returnvalue_22 (Rendering|Material|CreateDynamicMaterialInstance _figures_5_7_cube_374_2 0 (Rendering|Material|GetMaterial _figures_5_7_cube_374_2 0) "opacity" :!class /Script/Engine.PrimitiveComponent))
        (Rendering|Material|SetScalarParameterValue _returnvalue_22 "opacity" 0.25 :!class /Script/Engine.MaterialInstanceDynamic))
      (:then_22
        (bind _returnvalue_23 (Rendering|Material|CreateDynamicMaterialInstance _figures_5_7_cube_376_2 0 (Rendering|Material|GetMaterial _figures_5_7_cube_376_2 0) "opacity" :!class /Script/Engine.PrimitiveComponent))
        (Rendering|Material|SetScalarParameterValue _returnvalue_23 "opacity" 0.25 :!class /Script/Engine.MaterialInstanceDynamic)))
    (else
      (Utilities|FlowControl|Sequence
        (:then_0
          (bind _returnvalue_24 (Rendering|Material|CreateDynamicMaterialInstance _figures_5_7_cube_358_2 0 (Rendering|Material|GetMaterial _figures_5_7_cube_358_2 0) "opacity" :!class /Script/Engine.PrimitiveComponent))
          (Rendering|Material|SetScalarParameterValue _returnvalue_24 "opacity" 0.0 :!class /Script/Engine.MaterialInstanceDynamic))
        (:then_1
          (bind _returnvalue_25 (Rendering|Material|CreateDynamicMaterialInstance _figures_5_7_cube_369 0 (Rendering|Material|GetMaterial _figures_5_7_cube_369 0) "opacity" :!class /Script/Engine.PrimitiveComponent))
          (Rendering|Material|SetScalarParameterValue _returnvalue_25 "opacity" 0.0 :!class /Script/Engine.MaterialInstanceDynamic))
        (:then_2
          (bind _returnvalue_26 (Rendering|Material|CreateDynamicMaterialInstance _figures_5_7_cube_365 0 (Rendering|Material|GetMaterial _figures_5_7_cube_365 0) "opacity" :!class /Script/Engine.PrimitiveComponent))
          (Rendering|Material|SetScalarParameterValue _returnvalue_26 "opacity" 0.0 :!class /Script/Engine.MaterialInstanceDynamic))
        (:then_3
          (bind _returnvalue_27 (Rendering|Material|CreateDynamicMaterialInstance _figures_5_7_cube_366 0 (Rendering|Material|GetMaterial _figures_5_7_cube_366 0) "opacity" :!class /Script/Engine.PrimitiveComponent))
          (Rendering|Material|SetScalarParameterValue _returnvalue_27 "opacity" 0.0 :!class /Script/Engine.MaterialInstanceDynamic))
        (:then_4
          (bind _returnvalue_28 (Rendering|Material|CreateDynamicMaterialInstance _figures_5_7_cube_367_2 0 (Rendering|Material|GetMaterial _figures_5_7_cube_367_2 0) "opacity" :!class /Script/Engine.PrimitiveComponent))
          (Rendering|Material|SetScalarParameterValue _returnvalue_28 "opacity" 0.0 :!class /Script/Engine.MaterialInstanceDynamic))
        (:then_5
          (bind _returnvalue_29 (Rendering|Material|CreateDynamicMaterialInstance _figures_5_7_cube_368_2 0 (Rendering|Material|GetMaterial _figures_5_7_cube_368_2 0) "opacity" :!class /Script/Engine.PrimitiveComponent))
          (Rendering|Material|SetScalarParameterValue _returnvalue_29 "opacity" 0.0 :!class /Script/Engine.MaterialInstanceDynamic))
        (:then_6
          (bind _returnvalue_30 (Rendering|Material|CreateDynamicMaterialInstance _figures_5_7_cube_359_2 0 (Rendering|Material|GetMaterial _figures_5_7_cube_359_2 0) "opacity" :!class /Script/Engine.PrimitiveComponent))
          (Rendering|Material|SetScalarParameterValue _returnvalue_30 "opacity" 0.0 :!class /Script/Engine.MaterialInstanceDynamic))
        (:then_7
          (bind _returnvalue_31 (Rendering|Material|CreateDynamicMaterialInstance _figures_5_7_cube_360_2 0 (Rendering|Material|GetMaterial _figures_5_7_cube_360_2 0) "opacity" :!class /Script/Engine.PrimitiveComponent))
          (Rendering|Material|SetScalarParameterValue _returnvalue_31 "opacity" 0.0 :!class /Script/Engine.MaterialInstanceDynamic))
        (:then_8
          (bind _returnvalue_32 (Rendering|Material|CreateDynamicMaterialInstance _figures_5_7_cube_363_2 0 (Rendering|Material|GetMaterial _figures_5_7_cube_363_2 0) "opacity" :!class /Script/Engine.PrimitiveComponent))
          (Rendering|Material|SetScalarParameterValue _returnvalue_32 "opacity" 0.0 :!class /Script/Engine.MaterialInstanceDynamic))
        (:then_9
          (bind _returnvalue_33 (Rendering|Material|CreateDynamicMaterialInstance _figures_5_7_cube_361_2 0 (Rendering|Material|GetMaterial _figures_5_7_cube_361_2 0) "opacity" :!class /Script/Engine.PrimitiveComponent))
          (Rendering|Material|SetScalarParameterValue _returnvalue_33 "opacity" 0.0 :!class /Script/Engine.MaterialInstanceDynamic))
        (:then_10
          (bind _returnvalue_34 (Rendering|Material|CreateDynamicMaterialInstance _figures_5_7_cube_362 0 (Rendering|Material|GetMaterial _figures_5_7_cube_362 0) "opacity" :!class /Script/Engine.PrimitiveComponent))
          (Rendering|Material|SetScalarParameterValue _returnvalue_34 "opacity" 0.0 :!class /Script/Engine.MaterialInstanceDynamic))
        (:then_11
          (bind _returnvalue_35 (Rendering|Material|CreateDynamicMaterialInstance _figures_5_7_cube_364 0 (Rendering|Material|GetMaterial _figures_5_7_cube_364 0) "opacity" :!class /Script/Engine.PrimitiveComponent))
          (Rendering|Material|SetScalarParameterValue _returnvalue_35 "opacity" 0.0 :!class /Script/Engine.MaterialInstanceDynamic))
        (:then_12
          (bind _returnvalue_36 (Rendering|Material|CreateDynamicMaterialInstance _figures_5_7_cube_378 0 (Rendering|Material|GetMaterial _figures_5_7_cube_378 0) "opacity" :!class /Script/Engine.PrimitiveComponent))
          (Rendering|Material|SetScalarParameterValue _returnvalue_36 "opacity" 0.0 :!class /Script/Engine.MaterialInstanceDynamic))
        (:then_13
          (bind _returnvalue_37 (Rendering|Material|CreateDynamicMaterialInstance _figures_5_7_cube_379 0 (Rendering|Material|GetMaterial _figures_5_7_cube_379 0) "opacity" :!class /Script/Engine.PrimitiveComponent))
          (Rendering|Material|SetScalarParameterValue _returnvalue_37 "opacity" 0.0 :!class /Script/Engine.MaterialInstanceDynamic))
        (:then_14
          (bind _returnvalue_38 (Rendering|Material|CreateDynamicMaterialInstance _figures_5_7_cube_380 0 (Rendering|Material|GetMaterial _figures_5_7_cube_380 0) "opacity" :!class /Script/Engine.PrimitiveComponent))
          (Rendering|Material|SetScalarParameterValue _returnvalue_38 "opacity" 0.0 :!class /Script/Engine.MaterialInstanceDynamic))
        (:then_15
          (bind _returnvalue_39 (Rendering|Material|CreateDynamicMaterialInstance _figures_5_7_cube_381 0 (Rendering|Material|GetMaterial _figures_5_7_cube_381 0) "opacity" :!class /Script/Engine.PrimitiveComponent))
          (Rendering|Material|SetScalarParameterValue _returnvalue_39 "opacity" 0.0 :!class /Script/Engine.MaterialInstanceDynamic))
        (:then_16
          (bind _returnvalue_40 (Rendering|Material|CreateDynamicMaterialInstance _figures_5_7_cube_377 0 (Rendering|Material|GetMaterial _figures_5_7_cube_377 0) "opacity" :!class /Script/Engine.PrimitiveComponent))
          (Rendering|Material|SetScalarParameterValue _returnvalue_40 "opacity" 0.0 :!class /Script/Engine.MaterialInstanceDynamic))
        (:then_17
          (bind _returnvalue_41 (Rendering|Material|CreateDynamicMaterialInstance _figures_5_7_cube_370 0 (Rendering|Material|GetMaterial _figures_5_7_cube_370 0) "opacity" :!class /Script/Engine.PrimitiveComponent))
          (Rendering|Material|SetScalarParameterValue _returnvalue_41 "opacity" 0.0 :!class /Script/Engine.MaterialInstanceDynamic))
        (:then_18
          (bind _returnvalue_42 (Rendering|Material|CreateDynamicMaterialInstance _figures_5_7_cube_371 0 (Rendering|Material|GetMaterial _figures_5_7_cube_371 0) "opacity" :!class /Script/Engine.PrimitiveComponent))
          (Rendering|Material|SetScalarParameterValue _returnvalue_42 "opacity" 0.0 :!class /Script/Engine.MaterialInstanceDynamic))
        (:then_19
          (bind _returnvalue_43 (Rendering|Material|CreateDynamicMaterialInstance _figures_5_7_cube_372 0 (Rendering|Material|GetMaterial _figures_5_7_cube_372 0) "opacity" :!class /Script/Engine.PrimitiveComponent))
          (Rendering|Material|SetScalarParameterValue _returnvalue_43 "opacity" 0.0 :!class /Script/Engine.MaterialInstanceDynamic))
        (:then_20
          (bind _returnvalue_44 (Rendering|Material|CreateDynamicMaterialInstance _figures_5_7_cube_373 0 (Rendering|Material|GetMaterial _figures_5_7_cube_373 0) "opacity" :!class /Script/Engine.PrimitiveComponent))
          (Rendering|Material|SetScalarParameterValue _returnvalue_44 "opacity" 0.0 :!class /Script/Engine.MaterialInstanceDynamic))
        (:then_21
          (bind _returnvalue_45 (Rendering|Material|CreateDynamicMaterialInstance _figures_5_7_cube_374 0 (Rendering|Material|GetMaterial _figures_5_7_cube_374 0) "opacity" :!class /Script/Engine.PrimitiveComponent))
          (Rendering|Material|SetScalarParameterValue _returnvalue_45 "opacity" 0.0 :!class /Script/Engine.MaterialInstanceDynamic))
        (:then_22
          (bind _returnvalue_46 (Rendering|Material|CreateDynamicMaterialInstance _figures_5_7_cube_376 0 (Rendering|Material|GetMaterial _figures_5_7_cube_376 0) "opacity" :!class /Script/Engine.PrimitiveComponent))
          (Rendering|Material|SetScalarParameterValue _returnvalue_46 "opacity" 0.0 :!class /Script/Engine.MaterialInstanceDynamic))))))