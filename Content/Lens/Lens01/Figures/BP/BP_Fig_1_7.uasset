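; BP_Fig_1_7 is one of the selectable figures in round 1 of Lens01, picked by attaching it through its anchor connector component.
; Attaching sets Selected, waits two seconds, then asks BP_GameManager_01 to validate this actor if it is still selected.
; Detaching clears Selected.
; The older press-to-select logic, which deselected sibling figures, remains as an empty event and unconnected nodes.
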(event PressedSelect(Comp_Select)
  (params (Pawn :type BP%20Pawn%20Base%20Object%20Reference) (SourceActor :type Actor%20Object%20Reference) (ImpactLocation :type Vector :default "0, 0, 0") (ImpactComponent :type Actor%20Component%20Object%20Reference))
  ;[1 1 1] old
)

(event ConnectorDetached(Comp_Connector_Anchor)
  ;[1 1 1] if it is ready to validate selection
  (Variables|Default|Setselected false))

(event ConnectorAttached(Comp_Connector_Anchor)
  (params (Connector :type Comp%20Connector%20Object%20Reference) (AttachedToActor :type Actor%20Object%20Reference) (AttachedToComponent :type Scene%20Component%20Object%20Reference))
  ;[1 1 1] if it is ready to validate selection
  (Variables|Default|Setselected true)
  (bind _returnvalue (Actor|GetActorOfClass "/Game/Lens/Lens01/BP/BP_GameManager_01.BP_GameManager_01_C"))
  (Utilities|FlowControl|Delay 2.0)
  (if (Variables|Default|Getselected)
    (Default|ValidateSelection _returnvalue self 1)))

(fn ConstructionScript)