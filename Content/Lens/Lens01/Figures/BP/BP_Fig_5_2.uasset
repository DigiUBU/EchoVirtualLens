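; Selectable figure 2 for round 5 of Lens01, picked by attaching its anchor connector.
; Attaching sets Selected, waits two seconds, then asks BP_GameManager_01 to validate this actor if still selected; detaching clears Selected.
; SelectedOverlayColor toggles a faint opacity overlay on the figure's meshes through dynamic material instances, but its calls are disconnected.
; The older press-to-select flow that deselected sibling figures is also unwired.
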(event PressedSelect(Comp_Select)
  (params (Pawn :type BP%20Pawn%20Base%20Object%20Reference) (SourceActor :type Actor%20Object%20Reference) (ImpactLocation :type Vector :default "0, 0, 0") (ImpactComponent :type Actor%20Component%20Object%20Reference))
  ;[1 1 1] old
)

(event ConnectorAttached(Comp_Connector_Anchor)
  (params (Connector :type Comp%20Connector%20Object%20Reference) (AttachedToActor :type Actor%20Object%20Reference) (AttachedToComponent :type Scene%20Component%20Object%20Reference))
  ;[1 1 1] if it is ready to validate selection
  (Variables|Default|Setselected true)
  (bind _returnvalue (Actor|GetActorOfClass "/Game/Lens/Lens01/BP/BP_GameManager_01.BP_GameManager_01_C"))
  (Utilities|FlowControl|Delay 2.0)
  (if (Variables|Default|Getselected)
    (Default|ValidateSelection _returnvalue self 5)))

(event ConnectorDetached(Comp_Connector_Anchor)
  ;[1 1 1] if it is ready to validate selection
  (Variables|Default|Setselected false))

(fn ConstructionScript)

(fn SelectedOverlayColor
  (params (select :type Boolean))
  (bind _figures_5_2_cube_297 (Variables|Default|Getfigures_5_2_Cube_297))
  (bind _figures_5_2_cube_293 (Variables|Default|Getfigures_5_2_Cube_293))
  (bind _figures_5_2_cube_290 (Variables|Default|Getfigures_5_2_Cube_290))
  (bind _figures_5_2_cube_292 (Variables|Default|Getfigures_5_2_Cube_292))
  (bind _figures_5_2_cube_305 (Variables|Default|Getfigures_5_2_Cube_305))
  (bind _figures_5_2_cube_306 (Variables|Default|Getfigures_5_2_Cube_306))
  (bind _figures_5_2_cube_308 (Variables|Default|Getfigures_5_2_Cube_308))
  (bind _figures_5_2_cube_309 (Variables|Default|Getfigures_5_2_Cube_309))
  (bind _figures_5_2_cube_304 (Variables|Default|Getfigures_5_2_Cube_304))
  (bind _figures_5_2_cube_298 (Variables|Default|Getfigures_5_2_Cube_298))
  (bind _figures_5_2_cube_299 (Variables|Default|Getfigures_5_2_Cube_299))
  (bind _figures_5_2_cube_300 (Variables|Default|Getfigures_5_2_Cube_300))
  (bind _figures_5_2_cube_294 (Variables|Default|Getfigures_5_2_Cube_294))
  (bind _figures_5_2_cube_301 (Variables|Default|Getfigures_5_2_Cube_301))
  (bind _figures_5_2_cube_302 (Variables|Default|Getfigures_5_2_Cube_302))
  (bind _figures_5_2_cube_303 (Variables|Default|Getfigures_5_2_Cube_303))
  (bind _figures_5_2_cube_297_2 (Variables|Default|Getfigures_5_2_Cube_297))
  (bind _figures_5_2_cube_293_2 (Variables|Default|Getfigures_5_2_Cube_293))
  (bind _figures_5_2_cube_294_2 (Variables|Default|Getfigures_5_2_Cube_294))
  (bind _figures_5_2_cube_295 (Variables|Default|Getfigures_5_2_Cube_295))
  (bind _figures_5_2_cube_296 (Variables|Default|Getfigures_5_2_Cube_296))
  (bind _figures_5_2_cube_286 (Variables|Default|Getfigures_5_2_Cube_286))
  (bind _figures_5_2_cube_287 (Variables|Default|Getfigures_5_2_Cube_287))
  (bind _figures_5_2_cube_295_2 (Variables|Default|Getfigures_5_2_Cube_295))
  (bind _figures_5_2_cube_288 (Variables|Default|Getfigures_5_2_Cube_288))
  (bind _figures_5_2_cube_291 (Variables|Default|Getfigures_5_2_Cube_291))
  (bind _figures_5_2_cube_289 (Variables|Default|Getfigures_5_2_Cube_289))
  (bind _figures_5_2_cube_290_2 (Variables|Default|Getfigures_5_2_Cube_290))
  (bind _figures_5_2_cube_292_2 (Variables|Default|Getfigures_5_2_Cube_292))
  (bind _figures_5_2_cube_305_2 (Variables|Default|Getfigures_5_2_Cube_305))
  (bind _figures_5_2_cube_306_2 (Variables|Default|Getfigures_5_2_Cube_306))
  (bind _figures_5_2_cube_308_2 (Variables|Default|Getfigures_5_2_Cube_308))
  (bind _figures_5_2_cube_309_2 (Variables|Default|Getfigures_5_2_Cube_309))
  (bind _figures_5_2_cube_304_2 (Variables|Default|Getfigures_5_2_Cube_304))
  (bind _figures_5_2_cube_296_2 (Variables|Default|Getfigures_5_2_Cube_296))
  (bind _figures_5_2_cube_298_2 (Variables|Default|Getfigures_5_2_Cube_298))
  (bind _figures_5_2_cube_299_2 (Variables|Default|Getfigures_5_2_Cube_299))
  (bind _figures_5_2_cube_300_2 (Variables|Default|Getfigures_5_2_Cube_300))
  (bind _figures_5_2_cube_301_2 (Variables|Default|Getfigures_5_2_Cube_301))
  (bind _figures_5_2_cube_302_2 (Variables|Default|Getfigures_5_2_Cube_302))
  (bind _figures_5_2_cube_303_2 (Variables|Default|Getfigures_5_2_Cube_303))
  (bind _figures_5_2_cube_286_2 (Variables|Default|Getfigures_5_2_Cube_286))
  (bind _figures_5_2_cube_287_2 (Variables|Default|Getfigures_5_2_Cube_287))
  (bind _figures_5_2_cube_288_2 (Variables|Default|Getfigures_5_2_Cube_288))
  (bind _figures_5_2_cube_291_2 (Variables|Default|Getfigures_5_2_Cube_291))
  (bind _figures_5_2_cube_289_2 (Variables|Default|Getfigures_5_2_Cube_289))
  (if select
    (Utilities|FlowControl|Sequence
      (:then_0
        (bind _returnvalue (Rendering|Material|CreateDynamicMaterialInstance _figures_5_2_cube_286 0 (Rendering|Material|GetMaterial _figures_5_2_cube_286 0) "opacity" :!class /Script/Engine.PrimitiveComponent))
        (Rendering|Material|SetScalarParameterValue _returnvalue "opacity" 0.25 :!class /Script/Engine.MaterialInstanceDynamic))
      (:then_1
        (bind _returnvalue_2 (Rendering|Material|CreateDynamicMaterialInstance _figures_5_2_cube_297_2 0 (Rendering|Material|GetMaterial _figures_5_2_cube_297_2 0) "opacity" :!class /Script/Engine.PrimitiveComponent))
        (Rendering|Material|SetScalarParameterValue _returnvalue_2 "opacity" 0.25 :!class /Script/Engine.MaterialInstanceDynamic))
      (:then_2
        (bind _returnvalue_3 (Rendering|Material|CreateDynamicMaterialInstance _figures_5_2_cube_293_2 0 (Rendering|Material|GetMaterial _figures_5_2_cube_293_2 0) "opacity" :!class /Script/Engine.PrimitiveComponent))
        (Rendering|Material|SetScalarParameterValue _returnvalue_3 "opacity" 0.25 :!class /Script/Engine.MaterialInstanceDynamic))
      (:then_3
        (bind _returnvalue_4 (Rendering|Material|CreateDynamicMaterialInstance _figures_5_2_cube_294_2 0 (Rendering|Material|GetMaterial _figures_5_2_cube_294_2 0) "opacity" :!class /Script/Engine.PrimitiveComponent))
        (Rendering|Material|SetScalarParameterValue _returnvalue_4 "opacity" 0.25 :!class /Script/Engine.MaterialInstanceDynamic))
      (:then_4
        (bind _returnvalue_5 (Rendering|Material|CreateDynamicMaterialInstance _figures_5_2_cube_295 0 (Rendering|Material|GetMaterial _figures_5_2_cube_295 0) "opacity" :!class /Script/Engine.PrimitiveComponent))
        (Rendering|Material|SetScalarParameterValue _returnvalue_5 "opacity" 0.25 :!class /Script/Engine.MaterialInstanceDynamic))
      (:then_5
        (bind _returnvalue_6 (Rendering|Material|CreateDynamicMaterialInstance _figures_5_2_cube_296 0 (Rendering|Material|GetMaterial _figures_5_2_cube_296 0) "opacity" :!class /Script/Engine.PrimitiveComponent))
        (Rendering|Material|SetScalarParameterValue _returnvalue_6 "opacity" 0.25 :!class /Script/Engine.MaterialInstanceDynamic))
      (:then_6
        (bind _returnvalue_7 (Rendering|Material|CreateDynamicMaterialInstance _figures_5_2_cube_287 0 (Rendering|Material|GetMaterial _figures_5_2_cube_287 0) "opacity" :!class /Script/Engine.PrimitiveComponent))
        (Rendering|Material|SetScalarParameterValue _returnvalue_7 "opacity" 0.25 :!class /Script/Engine.MaterialInstanceDynamic))
      (:then_7
        (bind _returnvalue_8 (Rendering|Material|CreateDynamicMaterialInstance _figures_5_2_cube_288 0 (Rendering|Material|GetMaterial _figures_5_2_cube_288 0) "opacity" :!class /Script/Engine.PrimitiveComponent))
        (Rendering|Material|SetScalarParameterValue _returnvalue_8 "opacity" 0.25 :!class /Script/Engine.MaterialInstanceDynamic))
      (:then_8
        (bind _returnvalue_9 (Rendering|Material|CreateDynamicMaterialInstance _figures_5_2_cube_291 0 (Rendering|Material|GetMaterial _figures_5_2_cube_291 0) "opacity" :!class /Script/Engine.PrimitiveComponent))
        (Rendering|Material|SetScalarParameterValue _returnvalue_9 "opacity" 0.25 :!class /Script/Engine.MaterialInstanceDynamic))
      (:then_9
        (bind _returnvalue_10 (Rendering|Material|CreateDynamicMaterialInstance _figures_5_2_cube_289 0 (Rendering|Material|GetMaterial _figures_5_2_cube_289 0) "opacity" :!class /Script/Engine.PrimitiveComponent))
        (Rendering|Material|SetScalarParameterValue _returnvalue_10 "opacity" 0.25 :!class /Script/Engine.MaterialInstanceDynamic))
      (:then_10
        (bind _returnvalue_11 (Rendering|Material|CreateDynamicMaterialInstance _figures_5_2_cube_290_2 0 (Rendering|Material|GetMaterial _figures_5_2_cube_290_2 0) "opacity" :!class /Script/Engine.PrimitiveComponent))
        (Rendering|Material|SetScalarParameterValue _returnvalue_11 "opacity" 0.25 :!class /Script/Engine.MaterialInstanceDynamic))
      (:then_11
        (bind _returnvalue_12 (Rendering|Material|CreateDynamicMaterialInstance _figures_5_2_cube_292_2 0 (Rendering|Material|GetMaterial _figures_5_2_cube_292_2 0) "opacity" :!class /Script/Engine.PrimitiveComponent))
        (Rendering|Material|SetScalarParameterValue _returnvalue_12 "opacity" 0.25 :!class /Script/Engine.MaterialInstanceDynamic))
      (:then_12
        (bind _returnvalue_13 (Rendering|Material|CreateDynamicMaterialInstance _figures_5_2_cube_305_2 0 (Rendering|Material|GetMaterial _figures_5_2_cube_305_2 0) "opacity" :!class /Script/Engine.PrimitiveComponent))
        (Rendering|Material|SetScalarParameterValue _returnvalue_13 "opacity" 0.25 :!class /Script/Engine.MaterialInstanceDynamic))
      (:then_13
        (bind _returnvalue_14 (Rendering|Material|CreateDynamicMaterialInstance _figures_5_2_cube_306_2 0 (Rendering|Material|GetMaterial _figures_5_2_cube_306_2 0) "opacity" :!class /Script/Engine.PrimitiveComponent))
        (Rendering|Material|SetScalarParameterValue _returnvalue_14 "opacity" 0.25 :!class /Script/Engine.MaterialInstanceDynamic))
      (:then_14
        (bind _returnvalue_15 (Rendering|Material|CreateDynamicMaterialInstance _figures_5_2_cube_308_2 0 (Rendering|Material|GetMaterial _figures_5_2_cube_308_2 0) "opacity" :!class /Script/Engine.PrimitiveComponent))
        (Rendering|Material|SetScalarParameterValue _returnvalue_15 "opacity" 0.25 :!class /Script/Engine.MaterialInstanceDynamic))
      (:then_15
        (bind _returnvalue_16 (Rendering|Material|CreateDynamicMaterialInstance _figures_5_2_cube_309_2 0 (Rendering|Material|GetMaterial _figures_5_2_cube_309_2 0) "opacity" :!class /Script/Engine.PrimitiveComponent))
        (Rendering|Material|SetScalarParameterValue _returnvalue_16 "opacity" 0.25 :!class /Script/Engine.MaterialInstanceDynamic))
      (:then_16
        (bind _returnvalue_17 (Rendering|Material|CreateDynamicMaterialInstance _figures_5_2_cube_304_2 0 (Rendering|Material|GetMaterial _figures_5_2_cube_304_2 0) "opacity" :!class /Script/Engine.PrimitiveComponent))
        (Rendering|Material|SetScalarParameterValue _returnvalue_17 "opacity" 0.25 :!class /Script/Engine.MaterialInstanceDynamic))
      (:then_17
        (bind _returnvalue_18 (Rendering|Material|CreateDynamicMaterialInstance _figures_5_2_cube_298_2 0 (Rendering|Material|GetMaterial _figures_5_2_cube_298_2 0) "opacity" :!class /Script/Engine.PrimitiveComponent))
        (Rendering|Material|SetScalarParameterValue _returnvalue_18 "opacity" 0.25 :!class /Script/Engine.MaterialInstanceDynamic))
      (:then_18
        (bind _returnvalue_19 (Rendering|Material|CreateDynamicMaterialInstance _figures_5_2_cube_299_2 0 (Rendering|Material|GetMaterial _figures_5_2_cube_299_2 0) "opacity" :!class /Script/Engine.PrimitiveComponent))
        (Rendering|Material|SetScalarParameterValue _returnvalue_19 "opacity" 0.25 :!class /Script/Engine.MaterialInstanceDynamic))
      (:then_19
        (bind _returnvalue_20 (Rendering|Material|CreateDynamicMaterialInstance _figures_5_2_cube_300_2 0 (Rendering|Material|GetMaterial _figures_5_2_cube_300_2 0) "opacity" :!class /Script/Engine.PrimitiveComponent))
        (Rendering|Material|SetScalarParameterValue _returnvalue_20 "opacity" 0.25 :!class /Script/Engine.MaterialInstanceDynamic))
      (:then_20
        (bind _returnvalue_21 (Rendering|Material|CreateDynamicMaterialInstance _figures_5_2_cube_301_2 0 (Rendering|Material|GetMaterial _figures_5_2_cube_301_2 0) "opacity" :!class /Script/Engine.PrimitiveComponent))
        (Rendering|Material|SetScalarParameterValue _returnvalue_21 "opacity" 0.25 :!class /Script/Engine.MaterialInstanceDynamic))
      (:then_21
        (bind _returnvalue_22 (Rendering|Material|CreateDynamicMaterialInstance _figures_5_2_cube_302_2 0 (Rendering|Material|GetMaterial _figures_5_2_cube_302_2 0) "opacity" :!class /Script/Engine.PrimitiveComponent))
        (Rendering|Material|SetScalarParameterValue _returnvalue_22 "opacity" 0.25 :!class /Script/Engine.MaterialInstanceDynamic))
      (:then_22
        (bind _returnvalue_23 (Rendering|Material|CreateDynamicMaterialInstance _figures_5_2_cube_303_2 0 (Rendering|Material|GetMaterial _figures_5_2_cube_303_2 0) "opacity" :!class /Script/Engine.PrimitiveComponent))
        (Rendering|Material|SetScalarParameterValue _returnvalue_23 "opacity" 0.25 :!class /Script/Engine.MaterialInstanceDynamic)))
    (else
      (Utilities|FlowControl|Sequence
        (:then_0
          (bind _returnvalue_24 (Rendering|Material|CreateDynamicMaterialInstance _figures_5_2_cube_286_2 0 (Rendering|Material|GetMaterial _figures_5_2_cube_286_2 0) "opacity" :!class /Script/Engine.PrimitiveComponent))
          (Rendering|Material|SetScalarParameterValue _returnvalue_24 "opacity" 0.0 :!class /Script/Engine.MaterialInstanceDynamic))
        (:then_1
          (bind _returnvalue_25 (Rendering|Material|CreateDynamicMaterialInstance _figures_5_2_cube_297 0 (Rendering|Material|GetMaterial _figures_5_2_cube_297 0) "opacity" :!class /Script/Engine.PrimitiveComponent))
          (Rendering|Material|SetScalarParameterValue _returnvalue_25 "opacity" 0.0 :!class /Script/Engine.MaterialInstanceDynamic))
        (:then_2
          (bind _returnvalue_26 (Rendering|Material|CreateDynamicMaterialInstance _figures_5_2_cube_293 0 (Rendering|Material|GetMaterial _figures_5_2_cube_293 0) "opacity" :!class /Script/Engine.PrimitiveComponent))
          (Rendering|Material|SetScalarParameterValue _returnvalue_26 "opacity" 0.0 :!class /Script/Engine.MaterialInstanceDynamic))
        (:then_3
          (bind _returnvalue_27 (Rendering|Material|CreateDynamicMaterialInstance _figures_5_2_cube_294 0 (Rendering|Material|GetMaterial _figures_5_2_cube_294 0) "opacity" :!class /Script/Engine.PrimitiveComponent))
          (Rendering|Material|SetScalarParameterValue _returnvalue_27 "opacity" 0.0 :!class /Script/Engine.MaterialInstanceDynamic))
        (:then_4
          (bind _returnvalue_28 (Rendering|Material|CreateDynamicMaterialInstance _figures_5_2_cube_295_2 0 (Rendering|Material|GetMaterial _figures_5_2_cube_295_2 0) "opacity" :!class /Script/Engine.PrimitiveComponent))
          (Rendering|Material|SetScalarParameterValue _returnvalue_28 "opacity" 0.0 :!class /Script/Engine.MaterialInstanceDynamic))
        (:then_5
          (bind _returnvalue_29 (Rendering|Material|CreateDynamicMaterialInstance _figures_5_2_cube_296_2 0 (Rendering|Material|GetMaterial _figures_5_2_cube_296_2 0) "opacity" :!class /Script/Engine.PrimitiveComponent))
          (Rendering|Material|SetScalarParameterValue _returnvalue_29 "opacity" 0.0 :!class /Script/Engine.MaterialInstanceDynamic))
        (:then_6
          (bind _returnvalue_30 (Rendering|Material|CreateDynamicMaterialInstance _figures_5_2_cube_287_2 0 (Rendering|Material|GetMaterial _figures_5_2_cube_287_2 0) "opacity" :!class /Script/Engine.PrimitiveComponent))
          (Rendering|Material|SetScalarParameterValue _returnvalue_30 "opacity" 0.0 :!class /Script/Engine.MaterialInstanceDynamic))
        (:then_7
          (bind _returnvalue_31 (Rendering|Material|CreateDynamicMaterialInstance _figures_5_2_cube_288_2 0 (Rendering|Material|GetMaterial _figures_5_2_cube_288_2 0) "opacity" :!class /Script/Engine.PrimitiveComponent))
          (Rendering|Material|SetScalarParameterValue _returnvalue_31 "opacity" 0.0 :!class /Script/Engine.MaterialInstanceDynamic))
        (:then_8
          (bind _returnvalue_32 (Rendering|Material|CreateDynamicMaterialInstance _figures_5_2_cube_291_2 0 (Rendering|Material|GetMaterial _figures_5_2_cube_291_2 0) "opacity" :!class /Script/Engine.PrimitiveComponent))
          (Rendering|Material|SetScalarParameterValue _returnvalue_32 "opacity" 0.0 :!class /Script/Engine.MaterialInstanceDynamic))
        (:then_9
          (bind _returnvalue_33 (Rendering|Material|CreateDynamicMaterialInstance _figures_5_2_cube_289_2 0 (Rendering|Material|GetMaterial _figures_5_2_cube_289_2 0) "opacity" :!class /Script/Engine.PrimitiveComponent))
          (Rendering|Material|SetScalarParameterValue _returnvalue_33 "opacity" 0.0 :!class /Script/Engine.MaterialInstanceDynamic))
        (:then_10
          (bind _returnvalue_34 (Rendering|Material|CreateDynamicMaterialInstance _figures_5_2_cube_290 0 (Rendering|Material|GetMaterial _figures_5_2_cube_290 0) "opacity" :!class /Script/Engine.PrimitiveComponent))
          (Rendering|Material|SetScalarParameterValue _returnvalue_34 "opacity" 0.0 :!class /Script/Engine.MaterialInstanceDynamic))
        (:then_11
          (bind _returnvalue_35 (Rendering|Material|CreateDynamicMaterialInstance _figures_5_2_cube_292 0 (Rendering|Material|GetMaterial _figures_5_2_cube_292 0) "opacity" :!class /Script/Engine.PrimitiveComponent))
          (Rendering|Material|SetScalarParameterValue _returnvalue_35 "opacity" 0.0 :!class /Script/Engine.MaterialInstanceDynamic))
        (:then_12
          (bind _returnvalue_36 (Rendering|Material|CreateDynamicMaterialInstance _figures_5_2_cube_305 0 (Rendering|Material|GetMaterial _figures_5_2_cube_305 0) "opacity" :!class /Script/Engine.PrimitiveComponent))
          (Rendering|Material|SetScalarParameterValue _returnvalue_36 "opacity" 0.0 :!class /Script/Engine.MaterialInstanceDynamic))
        (:then_13
          (bind _returnvalue_37 (Rendering|Material|CreateDynamicMaterialInstance _figures_5_2_cube_306 0 (Rendering|Material|GetMaterial _figures_5_2_cube_306 0) "opacity" :!class /Script/Engine.PrimitiveComponent))
          (Rendering|Material|SetScalarParameterValue _returnvalue_37 "opacity" 0.0 :!class /Script/Engine.MaterialInstanceDynamic))
        (:then_14
          (bind _returnvalue_38 (Rendering|Material|CreateDynamicMaterialInstance _figures_5_2_cube_308 0 (Rendering|Material|GetMaterial _figures_5_2_cube_308 0) "opacity" :!class /Script/Engine.PrimitiveComponent))
          (Rendering|Material|SetScalarParameterValue _returnvalue_38 "opacity" 0.0 :!class /Script/Engine.MaterialInstanceDynamic))
        (:then_15
          (bind _returnvalue_39 (Rendering|Material|CreateDynamicMaterialInstance _figures_5_2_cube_309 0 (Rendering|Material|GetMaterial _figures_5_2_cube_309 0) "opacity" :!class /Script/Engine.PrimitiveComponent))
          (Rendering|Material|SetScalarParameterValue _returnvalue_39 "opacity" 0.0 :!class /Script/Engine.MaterialInstanceDynamic))
        (:then_16
          (bind _returnvalue_40 (Rendering|Material|CreateDynamicMaterialInstance _figures_5_2_cube_304 0 (Rendering|Material|GetMaterial _figures_5_2_cube_304 0) "opacity" :!class /Script/Engine.PrimitiveComponent))
          (Rendering|Material|SetScalarParameterValue _returnvalue_40 "opacity" 0.0 :!class /Script/Engine.MaterialInstanceDynamic))
        (:then_17
          (bind _returnvalue_41 (Rendering|Material|CreateDynamicMaterialInstance _figures_5_2_cube_298 0 (Rendering|Material|GetMaterial _figures_5_2_cube_298 0) "opacity" :!class /Script/Engine.PrimitiveComponent))
          (Rendering|Material|SetScalarParameterValue _returnvalue_41 "opacity" 0.0 :!class /Script/Engine.MaterialInstanceDynamic))
        (:then_18
          (bind _returnvalue_42 (Rendering|Material|CreateDynamicMaterialInstance _figures_5_2_cube_299 0 (Rendering|Material|GetMaterial _figures_5_2_cube_299 0) "opacity" :!class /Script/Engine.PrimitiveComponent))
          (Rendering|Material|SetScalarParameterValue _returnvalue_42 "opacity" 0.0 :!class /Script/Engine.MaterialInstanceDynamic))
        (:then_19
          (bind _returnvalue_43 (Rendering|Material|CreateDynamicMaterialInstance _figures_5_2_cube_300 0 (Rendering|Material|GetMaterial _figures_5_2_cube_300 0) "opacity" :!class /Script/Engine.PrimitiveComponent))
          (Rendering|Material|SetScalarParameterValue _returnvalue_43 "opacity" 0.0 :!class /Script/Engine.MaterialInstanceDynamic))
        (:then_20
          (bind _returnvalue_44 (Rendering|Material|CreateDynamicMaterialInstance _figures_5_2_cube_301 0 (Rendering|Material|GetMaterial _figures_5_2_cube_301 0) "opacity" :!class /Script/Engine.PrimitiveComponent))
          (Rendering|Material|SetScalarParameterValue _returnvalue_44 "opacity" 0.0 :!class /Script/Engine.MaterialInstanceDynamic))
        (:then_21
          (bind _returnvalue_45 (Rendering|Material|CreateDynamicMaterialInstance _figures_5_2_cube_302 0 (Rendering|Material|GetMaterial _figures_5_2_cube_302 0) "opacity" :!class /Script/Engine.PrimitiveComponent))
          (Rendering|Material|SetScalarParameterValue _returnvalue_45 "opacity" 0.0 :!class /Script/Engine.MaterialInstanceDynamic))
        (:then_22
          (bind _returnvalue_46 (Rendering|Material|CreateDynamicMaterialInstance _figures_5_2_cube_303 0 (Rendering|Material|GetMaterial _figures_5_2_cube_303 0) "opacity" :!class /Script/Engine.PrimitiveComponent))
          (Rendering|Material|SetScalarParameterValue _returnvalue_46 "opacity" 0.0 :!class /Script/Engine.MaterialInstanceDynamic))))))