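; Selectable figure 5_4 for round 5 of Lens01, chosen by attaching its anchor connector.
; Attaching sets Selected, waits two seconds, then asks BP_GameManager_01 to validate this actor if still selected; detaching clears the flag.
; SelectedOverlayColor toggles an opacity overlay on the cube meshes through dynamic material instances.
; The older press-to-select flow, including its overlay calls and deselection of sibling figures, is disconnected.
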(event PressedSelect(Comp_Select)
  (params (Pawn :type BP%20Pawn%20Base%20Object%20Reference) (SourceActor :type Actor%20Object%20Reference) (ImpactLocation :type Vector :default "0, 0, 0") (ImpactComponent :type Actor%20Component%20Object%20Reference))
  ;[1 1 1] old
)

(event ConnectorAttached(Comp_Connector_Anchor)
  (params (Connector :type Comp%20Connector%20Object%20Reference) (AttachedToActor :type Actor%20Object%20Reference) (AttachedToComponent :type Scene%20Component%20Object%20Reference))
  ;[1 1 1] if it is ready to validate selection
  (Variables|Default|Setselected true)
  (bind _returnvalue (Actor|GetActorOfClass "/Game/Lens/Lens01/BP/BP_GameManager_01.BP_GameManager_01_C"))
  (Utilities|FlowControl|Delay 2.0)
  (if (Variables|Default|Getselected)
    (Default|ValidateSelection _returnvalue self 5)))

(event ConnectorDetached(Comp_Connector_Anchor)
  ;[1 1 1] if it is ready to validate selection
  (Variables|Default|Setselected false))

(fn ConstructionScript)

(fn SelectedOverlayColor
  (params (select :type Boolean))
  (bind _figures_5_4_cube_258 (Variables|Default|Getfigures_5_4_Cube_258))
  (bind _figures_5_4_cube_246 (Variables|Default|Getfigures_5_4_Cube_246))
  (bind _figures_5_4_cube_240 (Variables|Default|Getfigures_5_4_Cube_240))
  (bind _figures_5_4_cube_241 (Variables|Default|Getfigures_5_4_Cube_241))
  (bind _figures_5_4_cube_244 (Variables|Default|Getfigures_5_4_Cube_244))
  (bind _figures_5_4_cube_259 (Variables|Default|Getfigures_5_4_Cube_259))
  (bind _figures_5_4_cube_257 (Variables|Default|Getfigures_5_4_Cube_257))
  (bind _figures_5_4_cube_260 (Variables|Default|Getfigures_5_4_Cube_260))
  (bind _figures_5_4_cube_261 (Variables|Default|Getfigures_5_4_Cube_261))
  (bind _figures_5_4_cube_250 (Variables|Default|Getfigures_5_4_Cube_250))
  (bind _figures_5_4_cube_256 (Variables|Default|Getfigures_5_4_Cube_256))
  (bind _figures_5_4_cube_251 (Variables|Default|Getfigures_5_4_Cube_251))
  (bind _figures_5_4_cube_247 (Variables|Default|Getfigures_5_4_Cube_247))
  (bind _figures_5_4_cube_252 (Variables|Default|Getfigures_5_4_Cube_252))
  (bind _figures_5_4_cube_253 (Variables|Default|Getfigures_5_4_Cube_253))
  (bind _figures_5_4_cube_254 (Variables|Default|Getfigures_5_4_Cube_254))
  (bind _figures_5_4_cube_255 (Variables|Default|Getfigures_5_4_Cube_255))
  (bind _figures_5_4_cube_258_2 (Variables|Default|Getfigures_5_4_Cube_258))
  (bind _figures_5_4_cube_246_2 (Variables|Default|Getfigures_5_4_Cube_246))
  (bind _figures_5_4_cube_247_2 (Variables|Default|Getfigures_5_4_Cube_247))
  (bind _figures_5_4_cube_248 (Variables|Default|Getfigures_5_4_Cube_248))
  (bind _figures_5_4_cube_249 (Variables|Default|Getfigures_5_4_Cube_249))
  (bind _figures_5_4_cube_243 (Variables|Default|Getfigures_5_4_Cube_243))
  (bind _figures_5_4_cube_248_2 (Variables|Default|Getfigures_5_4_Cube_248))
  (bind _figures_5_4_cube_038 (Variables|Default|Getfigures_5_4_Cube_038))
  (bind _figures_5_4_cube_238 (Variables|Default|Getfigures_5_4_Cube_238))
  (bind _figures_5_4_cube_239 (Variables|Default|Getfigures_5_4_Cube_239))
  (bind _figures_5_4_cube_242 (Variables|Default|Getfigures_5_4_Cube_242))
  (bind _figures_5_4_cube_240_2 (Variables|Default|Getfigures_5_4_Cube_240))
  (bind _figures_5_4_cube_241_2 (Variables|Default|Getfigures_5_4_Cube_241))
  (bind _figures_5_4_cube_244_2 (Variables|Default|Getfigures_5_4_Cube_244))
  (bind _figures_5_4_cube_259_2 (Variables|Default|Getfigures_5_4_Cube_259))
  (bind _figures_5_4_cube_257_2 (Variables|Default|Getfigures_5_4_Cube_257))
  (bind _figures_5_4_cube_260_2 (Variables|Default|Getfigures_5_4_Cube_260))
  (bind _figures_5_4_cube_249_2 (Variables|Default|Getfigures_5_4_Cube_249))
  (bind _figures_5_4_cube_261_2 (Variables|Default|Getfigures_5_4_Cube_261))
  (bind _figures_5_4_cube_250_2 (Variables|Default|Getfigures_5_4_Cube_250))
  (bind _figures_5_4_cube_256_2 (Variables|Default|Getfigures_5_4_Cube_256))
  (bind _figures_5_4_cube_251_2 (Variables|Default|Getfigures_5_4_Cube_251))
  (bind _figures_5_4_cube_252_2 (Variables|Default|Getfigures_5_4_Cube_252))
  (bind _figures_5_4_cube_253_2 (Variables|Default|Getfigures_5_4_Cube_253))
  (bind _figures_5_4_cube_254_2 (Variables|Default|Getfigures_5_4_Cube_254))
  (bind _figures_5_4_cube_255_2 (Variables|Default|Getfigures_5_4_Cube_255))
  (bind _figures_5_4_cube_243_2 (Variables|Default|Getfigures_5_4_Cube_243))
  (bind _figures_5_4_cube_038_2 (Variables|Default|Getfigures_5_4_Cube_038))
  (bind _figures_5_4_cube_238_2 (Variables|Default|Getfigures_5_4_Cube_238))
  (bind _figures_5_4_cube_239_2 (Variables|Default|Getfigures_5_4_Cube_239))
  (bind _figures_5_4_cube_242_2 (Variables|Default|Getfigures_5_4_Cube_242))
  (if select
    (Utilities|FlowControl|Sequence
      (:then_0
        (bind _returnvalue (Rendering|Material|CreateDynamicMaterialInstance _figures_5_4_cube_243 0 (Rendering|Material|GetMaterial _figures_5_4_cube_243 0) "opacity" :!class /Script/Engine.PrimitiveComponent))
        (Rendering|Material|SetScalarParameterValue _returnvalue "opacity" 0.25 :!class /Script/Engine.MaterialInstanceDynamic))
      (:then_1
        (bind _returnvalue_2 (Rendering|Material|CreateDynamicMaterialInstance _figures_5_4_cube_258_2 0 (Rendering|Material|GetMaterial _figures_5_4_cube_258_2 0) "opacity" :!class /Script/Engine.PrimitiveComponent))
        (Rendering|Material|SetScalarParameterValue _returnvalue_2 "opacity" 0.25 :!class /Script/Engine.MaterialInstanceDynamic))
      (:then_2
        (bind _returnvalue_3 (Rendering|Material|CreateDynamicMaterialInstance _figures_5_4_cube_246_2 0 (Rendering|Material|GetMaterial _figures_5_4_cube_246_2 0) "opacity" :!class /Script/Engine.PrimitiveComponent))
        (Rendering|Material|SetScalarParameterValue _returnvalue_3 "opacity" 0.25 :!class /Script/Engine.MaterialInstanceDynamic))
      (:then_3
        (bind _returnvalue_4 (Rendering|Material|CreateDynamicMaterialInstance _figures_5_4_cube_247_2 0 (Rendering|Material|GetMaterial _figures_5_4_cube_247_2 0) "opacity" :!class /Script/Engine.PrimitiveComponent))
        (Rendering|Material|SetScalarParameterValue _returnvalue_4 "opacity" 0.25 :!class /Script/Engine.MaterialInstanceDynamic))
      (:then_4
        (bind _returnvalue_5 (Rendering|Material|CreateDynamicMaterialInstance _figures_5_4_cube_248 0 (Rendering|Material|GetMaterial _figures_5_4_cube_248 0) "opacity" :!class /Script/Engine.PrimitiveComponent))
        (Rendering|Material|SetScalarParameterValue _returnvalue_5 "opacity" 0.25 :!class /Script/Engine.MaterialInstanceDynamic))
      (:then_5
        (bind _returnvalue_6 (Rendering|Material|CreateDynamicMaterialInstance _figures_5_4_cube_249 0 (Rendering|Material|GetMaterial _figures_5_4_cube_249 0) "opacity" :!class /Script/Engine.PrimitiveComponent))
        (Rendering|Material|SetScalarParameterValue _returnvalue_6 "opacity" 0.25 :!class /Script/Engine.MaterialInstanceDynamic))
      (:then_6
        (bind _returnvalue_7 (Rendering|Material|CreateDynamicMaterialInstance _figures_5_4_cube_038 0 (Rendering|Material|GetMaterial _figures_5_4_cube_038 0) "opacity" :!class /Script/Engine.PrimitiveComponent))
        (Rendering|Material|SetScalarParameterValue _returnvalue_7 "opacity" 0.25 :!class /Script/Engine.MaterialInstanceDynamic))
      (:then_7
        (bind _returnvalue_8 (Rendering|Material|CreateDynamicMaterialInstance _figures_5_4_cube_238 0 (Rendering|Material|GetMaterial _figures_5_4_cube_238 0) "opacity" :!class /Script/Engine.PrimitiveComponent))
        (Rendering|Material|SetScalarParameterValue _returnvalue_8 "opacity" 0.25 :!class /Script/Engine.MaterialInstanceDynamic))
      (:then_8
        (bind _returnvalue_9 (Rendering|Material|CreateDynamicMaterialInstance _figures_5_4_cube_239 0 (Rendering|Material|GetMaterial _figures_5_4_cube_239 0) "opacity" :!class /Script/Engine.PrimitiveComponent))
        (Rendering|Material|SetScalarParameterValue _returnvalue_9 "opacity" 0.25 :!class /Script/Engine.MaterialInstanceDynamic))
      (:then_9
        (bind _returnvalue_10 (Rendering|Material|CreateDynamicMaterialInstance _figures_5_4_cube_242 0 (Rendering|Material|GetMaterial _figures_5_4_cube_242 0) "opacity" :!class /Script/Engine.PrimitiveComponent))
        (Rendering|Material|SetScalarParameterValue _returnvalue_10 "opacity" 0.25 :!class /Script/Engine.MaterialInstanceDynamic))
      (:then_10
        (bind _returnvalue_11 (Rendering|Material|CreateDynamicMaterialInstance _figures_5_4_cube_240_2 0 (Rendering|Material|GetMaterial _figures_5_4_cube_240_2 0) "opacity" :!class /Script/Engine.PrimitiveComponent))
        (Rendering|Material|SetScalarParameterValue _returnvalue_11 "opacity" 0.25 :!class /Script/Engine.MaterialInstanceDynamic))
      (:then_11
        (bind _returnvalue_12 (Rendering|Material|CreateDynamicMaterialInstance _figures_5_4_cube_241_2 0 (Rendering|Material|GetMaterial _figures_5_4_cube_241_2 0) "opacity" :!class /Script/Engine.PrimitiveComponent))
        (Rendering|Material|SetScalarParameterValue _returnvalue_12 "opacity" 0.25 :!class /Script/Engine.MaterialInstanceDynamic))
      (:then_12
        (bind _returnvalue_13 (Rendering|Material|CreateDynamicMaterialInstance _figures_5_4_cube_244_2 0 (Rendering|Material|GetMaterial _figures_5_4_cube_244_2 0) "opacity" :!class /Script/Engine.PrimitiveComponent))
        (Rendering|Material|SetScalarParameterValue _returnvalue_13 "opacity" 0.25 :!class /Script/Engine.MaterialInstanceDynamic))
      (:then_13
        (bind _returnvalue_14 (Rendering|Material|CreateDynamicMaterialInstance _figures_5_4_cube_259_2 0 (Rendering|Material|GetMaterial _figures_5_4_cube_259_2 0) "opacity" :!class /Script/Engine.PrimitiveComponent))
        (Rendering|Material|SetScalarParameterValue _returnvalue_14 "opacity" 0.25 :!class /Script/Engine.MaterialInstanceDynamic))
      (:then_14
        (bind _returnvalue_15 (Rendering|Material|CreateDynamicMaterialInstance _figures_5_4_cube_257_2 0 (Rendering|Material|GetMaterial _figures_5_4_cube_257_2 0) "opacity" :!class /Script/Engine.PrimitiveComponent))
        (Rendering|Material|SetScalarParameterValue _returnvalue_15 "opacity" 0.25 :!class /Script/Engine.MaterialInstanceDynamic))
      (:then_15
        (bind _returnvalue_16 (Rendering|Material|CreateDynamicMaterialInstance _figures_5_4_cube_260_2 0 (Rendering|Material|GetMaterial _figures_5_4_cube_260_2 0) "opacity" :!class /Script/Engine.PrimitiveComponent))
        (Rendering|Material|SetScalarParameterValue _returnvalue_16 "opacity" 0.25 :!class /Script/Engine.MaterialInstanceDynamic))
      (:then_16
        (bind _returnvalue_17 (Rendering|Material|CreateDynamicMaterialInstance _figures_5_4_cube_261_2 0 (Rendering|Material|GetMaterial _figures_5_4_cube_261_2 0) "opacity" :!class /Script/Engine.PrimitiveComponent))
        (Rendering|Material|SetScalarParameterValue _returnvalue_17 "opacity" 0.25 :!class /Script/Engine.MaterialInstanceDynamic))
      (:then_17
        (bind _returnvalue_18 (Rendering|Material|CreateDynamicMaterialInstance _figures_5_4_cube_250_2 0 (Rendering|Material|GetMaterial _figures_5_4_cube_250_2 0) "opacity" :!class /Script/Engine.PrimitiveComponent))
        (Rendering|Material|SetScalarParameterValue _returnvalue_18 "opacity" 0.25 :!class /Script/Engine.MaterialInstanceDynamic))
      (:then_18
        (bind _returnvalue_19 (Rendering|Material|CreateDynamicMaterialInstance _figures_5_4_cube_256_2 0 (Rendering|Material|GetMaterial _figures_5_4_cube_256_2 0) "opacity" :!class /Script/Engine.PrimitiveComponent))
        (Rendering|Material|SetScalarParameterValue _returnvalue_19 "opacity" 0.25 :!class /Script/Engine.MaterialInstanceDynamic))
      (:then_19
        (bind _returnvalue_20 (Rendering|Material|CreateDynamicMaterialInstance _figures_5_4_cube_251_2 0 (Rendering|Material|GetMaterial _figures_5_4_cube_251_2 0) "opacity" :!class /Script/Engine.PrimitiveComponent))
        (Rendering|Material|SetScalarParameterValue _returnvalue_20 "opacity" 0.25 :!class /Script/Engine.MaterialInstanceDynamic))
      (:then_20
        (bind _returnvalue_21 (Rendering|Material|CreateDynamicMaterialInstance _figures_5_4_cube_252_2 0 (Rendering|Material|GetMaterial _figures_5_4_cube_252_2 0) "opacity" :!class /Script/Engine.PrimitiveComponent))
        (Rendering|Material|SetScalarParameterValue _returnvalue_21 "opacity" 0.25 :!class /Script/Engine.MaterialInstanceDynamic))
      (:then_21
        (bind _returnvalue_22 (Rendering|Material|CreateDynamicMaterialInstance _figures_5_4_cube_253_2 0 (Rendering|Material|GetMaterial _figures_5_4_cube_253_2 0) "opacity" :!class /Script/Engine.PrimitiveComponent))
        (Rendering|Material|SetScalarParameterValue _returnvalue_22 "opacity" 0.25 :!class /Script/Engine.MaterialInstanceDynamic))
      (:then_22
        (bind _returnvalue_23 (Rendering|Material|CreateDynamicMaterialInstance _figures_5_4_cube_254_2 0 (Rendering|Material|GetMaterial _figures_5_4_cube_254_2 0) "opacity" :!class /Script/Engine.PrimitiveComponent))
        (Rendering|Material|SetScalarParameterValue _returnvalue_23 "opacity" 0.25 :!class /Script/Engine.MaterialInstanceDynamic))
      (:then_23
        (bind _returnvalue_24 (Rendering|Material|CreateDynamicMaterialInstance _figures_5_4_cube_255_2 0 (Rendering|Material|GetMaterial _figures_5_4_cube_255_2 0) "opacity" :!class /Script/Engine.PrimitiveComponent))
        (Rendering|Material|SetScalarParameterValue _returnvalue_24 "opacity" 0.25 :!class /Script/Engine.MaterialInstanceDynamic)))
    (else
      (Utilities|FlowControl|Sequence
        (:then_0
          (bind _returnvalue_25 (Rendering|Material|CreateDynamicMaterialInstance _figures_5_4_cube_243_2 0 (Rendering|Material|GetMaterial _figures_5_4_cube_243_2 0) "opacity" :!class /Script/Engine.PrimitiveComponent))
          (Rendering|Material|SetScalarParameterValue _returnvalue_25 "opacity" 0.0 :!class /Script/Engine.MaterialInstanceDynamic))
        (:then_1
          (bind _returnvalue_26 (Rendering|Material|CreateDynamicMaterialInstance _figures_5_4_cube_258 0 (Rendering|Material|GetMaterial _figures_5_4_cube_258 0) "opacity" :!class /Script/Engine.PrimitiveComponent))
          (Rendering|Material|SetScalarParameterValue _returnvalue_26 "opacity" 0.0 :!class /Script/Engine.MaterialInstanceDynamic))
        (:then_2
          (bind _returnvalue_27 (Rendering|Material|CreateDynamicMaterialInstance _figures_5_4_cube_246 0 (Rendering|Material|GetMaterial _figures_5_4_cube_246 0) "opacity" :!class /Script/Engine.PrimitiveComponent))
          (Rendering|Material|SetScalarParameterValue _returnvalue_27 "opacity" 0.0 :!class /Script/Engine.MaterialInstanceDynamic))
        (:then_3
          (bind _returnvalue_28 (Rendering|Material|CreateDynamicMaterialInstance _figures_5_4_cube_247 0 (Rendering|Material|GetMaterial _figures_5_4_cube_247 0) "opacity" :!class /Script/Engine.PrimitiveComponent))
          (Rendering|Material|SetScalarParameterValue _returnvalue_28 "opacity" 0.0 :!class /Script/Engine.MaterialInstanceDynamic))
        (:then_4
          (bind _returnvalue_29 (Rendering|Material|CreateDynamicMaterialInstance _figures_5_4_cube_248_2 0 (Rendering|Material|GetMaterial _figures_5_4_cube_248_2 0) "opacity" :!class /Script/Engine.PrimitiveComponent))
          (Rendering|Material|SetScalarParameterValue _returnvalue_29 "opacity" 0.0 :!class /Script/Engine.MaterialInstanceDynamic))
        (:then_5
          (bind _returnvalue_30 (Rendering|Material|CreateDynamicMaterialInstance _figures_5_4_cube_249_2 0 (Rendering|Material|GetMaterial _figures_5_4_cube_249_2 0) "opacity" :!class /Script/Engine.PrimitiveComponent))
          (Rendering|Material|SetScalarParameterValue _returnvalue_30 "opacity" 0.0 :!class /Script/Engine.MaterialInstanceDynamic))
        (:then_6
          (bind _returnvalue_31 (Rendering|Material|CreateDynamicMaterialInstance _figures_5_4_cube_038_2 0 (Rendering|Material|GetMaterial _figures_5_4_cube_038_2 0) "opacity" :!class /Script/Engine.PrimitiveComponent))
          (Rendering|Material|SetScalarParameterValue _returnvalue_31 "opacity" 0.0 :!class /Script/Engine.MaterialInstanceDynamic))
        (:then_7
          (bind _returnvalue_32 (Rendering|Material|CreateDynamicMaterialInstance _figures_5_4_cube_238_2 0 (Rendering|Material|GetMaterial _figures_5_4_cube_238_2 0) "opacity" :!class /Script/Engine.PrimitiveComponent))
          (Rendering|Material|SetScalarParameterValue _returnvalue_32 "opacity" 0.0 :!class /Script/Engine.MaterialInstanceDynamic))
        (:then_8
          (bind _returnvalue_33 (Rendering|Material|CreateDynamicMaterialInstance _figures_5_4_cube_239_2 0 (Rendering|Material|GetMaterial _figures_5_4_cube_239_2 0) "opacity" :!class /Script/Engine.PrimitiveComponent))
          (Rendering|Material|SetScalarParameterValue _returnvalue_33 "opacity" 0.0 :!class /Script/Engine.MaterialInstanceDynamic))
        (:then_9
          (bind _returnvalue_34 (Rendering|Material|CreateDynamicMaterialInstance _figures_5_4_cube_242_2 0 (Rendering|Material|GetMaterial _figures_5_4_cube_242_2 0) "opacity" :!class /Script/Engine.PrimitiveComponent))
          (Rendering|Material|SetScalarParameterValue _returnvalue_34 "opacity" 0.0 :!class /Script/Engine.MaterialInstanceDynamic))
        (:then_10
          (bind _returnvalue_35 (Rendering|Material|CreateDynamicMaterialInstance _figures_5_4_cube_240 0 (Rendering|Material|GetMaterial _figures_5_4_cube_240 0) "opacity" :!class /Script/Engine.PrimitiveComponent))
          (Rendering|Material|SetScalarParameterValue _returnvalue_35 "opacity" 0.0 :!class /Script/Engine.MaterialInstanceDynamic))
        (:then_11
          (bind _returnvalue_36 (Rendering|Material|CreateDynamicMaterialInstance _figures_5_4_cube_241 0 (Rendering|Material|GetMaterial _figures_5_4_cube_241 0) "opacity" :!class /Script/Engine.PrimitiveComponent))
          (Rendering|Material|SetScalarParameterValue _returnvalue_36 "opacity" 0.0 :!class /Script/Engine.MaterialInstanceDynamic))
        (:then_12
          (bind _returnvalue_37 (Rendering|Material|CreateDynamicMaterialInstance _figures_5_4_cube_244 0 (Rendering|Material|GetMaterial _figures_5_4_cube_244 0) "opacity" :!class /Script/Engine.PrimitiveComponent))
          (Rendering|Material|SetScalarParameterValue _returnvalue_37 "opacity" 0.0 :!class /Script/Engine.MaterialInstanceDynamic))
        (:then_13
          (bind _returnvalue_38 (Rendering|Material|CreateDynamicMaterialInstance _figures_5_4_cube_259 0 (Rendering|Material|GetMaterial _figures_5_4_cube_259 0) "opacity" :!class /Script/Engine.PrimitiveComponent))
          (Rendering|Material|SetScalarParameterValue _returnvalue_38 "opacity" 0.0 :!class /Script/Engine.MaterialInstanceDynamic))
        (:then_14
          (bind _returnvalue_39 (Rendering|Material|CreateDynamicMaterialInstance _figures_5_4_cube_257 0 (Rendering|Material|GetMaterial _figures_5_4_cube_257 0) "opacity" :!class /Script/Engine.PrimitiveComponent))
          (Rendering|Material|SetScalarParameterValue _returnvalue_39 "opacity" 0.0 :!class /Script/Engine.MaterialInstanceDynamic))
        (:then_15
          (bind _returnvalue_40 (Rendering|Material|CreateDynamicMaterialInstance _figures_5_4_cube_260 0 (Rendering|Material|GetMaterial _figures_5_4_cube_260 0) "opacity" :!class /Script/Engine.PrimitiveComponent))
          (Rendering|Material|SetScalarParameterValue _returnvalue_40 "opacity" 0.0 :!class /Script/Engine.MaterialInstanceDynamic))
        (:then_16
          (bind _returnvalue_41 (Rendering|Material|CreateDynamicMaterialInstance _figures_5_4_cube_261 0 (Rendering|Material|GetMaterial _figures_5_4_cube_261 0) "opacity" :!class /Script/Engine.PrimitiveComponent))
          (Rendering|Material|SetScalarParameterValue _returnvalue_41 "opacity" 0.0 :!class /Script/Engine.MaterialInstanceDynamic))
        (:then_17
          (bind _returnvalue_42 (Rendering|Material|CreateDynamicMaterialInstance _figures_5_4_cube_250 0 (Rendering|Material|GetMaterial _figures_5_4_cube_250 0) "opacity" :!class /Script/Engine.PrimitiveComponent))
          (Rendering|Material|SetScalarParameterValue _returnvalue_42 "opacity" 0.0 :!class /Script/Engine.MaterialInstanceDynamic))
        (:then_18
          (bind _returnvalue_43 (Rendering|Material|CreateDynamicMaterialInstance _figures_5_4_cube_256 0 (Rendering|Material|GetMaterial _figures_5_4_cube_256 0) "opacity" :!class /Script/Engine.PrimitiveComponent))
          (Rendering|Material|SetScalarParameterValue _returnvalue_43 "opacity" 0.0 :!class /Script/Engine.MaterialInstanceDynamic))
        (:then_19
          (bind _returnvalue_44 (Rendering|Material|CreateDynamicMaterialInstance _figures_5_4_cube_251 0 (Rendering|Material|GetMaterial _figures_5_4_cube_251 0) "opacity" :!class /Script/Engine.PrimitiveComponent))
          (Rendering|Material|SetScalarParameterValue _returnvalue_44 "opacity" 0.0 :!class /Script/Engine.MaterialInstanceDynamic))
        (:then_20
          (bind _returnvalue_45 (Rendering|Material|CreateDynamicMaterialInstance _figures_5_4_cube_252 0 (Rendering|Material|GetMaterial _figures_5_4_cube_252 0) "opacity" :!class /Script/Engine.PrimitiveComponent))
          (Rendering|Material|SetScalarParameterValue _returnvalue_45 "opacity" 0.0 :!class /Script/Engine.MaterialInstanceDynamic))
        (:then_21
          (bind _returnvalue_46 (Rendering|Material|CreateDynamicMaterialInstance _figures_5_4_cube_253 0 (Rendering|Material|GetMaterial _figures_5_4_cube_253 0) "opacity" :!class /Script/Engine.PrimitiveComponent))
          (Rendering|Material|SetScalarParameterValue _returnvalue_46 "opacity" 0.0 :!class /Script/Engine.MaterialInstanceDynamic))
        (:then_22
          (bind _returnvalue_47 (Rendering|Material|CreateDynamicMaterialInstance _figures_5_4_cube_254 0 (Rendering|Material|GetMaterial _figures_5_4_cube_254 0) "opacity" :!class /Script/Engine.PrimitiveComponent))
          (Rendering|Material|SetScalarParameterValue _returnvalue_47 "opacity" 0.0 :!class /Script/Engine.MaterialInstanceDynamic))
        (:then_23
          (bind _returnvalue_48 (Rendering|Material|CreateDynamicMaterialInstance _figures_5_4_cube_255 0 (Rendering|Material|GetMaterial _figures_5_4_cube_255 0) "opacity" :!class /Script/Engine.PrimitiveComponent))
          (Rendering|Material|SetScalarParameterValue _returnvalue_48 "opacity" 0.0 :!class /Script/Engine.MaterialInstanceDynamic))))))