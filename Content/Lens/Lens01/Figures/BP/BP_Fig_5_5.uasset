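; Selectable figure actor for round 5 of the Lens01 game, chosen by attaching it through its anchor connector component.
; Attaching sets Selected and, after a two-second delay, asks BP_GameManager_01 to validate it if still attached; detaching clears Selected.
; SelectedOverlayColor toggles an opacity overlay on its cube meshes via dynamic materials, but it and the older press-to-select, sibling-deselect logic are no longer wired up.
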(event PressedSelect(Comp_Select)
  (params (Pawn :type BP%20Pawn%20Base%20Object%20Reference) (SourceActor :type Actor%20Object%20Reference) (ImpactLocation :type Vector :default "0, 0, 0") (ImpactComponent :type Actor%20Component%20Object%20Reference))
  ;[1 1 1] old
)

(event ConnectorAttached(Comp_Connector_Anchor)
  (params (Connector :type Comp%20Connector%20Object%20Reference) (AttachedToActor :type Actor%20Object%20Reference) (AttachedToComponent :type Scene%20Component%20Object%20Reference))
  ;[1 1 1] if it is ready to validate selection
  (Variables|Default|Setselected true)
  (bind _returnvalue (Actor|GetActorOfClass "/Game/Lens/Lens01/BP/BP_GameManager_01.BP_GameManager_01_C"))
  (Utilities|FlowControl|Delay 2.0)
  (if (Variables|Default|Getselected)
    (Default|ValidateSelection _returnvalue self 5)))

(event ConnectorDetached(Comp_Connector_Anchor)
  ;[1 1 1] if it is ready to validate selection
  (Variables|Default|Setselected false))

(fn ConstructionScript)

(fn SelectedOverlayColor
  (params (select :type Boolean))
  (bind _figures_5_5_cube_315 (Variables|Default|Getfigures_5_5_Cube_315))
  (bind _figures_5_5_cube_317 (Variables|Default|Getfigures_5_5_Cube_317))
  (bind _figures_5_5_cube_314 (Variables|Default|Getfigures_5_5_Cube_314))
  (bind _figures_5_5_cube_328 (Variables|Default|Getfigures_5_5_Cube_328))
  (bind _figures_5_5_cube_322 (Variables|Default|Getfigures_5_5_Cube_322))
  (bind _figures_5_5_cube_330 (Variables|Default|Getfigures_5_5_Cube_330))
  (bind _figures_5_5_cube_331 (Variables|Default|Getfigures_5_5_Cube_331))
  (bind _figures_5_5_cube_332 (Variables|Default|Getfigures_5_5_Cube_332))
  (bind _figures_5_5_cube_333 (Variables|Default|Getfigures_5_5_Cube_333))
  (bind _figures_5_5_cube_329 (Variables|Default|Getfigures_5_5_Cube_329))
  (bind _figures_5_5_cube_323 (Variables|Default|Getfigures_5_5_Cube_323))
  (bind _figures_5_5_cube_324 (Variables|Default|Getfigures_5_5_Cube_324))
  (bind _figures_5_5_cube_318 (Variables|Default|Getfigures_5_5_Cube_318))
  (bind _figures_5_5_cube_325 (Variables|Default|Getfigures_5_5_Cube_325))
  (bind _figures_5_5_cube_326 (Variables|Default|Getfigures_5_5_Cube_326))
  (bind _figures_5_5_cube_327 (Variables|Default|Getfigures_5_5_Cube_327))
  (bind _figures_5_5_cube_315_2 (Variables|Default|Getfigures_5_5_Cube_315))
  (bind _figures_5_5_cube_317_2 (Variables|Default|Getfigures_5_5_Cube_317))
  (bind _figures_5_5_cube_318_2 (Variables|Default|Getfigures_5_5_Cube_318))
  (bind _figures_5_5_cube_319 (Variables|Default|Getfigures_5_5_Cube_319))
  (bind _figures_5_5_cube_320 (Variables|Default|Getfigures_5_5_Cube_320))
  (bind _figures_5_5_cube_321 (Variables|Default|Getfigures_5_5_Cube_321))
  (bind _figures_5_5_cube_311 (Variables|Default|Getfigures_5_5_Cube_311))
  (bind _figures_5_5_cube_319_2 (Variables|Default|Getfigures_5_5_Cube_319))
  (bind _figures_5_5_cube_312 (Variables|Default|Getfigures_5_5_Cube_312))
  (bind _figures_5_5_cube_313 (Variables|Default|Getfigures_5_5_Cube_313))
  (bind _figures_5_5_cube_316 (Variables|Default|Getfigures_5_5_Cube_316))
  (bind _figures_5_5_cube_314_2 (Variables|Default|Getfigures_5_5_Cube_314))
  (bind _figures_5_5_cube_328_2 (Variables|Default|Getfigures_5_5_Cube_328))
  (bind _figures_5_5_cube_322_2 (Variables|Default|Getfigures_5_5_Cube_322))
  (bind _figures_5_5_cube_330_2 (Variables|Default|Getfigures_5_5_Cube_330))
  (bind _figures_5_5_cube_331_2 (Variables|Default|Getfigures_5_5_Cube_331))
  (bind _figures_5_5_cube_332_2 (Variables|Default|Getfigures_5_5_Cube_332))
  (bind _figures_5_5_cube_333_2 (Variables|Default|Getfigures_5_5_Cube_333))
  (bind _figures_5_5_cube_320_2 (Variables|Default|Getfigures_5_5_Cube_320))
  (bind _figures_5_5_cube_329_2 (Variables|Default|Getfigures_5_5_Cube_329))
  (bind _figures_5_5_cube_323_2 (Variables|Default|Getfigures_5_5_Cube_323))
  (bind _figures_5_5_cube_324_2 (Variables|Default|Getfigures_5_5_Cube_324))
  (bind _figures_5_5_cube_325_2 (Variables|Default|Getfigures_5_5_Cube_325))
  (bind _figures_5_5_cube_326_2 (Variables|Default|Getfigures_5_5_Cube_326))
  (bind _figures_5_5_cube_327_2 (Variables|Default|Getfigures_5_5_Cube_327))
  (bind _figures_5_5_cube_321_2 (Variables|Default|Getfigures_5_5_Cube_321))
  (bind _figures_5_5_cube_311_2 (Variables|Default|Getfigures_5_5_Cube_311))
  (bind _figures_5_5_cube_312_2 (Variables|Default|Getfigures_5_5_Cube_312))
  (bind _figures_5_5_cube_313_2 (Variables|Default|Getfigures_5_5_Cube_313))
  (bind _figures_5_5_cube_316_2 (Variables|Default|Getfigures_5_5_Cube_316))
  (if select
    (Utilities|FlowControl|Sequence
      (:then_0
        (bind _returnvalue (Rendering|Material|CreateDynamicMaterialInstance _figures_5_5_cube_321 0 (Rendering|Material|GetMaterial _figures_5_5_cube_321 0) "opacity" :!class /Script/Engine.PrimitiveComponent))
        (Rendering|Material|SetScalarParameterValue _returnvalue "opacity" 0.25 :!class /Script/Engine.MaterialInstanceDynamic))
      (:then_1
        (bind _returnvalue_2 (Rendering|Material|CreateDynamicMaterialInstance _figures_5_5_cube_315_2 0 (Rendering|Material|GetMaterial _figures_5_5_cube_315_2 0) "opacity" :!class /Script/Engine.PrimitiveComponent))
        (Rendering|Material|SetScalarParameterValue _returnvalue_2 "opacity" 0.25 :!class /Script/Engine.MaterialInstanceDynamic))
      (:then_2
        (bind _returnvalue_3 (Rendering|Material|CreateDynamicMaterialInstance _figures_5_5_cube_317_2 0 (Rendering|Material|GetMaterial _figures_5_5_cube_317_2 0) "opacity" :!class /Script/Engine.PrimitiveComponent))
        (Rendering|Material|SetScalarParameterValue _returnvalue_3 "opacity" 0.25 :!class /Script/Engine.MaterialInstanceDynamic))
      (:then_3
        (bind _returnvalue_4 (Rendering|Material|CreateDynamicMaterialInstance _figures_5_5_cube_318_2 0 (Rendering|Material|GetMaterial _figures_5_5_cube_318_2 0) "opacity" :!class /Script/Engine.PrimitiveComponent))
        (Rendering|Material|SetScalarParameterValue _returnvalue_4 "opacity" 0.25 :!class /Script/Engine.MaterialInstanceDynamic))
      (:then_4
        (bind _returnvalue_5 (Rendering|Material|CreateDynamicMaterialInstance _figures_5_5_cube_319 0 (Rendering|Material|GetMaterial _figures_5_5_cube_319 0) "opacity" :!class /Script/Engine.PrimitiveComponent))
        (Rendering|Material|SetScalarParameterValue _returnvalue_5 "opacity" 0.25 :!class /Script/Engine.MaterialInstanceDynamic))
      (:then_5
        (bind _returnvalue_6 (Rendering|Material|CreateDynamicMaterialInstance _figures_5_5_cube_320 0 (Rendering|Material|GetMaterial _figures_5_5_cube_320 0) "opacity" :!class /Script/Engine.PrimitiveComponent))
        (Rendering|Material|SetScalarParameterValue _returnvalue_6 "opacity" 0.25 :!class /Script/Engine.MaterialInstanceDynamic))
      (:then_6
        (bind _returnvalue_7 (Rendering|Material|CreateDynamicMaterialInstance _figures_5_5_cube_322_2 0 (Rendering|Material|GetMaterial _figures_5_5_cube_322_2 0) "opacity" :!class /Script/Engine.PrimitiveComponent))
        (Rendering|Material|SetScalarParameterValue _returnvalue_7 "opacity" 0.25 :!class /Script/Engine.MaterialInstanceDynamic))
      (:then_7
        (bind _returnvalue_8 (Rendering|Material|CreateDynamicMaterialInstance _figures_5_5_cube_330_2 0 (Rendering|Material|GetMaterial _figures_5_5_cube_330_2 0) "opacity" :!class /Script/Engine.PrimitiveComponent))
        (Rendering|Material|SetScalarParameterValue _returnvalue_8 "opacity" 0.25 :!class /Script/Engine.MaterialInstanceDynamic))
      (:then_8
        (bind _returnvalue_9 (Rendering|Material|CreateDynamicMaterialInstance _figures_5_5_cube_331_2 0 (Rendering|Material|GetMaterial _figures_5_5_cube_331_2 0) "opacity" :!class /Script/Engine.PrimitiveComponent))
        (Rendering|Material|SetScalarParameterValue _returnvalue_9 "opacity" 0.25 :!class /Script/Engine.MaterialInstanceDynamic))
      (:then_9
        (bind _returnvalue_10 (Rendering|Material|CreateDynamicMaterialInstance _figures_5_5_cube_332_2 0 (Rendering|Material|GetMaterial _figures_5_5_cube_332_2 0) "opacity" :!class /Script/Engine.PrimitiveComponent))
        (Rendering|Material|SetScalarParameterValue _returnvalue_10 "opacity" 0.25 :!class /Script/Engine.MaterialInstanceDynamic))
      (:then_10
        (bind _returnvalue_11 (Rendering|Material|CreateDynamicMaterialInstance _figures_5_5_cube_333_2 0 (Rendering|Material|GetMaterial _figures_5_5_cube_333_2 0) "opacity" :!class /Script/Engine.PrimitiveComponent))
        (Rendering|Material|SetScalarParameterValue _returnvalue_11 "opacity" 0.25 :!class /Script/Engine.MaterialInstanceDynamic))
      (:then_11
        (bind _returnvalue_12 (Rendering|Material|CreateDynamicMaterialInstance _figures_5_5_cube_327_2 0 (Rendering|Material|GetMaterial _figures_5_5_cube_327_2 0) "opacity" :!class /Script/Engine.PrimitiveComponent))
        (Rendering|Material|SetScalarParameterValue _returnvalue_12 "opacity" 0.25 :!class /Script/Engine.MaterialInstanceDynamic))
      (:then_12
        (bind _returnvalue_13 (Rendering|Material|CreateDynamicMaterialInstance _figures_5_5_cube_311 0 (Rendering|Material|GetMaterial _figures_5_5_cube_311 0) "opacity" :!class /Script/Engine.PrimitiveComponent))
        (Rendering|Material|SetScalarParameterValue _returnvalue_13 "opacity" 0.25 :!class /Script/Engine.MaterialInstanceDynamic))
      (:then_13
        (bind _returnvalue_14 (Rendering|Material|CreateDynamicMaterialInstance _figures_5_5_cube_312 0 (Rendering|Material|GetMaterial _figures_5_5_cube_312 0) "opacity" :!class /Script/Engine.PrimitiveComponent))
        (Rendering|Material|SetScalarParameterValue _returnvalue_14 "opacity" 0.25 :!class /Script/Engine.MaterialInstanceDynamic))
      (:then_14
        (bind _returnvalue_15 (Rendering|Material|CreateDynamicMaterialInstance _figures_5_5_cube_313 0 (Rendering|Material|GetMaterial _figures_5_5_cube_313 0) "opacity" :!class /Script/Engine.PrimitiveComponent))
        (Rendering|Material|SetScalarParameterValue _returnvalue_15 "opacity" 0.25 :!class /Script/Engine.MaterialInstanceDynamic))
      (:then_15
        (bind _returnvalue_16 (Rendering|Material|CreateDynamicMaterialInstance _figures_5_5_cube_316 0 (Rendering|Material|GetMaterial _figures_5_5_cube_316 0) "opacity" :!class /Script/Engine.PrimitiveComponent))
        (Rendering|Material|SetScalarParameterValue _returnvalue_16 "opacity" 0.25 :!class /Script/Engine.MaterialInstanceDynamic))
      (:then_16
        (bind _returnvalue_17 (Rendering|Material|CreateDynamicMaterialInstance _figures_5_5_cube_314_2 0 (Rendering|Material|GetMaterial _figures_5_5_cube_314_2 0) "opacity" :!class /Script/Engine.PrimitiveComponent))
        (Rendering|Material|SetScalarParameterValue _returnvalue_17 "opacity" 0.25 :!class /Script/Engine.MaterialInstanceDynamic))
      (:then_17
        (bind _returnvalue_18 (Rendering|Material|CreateDynamicMaterialInstance _figures_5_5_cube_328_2 0 (Rendering|Material|GetMaterial _figures_5_5_cube_328_2 0) "opacity" :!class /Script/Engine.PrimitiveComponent))
        (Rendering|Material|SetScalarParameterValue _returnvalue_18 "opacity" 0.25 :!class /Script/Engine.MaterialInstanceDynamic))
      (:then_18
        (bind _returnvalue_19 (Rendering|Material|CreateDynamicMaterialInstance _figures_5_5_cube_329_2 0 (Rendering|Material|GetMaterial _figures_5_5_cube_329_2 0) "opacity" :!class /Script/Engine.PrimitiveComponent))
        (Rendering|Material|SetScalarParameterValue _returnvalue_19 "opacity" 0.25 :!class /Script/Engine.MaterialInstanceDynamic))
      (:then_19
        (bind _returnvalue_20 (Rendering|Material|CreateDynamicMaterialInstance _figures_5_5_cube_323_2 0 (Rendering|Material|GetMaterial _figures_5_5_cube_323_2 0) "opacity" :!class /Script/Engine.PrimitiveComponent))
        (Rendering|Material|SetScalarParameterValue _returnvalue_20 "opacity" 0.25 :!class /Script/Engine.MaterialInstanceDynamic))
      (:then_20
        (bind _returnvalue_21 (Rendering|Material|CreateDynamicMaterialInstance _figures_5_5_cube_324_2 0 (Rendering|Material|GetMaterial _figures_5_5_cube_324_2 0) "opacity" :!class /Script/Engine.PrimitiveComponent))
        (Rendering|Material|SetScalarParameterValue _returnvalue_21 "opacity" 0.25 :!class /Script/Engine.MaterialInstanceDynamic))
      (:then_21
        (bind _returnvalue_22 (Rendering|Material|CreateDynamicMaterialInstance _figures_5_5_cube_325_2 0 (Rendering|Material|GetMaterial _figures_5_5_cube_325_2 0) "opacity" :!class /Script/Engine.PrimitiveComponent))
        (Rendering|Material|SetScalarParameterValue _returnvalue_22 "opacity" 0.25 :!class /Script/Engine.MaterialInstanceDynamic))
      (:then_22
        (bind _returnvalue_23 (Rendering|Material|CreateDynamicMaterialInstance _figures_5_5_cube_326_2 0 (Rendering|Material|GetMaterial _figures_5_5_cube_326_2 0) "opacity" :!class /Script/Engine.PrimitiveComponent))
        (Rendering|Material|SetScalarParameterValue _returnvalue_23 "opacity" 0.25 :!class /Script/Engine.MaterialInstanceDynamic)))
    (else
      (Utilities|FlowControl|Sequence
        (:then_0
          (bind _returnvalue_24 (Rendering|Material|CreateDynamicMaterialInstance _figures_5_5_cube_321_2 0 (Rendering|Material|GetMaterial _figures_5_5_cube_321_2 0) "opacity" :!class /Script/Engine.PrimitiveComponent))
          (Rendering|Material|SetScalarParameterValue _returnvalue_24 "opacity" 0.0 :!class /Script/Engine.MaterialInstanceDynamic))
        (:then_1
          (bind _returnvalue_25 (Rendering|Material|CreateDynamicMaterialInstance _figures_5_5_cube_315 0 (Rendering|Material|GetMaterial _figures_5_5_cube_315 0) "opacity" :!class /Script/Engine.PrimitiveComponent))
          (Rendering|Material|SetScalarParameterValue _returnvalue_25 "opacity" 0.0 :!class /Script/Engine.MaterialInstanceDynamic))
        (:then_2
          (bind _returnvalue_26 (Rendering|Material|CreateDynamicMaterialInstance _figures_5_5_cube_317 0 (Rendering|Material|GetMaterial _figures_5_5_cube_317 0) "opacity" :!class /Script/Engine.PrimitiveComponent))
          (Rendering|Material|SetScalarParameterValue _returnvalue_26 "opacity" 0.0 :!class /Script/Engine.MaterialInstanceDynamic))
        (:then_3
          (bind _returnvalue_27 (Rendering|Material|CreateDynamicMaterialInstance _figures_5_5_cube_318 0 (Rendering|Material|GetMaterial _figures_5_5_cube_318 0) "opacity" :!class /Script/Engine.PrimitiveComponent))
          (Rendering|Material|SetScalarParameterValue _returnvalue_27 "opacity" 0.0 :!class /Script/Engine.MaterialInstanceDynamic))
        (:then_4
          (bind _returnvalue_28 (Rendering|Material|CreateDynamicMaterialInstance _figures_5_5_cube_319_2 0 (Rendering|Material|GetMaterial _figures_5_5_cube_319_2 0) "opacity" :!class /Script/Engine.PrimitiveComponent))
          (Rendering|Material|SetScalarParameterValue _returnvalue_28 "opacity" 0.0 :!class /Script/Engine.MaterialInstanceDynamic))
        (:then_5
          (bind _returnvalue_29 (Rendering|Material|CreateDynamicMaterialInstance _figures_5_5_cube_320_2 0 (Rendering|Material|GetMaterial _figures_5_5_cube_320_2 0) "opacity" :!class /Script/Engine.PrimitiveComponent))
          (Rendering|Material|SetScalarParameterValue _returnvalue_29 "opacity" 0.0 :!class /Script/Engine.MaterialInstanceDynamic))
        (:then_6
          (bind _returnvalue_30 (Rendering|Material|CreateDynamicMaterialInstance _figures_5_5_cube_322 0 (Rendering|Material|GetMaterial _figures_5_5_cube_322 0) "opacity" :!class /Script/Engine.PrimitiveComponent))
          (Rendering|Material|SetScalarParameterValue _returnvalue_30 "opacity" 0.0 :!class /Script/Engine.MaterialInstanceDynamic))
        (:then_7
          (bind _returnvalue_31 (Rendering|Material|CreateDynamicMaterialInstance _figures_5_5_cube_330 0 (Rendering|Material|GetMaterial _figures_5_5_cube_330 0) "opacity" :!class /Script/Engine.PrimitiveComponent))
          (Rendering|Material|SetScalarParameterValue _returnvalue_31 "opacity" 0.0 :!class /Script/Engine.MaterialInstanceDynamic))
        (:then_8
          (bind _returnvalue_32 (Rendering|Material|CreateDynamicMaterialInstance _figures_5_5_cube_331 0 (Rendering|Material|GetMaterial _figures_5_5_cube_331 0) "opacity" :!class /Script/Engine.PrimitiveComponent))
          (Rendering|Material|SetScalarParameterValue _returnvalue_32 "opacity" 0.0 :!class /Script/Engine.MaterialInstanceDynamic))
        (:then_9
          (bind _returnvalue_33 (Rendering|Material|CreateDynamicMaterialInstance _figures_5_5_cube_332 0 (Rendering|Material|GetMaterial _figures_5_5_cube_332 0) "opacity" :!class /Script/Engine.PrimitiveComponent))
          (Rendering|Material|SetScalarParameterValue _returnvalue_33 "opacity" 0.0 :!class /Script/Engine.MaterialInstanceDynamic))
        (:then_10
          (bind _returnvalue_34 (Rendering|Material|CreateDynamicMaterialInstance _figures_5_5_cube_333 0 (Rendering|Material|GetMaterial _figures_5_5_cube_333 0) "opacity" :!class /Script/Engine.PrimitiveComponent))
          (Rendering|Material|SetScalarParameterValue _returnvalue_34 "opacity" 0.0 :!class /Script/Engine.MaterialInstanceDynamic))
        (:then_11
          (bind _returnvalue_35 (Rendering|Material|CreateDynamicMaterialInstance _figures_5_5_cube_327 0 (Rendering|Material|GetMaterial _figures_5_5_cube_327 0) "opacity" :!class /Script/Engine.PrimitiveComponent))
          (Rendering|Material|SetScalarParameterValue _returnvalue_35 "opacity" 0.0 :!class /Script/Engine.MaterialInstanceDynamic))
        (:then_12
          (bind _returnvalue_36 (Rendering|Material|CreateDynamicMaterialInstance _figures_5_5_cube_311_2 0 (Rendering|Material|GetMaterial _figures_5_5_cube_311_2 0) "opacity" :!class /Script/Engine.PrimitiveComponent))
          (Rendering|Material|SetScalarParameterValue _returnvalue_36 "opacity" 0.0 :!class /Script/Engine.MaterialInstanceDynamic))
        (:then_13
          (bind _returnvalue_37 (Rendering|Material|CreateDynamicMaterialInstance _figures_5_5_cube_312_2 0 (Rendering|Material|GetMaterial _figures_5_5_cube_312_2 0) "opacity" :!class /Script/Engine.PrimitiveComponent))
          (Rendering|Material|SetScalarParameterValue _returnvalue_37 "opacity" 0.0 :!class /Script/Engine.MaterialInstanceDynamic))
        (:then_14
          (bind _returnvalue_38 (Rendering|Material|CreateDynamicMaterialInstance _figures_5_5_cube_313_2 0 (Rendering|Material|GetMaterial _figures_5_5_cube_313_2 0) "opacity" :!class /Script/Engine.PrimitiveComponent))
          (Rendering|Material|SetScalarParameterValue _returnvalue_38 "opacity" 0.0 :!class /Script/Engine.MaterialInstanceDynamic))
        (:then_15
          (bind _returnvalue_39 (Rendering|Material|CreateDynamicMaterialInstance _figures_5_5_cube_316_2 0 (Rendering|Material|GetMaterial _figures_5_5_cube_316_2 0) "opacity" :!class /Script/Engine.PrimitiveComponent))
          (Rendering|Material|SetScalarParameterValue _returnvalue_39 "opacity" 0.0 :!class /Script/Engine.MaterialInstanceDynamic))
        (:then_16
          (bind _returnvalue_40 (Rendering|Material|CreateDynamicMaterialInstance _figures_5_5_cube_314 0 (Rendering|Material|GetMaterial _figures_5_5_cube_314 0) "opacity" :!class /Script/Engine.PrimitiveComponent))
          (Rendering|Material|SetScalarParameterValue _returnvalue_40 "opacity" 0.0 :!class /Script/Engine.MaterialInstanceDynamic))
        (:then_17
          (bind _returnvalue_41 (Rendering|Material|CreateDynamicMaterialInstance _figures_5_5_cube_328 0 (Rendering|Material|GetMaterial _figures_5_5_cube_328 0) "opacity" :!class /Script/Engine.PrimitiveComponent))
          (Rendering|Material|SetScalarParameterValue _returnvalue_41 "opacity" 0.0 :!class /Script/Engine.MaterialInstanceDynamic))
        (:then_18
          (bind _returnvalue_42 (Rendering|Material|CreateDynamicMaterialInstance _figures_5_5_cube_329 0 (Rendering|Material|GetMaterial _figures_5_5_cube_329 0) "opacity" :!class /Script/Engine.PrimitiveComponent))
          (Rendering|Material|SetScalarParameterValue _returnvalue_42 "opacity" 0.0 :!class /Script/Engine.MaterialInstanceDynamic))
        (:then_19
          (bind _returnvalue_43 (Rendering|Material|CreateDynamicMaterialInstance _figures_5_5_cube_323 0 (Rendering|Material|GetMaterial _figures_5_5_cube_323 0) "opacity" :!class /Script/Engine.PrimitiveComponent))
          (Rendering|Material|SetScalarParameterValue _returnvalue_43 "opacity" 0.0 :!class /Script/Engine.MaterialInstanceDynamic))
        (:then_20
          (bind _returnvalue_44 (Rendering|Material|CreateDynamicMaterialInstance _figures_5_5_cube_324 0 (Rendering|Material|GetMaterial _figures_5_5_cube_324 0) "opacity" :!class /Script/Engine.PrimitiveComponent))
          (Rendering|Material|SetScalarParameterValue _returnvalue_44 "opacity" 0.0 :!class /Script/Engine.MaterialInstanceDynamic))
        (:then_21
          (bind _returnvalue_45 (Rendering|Material|CreateDynamicMaterialInstance _figures_5_5_cube_325 0 (Rendering|Material|GetMaterial _figures_5_5_cube_325 0) "opacity" :!class /Script/Engine.PrimitiveComponent))
          (Rendering|Material|SetScalarParameterValue _returnvalue_45 "opacity" 0.0 :!class /Script/Engine.MaterialInstanceDynamic))
        (:then_22
          (bind _returnvalue_46 (Rendering|Material|CreateDynamicMaterialInstance _figures_5_5_cube_326 0 (Rendering|Material|GetMaterial _figures_5_5_cube_326 0) "opacity" :!class /Script/Engine.PrimitiveComponent))
          (Rendering|Material|SetScalarParameterValue _returnvalue_46 "opacity" 0.0 :!class /Script/Engine.MaterialInstanceDynamic))))))