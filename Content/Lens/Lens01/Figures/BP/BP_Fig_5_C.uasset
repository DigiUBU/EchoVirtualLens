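; BP_Fig_5_C is a selectable figure in Lens01 that submits itself as a round 5 choice when its anchor connector attaches.
; Attaching sets Selected, waits two seconds, then calls ValidateSelection on BP_GameManager_01 if still selected; detaching clears the flag.
; SelectedOverlayColor toggles overlay opacity across the cube meshes through new dynamic materials, but only disconnected nodes call it.
; Older press-to-select logic, including deselecting sibling figures, is also disconnected.
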(event PressedSelect(Comp_Select)
  (params (Pawn :type BP%20Pawn%20Base%20Object%20Reference) (SourceActor :type Actor%20Object%20Reference) (ImpactLocation :type Vector :default "0, 0, 0") (ImpactComponent :type Actor%20Component%20Object%20Reference))
  ;[1 1 1] old
)

(event ConnectorAttached(Comp_Connector_Anchor)
  (params (Connector :type Comp%20Connector%20Object%20Reference) (AttachedToActor :type Actor%20Object%20Reference) (AttachedToComponent :type Scene%20Component%20Object%20Reference))
  ;[1 1 1] if it is ready to validate selection
  (Variables|Default|Setselected true)
  (bind _returnvalue (Actor|GetActorOfClass "/Game/Lens/Lens01/BP/BP_GameManager_01.BP_GameManager_01_C"))
  (Utilities|FlowControl|Delay 2.0)
  (if (Variables|Default|Getselected)
    (Default|ValidateSelection _returnvalue self 5)))

(event ConnectorDetached(Comp_Connector_Anchor)
  ;[1 1 1] if it is ready to validate selection
  (Variables|Default|Setselected false))

(event EventBeginPlay
  ;[1 1 1] old
)

(fn ConstructionScript)

(fn SelectedOverlayColor
  (params (selected :type Boolean))
  (bind _figures_5_c_cube_282 (Variables|Default|Getfigures_5_C_Cube_282))
  (bind _figures_5_c_cube_270 (Variables|Default|Getfigures_5_C_Cube_270))
  (bind _figures_5_c_cube_265 (Variables|Default|Getfigures_5_C_Cube_265))
  (bind _figures_5_c_cube_266 (Variables|Default|Getfigures_5_C_Cube_266))
  (bind _figures_5_c_cube_269 (Variables|Default|Getfigures_5_C_Cube_269))
  (bind _figures_5_c_cube_283 (Variables|Default|Getfigures_5_C_Cube_283))
  (bind _figures_5_c_cube_281 (Variables|Default|Getfigures_5_C_Cube_281))
  (bind _figures_5_c_cube_284 (Variables|Default|Getfigures_5_C_Cube_284))
  (bind _figures_5_c_cube_285 (Variables|Default|Getfigures_5_C_Cube_285))
  (bind _figures_5_c_cube_274 (Variables|Default|Getfigures_5_C_Cube_274))
  (bind _figures_5_c_cube_280 (Variables|Default|Getfigures_5_C_Cube_280))
  (bind _figures_5_c_cube_275 (Variables|Default|Getfigures_5_C_Cube_275))
  (bind _figures_5_c_cube_271 (Variables|Default|Getfigures_5_C_Cube_271))
  (bind _figures_5_c_cube_276 (Variables|Default|Getfigures_5_C_Cube_276))
  (bind _figures_5_c_cube_277 (Variables|Default|Getfigures_5_C_Cube_277))
  (bind _figures_5_c_cube_278 (Variables|Default|Getfigures_5_C_Cube_278))
  (bind _figures_5_c_cube_279 (Variables|Default|Getfigures_5_C_Cube_279))
  (bind _figures_5_c_cube_282_2 (Variables|Default|Getfigures_5_C_Cube_282))
  (bind _figures_5_c_cube_270_2 (Variables|Default|Getfigures_5_C_Cube_270))
  (bind _figures_5_c_cube_271_2 (Variables|Default|Getfigures_5_C_Cube_271))
  (bind _figures_5_c_cube_272 (Variables|Default|Getfigures_5_C_Cube_272))
  (bind _figures_5_c_cube_273 (Variables|Default|Getfigures_5_C_Cube_273))
  (bind _figures_5_c_cube_268 (Variables|Default|Getfigures_5_C_Cube_268))
  (bind _figures_5_c_cube_272_2 (Variables|Default|Getfigures_5_C_Cube_272))
  (bind _figures_5_c_cube_262 (Variables|Default|Getfigures_5_C_Cube_262))
  (bind _figures_5_c_cube_263 (Variables|Default|Getfigures_5_C_Cube_263))
  (bind _figures_5_c_cube_264 (Variables|Default|Getfigures_5_C_Cube_264))
  (bind _figures_5_c_cube_267 (Variables|Default|Getfigures_5_C_Cube_267))
  (bind _figures_5_c_cube_265_2 (Variables|Default|Getfigures_5_C_Cube_265))
  (bind _figures_5_c_cube_266_2 (Variables|Default|Getfigures_5_C_Cube_266))
  (bind _figures_5_c_cube_269_2 (Variables|Default|Getfigures_5_C_Cube_269))
  (bind _figures_5_c_cube_283_2 (Variables|Default|Getfigures_5_C_Cube_283))
  (bind _figures_5_c_cube_281_2 (Variables|Default|Getfigures_5_C_Cube_281))
  (bind _figures_5_c_cube_284_2 (Variables|Default|Getfigures_5_C_Cube_284))
  (bind _figures_5_c_cube_273_2 (Variables|Default|Getfigures_5_C_Cube_273))
  (bind _figures_5_c_cube_285_2 (Variables|Default|Getfigures_5_C_Cube_285))
  (bind _figures_5_c_cube_274_2 (Variables|Default|Getfigures_5_C_Cube_274))
  (bind _figures_5_c_cube_280_2 (Variables|Default|Getfigures_5_C_Cube_280))
  (bind _figures_5_c_cube_275_2 (Variables|Default|Getfigures_5_C_Cube_275))
  (bind _figures_5_c_cube_276_2 (Variables|Default|Getfigures_5_C_Cube_276))
  (bind _figures_5_c_cube_277_2 (Variables|Default|Getfigures_5_C_Cube_277))
  (bind _figures_5_c_cube_278_2 (Variables|Default|Getfigures_5_C_Cube_278))
  (bind _figures_5_c_cube_279_2 (Variables|Default|Getfigures_5_C_Cube_279))
  (bind _figures_5_c_cube_268_2 (Variables|Default|Getfigures_5_C_Cube_268))
  (bind _figures_5_c_cube_262_2 (Variables|Default|Getfigures_5_C_Cube_262))
  (bind _figures_5_c_cube_263_2 (Variables|Default|Getfigures_5_C_Cube_263))
  (bind _figures_5_c_cube_264_2 (Variables|Default|Getfigures_5_C_Cube_264))
  (bind _figures_5_c_cube_267_2 (Variables|Default|Getfigures_5_C_Cube_267))
  (if selected
    (Utilities|FlowControl|Sequence
      (:then_0
        (bind _returnvalue (Rendering|Material|CreateDynamicMaterialInstance _figures_5_c_cube_268 0 (Rendering|Material|GetMaterial _figures_5_c_cube_268 0) "opacity" :!class /Script/Engine.PrimitiveComponent))
        (Rendering|Material|SetScalarParameterValue _returnvalue "opacity" 0.25 :!class /Script/Engine.MaterialInstanceDynamic))
      (:then_1
        (bind _returnvalue_2 (Rendering|Material|CreateDynamicMaterialInstance _figures_5_c_cube_282_2 0 (Rendering|Material|GetMaterial _figures_5_c_cube_282_2 0) "opacity" :!class /Script/Engine.PrimitiveComponent))
        (Rendering|Material|SetScalarParameterValue _returnvalue_2 "opacity" 0.25 :!class /Script/Engine.MaterialInstanceDynamic))
      (:then_2
        (bind _returnvalue_3 (Rendering|Material|CreateDynamicMaterialInstance _figures_5_c_cube_270_2 0 (Rendering|Material|GetMaterial _figures_5_c_cube_270_2 0) "opacity" :!class /Script/Engine.PrimitiveComponent))
        (Rendering|Material|SetScalarParameterValue _returnvalue_3 "opacity" 0.25 :!class /Script/Engine.MaterialInstanceDynamic))
      (:then_3
        (bind _returnvalue_4 (Rendering|Material|CreateDynamicMaterialInstance _figures_5_c_cube_271_2 0 (Rendering|Material|GetMaterial _figures_5_c_cube_271_2 0) "opacity" :!class /Script/Engine.PrimitiveComponent))
        (Rendering|Material|SetScalarParameterValue _returnvalue_4 "opacity" 0.25 :!class /Script/Engine.MaterialInstanceDynamic))
      (:then_4
        (bind _returnvalue_5 (Rendering|Material|CreateDynamicMaterialInstance _figures_5_c_cube_272 0 (Rendering|Material|GetMaterial _figures_5_c_cube_272 0) "opacity" :!class /Script/Engine.PrimitiveComponent))
        (Rendering|Material|SetScalarParameterValue _returnvalue_5 "opacity" 0.25 :!class /Script/Engine.MaterialInstanceDynamic))
      (:then_5
        (bind _returnvalue_6 (Rendering|Material|CreateDynamicMaterialInstance _figures_5_c_cube_273 0 (Rendering|Material|GetMaterial _figures_5_c_cube_273 0) "opacity" :!class /Script/Engine.PrimitiveComponent))
        (Rendering|Material|SetScalarParameterValue _returnvalue_6 "opacity" 0.25 :!class /Script/Engine.MaterialInstanceDynamic))
      (:then_6
        (bind _returnvalue_7 (Rendering|Material|CreateDynamicMaterialInstance _figures_5_c_cube_262 0 (Rendering|Material|GetMaterial _figures_5_c_cube_262 0) "opacity" :!class /Script/Engine.PrimitiveComponent))
        (Rendering|Material|SetScalarParameterValue _returnvalue_7 "opacity" 0.25 :!class /Script/Engine.MaterialInstanceDynamic))
      (:then_7
        (bind _returnvalue_8 (Rendering|Material|CreateDynamicMaterialInstance _figures_5_c_cube_263 0 (Rendering|Material|GetMaterial _figures_5_c_cube_263 0) "opacity" :!class /Script/Engine.PrimitiveComponent))
        (Rendering|Material|SetScalarParameterValue _returnvalue_8 "opacity" 0.25 :!class /Script/Engine.MaterialInstanceDynamic))
      (:then_8
        (bind _returnvalue_9 (Rendering|Material|CreateDynamicMaterialInstance _figures_5_c_cube_264 0 (Rendering|Material|GetMaterial _figures_5_c_cube_264 0) "opacity" :!class /Script/Engine.PrimitiveComponent))
        (Rendering|Material|SetScalarParameterValue _returnvalue_9 "opacity" 0.25 :!class /Script/Engine.MaterialInstanceDynamic))
      (:then_9
        (bind _returnvalue_10 (Rendering|Material|CreateDynamicMaterialInstance _figures_5_c_cube_267 0 (Rendering|Material|GetMaterial _figures_5_c_cube_267 0) "opacity" :!class /Script/Engine.PrimitiveComponent))
        (Rendering|Material|SetScalarParameterValue _returnvalue_10 "opacity" 0.25 :!class /Script/Engine.MaterialInstanceDynamic))
      (:then_10
        (bind _returnvalue_11 (Rendering|Material|CreateDynamicMaterialInstance _figures_5_c_cube_265_2 0 (Rendering|Material|GetMaterial _figures_5_c_cube_265_2 0) "opacity" :!class /Script/Engine.PrimitiveComponent))
        (Rendering|Material|SetScalarParameterValue _returnvalue_11 "opacity" 0.25 :!class /Script/Engine.MaterialInstanceDynamic))
      (:then_11
        (bind _returnvalue_12 (Rendering|Material|CreateDynamicMaterialInstance _figures_5_c_cube_266_2 0 (Rendering|Material|GetMaterial _figures_5_c_cube_266_2 0) "opacity" :!class /Script/Engine.PrimitiveComponent))
        (Rendering|Material|SetScalarParameterValue _returnvalue_12 "opacity" 0.25 :!class /Script/Engine.MaterialInstanceDynamic))
      (:then_12
        (bind _returnvalue_13 (Rendering|Material|CreateDynamicMaterialInstance _figures_5_c_cube_269_2 0 (Rendering|Material|GetMaterial _figures_5_c_cube_269_2 0) "opacity" :!class /Script/Engine.PrimitiveComponent))
        (Rendering|Material|SetScalarParameterValue _returnvalue_13 "opacity" 0.25 :!class /Script/Engine.MaterialInstanceDynamic))
      (:then_13
        (bind _returnvalue_14 (Rendering|Material|CreateDynamicMaterialInstance _figures_5_c_cube_283_2 0 (Rendering|Material|GetMaterial _figures_5_c_cube_283_2 0) "opacity" :!class /Script/Engine.PrimitiveComponent))
        (Rendering|Material|SetScalarParameterValue _returnvalue_14 "opacity" 0.25 :!class /Script/Engine.MaterialInstanceDynamic))
      (:then_14
        (bind _returnvalue_15 (Rendering|Material|CreateDynamicMaterialInstance _figures_5_c_cube_281_2 0 (Rendering|Material|GetMaterial _figures_5_c_cube_281_2 0) "opacity" :!class /Script/Engine.PrimitiveComponent))
        (Rendering|Material|SetScalarParameterValue _returnvalue_15 "opacity" 0.25 :!class /Script/Engine.MaterialInstanceDynamic))
      (:then_15
        (bind _returnvalue_16 (Rendering|Material|CreateDynamicMaterialInstance _figures_5_c_cube_284_2 0 (Rendering|Material|GetMaterial _figures_5_c_cube_284_2 0) "opacity" :!class /Script/Engine.PrimitiveComponent))
        (Rendering|Material|SetScalarParameterValue _returnvalue_16 "opacity" 0.25 :!class /Script/Engine.MaterialInstanceDynamic))
      (:then_16
        (bind _returnvalue_17 (Rendering|Material|CreateDynamicMaterialInstance _figures_5_c_cube_285_2 0 (Rendering|Material|GetMaterial _figures_5_c_cube_285_2 0) "opacity" :!class /Script/Engine.PrimitiveComponent))
        (Rendering|Material|SetScalarParameterValue _returnvalue_17 "opacity" 0.25 :!class /Script/Engine.MaterialInstanceDynamic))
      (:then_17
        (bind _returnvalue_18 (Rendering|Material|CreateDynamicMaterialInstance _figures_5_c_cube_274_2 0 (Rendering|Material|GetMaterial _figures_5_c_cube_274_2 0) "opacity" :!class /Script/Engine.PrimitiveComponent))
        (Rendering|Material|SetScalarParameterValue _returnvalue_18 "opacity" 0.25 :!class /Script/Engine.MaterialInstanceDynamic))
      (:then_18
        (bind _returnvalue_19 (Rendering|Material|CreateDynamicMaterialInstance _figures_5_c_cube_280_2 0 (Rendering|Material|GetMaterial _figures_5_c_cube_280_2 0) "opacity" :!class /Script/Engine.PrimitiveComponent))
        (Rendering|Material|SetScalarParameterValue _returnvalue_19 "opacity" 0.25 :!class /Script/Engine.MaterialInstanceDynamic))
      (:then_19
        (bind _returnvalue_20 (Rendering|Material|CreateDynamicMaterialInstance _figures_5_c_cube_275_2 0 (Rendering|Material|GetMaterial _figures_5_c_cube_275_2 0) "opacity" :!class /Script/Engine.PrimitiveComponent))
        (Rendering|Material|SetScalarParameterValue _returnvalue_20 "opacity" 0.25 :!class /Script/Engine.MaterialInstanceDynamic))
      (:then_20
        (bind _returnvalue_21 (Rendering|Material|CreateDynamicMaterialInstance _figures_5_c_cube_276_2 0 (Rendering|Material|GetMaterial _figures_5_c_cube_276_2 0) "opacity" :!class /Script/Engine.PrimitiveComponent))
        (Rendering|Material|SetScalarParameterValue _returnvalue_21 "opacity" 0.25 :!class /Script/Engine.MaterialInstanceDynamic))
      (:then_21
        (bind _returnvalue_22 (Rendering|Material|CreateDynamicMaterialInstance _figures_5_c_cube_277_2 0 (Rendering|Material|GetMaterial _figures_5_c_cube_277_2 0) "opacity" :!class /Script/Engine.PrimitiveComponent))
        (Rendering|Material|SetScalarParameterValue _returnvalue_22 "opacity" 0.25 :!class /Script/Engine.MaterialInstanceDynamic))
      (:then_22
        (bind _returnvalue_23 (Rendering|Material|CreateDynamicMaterialInstance _figures_5_c_cube_278_2 0 (Rendering|Material|GetMaterial _figures_5_c_cube_278_2 0) "opacity" :!class /Script/Engine.PrimitiveComponent))
        (Rendering|Material|SetScalarParameterValue _returnvalue_23 "opacity" 0.25 :!class /Script/Engine.MaterialInstanceDynamic))
      (:then_23
        (bind _returnvalue_24 (Rendering|Material|CreateDynamicMaterialInstance _figures_5_c_cube_279_2 0 (Rendering|Material|GetMaterial _figures_5_c_cube_279_2 0) "opacity" :!class /Script/Engine.PrimitiveComponent))
        (Rendering|Material|SetScalarParameterValue _returnvalue_24 "opacity" 0.25 :!class /Script/Engine.MaterialInstanceDynamic)))
    (else
      (Utilities|FlowControl|Sequence
        (:then_0
          (bind _returnvalue_25 (Rendering|Material|CreateDynamicMaterialInstance _figures_5_c_cube_268_2 0 (Rendering|Material|GetMaterial _figures_5_c_cube_268_2 0) "opacity" :!class /Script/Engine.PrimitiveComponent))
          (Rendering|Material|SetScalarParameterValue _returnvalue_25 "opacity" 0.0 :!class /Script/Engine.MaterialInstanceDynamic))
        (:then_1
          (bind _returnvalue_26 (Rendering|Material|CreateDynamicMaterialInstance _figures_5_c_cube_282 0 (Rendering|Material|GetMaterial _figures_5_c_cube_282 0) "opacity" :!class /Script/Engine.PrimitiveComponent))
          (Rendering|Material|SetScalarParameterValue _returnvalue_26 "opacity" 0.0 :!class /Script/Engine.MaterialInstanceDynamic))
        (:then_2
          (bind _returnvalue_27 (Rendering|Material|CreateDynamicMaterialInstance _figures_5_c_cube_270 0 (Rendering|Material|GetMaterial _figures_5_c_cube_270 0) "opacity" :!class /Script/Engine.PrimitiveComponent))
          (Rendering|Material|SetScalarParameterValue _returnvalue_27 "opacity" 0.0 :!class /Script/Engine.MaterialInstanceDynamic))
        (:then_3
          (bind _returnvalue_28 (Rendering|Material|CreateDynamicMaterialInstance _figures_5_c_cube_271 0 (Rendering|Material|GetMaterial _figures_5_c_cube_271 0) "opacity" :!class /Script/Engine.PrimitiveComponent))
          (Rendering|Material|SetScalarParameterValue _returnvalue_28 "opacity" 0.0 :!class /Script/Engine.MaterialInstanceDynamic))
        (:then_4
          (bind _returnvalue_29 (Rendering|Material|CreateDynamicMaterialInstance _figures_5_c_cube_272_2 0 (Rendering|Material|GetMaterial _figures_5_c_cube_272_2 0) "opacity" :!class /Script/Engine.PrimitiveComponent))
          (Rendering|Material|SetScalarParameterValue _returnvalue_29 "opacity" 0.0 :!class /Script/Engine.MaterialInstanceDynamic))
        (:then_5
          (bind _returnvalue_30 (Rendering|Material|CreateDynamicMaterialInstance _figures_5_c_cube_273_2 0 (Rendering|Material|GetMaterial _figures_5_c_cube_273_2 0) "opacity" :!class /Script/Engine.PrimitiveComponent))
          (Rendering|Material|SetScalarParameterValue _returnvalue_30 "opacity" 0.0 :!class /Script/Engine.MaterialInstanceDynamic))
        (:then_6
          (bind _returnvalue_31 (Rendering|Material|CreateDynamicMaterialInstance _figures_5_c_cube_262_2 0 (Rendering|Material|GetMaterial _figures_5_c_cube_262_2 0) "opacity" :!class /Script/Engine.PrimitiveComponent))
          (Rendering|Material|SetScalarParameterValue _returnvalue_31 "opacity" 0.0 :!class /Script/Engine.MaterialInstanceDynamic))
        (:then_7
          (bind _returnvalue_32 (Rendering|Material|CreateDynamicMaterialInstance _figures_5_c_cube_263_2 0 (Rendering|Material|GetMaterial _figures_5_c_cube_263_2 0) "opacity" :!class /Script/Engine.PrimitiveComponent))
          (Rendering|Material|SetScalarParameterValue _returnvalue_32 "opacity" 0.0 :!class /Script/Engine.MaterialInstanceDynamic))
        (:then_8
          (bind _returnvalue_33 (Rendering|Material|CreateDynamicMaterialInstance _figures_5_c_cube_264_2 0 (Rendering|Material|GetMaterial _figures_5_c_cube_264_2 0) "opacity" :!class /Script/Engine.PrimitiveComponent))
          (Rendering|Material|SetScalarParameterValue _returnvalue_33 "opacity" 0.0 :!class /Script/Engine.MaterialInstanceDynamic))
        (:then_9
          (bind _returnvalue_34 (Rendering|Material|CreateDynamicMaterialInstance _figures_5_c_cube_267_2 0 (Rendering|Material|GetMaterial _figures_5_c_cube_267_2 0) "opacity" :!class /Script/Engine.PrimitiveComponent))
          (Rendering|Material|SetScalarParameterValue _returnvalue_34 "opacity" 0.0 :!class /Script/Engine.MaterialInstanceDynamic))
        (:then_10
          (bind _returnvalue_35 (Rendering|Material|CreateDynamicMaterialInstance _figures_5_c_cube_265 0 (Rendering|Material|GetMaterial _figures_5_c_cube_265 0) "opacity" :!class /Script/Engine.PrimitiveComponent))
          (Rendering|Material|SetScalarParameterValue _returnvalue_35 "opacity" 0.0 :!class /Script/Engine.MaterialInstanceDynamic))
        (:then_11
          (bind _returnvalue_36 (Rendering|Material|CreateDynamicMaterialInstance _figures_5_c_cube_266 0 (Rendering|Material|GetMaterial _figures_5_c_cube_266 0) "opacity" :!class /Script/Engine.PrimitiveComponent))
          (Rendering|Material|SetScalarParameterValue _returnvalue_36 "opacity" 0.0 :!class /Script/Engine.MaterialInstanceDynamic))
        (:then_12
          (bind _returnvalue_37 (Rendering|Material|CreateDynamicMaterialInstance _figures_5_c_cube_269 0 (Rendering|Material|GetMaterial _figures_5_c_cube_269 0) "opacity" :!class /Script/Engine.PrimitiveComponent))
          (Rendering|Material|SetScalarParameterValue _returnvalue_37 "opacity" 0.0 :!class /Script/Engine.MaterialInstanceDynamic))
        (:then_13
          (bind _returnvalue_38 (Rendering|Material|CreateDynamicMaterialInstance _figures_5_c_cube_283 0 (Rendering|Material|GetMaterial _figures_5_c_cube_283 0) "opacity" :!class /Script/Engine.PrimitiveComponent))
          (Rendering|Material|SetScalarParameterValue _returnvalue_38 "opacity" 0.0 :!class /Script/Engine.MaterialInstanceDynamic))
        (:then_14
          (bind _returnvalue_39 (Rendering|Material|CreateDynamicMaterialInstance _figures_5_c_cube_281 0 (Rendering|Material|GetMaterial _figures_5_c_cube_281 0) "opacity" :!class /Script/Engine.PrimitiveComponent))
          (Rendering|Material|SetScalarParameterValue _returnvalue_39 "opacity" 0.0 :!class /Script/Engine.MaterialInstanceDynamic))
        (:then_15
          (bind _returnvalue_40 (Rendering|Material|CreateDynamicMaterialInstance _figures_5_c_cube_284 0 (Rendering|Material|GetMaterial _figures_5_c_cube_284 0) "opacity" :!class /Script/Engine.PrimitiveComponent))
          (Rendering|Material|SetScalarParameterValue _returnvalue_40 "opacity" 0.0 :!class /Script/Engine.MaterialInstanceDynamic))
        (:then_16
          (bind _returnvalue_41 (Rendering|Material|CreateDynamicMaterialInstance _figures_5_c_cube_285 0 (Rendering|Material|GetMaterial _figures_5_c_cube_285 0) "opacity" :!class /Script/Engine.PrimitiveComponent))
          (Rendering|Material|SetScalarParameterValue _returnvalue_41 "opacity" 0.0 :!class /Script/Engine.MaterialInstanceDynamic))
        (:then_17
          (bind _returnvalue_42 (Rendering|Material|CreateDynamicMaterialInstance _figures_5_c_cube_274 0 (Rendering|Material|GetMaterial _figures_5_c_cube_274 0) "opacity" :!class /Script/Engine.PrimitiveComponent))
          (Rendering|Material|SetScalarParameterValue _returnvalue_42 "opacity" 0.0 :!class /Script/Engine.MaterialInstanceDynamic))
        (:then_18
          (bind _returnvalue_43 (Rendering|Material|CreateDynamicMaterialInstance _figures_5_c_cube_280 0 (Rendering|Material|GetMaterial _figures_5_c_cube_280 0) "opacity" :!class /Script/Engine.PrimitiveComponent))
          (Rendering|Material|SetScalarParameterValue _returnvalue_43 "opacity" 0.0 :!class /Script/Engine.MaterialInstanceDynamic))
        (:then_19
          (bind _returnvalue_44 (Rendering|Material|CreateDynamicMaterialInstance _figures_5_c_cube_275 0 (Rendering|Material|GetMaterial _figures_5_c_cube_275 0) "opacity" :!class /Script/Engine.PrimitiveComponent))
          (Rendering|Material|SetScalarParameterValue _returnvalue_44 "opacity" 0.0 :!class /Script/Engine.MaterialInstanceDynamic))
        (:then_20
          (bind _returnvalue_45 (Rendering|Material|CreateDynamicMaterialInstance _figures_5_c_cube_276 0 (Rendering|Material|GetMaterial _figures_5_c_cube_276 0) "opacity" :!class /Script/Engine.PrimitiveComponent))
          (Rendering|Material|SetScalarParameterValue _returnvalue_45 "opacity" 0.0 :!class /Script/Engine.MaterialInstanceDynamic))
        (:then_21
          (bind _returnvalue_46 (Rendering|Material|CreateDynamicMaterialInstance _figures_5_c_cube_277 0 (Rendering|Material|GetMaterial _figures_5_c_cube_277 0) "opacity" :!class /Script/Engine.PrimitiveComponent))
          (Rendering|Material|SetScalarParameterValue _returnvalue_46 "opacity" 0.0 :!class /Script/Engine.MaterialInstanceDynamic))
        (:then_22
          (bind _returnvalue_47 (Rendering|Material|CreateDynamicMaterialInstance _figures_5_c_cube_278 0 (Rendering|Material|GetMaterial _figures_5_c_cube_278 0) "opacity" :!class /Script/Engine.PrimitiveComponent))
          (Rendering|Material|SetScalarParameterValue _returnvalue_47 "opacity" 0.0 :!class /Script/Engine.MaterialInstanceDynamic))
        (:then_23
          (bind _returnvalue_48 (Rendering|Material|CreateDynamicMaterialInstance _figures_5_c_cube_279 0 (Rendering|Material|GetMaterial _figures_5_c_cube_279 0) "opacity" :!class /Script/Engine.PrimitiveComponent))
          (Rendering|Material|SetScalarParameterValue _returnvalue_48 "opacity" 0.0 :!class /Script/Engine.MaterialInstanceDynamic))))))