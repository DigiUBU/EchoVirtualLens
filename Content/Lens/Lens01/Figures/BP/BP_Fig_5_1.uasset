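; Selectable figure 5_1 for Lens01, submitted to BP_GameManager_01 as a round 5 answer through its anchor connector.
; Attaching the connector sets Selected and, after a short delay, calls ValidateSelection if still selected; detaching clears the flag.
; SelectedOverlayColor toggles overlay opacity on the cube meshes through dynamic material instances, but its calls are disconnected.
; The older press-select handler is empty, and its toggle and sibling-deselect logic never runs.
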(event PressedSelect(Comp_Select)
  (params (Pawn :type BP%20Pawn%20Base%20Object%20Reference) (SourceActor :type Actor%20Object%20Reference) (ImpactLocation :type Vector :default "0, 0, 0") (ImpactComponent :type Actor%20Component%20Object%20Reference))
  ;[1 1 1] old
)

(event ConnectorAttached(Comp_Connector_Anchor)
  (params (Connector :type Comp%20Connector%20Object%20Reference) (AttachedToActor :type Actor%20Object%20Reference) (AttachedToComponent :type Scene%20Component%20Object%20Reference))
  ;[1 1 1] if it is ready to validate selection
  (Variables|Default|Setselected true)
  (bind _returnvalue (Actor|GetActorOfClass "/Game/Lens/Lens01/BP/BP_GameManager_01.BP_GameManager_01_C"))
  (Utilities|FlowControl|Delay 2.0)
  (if (Variables|Default|Getselected)
    (Default|ValidateSelection _returnvalue self 5)))

(event ConnectorDetached(Comp_Connector_Anchor)
  ;[1 1 1] if it is ready to validate selection
  (Variables|Default|Setselected false))

(fn ConstructionScript)

(fn SelectedOverlayColor
  (params (select :type Boolean))
  (bind _figures_5_1_cube_202 (Variables|Default|Getfigures_5_1_Cube_202))
  (bind _figures_5_1_cube_205 (Variables|Default|Getfigures_5_1_Cube_205))
  (bind _figures_5_1_cube_200 (Variables|Default|Getfigures_5_1_Cube_200))
  (bind _figures_5_1_cube_203 (Variables|Default|Getfigures_5_1_Cube_203))
  (bind _figures_5_1_cube_201 (Variables|Default|Getfigures_5_1_Cube_201))
  (bind _figures_5_1_cube_205_2 (Variables|Default|Getfigures_5_1_Cube_205))
  (bind _figures_5_1_cube_222 (Variables|Default|Getfigures_5_1_Cube_222))
  (bind _figures_5_1_cube_223 (Variables|Default|Getfigures_5_1_Cube_223))
  (bind _figures_5_1_cube_224 (Variables|Default|Getfigures_5_1_Cube_224))
  (bind _figures_5_1_cube_225 (Variables|Default|Getfigures_5_1_Cube_225))
  (bind _figures_5_1_cube_204 (Variables|Default|Getfigures_5_1_Cube_204))
  (bind _figures_5_1_cube_198 (Variables|Default|Getfigures_5_1_Cube_198))
  (bind _figures_5_1_cube_222_2 (Variables|Default|Getfigures_5_1_Cube_222))
  (bind _figures_5_1_cube_199 (Variables|Default|Getfigures_5_1_Cube_199))
  (bind _figures_5_1_cube_200_2 (Variables|Default|Getfigures_5_1_Cube_200))
  (bind _figures_5_1_cube_203_2 (Variables|Default|Getfigures_5_1_Cube_203))
  (bind _figures_5_1_cube_201_2 (Variables|Default|Getfigures_5_1_Cube_201))
  (bind _figures_5_1_cube_231 (Variables|Default|Getfigures_5_1_Cube_231))
  (bind _figures_5_1_cube_234 (Variables|Default|Getfigures_5_1_Cube_234))
  (bind _figures_5_1_cube_235 (Variables|Default|Getfigures_5_1_Cube_235))
  (bind _figures_5_1_cube_233 (Variables|Default|Getfigures_5_1_Cube_233))
  (bind _figures_5_1_cube_236 (Variables|Default|Getfigures_5_1_Cube_236))
  (bind _figures_5_1_cube_237 (Variables|Default|Getfigures_5_1_Cube_237))
  (bind _figures_5_1_cube_223_2 (Variables|Default|Getfigures_5_1_Cube_223))
  (bind _figures_5_1_cube_226 (Variables|Default|Getfigures_5_1_Cube_226))
  (bind _figures_5_1_cube_232 (Variables|Default|Getfigures_5_1_Cube_232))
  (bind _figures_5_1_cube_227 (Variables|Default|Getfigures_5_1_Cube_227))
  (bind _figures_5_1_cube_228 (Variables|Default|Getfigures_5_1_Cube_228))
  (bind _figures_5_1_cube_229 (Variables|Default|Getfigures_5_1_Cube_229))
  (bind _figures_5_1_cube_230 (Variables|Default|Getfigures_5_1_Cube_230))
  (bind _figures_5_1_cube_231_2 (Variables|Default|Getfigures_5_1_Cube_231))
  (bind _figures_5_1_cube_234_2 (Variables|Default|Getfigures_5_1_Cube_234))
  (bind _figures_5_1_cube_235_2 (Variables|Default|Getfigures_5_1_Cube_235))
  (bind _figures_5_1_cube_233_2 (Variables|Default|Getfigures_5_1_Cube_233))
  (bind _figures_5_1_cube_202_2 (Variables|Default|Getfigures_5_1_Cube_202))
  (bind _figures_5_1_cube_236_2 (Variables|Default|Getfigures_5_1_Cube_236))
  (bind _figures_5_1_cube_237_2 (Variables|Default|Getfigures_5_1_Cube_237))
  (bind _figures_5_1_cube_226_2 (Variables|Default|Getfigures_5_1_Cube_226))
  (bind _figures_5_1_cube_232_2 (Variables|Default|Getfigures_5_1_Cube_232))
  (bind _figures_5_1_cube_227_2 (Variables|Default|Getfigures_5_1_Cube_227))
  (bind _figures_5_1_cube_228_2 (Variables|Default|Getfigures_5_1_Cube_228))
  (bind _figures_5_1_cube_229_2 (Variables|Default|Getfigures_5_1_Cube_229))
  (bind _figures_5_1_cube_230_2 (Variables|Default|Getfigures_5_1_Cube_230))
  (bind _figures_5_1_cube_224_2 (Variables|Default|Getfigures_5_1_Cube_224))
  (bind _figures_5_1_cube_225_2 (Variables|Default|Getfigures_5_1_Cube_225))
  (bind _figures_5_1_cube_204_2 (Variables|Default|Getfigures_5_1_Cube_204))
  (bind _figures_5_1_cube_198_2 (Variables|Default|Getfigures_5_1_Cube_198))
  (bind _figures_5_1_cube_199_2 (Variables|Default|Getfigures_5_1_Cube_199))
  (if select
    (Utilities|FlowControl|Sequence
      (:then_0
        (bind _returnvalue (Rendering|Material|CreateDynamicMaterialInstance _figures_5_1_cube_225 0 (Rendering|Material|GetMaterial _figures_5_1_cube_225 0) "opacity" :!class /Script/Engine.PrimitiveComponent))
        (Rendering|Material|SetScalarParameterValue _returnvalue "opacity" 0.25 :!class /Script/Engine.MaterialInstanceDynamic))
      (:then_1
        (bind _returnvalue_2 (Rendering|Material|CreateDynamicMaterialInstance _figures_5_1_cube_202_2 0 (Rendering|Material|GetMaterial _figures_5_1_cube_202_2 0) "opacity" :!class /Script/Engine.PrimitiveComponent))
        (Rendering|Material|SetScalarParameterValue _returnvalue_2 "opacity" 0.25 :!class /Script/Engine.MaterialInstanceDynamic))
      (:then_2
        (bind _returnvalue_3 (Rendering|Material|CreateDynamicMaterialInstance _figures_5_1_cube_205_2 0 (Rendering|Material|GetMaterial _figures_5_1_cube_205_2 0) "opacity" :!class /Script/Engine.PrimitiveComponent))
        (Rendering|Material|SetScalarParameterValue _returnvalue_3 "opacity" 0.25 :!class /Script/Engine.MaterialInstanceDynamic))
      (:then_3
        (bind _returnvalue_4 (Rendering|Material|CreateDynamicMaterialInstance _figures_5_1_cube_222 0 (Rendering|Material|GetMaterial _figures_5_1_cube_222 0) "opacity" :!class /Script/Engine.PrimitiveComponent))
        (Rendering|Material|SetScalarParameterValue _returnvalue_4 "opacity" 0.25 :!class /Script/Engine.MaterialInstanceDynamic))
      (:then_4
        (bind _returnvalue_5 (Rendering|Material|CreateDynamicMaterialInstance _figures_5_1_cube_223 0 (Rendering|Material|GetMaterial _figures_5_1_cube_223 0) "opacity" :!class /Script/Engine.PrimitiveComponent))
        (Rendering|Material|SetScalarParameterValue _returnvalue_5 "opacity" 0.25 :!class /Script/Engine.MaterialInstanceDynamic))
      (:then_5
        (bind _returnvalue_6 (Rendering|Material|CreateDynamicMaterialInstance _figures_5_1_cube_224 0 (Rendering|Material|GetMaterial _figures_5_1_cube_224 0) "opacity" :!class /Script/Engine.PrimitiveComponent))
        (Rendering|Material|SetScalarParameterValue _returnvalue_6 "opacity" 0.25 :!class /Script/Engine.MaterialInstanceDynamic))
      (:then_6
        (bind _returnvalue_7 (Rendering|Material|CreateDynamicMaterialInstance _figures_5_1_cube_204 0 (Rendering|Material|GetMaterial _figures_5_1_cube_204 0) "opacity" :!class /Script/Engine.PrimitiveComponent))
        (Rendering|Material|SetScalarParameterValue _returnvalue_7 "opacity" 0.25 :!class /Script/Engine.MaterialInstanceDynamic))
      (:then_7
        (bind _returnvalue_8 (Rendering|Material|CreateDynamicMaterialInstance _figures_5_1_cube_198 0 (Rendering|Material|GetMaterial _figures_5_1_cube_198 0) "opacity" :!class /Script/Engine.PrimitiveComponent))
        (Rendering|Material|SetScalarParameterValue _returnvalue_8 "opacity" 0.25 :!class /Script/Engine.MaterialInstanceDynamic))
      (:then_8
        (bind _returnvalue_9 (Rendering|Material|CreateDynamicMaterialInstance _figures_5_1_cube_199 0 (Rendering|Material|GetMaterial _figures_5_1_cube_199 0) "opacity" :!class /Script/Engine.PrimitiveComponent))
        (Rendering|Material|SetScalarParameterValue _returnvalue_9 "opacity" 0.25 :!class /Script/Engine.MaterialInstanceDynamic))
      (:then_9
        (bind _returnvalue_10 (Rendering|Material|CreateDynamicMaterialInstance _figures_5_1_cube_200_2 0 (Rendering|Material|GetMaterial _figures_5_1_cube_200_2 0) "opacity" :!class /Script/Engine.PrimitiveComponent))
        (Rendering|Material|SetScalarParameterValue _returnvalue_10 "opacity" 0.25 :!class /Script/Engine.MaterialInstanceDynamic))
      (:then_10
        (bind _returnvalue_11 (Rendering|Material|CreateDynamicMaterialInstance _figures_5_1_cube_203_2 0 (Rendering|Material|GetMaterial _figures_5_1_cube_203_2 0) "opacity" :!class /Script/Engine.PrimitiveComponent))
        (Rendering|Material|SetScalarParameterValue _returnvalue_11 "opacity" 0.25 :!class /Script/Engine.MaterialInstanceDynamic))
      (:then_11
        (bind _returnvalue_12 (Rendering|Material|CreateDynamicMaterialInstance _figures_5_1_cube_201_2 0 (Rendering|Material|GetMaterial _figures_5_1_cube_201_2 0) "opacity" :!class /Script/Engine.PrimitiveComponent))
        (Rendering|Material|SetScalarParameterValue _returnvalue_12 "opacity" 0.25 :!class /Script/Engine.MaterialInstanceDynamic))
      (:then_12
        (bind _returnvalue_13 (Rendering|Material|CreateDynamicMaterialInstance _figures_5_1_cube_231_2 0 (Rendering|Material|GetMaterial _figures_5_1_cube_231_2 0) "opacity" :!class /Script/Engine.PrimitiveComponent))
        (Rendering|Material|SetScalarParameterValue _returnvalue_13 "opacity" 0.25 :!class /Script/Engine.MaterialInstanceDynamic))
      (:then_13
        (bind _returnvalue_14 (Rendering|Material|CreateDynamicMaterialInstance _figures_5_1_cube_234_2 0 (Rendering|Material|GetMaterial _figures_5_1_cube_234_2 0) "opacity" :!class /Script/Engine.PrimitiveComponent))
        (Rendering|Material|SetScalarParameterValue _returnvalue_14 "opacity" 0.25 :!class /Script/Engine.MaterialInstanceDynamic))
      (:then_14
        (bind _returnvalue_15 (Rendering|Material|CreateDynamicMaterialInstance _figures_5_1_cube_235_2 0 (Rendering|Material|GetMaterial _figures_5_1_cube_235_2 0) "opacity" :!class /Script/Engine.PrimitiveComponent))
        (Rendering|Material|SetScalarParameterValue _returnvalue_15 "opacity" 0.25 :!class /Script/Engine.MaterialInstanceDynamic))
      (:then_15
        (bind _returnvalue_16 (Rendering|Material|CreateDynamicMaterialInstance _figures_5_1_cube_233_2 0 (Rendering|Material|GetMaterial _figures_5_1_cube_233_2 0) "opacity" :!class /Script/Engine.PrimitiveComponent))
        (Rendering|Material|SetScalarParameterValue _returnvalue_16 "opacity" 0.25 :!class /Script/Engine.MaterialInstanceDynamic))
      (:then_16
        (bind _returnvalue_17 (Rendering|Material|CreateDynamicMaterialInstance _figures_5_1_cube_236_2 0 (Rendering|Material|GetMaterial _figures_5_1_cube_236_2 0) "opacity" :!class /Script/Engine.PrimitiveComponent))
        (Rendering|Material|SetScalarParameterValue _returnvalue_17 "opacity" 0.25 :!class /Script/Engine.MaterialInstanceDynamic))
      (:then_17
        (bind _returnvalue_18 (Rendering|Material|CreateDynamicMaterialInstance _figures_5_1_cube_237_2 0 (Rendering|Material|GetMaterial _figures_5_1_cube_237_2 0) "opacity" :!class /Script/Engine.PrimitiveComponent))
        (Rendering|Material|SetScalarParameterValue _returnvalue_18 "opacity" 0.25 :!class /Script/Engine.MaterialInstanceDynamic))
      (:then_18
        (bind _returnvalue_19 (Rendering|Material|CreateDynamicMaterialInstance _figures_5_1_cube_226_2 0 (Rendering|Material|GetMaterial _figures_5_1_cube_226_2 0) "opacity" :!class /Script/Engine.PrimitiveComponent))
        (Rendering|Material|SetScalarParameterValue _returnvalue_19 "opacity" 0.25 :!class /Script/Engine.MaterialInstanceDynamic))
      (:then_19
        (bind _returnvalue_20 (Rendering|Material|CreateDynamicMaterialInstance _figures_5_1_cube_232_2 0 (Rendering|Material|GetMaterial _figures_5_1_cube_232_2 0) "opacity" :!class /Script/Engine.PrimitiveComponent))
        (Rendering|Material|SetScalarParameterValue _returnvalue_20 "opacity" 0.25 :!class /Script/Engine.MaterialInstanceDynamic))
      (:then_20
        (bind _returnvalue_21 (Rendering|Material|CreateDynamicMaterialInstance _figures_5_1_cube_227_2 0 (Rendering|Material|GetMaterial _figures_5_1_cube_227_2 0) "opacity" :!class /Script/Engine.PrimitiveComponent))
        (Rendering|Material|SetScalarParameterValue _returnvalue_21 "opacity" 0.25 :!class /Script/Engine.MaterialInstanceDynamic))
      (:then_21
        (bind _returnvalue_22 (Rendering|Material|CreateDynamicMaterialInstance _figures_5_1_cube_228_2 0 (Rendering|Material|GetMaterial _figures_5_1_cube_228_2 0) "opacity" :!class /Script/Engine.PrimitiveComponent))
        (Rendering|Material|SetScalarParameterValue _returnvalue_22 "opacity" 0.25 :!class /Script/Engine.MaterialInstanceDynamic))
      (:then_22
        (bind _returnvalue_23 (Rendering|Material|CreateDynamicMaterialInstance _figures_5_1_cube_229_2 0 (Rendering|Material|GetMaterial _figures_5_1_cube_229_2 0) "opacity" :!class /Script/Engine.PrimitiveComponent))
        (Rendering|Material|SetScalarParameterValue _returnvalue_23 "opacity" 0.25 :!class /Script/Engine.MaterialInstanceDynamic))
      (:then_23
        (bind _returnvalue_24 (Rendering|Material|CreateDynamicMaterialInstance _figures_5_1_cube_230_2 0 (Rendering|Material|GetMaterial _figures_5_1_cube_230_2 0) "opacity" :!class /Script/Engine.PrimitiveComponent))
        (Rendering|Material|SetScalarParameterValue _returnvalue_24 "opacity" 0.25 :!class /Script/Engine.MaterialInstanceDynamic)))
    (else
      (Utilities|FlowControl|Sequence
        (:then_0
          (bind _returnvalue_25 (Rendering|Material|CreateDynamicMaterialInstance _figures_5_1_cube_225_2 0 (Rendering|Material|GetMaterial _figures_5_1_cube_225_2 0) "opacity" :!class /Script/Engine.PrimitiveComponent))
          (Rendering|Material|SetScalarParameterValue _returnvalue_25 "opacity" 0.0 :!class /Script/Engine.MaterialInstanceDynamic))
        (:then_1
          (bind _returnvalue_26 (Rendering|Material|CreateDynamicMaterialInstance _figures_5_1_cube_202 0 (Rendering|Material|GetMaterial _figures_5_1_cube_202 0) "opacity" :!class /Script/Engine.PrimitiveComponent))
          (Rendering|Material|SetScalarParameterValue _returnvalue_26 "opacity" 0.0 :!class /Script/Engine.MaterialInstanceDynamic))
        (:then_2
          (bind _returnvalue_27 (Rendering|Material|CreateDynamicMaterialInstance _figures_5_1_cube_205 0 (Rendering|Material|GetMaterial _figures_5_1_cube_205 0) "opacity" :!class /Script/Engine.PrimitiveComponent))
          (Rendering|Material|SetScalarParameterValue _returnvalue_27 "opacity" 0.0 :!class /Script/Engine.MaterialInstanceDynamic))
        (:then_3
          (bind _returnvalue_28 (Rendering|Material|CreateDynamicMaterialInstance _figures_5_1_cube_222_2 0 (Rendering|Material|GetMaterial _figures_5_1_cube_222_2 0) "opacity" :!class /Script/Engine.PrimitiveComponent))
          (Rendering|Material|SetScalarParameterValue _returnvalue_28 "opacity" 0.0 :!class /Script/Engine.MaterialInstanceDynamic))
        (:then_4
          (bind _returnvalue_29 (Rendering|Material|CreateDynamicMaterialInstance _figures_5_1_cube_223_2 0 (Rendering|Material|GetMaterial _figures_5_1_cube_223_2 0) "opacity" :!class /Script/Engine.PrimitiveComponent))
          (Rendering|Material|SetScalarParameterValue _returnvalue_29 "opacity" 0.0 :!class /Script/Engine.MaterialInstanceDynamic))
        (:then_5
          (bind _returnvalue_30 (Rendering|Material|CreateDynamicMaterialInstance _figures_5_1_cube_224_2 0 (Rendering|Material|GetMaterial _figures_5_1_cube_224_2 0) "opacity" :!class /Script/Engine.PrimitiveComponent))
          (Rendering|Material|SetScalarParameterValue _returnvalue_30 "opacity" 0.0 :!class /Script/Engine.MaterialInstanceDynamic))
        (:then_6
          (bind _returnvalue_31 (Rendering|Material|CreateDynamicMaterialInstance _figures_5_1_cube_204_2 0 (Rendering|Material|GetMaterial _figures_5_1_cube_204_2 0) "opacity" :!class /Script/Engine.PrimitiveComponent))
          (Rendering|Material|SetScalarParameterValue _returnvalue_31 "opacity" 0.0 :!class /Script/Engine.MaterialInstanceDynamic))
        (:then_7
          (bind _returnvalue_32 (Rendering|Material|CreateDynamicMaterialInstance _figures_5_1_cube_198_2 0 (Rendering|Material|GetMaterial _figures_5_1_cube_198_2 0) "opacity" :!class /Script/Engine.PrimitiveComponent))
          (Rendering|Material|SetScalarParameterValue _returnvalue_32 "opacity" 0.0 :!class /Script/Engine.MaterialInstanceDynamic))
        (:then_8
          (bind _returnvalue_33 (Rendering|Material|CreateDynamicMaterialInstance _figures_5_1_cube_199_2 0 (Rendering|Material|GetMaterial _figures_5_1_cube_199_2 0) "opacity" :!class /Script/Engine.PrimitiveComponent))
          (Rendering|Material|SetScalarParameterValue _returnvalue_33 "opacity" 0.0 :!class /Script/Engine.MaterialInstanceDynamic))
        (:then_9
          (bind _returnvalue_34 (Rendering|Material|CreateDynamicMaterialInstance _figures_5_1_cube_200 0 (Rendering|Material|GetMaterial _figures_5_1_cube_200 0) "opacity" :!class /Script/Engine.PrimitiveComponent))
          (Rendering|Material|SetScalarParameterValue _returnvalue_34 "opacity" 0.0 :!class /Script/Engine.MaterialInstanceDynamic))
        (:then_10
          (bind _returnvalue_35 (Rendering|Material|CreateDynamicMaterialInstance _figures_5_1_cube_203 0 (Rendering|Material|GetMaterial _figures_5_1_cube_203 0) "opacity" :!class /Script/Engine.PrimitiveComponent))
          (Rendering|Material|SetScalarParameterValue _returnvalue_35 "opacity" 0.0 :!class /Script/Engine.MaterialInstanceDynamic))
        (:then_11
          (bind _returnvalue_36 (Rendering|Material|CreateDynamicMaterialInstance _figures_5_1_cube_201 0 (Rendering|Material|GetMaterial _figures_5_1_cube_201 0) "opacity" :!class /Script/Engine.PrimitiveComponent))
          (Rendering|Material|SetScalarParameterValue _returnvalue_36 "opacity" 0.0 :!class /Script/Engine.MaterialInstanceDynamic))
        (:then_12
          (bind _returnvalue_37 (Rendering|Material|CreateDynamicMaterialInstance _figures_5_1_cube_231 0 (Rendering|Material|GetMaterial _figures_5_1_cube_231 0) "opacity" :!class /Script/Engine.PrimitiveComponent))
          (Rendering|Material|SetScalarParameterValue _returnvalue_37 "opacity" 0.0 :!class /Script/Engine.MaterialInstanceDynamic))
        (:then_13
          (bind _returnvalue_38 (Rendering|Material|CreateDynamicMaterialInstance _figures_5_1_cube_234 0 (Rendering|Material|GetMaterial _figures_5_1_cube_234 0) "opacity" :!class /Script/Engine.PrimitiveComponent))
          (Rendering|Material|SetScalarParameterValue _returnvalue_38 "opacity" 0.0 :!class /Script/Engine.MaterialInstanceDynamic))
        (:then_14
          (bind _returnvalue_39 (Rendering|Material|CreateDynamicMaterialInstance _figures_5_1_cube_235 0 (Rendering|Material|GetMaterial _figures_5_1_cube_235 0) "opacity" :!class /Script/Engine.PrimitiveComponent))
          (Rendering|Material|SetScalarParameterValue _returnvalue_39 "opacity" 0.0 :!class /Script/Engine.MaterialInstanceDynamic))
        (:then_15
          (bind _returnvalue_40 (Rendering|Material|CreateDynamicMaterialInstance _figures_5_1_cube_233 0 (Rendering|Material|GetMaterial _figures_5_1_cube_233 0) "opacity" :!class /Script/Engine.PrimitiveComponent))
          (Rendering|Material|SetScalarParameterValue _returnvalue_40 "opacity" 0.0 :!class /Script/Engine.MaterialInstanceDynamic))
        (:then_16
          (bind _returnvalue_41 (Rendering|Material|CreateDynamicMaterialInstance _figures_5_1_cube_236 0 (Rendering|Material|GetMaterial _figures_5_1_cube_236 0) "opacity" :!class /Script/Engine.PrimitiveComponent))
          (Rendering|Material|SetScalarParameterValue _returnvalue_41 "opacity" 0.0 :!class /Script/Engine.MaterialInstanceDynamic))
        (:then_17
          (bind _returnvalue_42 (Rendering|Material|CreateDynamicMaterialInstance _figures_5_1_cube_237 0 (Rendering|Material|GetMaterial _figures_5_1_cube_237 0) "opacity" :!class /Script/Engine.PrimitiveComponent))
          (Rendering|Material|SetScalarParameterValue _returnvalue_42 "opacity" 0.0 :!class /Script/Engine.MaterialInstanceDynamic))
        (:then_18
          (bind _returnvalue_43 (Rendering|Material|CreateDynamicMaterialInstance _figures_5_1_cube_226 0 (Rendering|Material|GetMaterial _figures_5_1_cube_226 0) "opacity" :!class /Script/Engine.PrimitiveComponent))
          (Rendering|Material|SetScalarParameterValue _returnvalue_43 "opacity" 0.0 :!class /Script/Engine.MaterialInstanceDynamic))
        (:then_19
          (bind _returnvalue_44 (Rendering|Material|CreateDynamicMaterialInstance _figures_5_1_cube_232 0 (Rendering|Material|GetMaterial _figures_5_1_cube_232 0) "opacity" :!class /Script/Engine.PrimitiveComponent))
          (Rendering|Material|SetScalarParameterValue _returnvalue_44 "opacity" 0.0 :!class /Script/Engine.MaterialInstanceDynamic))
        (:then_20
          (bind _returnvalue_45 (Rendering|Material|CreateDynamicMaterialInstance _figures_5_1_cube_227 0 (Rendering|Material|GetMaterial _figures_5_1_cube_227 0) "opacity" :!class /Script/Engine.PrimitiveComponent))
          (Rendering|Material|SetScalarParameterValue _returnvalue_45 "opacity" 0.0 :!class /Script/Engine.MaterialInstanceDynamic))
        (:then_21
          (bind _returnvalue_46 (Rendering|Material|CreateDynamicMaterialInstance _figures_5_1_cube_228 0 (Rendering|Material|GetMaterial _figures_5_1_cube_228 0) "opacity" :!class /Script/Engine.PrimitiveComponent))
          (Rendering|Material|SetScalarParameterValue _returnvalue_46 "opacity" 0.0 :!class /Script/Engine.MaterialInstanceDynamic))
        (:then_22
          (bind _returnvalue_47 (Rendering|Material|CreateDynamicMaterialInstance _figures_5_1_cube_229 0 (Rendering|Material|GetMaterial _figures_5_1_cube_229 0) "opacity" :!class /Script/Engine.PrimitiveComponent))
          (Rendering|Material|SetScalarParameterValue _returnvalue_47 "opacity" 0.0 :!class /Script/Engine.MaterialInstanceDynamic))
        (:then_23
          (bind _returnvalue_48 (Rendering|Material|CreateDynamicMaterialInstance _figures_5_1_cube_230 0 (Rendering|Material|GetMaterial _figures_5_1_cube_230 0) "opacity" :!class /Script/Engine.PrimitiveComponent))
          (Rendering|Material|SetScalarParameterValue _returnvalue_48 "opacity" 0.0 :!class /Script/Engine.MaterialInstanceDynamic))))))