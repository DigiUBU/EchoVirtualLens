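; Selectable figure 6 of round 5 in the Lens01 level, validated by the game manager when chosen.
; Attaching its anchor connector sets Selected and, after a two-second delay, calls ValidateSelection on BP_GameManager_01 if still selected; detaching clears the flag.
; SelectedOverlayColor toggles an opacity overlay across the cube meshes through dynamic material instances, but its calls and the sibling-figure deselect chain are disconnected, and the press event is empty.
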(event PressedSelect(Comp_Select)
  (params (Pawn :type BP%20Pawn%20Base%20Object%20Reference) (SourceActor :type Actor%20Object%20Reference) (ImpactLocation :type Vector :default "0, 0, 0") (ImpactComponent :type Actor%20Component%20Object%20Reference)))

(event ConnectorAttached(Comp_Connector_Anchor)
  (params (Connector :type Comp%20Connector%20Object%20Reference) (AttachedToActor :type Actor%20Object%20Reference) (AttachedToComponent :type Scene%20Component%20Object%20Reference))
  ;[1 1 1] if it is ready to validate selection
  (Variables|Default|Setselected true)
  (bind _returnvalue (Actor|GetActorOfClass "/Game/Lens/Lens01/BP/BP_GameManager_01.BP_GameManager_01_C"))
  (Utilities|FlowControl|Delay 2.0)
  (if (Variables|Default|Getselected)
    (Default|ValidateSelection _returnvalue self 5)))

(event ConnectorDetached(Comp_Connector_Anchor)
  ;[1 1 1] if it is ready to validate selection
  (Variables|Default|Setselected false))

(fn ConstructionScript)

(fn SelectedOverlayColor
  (params (select :type Boolean))
  (bind _figures_5_6_cube_394 (Variables|Default|Getfigures_5_6_Cube_394))
  (bind _figures_5_6_cube_390 (Variables|Default|Getfigures_5_6_Cube_390))
  (bind _figures_5_6_cube_387 (Variables|Default|Getfigures_5_6_Cube_387))
  (bind _figures_5_6_cube_389 (Variables|Default|Getfigures_5_6_Cube_389))
  (bind _figures_5_6_cube_402 (Variables|Default|Getfigures_5_6_Cube_402))
  (bind _figures_5_6_cube_403 (Variables|Default|Getfigures_5_6_Cube_403))
  (bind _figures_5_6_cube_404 (Variables|Default|Getfigures_5_6_Cube_404))
  (bind _figures_5_6_cube_405 (Variables|Default|Getfigures_5_6_Cube_405))
  (bind _figures_5_6_cube_401 (Variables|Default|Getfigures_5_6_Cube_401))
  (bind _figures_5_6_cube_395 (Variables|Default|Getfigures_5_6_Cube_395))
  (bind _figures_5_6_cube_396 (Variables|Default|Getfigures_5_6_Cube_396))
  (bind _figures_5_6_cube_397 (Variables|Default|Getfigures_5_6_Cube_397))
  (bind _figures_5_6_cube_391 (Variables|Default|Getfigures_5_6_Cube_391))
  (bind _figures_5_6_cube_398 (Variables|Default|Getfigures_5_6_Cube_398))
  (bind _figures_5_6_cube_399 (Variables|Default|Getfigures_5_6_Cube_399))
  (bind _figures_5_6_cube_400 (Variables|Default|Getfigures_5_6_Cube_400))
  (bind _figures_5_6_cube_394_2 (Variables|Default|Getfigures_5_6_Cube_394))
  (bind _figures_5_6_cube_390_2 (Variables|Default|Getfigures_5_6_Cube_390))
  (bind _figures_5_6_cube_391_2 (Variables|Default|Getfigures_5_6_Cube_391))
  (bind _figures_5_6_cube_392 (Variables|Default|Getfigures_5_6_Cube_392))
  (bind _figures_5_6_cube_393 (Variables|Default|Getfigures_5_6_Cube_393))
  (bind _figures_5_6_cube_382 (Variables|Default|Getfigures_5_6_Cube_382))
  (bind _figures_5_6_cube_384 (Variables|Default|Getfigures_5_6_Cube_384))
  (bind _figures_5_6_cube_392_2 (Variables|Default|Getfigures_5_6_Cube_392))
  (bind _figures_5_6_cube_385 (Variables|Default|Getfigures_5_6_Cube_385))
  (bind _figures_5_6_cube_388 (Variables|Default|Getfigures_5_6_Cube_388))
  (bind _figures_5_6_cube_386 (Variables|Default|Getfigures_5_6_Cube_386))
  (bind _figures_5_6_cube_387_2 (Variables|Default|Getfigures_5_6_Cube_387))
  (bind _figures_5_6_cube_389_2 (Variables|Default|Getfigures_5_6_Cube_389))
  (bind _figures_5_6_cube_402_2 (Variables|Default|Getfigures_5_6_Cube_402))
  (bind _figures_5_6_cube_403_2 (Variables|Default|Getfigures_5_6_Cube_403))
  (bind _figures_5_6_cube_404_2 (Variables|Default|Getfigures_5_6_Cube_404))
  (bind _figures_5_6_cube_405_2 (Variables|Default|Getfigures_5_6_Cube_405))
  (bind _figures_5_6_cube_401_2 (Variables|Default|Getfigures_5_6_Cube_401))
  (bind _figures_5_6_cube_393_2 (Variables|Default|Getfigures_5_6_Cube_393))
  (bind _figures_5_6_cube_395_2 (Variables|Default|Getfigures_5_6_Cube_395))
  (bind _figures_5_6_cube_396_2 (Variables|Default|Getfigures_5_6_Cube_396))
  (bind _figures_5_6_cube_397_2 (Variables|Default|Getfigures_5_6_Cube_397))
  (bind _figures_5_6_cube_398_2 (Variables|Default|Getfigures_5_6_Cube_398))
  (bind _figures_5_6_cube_399_2 (Variables|Default|Getfigures_5_6_Cube_399))
  (bind _figures_5_6_cube_400_2 (Variables|Default|Getfigures_5_6_Cube_400))
  (bind _figures_5_6_cube_382_2 (Variables|Default|Getfigures_5_6_Cube_382))
  (bind _figures_5_6_cube_384_2 (Variables|Default|Getfigures_5_6_Cube_384))
  (bind _figures_5_6_cube_385_2 (Variables|Default|Getfigures_5_6_Cube_385))
  (bind _figures_5_6_cube_388_2 (Variables|Default|Getfigures_5_6_Cube_388))
  (bind _figures_5_6_cube_386_2 (Variables|Default|Getfigures_5_6_Cube_386))
  (if select
    (Utilities|FlowControl|Sequence
      (:then_0
        (bind _returnvalue (Rendering|Material|CreateDynamicMaterialInstance _figures_5_6_cube_382 0 (Rendering|Material|GetMaterial _figures_5_6_cube_382 0) "opacity" :!class /Script/Engine.PrimitiveComponent))
        (Rendering|Material|SetScalarParameterValue _returnvalue "opacity" 0.25 :!class /Script/Engine.MaterialInstanceDynamic))
      (:then_1
        (bind _returnvalue_2 (Rendering|Material|CreateDynamicMaterialInstance _figures_5_6_cube_394_2 0 (Rendering|Material|GetMaterial _figures_5_6_cube_394_2 0) "opacity" :!class /Script/Engine.PrimitiveComponent))
        (Rendering|Material|SetScalarParameterValue _returnvalue_2 "opacity" 0.25 :!class /Script/Engine.MaterialInstanceDynamic))
      (:then_2
        (bind _returnvalue_3 (Rendering|Material|CreateDynamicMaterialInstance _figures_5_6_cube_390_2 0 (Rendering|Material|GetMaterial _figures_5_6_cube_390_2 0) "opacity" :!class /Script/Engine.PrimitiveComponent))
        (Rendering|Material|SetScalarParameterValue _returnvalue_3 "opacity" 0.25 :!class /Script/Engine.MaterialInstanceDynamic))
      (:then_3
        (bind _returnvalue_4 (Rendering|Material|CreateDynamicMaterialInstance _figures_5_6_cube_391_2 0 (Rendering|Material|GetMaterial _figures_5_6_cube_391_2 0) "opacity" :!class /Script/Engine.PrimitiveComponent))
        (Rendering|Material|SetScalarParameterValue _returnvalue_4 "opacity" 0.25 :!class /Script/Engine.MaterialInstanceDynamic))
      (:then_4
        (bind _returnvalue_5 (Rendering|Material|CreateDynamicMaterialInstance _figures_5_6_cube_392 0 (Rendering|Material|GetMaterial _figures_5_6_cube_392 0) "opacity" :!class /Script/Engine.PrimitiveComponent))
        (Rendering|Material|SetScalarParameterValue _returnvalue_5 "opacity" 0.25 :!class /Script/Engine.MaterialInstanceDynamic))
      (:then_5
        (bind _returnvalue_6 (Rendering|Material|CreateDynamicMaterialInstance _figures_5_6_cube_393 0 (Rendering|Material|GetMaterial _figures_5_6_cube_393 0) "opacity" :!class /Script/Engine.PrimitiveComponent))
        (Rendering|Material|SetScalarParameterValue _returnvalue_6 "opacity" 0.25 :!class /Script/Engine.MaterialInstanceDynamic))
      (:then_6
        (bind _returnvalue_7 (Rendering|Material|CreateDynamicMaterialInstance _figures_5_6_cube_384 0 (Rendering|Material|GetMaterial _figures_5_6_cube_384 0) "opacity" :!class /Script/Engine.PrimitiveComponent))
        (Rendering|Material|SetScalarParameterValue _returnvalue_7 "opacity" 0.25 :!class /Script/Engine.MaterialInstanceDynamic))
      (:then_7
        (bind _returnvalue_8 (Rendering|Material|CreateDynamicMaterialInstance _figures_5_6_cube_385 0 (Rendering|Material|GetMaterial _figures_5_6_cube_385 0) "opacity" :!class /Script/Engine.PrimitiveComponent))
        (Rendering|Material|SetScalarParameterValue _returnvalue_8 "opacity" 0.25 :!class /Script/Engine.MaterialInstanceDynamic))
      (:then_8
        (bind _returnvalue_9 (Rendering|Material|CreateDynamicMaterialInstance _figures_5_6_cube_388 0 (Rendering|Material|GetMaterial _figures_5_6_cube_388 0) "opacity" :!class /Script/Engine.PrimitiveComponent))
        (Rendering|Material|SetScalarParameterValue _returnvalue_9 "opacity" 0.25 :!class /Script/Engine.MaterialInstanceDynamic))
      (:then_9
        (bind _returnvalue_10 (Rendering|Material|CreateDynamicMaterialInstance _figures_5_6_cube_386 0 (Rendering|Material|GetMaterial _figures_5_6_cube_386 0) "opacity" :!class /Script/Engine.PrimitiveComponent))
        (Rendering|Material|SetScalarParameterValue _returnvalue_10 "opacity" 0.25 :!class /Script/Engine.MaterialInstanceDynamic))
      (:then_10
        (bind _returnvalue_11 (Rendering|Material|CreateDynamicMaterialInstance _figures_5_6_cube_387_2 0 (Rendering|Material|GetMaterial _figures_5_6_cube_387_2 0) "opacity" :!class /Script/Engine.PrimitiveComponent))
        (Rendering|Material|SetScalarParameterValue _returnvalue_11 "opacity" 0.25 :!class /Script/Engine.MaterialInstanceDynamic))
      (:then_11
        (bind _returnvalue_12 (Rendering|Material|CreateDynamicMaterialInstance _figures_5_6_cube_389_2 0 (Rendering|Material|GetMaterial _figures_5_6_cube_389_2 0) "opacity" :!class /Script/Engine.PrimitiveComponent))
        (Rendering|Material|SetScalarParameterValue _returnvalue_12 "opacity" 0.25 :!class /Script/Engine.MaterialInstanceDynamic))
      (:then_12
        (bind _returnvalue_13 (Rendering|Material|CreateDynamicMaterialInstance _figures_5_6_cube_402_2 0 (Rendering|Material|GetMaterial _figures_5_6_cube_402_2 0) "opacity" :!class /Script/Engine.PrimitiveComponent))
        (Rendering|Material|SetScalarParameterValue _returnvalue_13 "opacity" 0.25 :!class /Script/Engine.MaterialInstanceDynamic))
      (:then_13
        (bind _returnvalue_14 (Rendering|Material|CreateDynamicMaterialInstance _figures_5_6_cube_403_2 0 (Rendering|Material|GetMaterial _figures_5_6_cube_403_2 0) "opacity" :!class /Script/Engine.PrimitiveComponent))
        (Rendering|Material|SetScalarParameterValue _returnvalue_14 "opacity" 0.25 :!class /Script/Engine.MaterialInstanceDynamic))
      (:then_14
        (bind _returnvalue_15 (Rendering|Material|CreateDynamicMaterialInstance _figures_5_6_cube_404_2 0 (Rendering|Material|GetMaterial _figures_5_6_cube_404_2 0) "opacity" :!class /Script/Engine.PrimitiveComponent))
        (Rendering|Material|SetScalarParameterValue _returnvalue_15 "opacity" 0.25 :!class /Script/Engine.MaterialInstanceDynamic))
      (:then_15
        (bind _returnvalue_16 (Rendering|Material|CreateDynamicMaterialInstance _figures_5_6_cube_405_2 0 (Rendering|Material|GetMaterial _figures_5_6_cube_405_2 0) "opacity" :!class /Script/Engine.PrimitiveComponent))
        (Rendering|Material|SetScalarParameterValue _returnvalue_16 "opacity" 0.25 :!class /Script/Engine.MaterialInstanceDynamic))
      (:then_16
        (bind _returnvalue_17 (Rendering|Material|CreateDynamicMaterialInstance _figures_5_6_cube_401_2 0 (Rendering|Material|GetMaterial _figures_5_6_cube_401_2 0) "opacity" :!class /Script/Engine.PrimitiveComponent))
        (Rendering|Material|SetScalarParameterValue _returnvalue_17 "opacity" 0.25 :!class /Script/Engine.MaterialInstanceDynamic))
      (:then_17
        (bind _returnvalue_18 (Rendering|Material|CreateDynamicMaterialInstance _figures_5_6_cube_395_2 0 (Rendering|Material|GetMaterial _figures_5_6_cube_395_2 0) "opacity" :!class /Script/Engine.PrimitiveComponent))
        (Rendering|Material|SetScalarParameterValue _returnvalue_18 "opacity" 0.25 :!class /Script/Engine.MaterialInstanceDynamic))
      (:then_18
        (bind _returnvalue_19 (Rendering|Material|CreateDynamicMaterialInstance _figures_5_6_cube_396_2 0 (Rendering|Material|GetMaterial _figures_5_6_cube_396_2 0) "opacity" :!class /Script/Engine.PrimitiveComponent))
        (Rendering|Material|SetScalarParameterValue _returnvalue_19 "opacity" 0.25 :!class /Script/Engine.MaterialInstanceDynamic))
      (:then_19
        (bind _returnvalue_20 (Rendering|Material|CreateDynamicMaterialInstance _figures_5_6_cube_397_2 0 (Rendering|Material|GetMaterial _figures_5_6_cube_397_2 0) "opacity" :!class /Script/Engine.PrimitiveComponent))
        (Rendering|Material|SetScalarParameterValue _returnvalue_20 "opacity" 0.25 :!class /Script/Engine.MaterialInstanceDynamic))
      (:then_20
        (bind _returnvalue_21 (Rendering|Material|CreateDynamicMaterialInstance _figures_5_6_cube_398_2 0 (Rendering|Material|GetMaterial _figures_5_6_cube_398_2 0) "opacity" :!class /Script/Engine.PrimitiveComponent))
        (Rendering|Material|SetScalarParameterValue _returnvalue_21 "opacity" 0.25 :!class /Script/Engine.MaterialInstanceDynamic))
      (:then_21
        (bind _returnvalue_22 (Rendering|Material|CreateDynamicMaterialInstance _figures_5_6_cube_399_2 0 (Rendering|Material|GetMaterial _figures_5_6_cube_399_2 0) "opacity" :!class /Script/Engine.PrimitiveComponent))
        (Rendering|Material|SetScalarParameterValue _returnvalue_22 "opacity" 0.25 :!class /Script/Engine.MaterialInstanceDynamic))
      (:then_22
        (bind _returnvalue_23 (Rendering|Material|CreateDynamicMaterialInstance _figures_5_6_cube_400_2 0 (Rendering|Material|GetMaterial _figures_5_6_cube_400_2 0) "opacity" :!class /Script/Engine.PrimitiveComponent))
        (Rendering|Material|SetScalarParameterValue _returnvalue_23 "opacity" 0.25 :!class /Script/Engine.MaterialInstanceDynamic)))
    (else
      (Utilities|FlowControl|Sequence
        (:then_0
          (bind _returnvalue_24 (Rendering|Material|CreateDynamicMaterialInstance _figures_5_6_cube_382_2 0 (Rendering|Material|GetMaterial _figures_5_6_cube_382_2 0) "opacity" :!class /Script/Engine.PrimitiveComponent))
          (Rendering|Material|SetScalarParameterValue _returnvalue_24 "opacity" 0.0 :!class /Script/Engine.MaterialInstanceDynamic))
        (:then_1
          (bind _returnvalue_25 (Rendering|Material|CreateDynamicMaterialInstance _figures_5_6_cube_394 0 (Rendering|Material|GetMaterial _figures_5_6_cube_394 0) "opacity" :!class /Script/Engine.PrimitiveComponent))
          (Rendering|Material|SetScalarParameterValue _returnvalue_25 "opacity" 0.0 :!class /Script/Engine.MaterialInstanceDynamic))
        (:then_2
          (bind _returnvalue_26 (Rendering|Material|CreateDynamicMaterialInstance _figures_5_6_cube_390 0 (Rendering|Material|GetMaterial _figures_5_6_cube_390 0) "opacity" :!class /Script/Engine.PrimitiveComponent))
          (Rendering|Material|SetScalarParameterValue _returnvalue_26 "opacity" 0.0 :!class /Script/Engine.MaterialInstanceDynamic))
        (:then_3
          (bind _returnvalue_27 (Rendering|Material|CreateDynamicMaterialInstance _figures_5_6_cube_391 0 (Rendering|Material|GetMaterial _figures_5_6_cube_391 0) "opacity" :!class /Script/Engine.PrimitiveComponent))
          (Rendering|Material|SetScalarParameterValue _returnvalue_27 "opacity" 0.0 :!class /Script/Engine.MaterialInstanceDynamic))
        (:then_4
          (bind _returnvalue_28 (Rendering|Material|CreateDynamicMaterialInstance _figures_5_6_cube_392_2 0 (Rendering|Material|GetMaterial _figures_5_6_cube_392_2 0) "opacity" :!class /Script/Engine.PrimitiveComponent))
          (Rendering|Material|SetScalarParameterValue _returnvalue_28 "opacity" 0.0 :!class /Script/Engine.MaterialInstanceDynamic))
        (:then_5
          (bind _returnvalue_29 (Rendering|Material|CreateDynamicMaterialInstance _figures_5_6_cube_393_2 0 (Rendering|Material|GetMaterial _figures_5_6_cube_393_2 0) "opacity" :!class /Script/Engine.PrimitiveComponent))
          (Rendering|Material|SetScalarParameterValue _returnvalue_29 "opacity" 0.0 :!class /Script/Engine.MaterialInstanceDynamic))
        (:then_6
          (bind _returnvalue_30 (Rendering|Material|CreateDynamicMaterialInstance _figures_5_6_cube_384_2 0 (Rendering|Material|GetMaterial _figures_5_6_cube_384_2 0) "opacity" :!class /Script/Engine.PrimitiveComponent))
          (Rendering|Material|SetScalarParameterValue _returnvalue_30 "opacity" 0.0 :!class /Script/Engine.MaterialInstanceDynamic))
        (:then_7
          (bind _returnvalue_31 (Rendering|Material|CreateDynamicMaterialInstance _figures_5_6_cube_385_2 0 (Rendering|Material|GetMaterial _figures_5_6_cube_385_2 0) "opacity" :!class /Script/Engine.PrimitiveComponent))
          (Rendering|Material|SetScalarParameterValue _returnvalue_31 "opacity" 0.0 :!class /Script/Engine.MaterialInstanceDynamic))
        (:then_8
          (bind _returnvalue_32 (Rendering|Material|CreateDynamicMaterialInstance _figures_5_6_cube_388_2 0 (Rendering|Material|GetMaterial _figures_5_6_cube_388_2 0) "opacity" :!class /Script/Engine.PrimitiveComponent))
          (Rendering|Material|SetScalarParameterValue _returnvalue_32 "opacity" 0.0 :!class /Script/Engine.MaterialInstanceDynamic))
        (:then_9
          (bind _returnvalue_33 (Rendering|Material|CreateDynamicMaterialInstance _figures_5_6_cube_386_2 0 (Rendering|Material|GetMaterial _figures_5_6_cube_386_2 0) "opacity" :!class /Script/Engine.PrimitiveComponent))
          (Rendering|Material|SetScalarParameterValue _returnvalue_33 "opacity" 0.0 :!class /Script/Engine.MaterialInstanceDynamic))
        (:then_10
          (bind _returnvalue_34 (Rendering|Material|CreateDynamicMaterialInstance _figures_5_6_cube_387 0 (Rendering|Material|GetMaterial _figures_5_6_cube_387 0) "opacity" :!class /Script/Engine.PrimitiveComponent))
          (Rendering|Material|SetScalarParameterValue _returnvalue_34 "opacity" 0.0 :!class /Script/Engine.MaterialInstanceDynamic))
        (:then_11
          (bind _returnvalue_35 (Rendering|Material|CreateDynamicMaterialInstance _figures_5_6_cube_389 0 (Rendering|Material|GetMaterial _figures_5_6_cube_389 0) "opacity" :!class /Script/Engine.PrimitiveComponent))
          (Rendering|Material|SetScalarParameterValue _returnvalue_35 "opacity" 0.0 :!class /Script/Engine.MaterialInstanceDynamic))
        (:then_12
          (bind _returnvalue_36 (Rendering|Material|CreateDynamicMaterialInstance _figures_5_6_cube_402 0 (Rendering|Material|GetMaterial _figures_5_6_cube_402 0) "opacity" :!class /Script/Engine.PrimitiveComponent))
          (Rendering|Material|SetScalarParameterValue _returnvalue_36 "opacity" 0.0 :!class /Script/Engine.MaterialInstanceDynamic))
        (:then_13
          (bind _returnvalue_37 (Rendering|Material|CreateDynamicMaterialInstance _figures_5_6_cube_403 0 (Rendering|Material|GetMaterial _figures_5_6_cube_403 0) "opacity" :!class /Script/Engine.PrimitiveComponent))
          (Rendering|Material|SetScalarParameterValue _returnvalue_37 "opacity" 0.0 :!class /Script/Engine.MaterialInstanceDynamic))
        (:then_14
          (bind _returnvalue_38 (Rendering|Material|CreateDynamicMaterialInstance _figures_5_6_cube_404 0 (Rendering|Material|GetMaterial _figures_5_6_cube_404 0) "opacity" :!class /Script/Engine.PrimitiveComponent))
          (Rendering|Material|SetScalarParameterValue _returnvalue_38 "opacity" 0.0 :!class /Script/Engine.MaterialInstanceDynamic))
        (:then_15
          (bind _returnvalue_39 (Rendering|Material|CreateDynamicMaterialInstance _figures_5_6_cube_405 0 (Rendering|Material|GetMaterial _figures_5_6_cube_405 0) "opacity" :!class /Script/Engine.PrimitiveComponent))
          (Rendering|Material|SetScalarParameterValue _returnvalue_39 "opacity" 0.0 :!class /Script/Engine.MaterialInstanceDynamic))
        (:then_16
          (bind _returnvalue_40 (Rendering|Material|CreateDynamicMaterialInstance _figures_5_6_cube_401 0 (Rendering|Material|GetMaterial _figures_5_6_cube_401 0) "opacity" :!class /Script/Engine.PrimitiveComponent))
          (Rendering|Material|SetScalarParameterValue _returnvalue_40 "opacity" 0.0 :!class /Script/Engine.MaterialInstanceDynamic))
        (:then_17
          (bind _returnvalue_41 (Rendering|Material|CreateDynamicMaterialInstance _figures_5_6_cube_395 0 (Rendering|Material|GetMaterial _figures_5_6_cube_395 0) "opacity" :!class /Script/Engine.PrimitiveComponent))
          (Rendering|Material|SetScalarParameterValue _returnvalue_41 "opacity" 0.0 :!class /Script/Engine.MaterialInstanceDynamic))
        (:then_18
          (bind _returnvalue_42 (Rendering|Material|CreateDynamicMaterialInstance _figures_5_6_cube_396 0 (Rendering|Material|GetMaterial _figures_5_6_cube_396 0) "opacity" :!class /Script/Engine.PrimitiveComponent))
          (Rendering|Material|SetScalarParameterValue _returnvalue_42 "opacity" 0.0 :!class /Script/Engine.MaterialInstanceDynamic))
        (:then_19
          (bind _returnvalue_43 (Rendering|Material|CreateDynamicMaterialInstance _figures_5_6_cube_397 0 (Rendering|Material|GetMaterial _figures_5_6_cube_397 0) "opacity" :!class /Script/Engine.PrimitiveComponent))
          (Rendering|Material|SetScalarParameterValue _returnvalue_43 "opacity" 0.0 :!class /Script/Engine.MaterialInstanceDynamic))
        (:then_20
          (bind _returnvalue_44 (Rendering|Material|CreateDynamicMaterialInstance _figures_5_6_cube_398 0 (Rendering|Material|GetMaterial _figures_5_6_cube_398 0) "opacity" :!class /Script/Engine.PrimitiveComponent))
          (Rendering|Material|SetScalarParameterValue _returnvalue_44 "opacity" 0.0 :!class /Script/Engine.MaterialInstanceDynamic))
        (:then_21
          (bind _returnvalue_45 (Rendering|Material|CreateDynamicMaterialInstance _figures_5_6_cube_399 0 (Rendering|Material|GetMaterial _figures_5_6_cube_399 0) "opacity" :!class /Script/Engine.PrimitiveComponent))
          (Rendering|Material|SetScalarParameterValue _returnvalue_45 "opacity" 0.0 :!class /Script/Engine.MaterialInstanceDynamic))
        (:then_22
          (bind _returnvalue_46 (Rendering|Material|CreateDynamicMaterialInstance _figures_5_6_cube_400 0 (Rendering|Material|GetMaterial _figures_5_6_cube_400 0) "opacity" :!class /Script/Engine.PrimitiveComponent))
          (Rendering|Material|SetScalarParameterValue _returnvalue_46 "opacity" 0.0 :!class /Script/Engine.MaterialInstanceDynamic))))))