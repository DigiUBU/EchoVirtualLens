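; BP_Fig_5_3 is a selectable figure for round 5 of Lens01, chosen by attaching its connector anchor.
; Attaching sets Selected and, after a two-second delay, asks BP_GameManager_01 to validate the selection; detaching clears the overlay but leaves Selected set.
; SelectedOverlayColor sets opacity through dynamic material instances on each cube mesh.
; Older press-to-select logic, including overlay highlighting and sibling deselection, is disconnected.
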(event PressedSelect(Comp_Select)
  (params (Pawn :type BP%20Pawn%20Base%20Object%20Reference) (SourceActor :type Actor%20Object%20Reference) (ImpactLocation :type Vector :default "0, 0, 0") (ImpactComponent :type Actor%20Component%20Object%20Reference))
  ;[1 1 1] old
)

(event ConnectorAttached(Comp_Connector_Anchor)
  (params (Connector :type Comp%20Connector%20Object%20Reference) (AttachedToActor :type Actor%20Object%20Reference) (AttachedToComponent :type Scene%20Component%20Object%20Reference))
  ;[1 1 1] if it is ready to validate selection
  (Variables|Default|Setselected true)
  (bind _returnvalue (Actor|GetActorOfClass "/Game/Lens/Lens01/BP/BP_GameManager_01.BP_GameManager_01_C"))
  (Utilities|FlowControl|Delay 2.0)
  (if (Variables|Default|Getselected)
    (Default|ValidateSelection _returnvalue self 5)))

(event ConnectorDetached(Comp_Connector_Anchor)
  ;[1 1 1] if it is ready to validate selection
  (CallFunction|SelectedOverlayColor false))

(fn ConstructionScript)

(fn SelectedOverlayColor
  (params (select :type Boolean))
  (bind _figures_5_3_cube_034 (Variables|Default|Getfigures_5_3_Cube_034))
  (bind _figures_5_3_cube_021 (Variables|Default|Getfigures_5_3_Cube_021))
  (bind _figures_5_3_cube_022 (Variables|Default|Getfigures_5_3_Cube_022))
  (bind _figures_5_3_cube_023 (Variables|Default|Getfigures_5_3_Cube_023))
  (bind _figures_5_3_cube_025 (Variables|Default|Getfigures_5_3_Cube_025))
  (bind _figures_5_3_cube_019 (Variables|Default|Getfigures_5_3_Cube_019))
  (bind _figures_5_3_cube_012 (Variables|Default|Getfigures_5_3_Cube_012))
  (bind _figures_5_3_cube_014 (Variables|Default|Getfigures_5_3_Cube_014))
  (bind _figures_5_3_cube_015 (Variables|Default|Getfigures_5_3_Cube_015))
  (bind _figures_5_3_cube_018 (Variables|Default|Getfigures_5_3_Cube_018))
  (bind _figures_5_3_cube_016 (Variables|Default|Getfigures_5_3_Cube_016))
  (bind _figures_5_3_cube_017 (Variables|Default|Getfigures_5_3_Cube_017))
  (bind _figures_5_3_cube_020 (Variables|Default|Getfigures_5_3_Cube_020))
  (bind _figures_5_3_cube_035 (Variables|Default|Getfigures_5_3_Cube_035))
  (bind _figures_5_3_cube_033 (Variables|Default|Getfigures_5_3_Cube_033))
  (bind _figures_5_3_cube_036 (Variables|Default|Getfigures_5_3_Cube_036))
  (bind _figures_5_3_cube_307 (Variables|Default|Getfigures_5_3_Cube_307))
  (bind _figures_5_3_cube_026 (Variables|Default|Getfigures_5_3_Cube_026))
  (bind _figures_5_3_cube_032 (Variables|Default|Getfigures_5_3_Cube_032))
  (bind _figures_5_3_cube_027 (Variables|Default|Getfigures_5_3_Cube_027))
  (bind _figures_5_3_cube_028 (Variables|Default|Getfigures_5_3_Cube_028))
  (bind _figures_5_3_cube_029 (Variables|Default|Getfigures_5_3_Cube_029))
  (bind _figures_5_3_cube_030 (Variables|Default|Getfigures_5_3_Cube_030))
  (bind _figures_5_3_cube_031 (Variables|Default|Getfigures_5_3_Cube_031))
  (bind _figures_5_3_cube_034_2 (Variables|Default|Getfigures_5_3_Cube_034))
  (bind _figures_5_3_cube_021_2 (Variables|Default|Getfigures_5_3_Cube_021))
  (bind _figures_5_3_cube_022_2 (Variables|Default|Getfigures_5_3_Cube_022))
  (bind _figures_5_3_cube_023_2 (Variables|Default|Getfigures_5_3_Cube_023))
  (bind _figures_5_3_cube_025_2 (Variables|Default|Getfigures_5_3_Cube_025))
  (bind _figures_5_3_cube_019_2 (Variables|Default|Getfigures_5_3_Cube_019))
  (bind _figures_5_3_cube_012_2 (Variables|Default|Getfigures_5_3_Cube_012))
  (bind _figures_5_3_cube_014_2 (Variables|Default|Getfigures_5_3_Cube_014))
  (bind _figures_5_3_cube_015_2 (Variables|Default|Getfigures_5_3_Cube_015))
  (bind _figures_5_3_cube_018_2 (Variables|Default|Getfigures_5_3_Cube_018))
  (bind _figures_5_3_cube_016_2 (Variables|Default|Getfigures_5_3_Cube_016))
  (bind _figures_5_3_cube_017_2 (Variables|Default|Getfigures_5_3_Cube_017))
  (bind _figures_5_3_cube_020_2 (Variables|Default|Getfigures_5_3_Cube_020))
  (bind _figures_5_3_cube_035_2 (Variables|Default|Getfigures_5_3_Cube_035))
  (bind _figures_5_3_cube_033_2 (Variables|Default|Getfigures_5_3_Cube_033))
  (bind _figures_5_3_cube_036_2 (Variables|Default|Getfigures_5_3_Cube_036))
  (bind _figures_5_3_cube_307_2 (Variables|Default|Getfigures_5_3_Cube_307))
  (bind _figures_5_3_cube_026_2 (Variables|Default|Getfigures_5_3_Cube_026))
  (bind _figures_5_3_cube_032_2 (Variables|Default|Getfigures_5_3_Cube_032))
  (bind _figures_5_3_cube_027_2 (Variables|Default|Getfigures_5_3_Cube_027))
  (bind _figures_5_3_cube_028_2 (Variables|Default|Getfigures_5_3_Cube_028))
  (bind _figures_5_3_cube_029_2 (Variables|Default|Getfigures_5_3_Cube_029))
  (bind _figures_5_3_cube_030_2 (Variables|Default|Getfigures_5_3_Cube_030))
  (bind _figures_5_3_cube_031_2 (Variables|Default|Getfigures_5_3_Cube_031))
  (if select
    (Utilities|FlowControl|Sequence
      (:then_0
        (bind _returnvalue (Rendering|Material|CreateDynamicMaterialInstance _figures_5_3_cube_019_2 0 (Rendering|Material|GetMaterial _figures_5_3_cube_019_2 0) "opacity" :!class /Script/Engine.PrimitiveComponent))
        (Rendering|Material|SetScalarParameterValue _returnvalue "opacity" 0.25 :!class /Script/Engine.MaterialInstanceDynamic))
      (:then_1
        (bind _returnvalue_2 (Rendering|Material|CreateDynamicMaterialInstance _figures_5_3_cube_034_2 0 (Rendering|Material|GetMaterial _figures_5_3_cube_034_2 0) "opacity" :!class /Script/Engine.PrimitiveComponent))
        (Rendering|Material|SetScalarParameterValue _returnvalue_2 "opacity" 0.25 :!class /Script/Engine.MaterialInstanceDynamic))
      (:then_2
        (bind _returnvalue_3 (Rendering|Material|CreateDynamicMaterialInstance _figures_5_3_cube_021_2 0 (Rendering|Material|GetMaterial _figures_5_3_cube_021_2 0) "opacity" :!class /Script/Engine.PrimitiveComponent))
        (Rendering|Material|SetScalarParameterValue _returnvalue_3 "opacity" 0.25 :!class /Script/Engine.MaterialInstanceDynamic))
      (:then_3
        (bind _returnvalue_4 (Rendering|Material|CreateDynamicMaterialInstance _figures_5_3_cube_022_2 0 (Rendering|Material|GetMaterial _figures_5_3_cube_022_2 0) "opacity" :!class /Script/Engine.PrimitiveComponent))
        (Rendering|Material|SetScalarParameterValue _returnvalue_4 "opacity" 0.25 :!class /Script/Engine.MaterialInstanceDynamic))
      (:then_4
        (bind _returnvalue_5 (Rendering|Material|CreateDynamicMaterialInstance _figures_5_3_cube_023_2 0 (Rendering|Material|GetMaterial _figures_5_3_cube_023_2 0) "opacity" :!class /Script/Engine.PrimitiveComponent))
        (Rendering|Material|SetScalarParameterValue _returnvalue_5 "opacity" 0.25 :!class /Script/Engine.MaterialInstanceDynamic))
      (:then_5
        (bind _returnvalue_6 (Rendering|Material|CreateDynamicMaterialInstance _figures_5_3_cube_025_2 0 (Rendering|Material|GetMaterial _figures_5_3_cube_025_2 0) "opacity" :!class /Script/Engine.PrimitiveComponent))
        (Rendering|Material|SetScalarParameterValue _returnvalue_6 "opacity" 0.25 :!class /Script/Engine.MaterialInstanceDynamic))
      (:then_6
        (bind _returnvalue_7 (Rendering|Material|CreateDynamicMaterialInstance _figures_5_3_cube_012_2 0 (Rendering|Material|GetMaterial _figures_5_3_cube_012_2 0) "opacity" :!class /Script/Engine.PrimitiveComponent))
        (Rendering|Material|SetScalarParameterValue _returnvalue_7 "opacity" 0.25 :!class /Script/Engine.MaterialInstanceDynamic))
      (:then_7
        (bind _returnvalue_8 (Rendering|Material|CreateDynamicMaterialInstance _figures_5_3_cube_014_2 0 (Rendering|Material|GetMaterial _figures_5_3_cube_014_2 0) "opacity" :!class /Script/Engine.PrimitiveComponent))
        (Rendering|Material|SetScalarParameterValue _returnvalue_8 "opacity" 0.25 :!class /Script/Engine.MaterialInstanceDynamic))
      (:then_8
        (bind _returnvalue_9 (Rendering|Material|CreateDynamicMaterialInstance _figures_5_3_cube_015_2 0 (Rendering|Material|GetMaterial _figures_5_3_cube_015_2 0) "opacity" :!class /Script/Engine.PrimitiveComponent))
        (Rendering|Material|SetScalarParameterValue _returnvalue_9 "opacity" 0.25 :!class /Script/Engine.MaterialInstanceDynamic))
      (:then_9
        (bind _returnvalue_10 (Rendering|Material|CreateDynamicMaterialInstance _figures_5_3_cube_018_2 0 (Rendering|Material|GetMaterial _figures_5_3_cube_018_2 0) "opacity" :!class /Script/Engine.PrimitiveComponent))
        (Rendering|Material|SetScalarParameterValue _returnvalue_10 "opacity" 0.25 :!class /Script/Engine.MaterialInstanceDynamic))
      (:then_10
        (bind _returnvalue_11 (Rendering|Material|CreateDynamicMaterialInstance _figures_5_3_cube_016_2 0 (Rendering|Material|GetMaterial _figures_5_3_cube_016_2 0) "opacity" :!class /Script/Engine.PrimitiveComponent))
        (Rendering|Material|SetScalarParameterValue _returnvalue_11 "opacity" 0.25 :!class /Script/Engine.MaterialInstanceDynamic))
      (:then_11
        (bind _returnvalue_12 (Rendering|Material|CreateDynamicMaterialInstance _figures_5_3_cube_017_2 0 (Rendering|Material|GetMaterial _figures_5_3_cube_017_2 0) "opacity" :!class /Script/Engine.PrimitiveComponent))
        (Rendering|Material|SetScalarParameterValue _returnvalue_12 "opacity" 0.25 :!class /Script/Engine.MaterialInstanceDynamic))
      (:then_12
        (bind _returnvalue_13 (Rendering|Material|CreateDynamicMaterialInstance _figures_5_3_cube_020_2 0 (Rendering|Material|GetMaterial _figures_5_3_cube_020_2 0) "opacity" :!class /Script/Engine.PrimitiveComponent))
        (Rendering|Material|SetScalarParameterValue _returnvalue_13 "opacity" 0.25 :!class /Script/Engine.MaterialInstanceDynamic))
      (:then_13
        (bind _returnvalue_14 (Rendering|Material|CreateDynamicMaterialInstance _figures_5_3_cube_035_2 0 (Rendering|Material|GetMaterial _figures_5_3_cube_035_2 0) "opacity" :!class /Script/Engine.PrimitiveComponent))
        (Rendering|Material|SetScalarParameterValue _returnvalue_14 "opacity" 0.25 :!class /Script/Engine.MaterialInstanceDynamic))
      (:then_14
        (bind _returnvalue_15 (Rendering|Material|CreateDynamicMaterialInstance _figures_5_3_cube_033_2 0 (Rendering|Material|GetMaterial _figures_5_3_cube_033_2 0) "opacity" :!class /Script/Engine.PrimitiveComponent))
        (Rendering|Material|SetScalarParameterValue _returnvalue_15 "opacity" 0.25 :!class /Script/Engine.MaterialInstanceDynamic))
      (:then_15
        (bind _returnvalue_16 (Rendering|Material|CreateDynamicMaterialInstance _figures_5_3_cube_036_2 0 (Rendering|Material|GetMaterial _figures_5_3_cube_036_2 0) "opacity" :!class /Script/Engine.PrimitiveComponent))
        (Rendering|Material|SetScalarParameterValue _returnvalue_16 "opacity" 0.25 :!class /Script/Engine.MaterialInstanceDynamic))
      (:then_16
        (bind _returnvalue_17 (Rendering|Material|CreateDynamicMaterialInstance _figures_5_3_cube_307_2 0 (Rendering|Material|GetMaterial _figures_5_3_cube_307_2 0) "opacity" :!class /Script/Engine.PrimitiveComponent))
        (Rendering|Material|SetScalarParameterValue _returnvalue_17 "opacity" 0.25 :!class /Script/Engine.MaterialInstanceDynamic))
      (:then_17
        (bind _returnvalue_18 (Rendering|Material|CreateDynamicMaterialInstance _figures_5_3_cube_026_2 0 (Rendering|Material|GetMaterial _figures_5_3_cube_026_2 0) "opacity" :!class /Script/Engine.PrimitiveComponent))
        (Rendering|Material|SetScalarParameterValue _returnvalue_18 "opacity" 0.25 :!class /Script/Engine.MaterialInstanceDynamic))
      (:then_18
        (bind _returnvalue_19 (Rendering|Material|CreateDynamicMaterialInstance _figures_5_3_cube_032_2 0 (Rendering|Material|GetMaterial _figures_5_3_cube_032_2 0) "opacity" :!class /Script/Engine.PrimitiveComponent))
        (Rendering|Material|SetScalarParameterValue _returnvalue_19 "opacity" 0.25 :!class /Script/Engine.MaterialInstanceDynamic))
      (:then_19
        (bind _returnvalue_20 (Rendering|Material|CreateDynamicMaterialInstance _figures_5_3_cube_027_2 0 (Rendering|Material|GetMaterial _figures_5_3_cube_027_2 0) "opacity" :!class /Script/Engine.PrimitiveComponent))
        (Rendering|Material|SetScalarParameterValue _returnvalue_20 "opacity" 0.25 :!class /Script/Engine.MaterialInstanceDynamic))
      (:then_20
        (bind _returnvalue_21 (Rendering|Material|CreateDynamicMaterialInstance _figures_5_3_cube_028_2 0 (Rendering|Material|GetMaterial _figures_5_3_cube_028_2 0) "opacity" :!class /Script/Engine.PrimitiveComponent))
        (Rendering|Material|SetScalarParameterValue _returnvalue_21 "opacity" 0.25 :!class /Script/Engine.MaterialInstanceDynamic))
      (:then_21
        (bind _returnvalue_22 (Rendering|Material|CreateDynamicMaterialInstance _figures_5_3_cube_029_2 0 (Rendering|Material|GetMaterial _figures_5_3_cube_029_2 0) "opacity" :!class /Script/Engine.PrimitiveComponent))
        (Rendering|Material|SetScalarParameterValue _returnvalue_22 "opacity" 0.25 :!class /Script/Engine.MaterialInstanceDynamic))
      (:then_22
        (bind _returnvalue_23 (Rendering|Material|CreateDynamicMaterialInstance _figures_5_3_cube_030_2 0 (Rendering|Material|GetMaterial _figures_5_3_cube_030_2 0) "opacity" :!class /Script/Engine.PrimitiveComponent))
        (Rendering|Material|SetScalarParameterValue _returnvalue_23 "opacity" 0.25 :!class /Script/Engine.MaterialInstanceDynamic))
      (:then_23
        (bind _returnvalue_24 (Rendering|Material|CreateDynamicMaterialInstance _figures_5_3_cube_031_2 0 (Rendering|Material|GetMaterial _figures_5_3_cube_031_2 0) "opacity" :!class /Script/Engine.PrimitiveComponent))
        (Rendering|Material|SetScalarParameterValue _returnvalue_24 "opacity" 0.25 :!class /Script/Engine.MaterialInstanceDynamic)))
    (else
      (Utilities|FlowControl|Sequence
        (:then_0
          (bind _returnvalue_25 (Rendering|Material|CreateDynamicMaterialInstance _figures_5_3_cube_019 0 (Rendering|Material|GetMaterial _figures_5_3_cube_019 0) "opacity" :!class /Script/Engine.PrimitiveComponent))
          (Rendering|Material|SetScalarParameterValue _returnvalue_25 "opacity" 0.0 :!class /Script/Engine.MaterialInstanceDynamic))
        (:then_1
          (bind _returnvalue_26 (Rendering|Material|CreateDynamicMaterialInstance _figures_5_3_cube_034 0 (Rendering|Material|GetMaterial _figures_5_3_cube_034 0) "opacity" :!class /Script/Engine.PrimitiveComponent))
          (Rendering|Material|SetScalarParameterValue _returnvalue_26 "opacity" 0.0 :!class /Script/Engine.MaterialInstanceDynamic))
        (:then_2
          (bind _returnvalue_27 (Rendering|Material|CreateDynamicMaterialInstance _figures_5_3_cube_021 0 (Rendering|Material|GetMaterial _figures_5_3_cube_021 0) "opacity" :!class /Script/Engine.PrimitiveComponent))
          (Rendering|Material|SetScalarParameterValue _returnvalue_27 "opacity" 0.0 :!class /Script/Engine.MaterialInstanceDynamic))
        (:then_3
          (bind _returnvalue_28 (Rendering|Material|CreateDynamicMaterialInstance _figures_5_3_cube_022 0 (Rendering|Material|GetMaterial _figures_5_3_cube_022 0) "opacity" :!class /Script/Engine.PrimitiveComponent))
          (Rendering|Material|SetScalarParameterValue _returnvalue_28 "opacity" 0.0 :!class /Script/Engine.MaterialInstanceDynamic))
        (:then_4
          (bind _returnvalue_29 (Rendering|Material|CreateDynamicMaterialInstance _figures_5_3_cube_023 0 (Rendering|Material|GetMaterial _figures_5_3_cube_023 0) "opacity" :!class /Script/Engine.PrimitiveComponent))
          (Rendering|Material|SetScalarParameterValue _returnvalue_29 "opacity" 0.0 :!class /Script/Engine.MaterialInstanceDynamic))
        (:then_5
          (bind _returnvalue_30 (Rendering|Material|CreateDynamicMaterialInstance _figures_5_3_cube_025 0 (Rendering|Material|GetMaterial _figures_5_3_cube_025 0) "opacity" :!class /Script/Engine.PrimitiveComponent))
          (Rendering|Material|SetScalarParameterValue _returnvalue_30 "opacity" 0.0 :!class /Script/Engine.MaterialInstanceDynamic))
        (:then_6
          (bind _returnvalue_31 (Rendering|Material|CreateDynamicMaterialInstance _figures_5_3_cube_012 0 (Rendering|Material|GetMaterial _figures_5_3_cube_012 0) "opacity" :!class /Script/Engine.PrimitiveComponent))
          (Rendering|Material|SetScalarParameterValue _returnvalue_31 "opacity" 0.0 :!class /Script/Engine.MaterialInstanceDynamic))
        (:then_7
          (bind _returnvalue_32 (Rendering|Material|CreateDynamicMaterialInstance _figures_5_3_cube_014 0 (Rendering|Material|GetMaterial _figures_5_3_cube_014 0) "opacity" :!class /Script/Engine.PrimitiveComponent))
          (Rendering|Material|SetScalarParameterValue _returnvalue_32 "opacity" 0.0 :!class /Script/Engine.MaterialInstanceDynamic))
        (:then_8
          (bind _returnvalue_33 (Rendering|Material|CreateDynamicMaterialInstance _figures_5_3_cube_015 0 (Rendering|Material|GetMaterial _figures_5_3_cube_015 0) "opacity" :!class /Script/Engine.PrimitiveComponent))
          (Rendering|Material|SetScalarParameterValue _returnvalue_33 "opacity" 0.0 :!class /Script/Engine.MaterialInstanceDynamic))
        (:then_9
          (bind _returnvalue_34 (Rendering|Material|CreateDynamicMaterialInstance _figures_5_3_cube_018 0 (Rendering|Material|GetMaterial _figures_5_3_cube_018 0) "opacity" :!class /Script/Engine.PrimitiveComponent))
          (Rendering|Material|SetScalarParameterValue _returnvalue_34 "opacity" 0.0 :!class /Script/Engine.MaterialInstanceDynamic))
        (:then_10
          (bind _returnvalue_35 (Rendering|Material|CreateDynamicMaterialInstance _figures_5_3_cube_016 0 (Rendering|Material|GetMaterial _figures_5_3_cube_016 0) "opacity" :!class /Script/Engine.PrimitiveComponent))
          (Rendering|Material|SetScalarParameterValue _returnvalue_35 "opacity" 0.0 :!class /Script/Engine.MaterialInstanceDynamic))
        (:then_11
          (bind _returnvalue_36 (Rendering|Material|CreateDynamicMaterialInstance _figures_5_3_cube_017 0 (Rendering|Material|GetMaterial _figures_5_3_cube_017 0) "opacity" :!class /Script/Engine.PrimitiveComponent))
          (Rendering|Material|SetScalarParameterValue _returnvalue_36 "opacity" 0.0 :!class /Script/Engine.MaterialInstanceDynamic))
        (:then_12
          (bind _returnvalue_37 (Rendering|Material|CreateDynamicMaterialInstance _figures_5_3_cube_020 0 (Rendering|Material|GetMaterial _figures_5_3_cube_020 0) "opacity" :!class /Script/Engine.PrimitiveComponent))
          (Rendering|Material|SetScalarParameterValue _returnvalue_37 "opacity" 0.0 :!class /Script/Engine.MaterialInstanceDynamic))
        (:then_13
          (bind _returnvalue_38 (Rendering|Material|CreateDynamicMaterialInstance _figures_5_3_cube_035 0 (Rendering|Material|GetMaterial _figures_5_3_cube_035 0) "opacity" :!class /Script/Engine.PrimitiveComponent))
          (Rendering|Material|SetScalarParameterValue _returnvalue_38 "opacity" 0.0 :!class /Script/Engine.MaterialInstanceDynamic))
        (:then_14
          (bind _returnvalue_39 (Rendering|Material|CreateDynamicMaterialInstance _figures_5_3_cube_033 0 (Rendering|Material|GetMaterial _figures_5_3_cube_033 0) "opacity" :!class /Script/Engine.PrimitiveComponent))
          (Rendering|Material|SetScalarParameterValue _returnvalue_39 "opacity" 0.0 :!class /Script/Engine.MaterialInstanceDynamic))
        (:then_15
          (bind _returnvalue_40 (Rendering|Material|CreateDynamicMaterialInstance _figures_5_3_cube_036 0 (Rendering|Material|GetMaterial _figures_5_3_cube_036 0) "opacity" :!class /Script/Engine.PrimitiveComponent))
          (Rendering|Material|SetScalarParameterValue _returnvalue_40 "opacity" 0.0 :!class /Script/Engine.MaterialInstanceDynamic))
        (:then_16
          (bind _returnvalue_41 (Rendering|Material|CreateDynamicMaterialInstance _figures_5_3_cube_307 0 (Rendering|Material|GetMaterial _figures_5_3_cube_307 0) "opacity" :!class /Script/Engine.PrimitiveComponent))
          (Rendering|Material|SetScalarParameterValue _returnvalue_41 "opacity" 0.0 :!class /Script/Engine.MaterialInstanceDynamic))
        (:then_17
          (bind _returnvalue_42 (Rendering|Material|CreateDynamicMaterialInstance _figures_5_3_cube_026 0 (Rendering|Material|GetMaterial _figures_5_3_cube_026 0) "opacity" :!class /Script/Engine.PrimitiveComponent))
          (Rendering|Material|SetScalarParameterValue _returnvalue_42 "opacity" 0.0 :!class /Script/Engine.MaterialInstanceDynamic))
        (:then_18
          (bind _returnvalue_43 (Rendering|Material|CreateDynamicMaterialInstance _figures_5_3_cube_032 0 (Rendering|Material|GetMaterial _figures_5_3_cube_032 0) "opacity" :!class /Script/Engine.PrimitiveComponent))
          (Rendering|Material|SetScalarParameterValue _returnvalue_43 "opacity" 0.0 :!class /Script/Engine.MaterialInstanceDynamic))
        (:then_19
          (bind _returnvalue_44 (Rendering|Material|CreateDynamicMaterialInstance _figures_5_3_cube_027 0 (Rendering|Material|GetMaterial _figures_5_3_cube_027 0) "opacity" :!class /Script/Engine.PrimitiveComponent))
          (Rendering|Material|SetScalarParameterValue _returnvalue_44 "opacity" 0.0 :!class /Script/Engine.MaterialInstanceDynamic))
        (:then_20
          (bind _returnvalue_45 (Rendering|Material|CreateDynamicMaterialInstance _figures_5_3_cube_028 0 (Rendering|Material|GetMaterial _figures_5_3_cube_028 0) "opacity" :!class /Script/Engine.PrimitiveComponent))
          (Rendering|Material|SetScalarParameterValue _returnvalue_45 "opacity" 0.0 :!class /Script/Engine.MaterialInstanceDynamic))
        (:then_21
          (bind _returnvalue_46 (Rendering|Material|CreateDynamicMaterialInstance _figures_5_3_cube_029 0 (Rendering|Material|GetMaterial _figures_5_3_cube_029 0) "opacity" :!class /Script/Engine.PrimitiveComponent))
          (Rendering|Material|SetScalarParameterValue _returnvalue_46 "opacity" 0.0 :!class /Script/Engine.MaterialInstanceDynamic))
        (:then_22
          (bind _returnvalue_47 (Rendering|Material|CreateDynamicMaterialInstance _figures_5_3_cube_030 0 (Rendering|Material|GetMaterial _figures_5_3_cube_030 0) "opacity" :!class /Script/Engine.PrimitiveComponent))
          (Rendering|Material|SetScalarParameterValue _returnvalue_47 "opacity" 0.0 :!class /Script/Engine.MaterialInstanceDynamic))
        (:then_23
          (bind _returnvalue_48 (Rendering|Material|CreateDynamicMaterialInstance _figures_5_3_cube_031 0 (Rendering|Material|GetMaterial _figures_5_3_cube_031 0) "opacity" :!class /Script/Engine.PrimitiveComponent))
          (Rendering|Material|SetScalarParameterValue _returnvalue_48 "opacity" 0.0 :!class /Script/Engine.MaterialInstanceDynamic))))))