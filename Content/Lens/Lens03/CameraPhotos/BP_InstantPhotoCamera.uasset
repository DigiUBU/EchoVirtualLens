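; BP_InstantPhotoCamera is an in-game camera with four photo slots, saving shots and where the player stood.
; SavePhotos fills the first free slot by capturing its SceneCapture2D into a new render target, exporting a per-player PNG and freezing that capture.
; It records the VR or desktop pawn's transform alongside the Reel, then writes photo-and-transform strings to a timestamped text file.
; RemovePhoto clears a slot and restores its live capture.
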(fn ConstructionScript)

(fn TakePhoto01
  (bind _scenecapturecomponent2d01 (Variables|Default|GetSceneCaptureComponent2D01))
  ;[1 1 1] the first photo is taken and saved
  (bind _result (Math|Integer|IncrementInt (Variables|Default|GettimesPhotoTaken01))
    (:%20%20
      (bind _asbp_game_instance_main (Utilities|Casting|CastToBP_GameInstance_Main (Game|GetGameInstance)))
      (bind _returnvalue (Rendering|CreateRenderTarget2D 256 256 "RTF_RGBA8"))
      (bind _output_get (Variables|/Script/Engine.SceneCaptureComponent2D|SetTextureTarget _scenecapturecomponent2d01 _returnvalue))
      (Rendering|SceneCapture|CaptureScene _scenecapturecomponent2d01 :!class /Script/Engine.SceneCaptureComponent2D)
      (Rendering|ExportRenderTarget _output_get (Class|KismetSystemLibrary|GetProjectSavedDirectory) (Utilities|String|Append "photo_" (Variables|/Game/AFCore/Blueprints/Game/BP_GameInstance_Main.BP_GameInstance_Main_C|GetplayerName _asbp_game_instance_main) "_" "01" "_" (Utilities|String|ToString(Integer) _result) ".png"))
      (Variables|/Script/Engine.SceneCaptureComponent|SetbCaptureEveryFrame _scenecapturecomponent2d01 false)
      (Utilities|Array|Add (Variables|Default|Getreel) _returnvalue)
      (Variables|Default|SetphotoTaken01 true)
      (return true))))

(fn TakePhoto02
  (bind _scenecapturecomponent2d02 (Variables|Default|GetSceneCaptureComponent2D02))
  ;[1 1 1] the second photo is taken and saved
  (bind _result (Math|Integer|IncrementInt (Variables|Default|GettimesPhotoTaken02))
    (:%20%20
      (bind _asbp_game_instance_main (Utilities|Casting|CastToBP_GameInstance_Main (Game|GetGameInstance)))
      (bind _returnvalue (Rendering|CreateRenderTarget2D 256 256 "RTF_RGBA8"))
      (bind _output_get (Variables|/Script/Engine.SceneCaptureComponent2D|SetTextureTarget _scenecapturecomponent2d02 _returnvalue))
      (Rendering|SceneCapture|CaptureScene _scenecapturecomponent2d02 :!class /Script/Engine.SceneCaptureComponent2D)
      (Rendering|ExportRenderTarget _output_get (Class|KismetSystemLibrary|GetProjectSavedDirectory) (Utilities|String|Append "photo_" (Variables|/Game/AFCore/Blueprints/Game/BP_GameInstance_Main.BP_GameInstance_Main_C|GetplayerName _asbp_game_instance_main) "_" "02" "_" (Utilities|String|ToString(Integer) _result) ".png"))
      (Variables|/Script/Engine.SceneCaptureComponent|SetbCaptureEveryFrame _scenecapturecomponent2d02 false)
      (Utilities|Array|Add (Variables|Default|Getreel) _returnvalue)
      (Variables|Default|SetphotoTaken02 true)
      (return true))))

(fn TakePhoto03
  (bind _scenecapturecomponent2d03 (Variables|Default|GetSceneCaptureComponent2D03))
  ;[1 1 1] the third photo is taken and saved
  (bind _result (Math|Integer|IncrementInt (Variables|Default|GettimesPhotoTaken03))
    (:%20%20
      (bind _asbp_game_instance_main (Utilities|Casting|CastToBP_GameInstance_Main (Game|GetGameInstance)))
      (bind _returnvalue (Rendering|CreateRenderTarget2D 256 256 "RTF_RGBA8"))
      (bind _output_get (Variables|/Script/Engine.SceneCaptureComponent2D|SetTextureTarget _scenecapturecomponent2d03 _returnvalue))
      (Rendering|SceneCapture|CaptureScene _scenecapturecomponent2d03 :!class /Script/Engine.SceneCaptureComponent2D)
      (Rendering|ExportRenderTarget _output_get (Class|KismetSystemLibrary|GetProjectSavedDirectory) (Utilities|String|Append "photo_" (Variables|/Game/AFCore/Blueprints/Game/BP_GameInstance_Main.BP_GameInstance_Main_C|GetplayerName _asbp_game_instance_main) "_" "03" "_" (Utilities|String|ToString(Integer) _result) ".png"))
      (Variables|/Script/Engine.SceneCaptureComponent|SetbCaptureEveryFrame _scenecapturecomponent2d03 false)
      (Utilities|Array|Add (Variables|Default|Getreel) _returnvalue)
      (Variables|Default|SetphotoTaken03 true)
      (return true))))

(fn TakePhoto04
  (bind _scenecapturecomponent2d04 (Variables|Default|GetSceneCaptureComponent2D04))
  ;[1 1 1] the fourth photo is taken and saved
  (bind _result (Math|Integer|IncrementInt (Variables|Default|GettimesPhotoTaken04))
    (:%20%20
      (bind _asbp_game_instance_main (Utilities|Casting|CastToBP_GameInstance_Main (Game|GetGameInstance)))
      (bind _returnvalue (Rendering|CreateRenderTarget2D 256 256 "RTF_RGBA8"))
      (bind _output_get (Variables|/Script/Engine.SceneCaptureComponent2D|SetTextureTarget _scenecapturecomponent2d04 _returnvalue))
      (Rendering|SceneCapture|CaptureScene _scenecapturecomponent2d04 :!class /Script/Engine.SceneCaptureComponent2D)
      (Rendering|ExportRenderTarget _output_get (Class|KismetSystemLibrary|GetProjectSavedDirectory) (Utilities|String|Append "photo_" (Variables|/Game/AFCore/Blueprints/Game/BP_GameInstance_Main.BP_GameInstance_Main_C|GetplayerName _asbp_game_instance_main) "_" "04" "_" (Utilities|String|ToString(Integer) _result) ".png"))
      (Variables|/Script/Engine.SceneCaptureComponent|SetbCaptureEveryFrame _scenecapturecomponent2d04 false)
      (Utilities|Array|Add (Variables|Default|Getreel) _returnvalue)
      (Variables|Default|SetphotoTaken04 true)
      (return true))))

(fn SavePhotos
  ;[1 1 1] the photos are taken so now need to be saved
  (if (Variables|Default|GetphotoTaken01)
    (if (Variables|Default|GetphotoTaken02)
      (if (Variables|Default|GetphotoTaken03)
        (if (not (Variables|Default|GetphotoTaken04))
          (bind _phototaken (CallFunction|TakePhoto04))
          (bind _pawnlocrot (CallFunction|SaveLocationRotationPawn _phototaken))
          (bind _returnvalue (Utilities|Array|Add (Variables|Default|GetpawnLocRot) _pawnlocrot))
          (CallFunction|CollectDataOfTakenPhotos _returnvalue)
          (CallFunction|SaveDataOfTakenPhotos :!label _label))
        (else
          (bind _phototaken_2 (CallFunction|TakePhoto03))
          (bind _pawnlocrot_2 (CallFunction|SaveLocationRotationPawn _phototaken_2))
          (bind _returnvalue_2 (Utilities|Array|Add (Variables|Default|GetpawnLocRot) _pawnlocrot_2))
          (CallFunction|CollectDataOfTakenPhotos _returnvalue_2)
          (goto _label)))
      (else
        (bind _phototaken_3 (CallFunction|TakePhoto02))
        (bind _pawnlocrot_3 (CallFunction|SaveLocationRotationPawn _phototaken_3))
        (bind _returnvalue_3 (Utilities|Array|Add (Variables|Default|GetpawnLocRot) _pawnlocrot_3))
        (CallFunction|CollectDataOfTakenPhotos _returnvalue_3)
        (goto _label)))
    (else
      (bind _phototaken_4 (CallFunction|TakePhoto01))
      (bind _pawnlocrot_4 (CallFunction|SaveLocationRotationPawn _phototaken_4))
      (bind _returnvalue_4 (Utilities|Array|Add (Variables|Default|GetpawnLocRot) _pawnlocrot_4))
      (CallFunction|CollectDataOfTakenPhotos _returnvalue_4)
      (goto _label))))

(fn SaveLocationRotationPawn
  (params (readyToSave :type Boolean))
  (bind _returnvalue (Game|GetPlayerCharacter 0))
  ;[1 1 1] where is the photographer
  (if readyToSave
    (bind _asbp_pawn_vr_hands (Utilities|Casting|CastToBP_Pawn_VR_Hands _returnvalue)
      (:then
        (return (Math|Transform|MakeTransform (Transformation|GetActorLocation _asbp_pawn_vr_hands) (Transformation|GetActorRotation _asbp_pawn_vr_hands))))
      (:CastFailed
        (bind _asbp_pawn_desktop_hands (Utilities|Casting|CastToBP_Pawn_Desktop_Hands _returnvalue))
        (return (Math|Transform|MakeTransform (Transformation|GetActorLocation _asbp_pawn_desktop_hands) (Transformation|GetActorRotation _asbp_pawn_desktop_hands)))))))

(fn ClearPhoto
  (params (index :type Integer))
  ;[1 1 1] when the photo is removed, need to update the indexes of the arrays
  (Utilities|Array|RemoveIndex (Variables|Default|Getreel) index)
  (Utilities|Array|RemoveIndex (Variables|Default|GetpawnLocRot) index))

(fn RemovePhoto
  (params (photoToRemove :type Integer))
  (bind _scenecapturecomponent2d01 (Variables|Default|GetSceneCaptureComponent2D01))
  (bind _scenecapturecomponent2d02 (Variables|Default|GetSceneCaptureComponent2D02))
  (bind _scenecapturecomponent2d03 (Variables|Default|GetSceneCaptureComponent2D03))
  (bind _scenecapturecomponent2d04 (Variables|Default|GetSceneCaptureComponent2D04))
  ;[1 1 1] update arrays and variables
  (switch int photoToRemove
    (:0
      (CallFunction|ClearPhoto photoToRemove)
      (Variables|Default|SetphotoTaken01 false)
      (Variables|/Script/Engine.SceneCaptureComponent|SetbCaptureEveryFrame _scenecapturecomponent2d01 true)
      (Variables|/Script/Engine.SceneCaptureComponent2D|SetTextureTarget _scenecapturecomponent2d01 "/Game/Lens/Lens03/CameraPhotos/Texture_Photos/RT_InstantPhoto01.RT_InstantPhoto01"))
    (:1
      (CallFunction|ClearPhoto photoToRemove)
      (Variables|Default|SetphotoTaken02 false)
      (Variables|/Script/Engine.SceneCaptureComponent|SetbCaptureEveryFrame _scenecapturecomponent2d02 true)
      (Variables|/Script/Engine.SceneCaptureComponent2D|SetTextureTarget _scenecapturecomponent2d02 "/Game/Lens/Lens03/CameraPhotos/Texture_Photos/RT_InstantPhoto01.RT_InstantPhoto01"))
    (:2
      (CallFunction|ClearPhoto photoToRemove)
      (Variables|Default|SetphotoTaken03 false)
      (Variables|/Script/Engine.SceneCaptureComponent|SetbCaptureEveryFrame _scenecapturecomponent2d03 true)
      (Variables|/Script/Engine.SceneCaptureComponent2D|SetTextureTarget _scenecapturecomponent2d03 "/Game/Lens/Lens03/CameraPhotos/Texture_Photos/RT_InstantPhoto01.RT_InstantPhoto01"))
    (:3
      (CallFunction|ClearPhoto photoToRemove)
      (Variables|Default|SetphotoTaken04 false)
      (Variables|/Script/Engine.SceneCaptureComponent|SetbCaptureEveryFrame _scenecapturecomponent2d04 true)
      (Variables|/Script/Engine.SceneCaptureComponent2D|SetTextureTarget _scenecapturecomponent2d04 "/Game/Lens/Lens03/CameraPhotos/Texture_Photos/RT_InstantPhoto01.RT_InstantPhoto01"))))

(fn CollectDataOfTakenPhotos
  (params (index :type Integer))
  ;[1 1 1] saves data to string array
  (for (_array_element _array_index) (Variables|Default|Getreel)
    (if (== _array_index index)
      (Utilities|Array|Add (Variables|Default|GetphotoTakenANDpawnLocRot) (Utilities|GetDisplayName _array_element))
      (for (_array_element_2 _array_index_2) (Variables|Default|GetpawnLocRot)
        (if (== _array_index_2 index)
          (Utilities|Array|Add (Variables|Default|GetphotoTakenANDpawnLocRot) (Utilities|String|ToString(Transform) _array_element_2)))))))

(fn SaveDataOfTakenPhotos
  (bind _returnvalue (Math|DateTime|Now))
  ;[1 1 1] saves the data of the photographer
  (bind _asbp_game_instance_main (Utilities|Casting|CastToBP_GameInstance_Main (Game|GetGameInstance)))
  (Class|VictoryBPFunctionLibrary|FileIOSaveStringArraytoFile (Class|KismetSystemLibrary|GetProjectSavedDirectory) (Utilities|String|Append "EVL_" (Utilities|String|ToString(Integer) (.year _returnvalue)) (Utilities|String|ToString(Integer) (.month _returnvalue)) (Utilities|String|ToString(Integer) (.day _returnvalue)) (Utilities|String|ToString(Integer) (.hour _returnvalue)) (Utilities|String|ToString(Integer) (.minute _returnvalue)) (Utilities|String|ToString(Integer) (.second _returnvalue)) "_DataPhotoWhereTook_" (Variables|/Game/AFCore/Blueprints/Game/BP_GameInstance_Main.BP_GameInstance_Main_C|GetplayerName _asbp_game_instance_main) ".txt") (Variables|Default|GetphotoTakenANDpawnLocRot) true true))