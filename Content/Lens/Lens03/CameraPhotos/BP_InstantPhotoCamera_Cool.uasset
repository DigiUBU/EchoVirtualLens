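; Four-shot instant photo camera for the Lens03 level that captures photos and records where and when each is taken.
; Each TakePhoto event freezes its own SceneCapture2D into a new render target in Reel, while RemovePhoto restores that slot's live preview.
; Outside the tutorial, SavePhotos reports camera transform and time to BP_GameManager_03 and builds a string log.
; PNG export, text-file saving and HTTP upload are disconnected.
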(event Custom|TakePhoto4
  (bind _scenecapturecomponent2d04 (Variables|Default|GetSceneCaptureComponent2D04))
  ;[1 1 1] the fourth photo is taken and saved
  (bind _result (Math|Integer|IncrementInt (Variables|Default|GettimesPhotoTaken04))
    (:%20%20
      (bind _asbp_game_instance_main (Utilities|Casting|CastToBP_GameInstance_Main (Game|GetGameInstance)))
      (bind _returnvalue (Rendering|CreateRenderTarget2D 256 256 "RTF_RGBA8"))
      (Utilities|FlowControl|Delay 0.01)
      (Rendering|SceneCapture|CaptureScene _scenecapturecomponent2d04 :!class /Script/Engine.SceneCaptureComponent2D)
      (bind _output_get (Variables|/Script/Engine.SceneCaptureComponent2D|SetTextureTarget _scenecapturecomponent2d04 _returnvalue))
      (Utilities|FlowControl|Delay 0.01)
      (bind _returnvalue_2 (Actor|GetActorOfClass "/Script/TheVirtualCode.HttpSenderActor"))
      (Variables|/Script/Engine.SceneCaptureComponent|SetbCaptureEveryFrame _scenecapturecomponent2d04 false)
      (Utilities|Array|SetArrayElem (Variables|Default|Getreel) 3 _returnvalue true)
      (Variables|Default|SetphotoTaken04 true)
      (CallFunction|SavePhotos 4))))

(event Custom|TakePhoto3
  (bind _scenecapturecomponent2d03 (Variables|Default|GetSceneCaptureComponent2D03))
  ;[1 1 1] the third photo is taken and saved
  (bind _result (Math|Integer|IncrementInt (Variables|Default|GettimesPhotoTaken03))
    (:%20%20
      (bind _asbp_game_instance_main (Utilities|Casting|CastToBP_GameInstance_Main (Game|GetGameInstance)))
      (bind _returnvalue (Rendering|CreateRenderTarget2D 256 256 "RTF_RGBA8"))
      (Utilities|FlowControl|Delay 0.01)
      (Rendering|SceneCapture|CaptureScene _scenecapturecomponent2d03 :!class /Script/Engine.SceneCaptureComponent2D)
      (bind _output_get (Variables|/Script/Engine.SceneCaptureComponent2D|SetTextureTarget _scenecapturecomponent2d03 _returnvalue))
      (Utilities|FlowControl|Delay 0.01)
      (bind _returnvalue_2 (Actor|GetActorOfClass "/Script/TheVirtualCode.HttpSenderActor"))
      (Variables|/Script/Engine.SceneCaptureComponent|SetbCaptureEveryFrame _scenecapturecomponent2d03 false)
      (Utilities|Array|SetArrayElem (Variables|Default|Getreel) 2 _returnvalue true)
      (Variables|Default|SetphotoTaken03 true)
      (CallFunction|SavePhotos 3))))

(event Custom|TakePhoto1
  (bind _scenecapturecomponent2d01 (Variables|Default|GetSceneCaptureComponent2D01))
  ;[1 1 1] the first photo is taken and saved
  (bind _result (Math|Integer|IncrementInt (Variables|Default|GettimesPhotoTaken01))
    (:%20%20
      (bind _asbp_game_instance_main (Utilities|Casting|CastToBP_GameInstance_Main (Game|GetGameInstance)))
      (bind _returnvalue (Rendering|CreateRenderTarget2D 256 256 "RTF_RGBA8"))
      (Utilities|FlowControl|Delay 0.01)
      (Rendering|SceneCapture|CaptureScene _scenecapturecomponent2d01 :!class /Script/Engine.SceneCaptureComponent2D)
      (bind _output_get (Variables|/Script/Engine.SceneCaptureComponent2D|SetTextureTarget _scenecapturecomponent2d01 _returnvalue))
      (Utilities|FlowControl|Delay 0.01)
      (bind _returnvalue_2 (Actor|GetActorOfClass "/Script/TheVirtualCode.HttpSenderActor"))
      (Variables|/Script/Engine.SceneCaptureComponent|SetbCaptureEveryFrame _scenecapturecomponent2d01 false)
      (Utilities|Array|SetArrayElem (Variables|Default|Getreel) 0 _returnvalue true)
      (Variables|Default|SetphotoTaken01 true)
      (CallFunction|SavePhotos 1))))

(event Custom|TakePhoto2
  (bind _scenecapturecomponent2d02 (Variables|Default|GetSceneCaptureComponent2D02))
  ;[1 1 1] the second photo is taken and saved
  (bind _result (Math|Integer|IncrementInt (Variables|Default|GettimesPhotoTaken02))
    (:%20%20
      (bind _asbp_game_instance_main (Utilities|Casting|CastToBP_GameInstance_Main (Game|GetGameInstance)))
      (bind _returnvalue (Rendering|CreateRenderTarget2D 256 256 "RTF_RGBA8"))
      (Utilities|FlowControl|Delay 0.01)
      (Rendering|SceneCapture|CaptureScene _scenecapturecomponent2d02 :!class /Script/Engine.SceneCaptureComponent2D)
      (bind _output_get (Variables|/Script/Engine.SceneCaptureComponent2D|SetTextureTarget _scenecapturecomponent2d02 _returnvalue))
      (Utilities|FlowControl|Delay 0.01)
      (bind _returnvalue_2 (Actor|GetActorOfClass "/Script/TheVirtualCode.HttpSenderActor"))
      (Variables|/Script/Engine.SceneCaptureComponent|SetbCaptureEveryFrame _scenecapturecomponent2d02 false)
      (Utilities|Array|SetArrayElem (Variables|Default|Getreel) 1 _returnvalue true)
      (Variables|Default|SetphotoTaken02 true)
      (CallFunction|SavePhotos 2))))

(fn ConstructionScript)

(fn SaveLocationRotationPawn
  (params (readyToSave :type Boolean))
  (bind _returnvalue (Game|GetPlayerCharacter 0))
  ;[1 1 1] the location of the pawn is saved
  (if readyToSave
    (bind _asbp_pawn_vr_hands (Utilities|Casting|CastToBP_Pawn_VR_Hands _returnvalue)
      (:then
        (return (Math|Transform|MakeTransform (Transformation|GetActorLocation _asbp_pawn_vr_hands) (Transformation|GetActorRotation _asbp_pawn_vr_hands))))
      (:CastFailed
        (bind _asbp_pawn_desktop_hands (Utilities|Casting|CastToBP_Pawn_Desktop_Hands _returnvalue))
        (return (Math|Transform|MakeTransform (Transformation|GetActorLocation _asbp_pawn_desktop_hands) (Transformation|GetActorRotation _asbp_pawn_desktop_hands)))))))

(fn SavePhotos
  (params (photo :type Integer))
  (bind _returnvalue (Class|Actor|GetLevel))
  (bind _infolevels (CallFunction|GetInfoLevels _returnvalue))
  (bind _returnvalue_2 (Utilities|GetDisplayName _infolevels))
  ;[1 1 1] save photos but not from the tutorial level
  (switch int photo
    (:1
      (if (Utilities|Enum|NotEqual(Enum) _returnvalue_2 "DA_Lens_Tutorial")
        ;[1 1 1] photos are saved ans data collected
        (Variables|Default|SetcaptureTime (Utilities|Time|GetGameTimeinSeconds))
        (bind _pawnlocrot (CallFunction|SaveLocationRotationCamera true))
        (bind _returnvalue_3 (Utilities|Array|Add (Variables|Default|GetpawnLocRot) _pawnlocrot))
        (bind _returnvalue_4 (Actor|GetActorOfClass "/Game/Lens/Lens03/BP/BP_GameManager_03.BP_GameManager_03_C"))
        (Default|PhotoTaken _returnvalue_4 (.Location (Math|Transform|BreakTransform _pawnlocrot)) (.Rotation (Math|Transform|BreakTransform _pawnlocrot)) (Variables|Default|GetcaptureTime))
        (CallFunction|CollectDataOfTakenPhotos _returnvalue_3 (Variables|Default|GetcaptureTime))
        (CallFunction|SaveDataOfTakenPhotos :!label _label)))
    (:2
      (if (Utilities|Enum|NotEqual(Enum) _returnvalue_2 "DA_Lens_Tutorial")
        (Variables|Default|SetcaptureTime (Utilities|Time|GetGameTimeinSeconds))
        (bind _pawnlocrot_2 (CallFunction|SaveLocationRotationCamera true))
        (bind _returnvalue_5 (Utilities|Array|Add (Variables|Default|GetpawnLocRot) _pawnlocrot_2))
        (bind _returnvalue_6 (Actor|GetActorOfClass "/Game/Lens/Lens03/BP/BP_GameManager_03.BP_GameManager_03_C"))
        (Default|PhotoTaken _returnvalue_6 (.Location (Math|Transform|BreakTransform _pawnlocrot_2)) (.Rotation (Math|Transform|BreakTransform _pawnlocrot_2)) (Variables|Default|GetcaptureTime))
        (CallFunction|CollectDataOfTakenPhotos _returnvalue_5 (Variables|Default|GetcaptureTime))
        (goto _label)))
    (:3
      (if (Utilities|Enum|NotEqual(Enum) _returnvalue_2 "DA_Lens_Tutorial")
        (Variables|Default|SetcaptureTime (Utilities|Time|GetGameTimeinSeconds))
        (bind _pawnlocrot_3 (CallFunction|SaveLocationRotationCamera true))
        (bind _returnvalue_7 (Utilities|Array|Add (Variables|Default|GetpawnLocRot) _pawnlocrot_3))
        (bind _returnvalue_8 (Actor|GetActorOfClass "/Game/Lens/Lens03/BP/BP_GameManager_03.BP_GameManager_03_C"))
        (Default|PhotoTaken _returnvalue_8 (.Location (Math|Transform|BreakTransform _pawnlocrot_3)) (.Rotation (Math|Transform|BreakTransform _pawnlocrot_3)) (Variables|Default|GetcaptureTime))
        (CallFunction|CollectDataOfTakenPhotos _returnvalue_7 (Variables|Default|GetcaptureTime))
        (goto _label)))
    (:4
      (if (Utilities|Enum|NotEqual(Enum) _returnvalue_2 "DA_Lens_Tutorial")
        (Variables|Default|SetcaptureTime (Utilities|Time|GetGameTimeinSeconds))
        (bind _pawnlocrot_4 (CallFunction|SaveLocationRotationCamera true))
        (bind _returnvalue_9 (Utilities|Array|Add (Variables|Default|GetpawnLocRot) _pawnlocrot_4))
        (bind _returnvalue_10 (Actor|GetActorOfClass "/Game/Lens/Lens03/BP/BP_GameManager_03.BP_GameManager_03_C"))
        (Default|PhotoTaken _returnvalue_10 (.Location (Math|Transform|BreakTransform _pawnlocrot_4)) (.Rotation (Math|Transform|BreakTransform _pawnlocrot_4)) (Variables|Default|GetcaptureTime))
        (CallFunction|CollectDataOfTakenPhotos _returnvalue_9 (Variables|Default|GetcaptureTime))
        (goto _label)))))

(fn ClearPhoto
  (params (index :type Integer))
  ;[1 1 1] arrays are cleared
  (Utilities|Array|SetArrayElem (Variables|Default|Getreel) index (Variables|Default|GettextureRenderNone))
  (Utilities|Array|SetArrayElem :TargetArray (Variables|Default|GetpawnLocRot) :Index index))

(fn RemovePhoto
  (params (photoToRemove :type Integer))
  (bind _scenecapturecomponent2d01 (Variables|Default|GetSceneCaptureComponent2D01))
  (bind _scenecapturecomponent2d02 (Variables|Default|GetSceneCaptureComponent2D02))
  (bind _scenecapturecomponent2d03 (Variables|Default|GetSceneCaptureComponent2D03))
  (bind _scenecapturecomponent2d04 (Variables|Default|GetSceneCaptureComponent2D04))
  ;[1 1 1] to remove a photo and reset variables
  (switch int photoToRemove
    (:0
      (CallFunction|ClearPhoto photoToRemove)
      (Variables|Default|SetphotoTaken01 false)
      (Variables|/Script/Engine.SceneCaptureComponent|SetbCaptureEveryFrame _scenecapturecomponent2d01 true)
      (Variables|/Script/Engine.SceneCaptureComponent2D|SetTextureTarget _scenecapturecomponent2d01 "/Game/Lens/Lens03/CameraPhotos/Texture_Photos/RT_InstantPhoto01.RT_InstantPhoto01"))
    (:1
      (CallFunction|ClearPhoto photoToRemove)
      (Variables|Default|SetphotoTaken02 false)
      (Variables|/Script/Engine.SceneCaptureComponent|SetbCaptureEveryFrame _scenecapturecomponent2d02 true)
      (Variables|/Script/Engine.SceneCaptureComponent2D|SetTextureTarget _scenecapturecomponent2d02 "/Game/Lens/Lens03/CameraPhotos/Texture_Photos/RT_InstantPhoto02.RT_InstantPhoto02"))
    (:2
      (CallFunction|ClearPhoto photoToRemove)
      (Variables|Default|SetphotoTaken03 false)
      (Variables|/Script/Engine.SceneCaptureComponent|SetbCaptureEveryFrame _scenecapturecomponent2d03 true)
      (Variables|/Script/Engine.SceneCaptureComponent2D|SetTextureTarget _scenecapturecomponent2d03 "/Game/Lens/Lens03/CameraPhotos/Texture_Photos/RT_InstantPhoto03.RT_InstantPhoto03"))
    (:3
      (CallFunction|ClearPhoto photoToRemove)
      (Variables|Default|SetphotoTaken04 false)
      (Variables|/Script/Engine.SceneCaptureComponent|SetbCaptureEveryFrame _scenecapturecomponent2d04 true)
      (Variables|/Script/Engine.SceneCaptureComponent2D|SetTextureTarget _scenecapturecomponent2d04 "/Game/Lens/Lens03/CameraPhotos/Texture_Photos/RT_InstantPhoto04.RT_InstantPhoto04"))))

(fn CollectDataOfTakenPhotos
  (params (index :type Integer) (captureTime :type Float%20%28double-precision%29))
  (bind _phototakenandpawnlocrot (Variables|Default|GetphotoTakenANDpawnLocRot))
  ;[1 1 1] prepare data to save from where the photos were taken
  (for (_array_element _array_index) (Variables|Default|Getreel)
    (if (== _array_index index)
      (Utilities|Array|Add (Variables|Default|GetphotoTakenANDpawnLocRot) (Utilities|GetDisplayName _array_element))
      (for (_array_element_2 _array_index_2) (Variables|Default|GetpawnLocRot)
        (if (== _array_index_2 index)
          (Utilities|Array|Add _phototakenandpawnlocrot (Utilities|String|ToString(Transform) _array_element_2))
          (Utilities|Array|Add _phototakenandpawnlocrot (Utilities|String|Append "Time: " (Utilities|String|ToString(Float) captureTime))))))))

(fn SaveDataOfTakenPhotos
  ;[1 1 1] save data in txt
)

(fn SaveLocationRotationCamera
  (params (readyToSave :type Boolean))
  (bind _camera (Variables|Default|GetCamera))
  ;[1 1 1] save data of the position of the camera
  (if readyToSave
    (return (Math|Transform|MakeTransform (Transformation|GetWorldLocation _camera) (Transformation|GetWorldRotation _camera)))))