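; Feedback actor that compares current and previous score and time, then picks a performance message for the player.
; CalculatePerformance computes percentage changes with a divide-by-zero guard and writes them to its UI_FeedbackMessage widget through SetScore and SetTime.
; Strong-threshold tests select one of five outcomes, returning a random phrase of three from DT_FeedbackMessages.
; Positive time change counts as improvement despite a comment calling it slower; the minor-threshold check has no effect.
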(event EventBeginPlay)

(event Collision|EventActorBeginOverlap
  (params (OtherActor :type Actor%20Object%20Reference)))

(event EventTick
  (params (DeltaSeconds :type Float%20%28single-precision%29)))

(fn ConstructionScript)

(fn SetScore
  ;[1 1 1] sets the score performance
  (return (Utilities|Text|ToText(String) (Utilities|String|Append (Utilities|String|ToString(Text) (Utilities|Text|MakeLiteralText "Score: ")) (Utilities|String|ToString(Text) (Utilities|Text|ToText(Float) (Variables|Default|GetscoreEvol) "HalfToEven" false true 1 324 2 2)) "%"))))

(fn SetTime
  ;[1 1 1] sets time performance
  (return (Utilities|Text|ToText(String) (Utilities|String|Append (Utilities|String|ToString(Text) (Utilities|Text|MakeLiteralText "Time: ")) (Utilities|String|ToString(Text) (Utilities|Text|ToText(Float) (Variables|Default|GettimeEvol) "HalfToEven" false true 1 324 2 2)) "%"))))

(fn CalculatePerformance
  (params (scoreCurrent :type Float%20%28double-precision%29) (scorePrevious :type Float%20%28double-precision%29) (timeCurrent :type Float%20%28double-precision%29) (timePrevious :type Float%20%28double-precision%29))
  (bind _returnvalue (Math|Float|Max(Float) timePrevious 0.0001))
  (bind _returnvalue_2 (Math|Float|Max(Float) scorePrevious 0.1))
  (bind _returnvalue_3 (- timeCurrent timePrevious))
  (bind _returnvalue_4 (- scoreCurrent scorePrevious))
  (bind _returnvalue_5 (/ _returnvalue_3 _returnvalue))
  (bind _returnvalue_6 (/ _returnvalue_4 _returnvalue_2))
  (bind _returnvalue_7 (* _returnvalue_5 1e+02))
  (bind _returnvalue_8 (* _returnvalue_6 1e+02))
  ;[1 1 1] if score thrshold is positive, there is improvement, in contrast if time threshold is positive, the performance has been slower
  (Variables|Default|SetscoreDelta _returnvalue_8)
  (Variables|Default|SettimeDelta _returnvalue_7)
  (bind _asui_feedback_message (Utilities|Casting|CastToUI_FeedbackMessage (UserInterface|GetWidget (Variables|Default|GetWidget))))
  (Variables|Default|SetscoreEvol _returnvalue_8)
  (Variables|Default|SettimeEvol _returnvalue_7)
  (bind _score (CallFunction|SetScore))
  (bind _time (CallFunction|SetTime))
  (Variables|/Script/UMG.TextBlock|SetText (Variables|/Game/Lens/BluePrints/Widgets/UI_FeedbackMessage.UI_FeedbackMessage_C|GetfeedbackMessage_time _asui_feedback_message) _time)
  (Variables|/Script/UMG.TextBlock|SetText (Variables|/Game/Lens/BluePrints/Widgets/UI_FeedbackMessage.UI_FeedbackMessage_C|GetfeedbackMessage_score _asui_feedback_message) _score)
  ;[1 1 1] if both improve
  (if (and (>= (Variables|Default|GetscoreDelta) (Variables|Default|GetthresholdStrong)) (>= (Variables|Default|GettimeDelta) (Variables|Default|GetthresholdStrong)))
    ;[1 1 1] from a data table the feedback message is established
    (switch int (Math|Random|RandomIntegerinRange 1 3)
      (:1
        (bind _outrownames (DataTable|GetDataTableRowNames (Variables|Default|Getdatatable)))
        (for _array_element _outrownames
          (bind _returnvalue_9 (Utilities|GetDataTableRow "/Game/Lens/BluePrints/DA_Structs/DT_FeedbackMessages.DT_FeedbackMessages" _array_element)
            (:then
              (if (== _array_element "improve2_1")
                (return (.phrase _returnvalue_9)))))))
      (:2
        (bind _outrownames_2 (DataTable|GetDataTableRowNames (Variables|Default|Getdatatable)))
        (for _array_element_2 _outrownames_2
          (bind _returnvalue_10 (Utilities|GetDataTableRow "/Game/Lens/BluePrints/DA_Structs/DT_FeedbackMessages.DT_FeedbackMessages" _array_element_2)
            (:then
              (if (== _array_element_2 "improve2_2")
                (return (.phrase _returnvalue_10)))))))
      (:3
        (bind _outrownames_3 (DataTable|GetDataTableRowNames (Variables|Default|Getdatatable)))
        (for _array_element_3 _outrownames_3
          (bind _returnvalue_11 (Utilities|GetDataTableRow "/Game/Lens/BluePrints/DA_Structs/DT_FeedbackMessages.DT_FeedbackMessages" _array_element_3)
            (:then
              (if (== _array_element_3 "improve2_3")
                (return (.phrase _returnvalue_11))))))))
    (else
      ;[1 1 1] if score is improved, but time not
      (if (and (>= (Variables|Default|GetscoreDelta) (Variables|Default|GetthresholdStrong)) (<= (Variables|Default|GettimeDelta) (.Negative (Utilities|ValueandNegative (Variables|Default|GetthresholdStrong)))))
        ;[1 1 1] from a data table the feedback message is established
        (switch int (Math|Random|RandomIntegerinRange 1 3)
          (:1
            (bind _outrownames_4 (DataTable|GetDataTableRowNames (Variables|Default|Getdatatable)))
            (for _array_element_4 _outrownames_4
              (bind _returnvalue_12 (Utilities|GetDataTableRow "/Game/Lens/BluePrints/DA_Structs/DT_FeedbackMessages.DT_FeedbackMessages" _array_element_4)
                (:then
                  (if (== _array_element_4 "score_1")
                    (return (.phrase _returnvalue_12)))))))
          (:2
            (bind _outrownames_5 (DataTable|GetDataTableRowNames (Variables|Default|Getdatatable)))
            (for _array_element_5 _outrownames_5
              (bind _returnvalue_13 (Utilities|GetDataTableRow "/Game/Lens/BluePrints/DA_Structs/DT_FeedbackMessages.DT_FeedbackMessages" _array_element_5)
                (:then
                  (if (== _array_element_5 "score_2")
                    (return (.phrase _returnvalue_13)))))))
          (:3
            (bind _outrownames_6 (DataTable|GetDataTableRowNames (Variables|Default|Getdatatable)))
            (for _array_element_6 _outrownames_6
              (bind _returnvalue_14 (Utilities|GetDataTableRow "/Game/Lens/BluePrints/DA_Structs/DT_FeedbackMessages.DT_FeedbackMessages" _array_element_6)
                (:then
                  (if (== _array_element_6 "score_3")
                    (return (.phrase _returnvalue_14))))))))
        (else
          ;[1 1 1] if time is improved, but score not
          (if (and (>= (Variables|Default|GettimeDelta) (Variables|Default|GetthresholdStrong)) (<= (Variables|Default|GetscoreDelta) (.Negative (Utilities|ValueandNegative (Variables|Default|GetthresholdStrong)))))
            ;[1 1 1] from a data table the feedback message is established
            (switch int (Math|Random|RandomIntegerinRange 1 3)
              (:1
                (bind _outrownames_7 (DataTable|GetDataTableRowNames (Variables|Default|Getdatatable)))
                (for _array_element_7 _outrownames_7
                  (bind _returnvalue_15 (Utilities|GetDataTableRow "/Game/Lens/BluePrints/DA_Structs/DT_FeedbackMessages.DT_FeedbackMessages" _array_element_7)
                    (:then
                      (if (== _array_element_7 "time_1")
                        (return (.phrase _returnvalue_15)))))))
              (:2
                (bind _outrownames_8 (DataTable|GetDataTableRowNames (Variables|Default|Getdatatable)))
                (for _array_element_8 _outrownames_8
                  (bind _returnvalue_16 (Utilities|GetDataTableRow "/Game/Lens/BluePrints/DA_Structs/DT_FeedbackMessages.DT_FeedbackMessages" _array_element_8)
                    (:then
                      (if (== _array_element_8 "time_2")
                        (return (.phrase _returnvalue_16)))))))
              (:3
                (bind _outrownames_9 (DataTable|GetDataTableRowNames (Variables|Default|Getdatatable)))
                (for _array_element_9 _outrownames_9
                  (bind _returnvalue_17 (Utilities|GetDataTableRow "/Game/Lens/BluePrints/DA_Structs/DT_FeedbackMessages.DT_FeedbackMessages" _array_element_9)
                    (:then
                      (if (== _array_element_9 "time_3")
                        (return (.phrase _returnvalue_17))))))))
            (else
              ;[1 1 1] anyone is improved
              (if (and (<= (Variables|Default|GettimeDelta) (.Negative (Utilities|ValueandNegative (Variables|Default|GetthresholdStrong)))) (<= (Variables|Default|GetscoreDelta) (.Negative (Utilities|ValueandNegative (Variables|Default|GetthresholdStrong)))))
                ;[1 1 1] from a data table the feedback message is established
                (switch int (Math|Random|RandomIntegerinRange 1 3)
                  (:1
                    (bind _outrownames_10 (DataTable|GetDataTableRowNames (Variables|Default|Getdatatable)))
                    (for _array_element_10 _outrownames_10
                      (bind _returnvalue_18 (Utilities|GetDataTableRow "/Game/Lens/BluePrints/DA_Structs/DT_FeedbackMessages.DT_FeedbackMessages" _array_element_10)
                        (:then
                          (if (== _array_element_10 "worse_1")
                            (return (.phrase _returnvalue_18)))))))
                  (:2
                    (bind _outrownames_11 (DataTable|GetDataTableRowNames (Variables|Default|Getdatatable)))
                    (for _array_element_11 _outrownames_11
                      (bind _returnvalue_19 (Utilities|GetDataTableRow "/Game/Lens/BluePrints/DA_Structs/DT_FeedbackMessages.DT_FeedbackMessages" _array_element_11)
                        (:then
                          (if (== _array_element_11 "worse_2")
                            (return (.phrase _returnvalue_19)))))))
                  (:3
                    (bind _outrownames_12 (DataTable|GetDataTableRowNames (Variables|Default|Getdatatable)))
                    (for _array_element_12 _outrownames_12
                      (bind _returnvalue_20 (Utilities|GetDataTableRow "/Game/Lens/BluePrints/DA_Structs/DT_FeedbackMessages.DT_FeedbackMessages" _array_element_12)
                        (:then
                          (if (== _array_element_12 "worse_3")
                            (return (.phrase _returnvalue_20))))))))
                (else
                  ;[1 1 1] the improvement or orsening are not significative in any case
                  (if (and (<= (Math|Float|Absolute(Float) (Variables|Default|GetscoreDelta)) (Variables|Default|GetthresholdMinor)) (<= (Math|Float|Absolute(Float) (Variables|Default|GettimeDelta)) (Variables|Default|GetthresholdMinor)))
                    _
                    (else
                      _))
                  ;[1 1 1] from a data table the feedback message is established
                  (switch int (Math|Random|RandomIntegerinRange 1 3)
                    (:1
                      (bind _outrownames_13 (DataTable|GetDataTableRowNames (Variables|Default|Getdatatable)))
                      (for _array_element_13 _outrownames_13
                        (bind _returnvalue_21 (Utilities|GetDataTableRow "/Game/Lens/BluePrints/DA_Structs/DT_FeedbackMessages.DT_FeedbackMessages" _array_element_13)
                          (:then
                            (if (== _array_element_13 "neutral_1")
                              (return (.phrase _returnvalue_21)))))))
                    (:2
                      (bind _outrownames_14 (DataTable|GetDataTableRowNames (Variables|Default|Getdatatable)))
                      (for _array_element_14 _outrownames_14
                        (bind _returnvalue_22 (Utilities|GetDataTableRow "/Game/Lens/BluePrints/DA_Structs/DT_FeedbackMessages.DT_FeedbackMessages" _array_element_14)
                          (:then
                            (if (== _array_element_14 "neutral_2")
                              (return (.phrase _returnvalue_22)))))))
                    (:3
                      (bind _outrownames_15 (DataTable|GetDataTableRowNames (Variables|Default|Getdatatable)))
                      (for _array_element_15 _outrownames_15
                        (bind _returnvalue_23 (Utilities|GetDataTableRow "/Game/Lens/BluePrints/DA_Structs/DT_FeedbackMessages.DT_FeedbackMessages" _array_element_15)
                          (:then
                            (if (== _array_element_15 "neutral_3")
                              (return (.phrase _returnvalue_23)))))))))))))))))