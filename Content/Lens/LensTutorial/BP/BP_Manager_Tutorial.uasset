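; Tutorial level manager for the Lens game that tracks three tasks: grabbing the phone, attaching the cube and taking a photo.
; Tick polls each task's actor, ticking its checklist box and playing a one-time sound.
; Completion clears polaroids, saves eye-tracking data, fades music and switches level; SaveData is an empty stub, so round stats are never written.
; GiveHint has the robot speak successive hints and counts their use.
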(event Custom|PhoneGrabbed
  ;[1 1 1] if phone is grabbed, check box is ticked
  (bind _returnvalue (Actor|GetActorOfClass "/Game/Lens/Lens03/Figures/BP/BP_Phone.BP_Phone_C"))
  (if (Default|IsBeingGrabbed (Variables|/Game/Lens/Lens03/Figures/BP/BP_Phone.BP_Phone_C|GetComp_Grab _returnvalue))
    (Variables|Default|SetisGrabbed true)
    (Utilities|FlowControl|Sequence
      (:then_0
        (bind _returnvalue_2 (Actor|GetActorOfClass "/Game/Lens/LensTutorial/BP/BP_Tutorial_Instructions.BP_Tutorial_Instructions_C"))
        (bind _asui_tutorial (Utilities|Casting|CastToUI_Tutorial (UserInterface|GetWidget (Variables|/Game/Lens/LensTutorial/BP/BP_Tutorial_Instructions.BP_Tutorial_Instructions_C|GetWidget _returnvalue_2))))
        (Class|CheckBox|SetCheckedState (Variables|/Game/Lens/LensTutorial/Widget/UI_Tutorial.UI_Tutorial_C|GetCheckBox_0 _asui_tutorial) "Checked"))
      (:then_1
        (Utilities|FlowControl|DoOnce false
          (:Completed
            (Audio|PlaySound2D "/Game/Lens/Sounds/evl_correct.evl_correct" 1.0 1.0 0.0 0 0)))))))

(event Custom|PhotoTaken
  ;[1 1 1] if photo is taken, check box is ticked
  (bind _returnvalue (Actor|GetActorOfClass "/Game/Lens/Lens03/CameraPhotos/BP_InstantPhotoCamera_Cool.BP_InstantPhotoCamera_Cool_C"))
  (if (Math|Boolean|ORBoolean (Variables|/Game/Lens/Lens03/CameraPhotos/BP_InstantPhotoCamera_Cool.BP_InstantPhotoCamera_Cool_C|GetphotoTaken01 _returnvalue) (Variables|/Game/Lens/Lens03/CameraPhotos/BP_InstantPhotoCamera_Cool.BP_InstantPhotoCamera_Cool_C|GetphotoTaken02 _returnvalue) (Variables|/Game/Lens/Lens03/CameraPhotos/BP_InstantPhotoCamera_Cool.BP_InstantPhotoCamera_Cool_C|GetphotoTaken03 _returnvalue) (Variables|/Game/Lens/Lens03/CameraPhotos/BP_InstantPhotoCamera_Cool.BP_InstantPhotoCamera_Cool_C|GetphotoTaken04 _returnvalue))
    (Variables|Default|SetisPhoto true)
    (Utilities|FlowControl|Sequence
      (:then_0
        (bind _returnvalue_2 (Actor|GetActorOfClass "/Game/Lens/LensTutorial/BP/BP_Tutorial_Instructions.BP_Tutorial_Instructions_C"))
        (bind _asui_tutorial (Utilities|Casting|CastToUI_Tutorial (UserInterface|GetWidget (Variables|/Game/Lens/LensTutorial/BP/BP_Tutorial_Instructions.BP_Tutorial_Instructions_C|GetWidget _returnvalue_2))))
        (Class|CheckBox|SetCheckedState (Variables|/Game/Lens/LensTutorial/Widget/UI_Tutorial.UI_Tutorial_C|GetCheckBox_2 _asui_tutorial) "Checked"))
      (:then_1
        (Utilities|FlowControl|DoOnce false
          (:Completed
            (Audio|PlaySound2D "/Game/Lens/Sounds/evl_correct.evl_correct" 1.0 1.0 0.0 0 0)))))))

(event Custom|CubeAttached
  ;[1 1 1] if cube is attached, check box is ticked
  (bind _returnvalue (Actor|GetActorOfClass "/Game/Lens/LensTutorial/BP/BP_AttachingCubes.BP_AttachingCubes_C"))
  (if (Variables|/Game/AFCore/Blueprints/Components/Snapping/Comp_Anchor.Comp_Anchor_C|GetOccupied (Variables|/Game/Lens/LensTutorial/BP/BP_AttachingCubes.BP_AttachingCubes_C|GetComp_Anchor _returnvalue))
    (Variables|Default|SetisAttached true)
    (Utilities|FlowControl|Sequence
      (:then_0
        (bind _returnvalue_2 (Actor|GetActorOfClass "/Game/Lens/LensTutorial/BP/BP_Tutorial_Instructions.BP_Tutorial_Instructions_C"))
        (bind _asui_tutorial (Utilities|Casting|CastToUI_Tutorial (UserInterface|GetWidget (Variables|/Game/Lens/LensTutorial/BP/BP_Tutorial_Instructions.BP_Tutorial_Instructions_C|GetWidget _returnvalue_2))))
        (Class|CheckBox|SetCheckedState (Variables|/Game/Lens/LensTutorial/Widget/UI_Tutorial.UI_Tutorial_C|GetCheckBox _asui_tutorial) "Checked"))
      (:then_1
        (Utilities|FlowControl|DoOnce false
          (:Completed
            (Audio|PlaySound2D "/Game/Lens/Sounds/evl_correct.evl_correct" 1.0 1.0 0.0 0 0)))))))

(event Custom|GiveHint
  (bind _hints (Variables|Default|Gethints))
  (bind _hintnum (Variables|Default|GethintNum))
  ;[1 1 1] to give hint
  (bind _returnvalue (Actor|GetActorOfClass "/Game/Lens/BluePrints/BP/BP_Clue.BP_Clue_C"))
  (Rendering|SetActorHiddenInGame _returnvalue true)
  (Math|Integer|IncrementInt (Variables|Default|GethintsUsed)
    (:%20%20
      (if (>= _hintnum (Utilities|Array|Length _hints))
        (bind _returnvalue_2 (Actor|GetActorOfClass "/Game/Coding/Character_PitXY/pitxy_v2/animations/C_PitXY_v5.C_PitXY_v5_C"))
        (Default|IsTalking _returnvalue_2 true "I do not have more clues" 5.0)
        (Utilities|FlowControl|Delay 5.0)
        (else
          (bind _returnvalue_3 (Actor|GetActorOfClass "/Game/Coding/Character_PitXY/pitxy_v2/animations/C_PitXY_v5.C_PitXY_v5_C"))
          (Default|IsTalking _returnvalue_3 true (.hinttext (Utilities|Array|Get(acopy) _hints _hintnum)) 5.0)
          (Math|Integer|IncrementInt (Variables|Default|GethintNum)
            (:%20%20
              (Utilities|FlowControl|Delay 5.0)
              (bind _returnvalue_4 (Actor|GetActorOfClass "/Game/Lens/BluePrints/BP/BP_Clue.BP_Clue_C"))
              (bind _asui_clue (Utilities|Casting|CastToUI_Clue (UserInterface|GetWidget (Variables|/Game/Lens/BluePrints/BP/BP_Clue.BP_Clue_C|GetWidget _returnvalue_4))))
              (Widget|SetVisibility _asui_clue "Visible")
              (bind _returnvalue_5 (Actor|GetActorOfClass "/Game/Lens/BluePrints/BP/BP_Clue.BP_Clue_C"))
              (Collision|SetActorEnableCollision _returnvalue_5 true))))))))

(event Custom|StopMusic
  (bind _musicref (Variables|Default|GetmusicRef))
  ;[1 1 1] stops the ambient sound music
  (Audio|Components|Audio|FadeOut _musicref 2.0 0.0 "Linear" :!class /Script/Engine.AudioComponent)
  (Utilities|FlowControl|Delay 2.0)
  (Audio|Components|Audio|Stop _musicref))

(event EventBeginPlay
  ;[1 1 1] time is saved
  (Utilities|FlowControl|Sequence
    (:then_0
      (Variables|Default|SettimeStart (Utilities|Time|GetGameTimeinSeconds)))
    (:then_1
      ;[1 1 1] music starts playing
      (Utilities|FlowControl|Delay 2.0)
      (bind _returnvalue (Audio|SpawnSound2D (Variables|Default|GetlevelMusic) 1.0 1.0 0.0 0 false false))
      (bind _output_get (Variables|Default|SetmusicRef _returnvalue))
      (Audio|Components|Audio|FadeIn _output_get 5.0 1.0 0.0 "Linear" :!class /Script/Engine.AudioComponent))))

(event EventTick
  (params (DeltaSeconds :type Float%20%28single-precision%29))
  (bind _returnvalue (Utilities|Time|GetGameTimeinSeconds))
  (bind _timestart (Variables|Default|GettimeStart))
  (bind _duration (Utilities|Duration _timestart _returnvalue))
  ;[1 1 1] evaluates if tutorial is completed
  (Utilities|FlowControl|Sequence
    (:then_0
      (CallFunction|PhoneGrabbed))
    (:then_1
      (CallFunction|CubeAttached))
    (:then_2
      (CallFunction|PhotoTaken))
    (:then_3
      (if (Math|Boolean|ANDBoolean (Variables|Default|GetisGrabbed) (Variables|Default|GetisAttached) (Variables|Default|GetisPhoto))
        (bind _returnvalue_2 (Actor|GetActorOfClass "/Game/Lens/BluePrints/BP/BP_Clue.BP_Clue_C"))
        (Rendering|SetActorHiddenInGame _returnvalue_2 true)
        (Utilities|FlowControl|Delay 5.0)
        ;[1 1 1] prepares everything for the next level
        (Utilities|FlowControl|DoOnce false
          (:Completed
            (bind _returnvalue_3 (Actor|GetActorOfClass "/Game/Lens/Lens03/BP/BP_GameManager_03.BP_GameManager_03_C"))
            (bind _asbp_game_instance_main (Utilities|Casting|CastToBP_GameInstance_Main (Game|GetGameInstance)))
            (bind _returnvalue_4 (Actor|GetActorOfClass "/Game/Lens/Lens03/CameraPhotos/BP_PaperBin.BP_PaperBin_C"))
            (Default|DestroyPolaroid _returnvalue_4 (Variables|/Game/Lens/Lens03/BP/BP_GameManager_03.BP_GameManager_03_C|Getphoto_2 _returnvalue_3))
            (Default|DestroyPolaroid _returnvalue_4 (Variables|/Game/Lens/Lens03/BP/BP_GameManager_03.BP_GameManager_03_C|Getphoto_3 _returnvalue_3))
            (Default|DestroyPolaroid _returnvalue_4 (Variables|/Game/Lens/Lens03/BP/BP_GameManager_03.BP_GameManager_03_C|Getphoto_4 _returnvalue_3))
            (Default|DestroyPolaroid _returnvalue_4 (Variables|/Game/Lens/Lens03/BP/BP_GameManager_03.BP_GameManager_03_C|Getphoto_1 _returnvalue_3))
            (bind _returnvalue_5 (Actor|GetActorOfClass "/Game/Lens/BluePrints/BP/BP_Data.BP_Data_C"))
            (bind _filename (Default|SaveEyeTrackingData _returnvalue_5))
            (Variables|Default|SettutorialTime _duration)
            (Utilities|Array|Add (Variables|Default|GetdataToSave) (Utilities|String|Append "Player: " (Variables|/Game/AFCore/Blueprints/Game/BP_GameInstance_Main.BP_GameInstance_Main_C|GetplayerName _asbp_game_instance_main) " 
Duration: " (Utilities|String|ToString(Float) _duration) " 
Clues: " (Utilities|String|ToString(Integer) (Variables|Default|GethintsUsed))))
            (CallFunction|SaveData)
            (Utilities|FlowControl|Delay 1.0)
            (Utilities|FlowControl|Delay 1.0)
            (CallFunction|StopMusic)
            (bind _asbp_game_instance_main_2 (Utilities|Casting|CastToBP_GameInstance_Main (Game|GetGameInstance)))
            (Default|SwitchLevel _asbp_game_instance_main_2 "/Game/Lens/DA_Lens_001.DA_Lens_001" false false)))))))

(fn ConstructionScript)

(fn SaveData
  ;[1 1 1] save the data of the round performance
)