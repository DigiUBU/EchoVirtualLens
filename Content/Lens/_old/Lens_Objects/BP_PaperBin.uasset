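; Paper bin that discards polaroid photos dropped into its box trigger.
; On overlap, it matches the actor's display name to one of four polaroid slots and calls RemovePhoto with that index on the BP_InstantPhotoCamera_Cool found in the level.
; The polaroid is hidden with collision disabled rather than destroyed.
; Leftover nodes that remove render targets from the camera's Reel are disconnected and never run.
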(event OnComponentBeginOverlap(Box)
  (params (OverlappedComponent :type Primitive%20Component%20Object%20Reference) (OtherActor :type Actor%20Object%20Reference) (OtherComp :type Primitive%20Component%20Object%20Reference) (OtherBodyIndex :type Integer) (bFromSweep :type Boolean) (SweepResult :type Hit%20Result%20Structure%20%28by%20ref%29))
  (CallFunction|DestroyPolaroid OtherActor))

(event Custom|DestroyPolaroid
  (params (object :type Actor%20Object%20Reference))
  (switch string (Utilities|GetDisplayName object)
    (:BP_Polaroid01
      (bind _returnvalue (Actor|GetActorOfClass "/Game/Lens/_old/Lens_Objects/BP_InstantPhotoCamera_Cool.BP_InstantPhotoCamera_Cool_C"))
      (Default|RemovePhoto _returnvalue))
    (:BP_Polaroid02
      (bind _returnvalue_2 (Actor|GetActorOfClass "/Game/Lens/_old/Lens_Objects/BP_InstantPhotoCamera_Cool.BP_InstantPhotoCamera_Cool_C"))
      (Default|RemovePhoto _returnvalue_2 1))
    (:BP_Polaroid03
      (bind _returnvalue_3 (Actor|GetActorOfClass "/Game/Lens/_old/Lens_Objects/BP_InstantPhotoCamera_Cool.BP_InstantPhotoCamera_Cool_C"))
      (Default|RemovePhoto _returnvalue_3 2))
    (:BP_Polaroid04
      (bind _returnvalue_4 (Actor|GetActorOfClass "/Game/Lens/_old/Lens_Objects/BP_InstantPhotoCamera_Cool.BP_InstantPhotoCamera_Cool_C"))
      (Default|RemovePhoto _returnvalue_4 3)))
  (Rendering|SetActorHiddenInGame object true)
  (Collision|SetActorEnableCollision object false))

(fn ConstructionScript)