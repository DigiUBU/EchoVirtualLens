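; Shutter button for the instant photo camera, allowing up to four photos, each paired with its own polaroid actor.
; On BeginPlay it hides the four polaroids and disables their grab and collision.
; Each press checks the camera's PhotoTaken flags, triggers the next TakePhoto, and reveals the matching polaroid, scaled down and grabbable, at the camera's Arrow.
; The switch toggles itself back after a short delay; photo-clearing nodes are left unconnected.
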(event OnStateChanged(Comp_Switch)
  (params (SourceInfo :type Struct%20Component%20Source%20Info%20Structure) (Value :type Boolean))
  ;[1 1 1] takes a photo and prepares for the next one
  (if Value
    (Utilities|FlowControl|Sequence
      (:then_0
        (bind _returnvalue (Actor|GetActorOfClass "/Game/Lens/Lens03/CameraPhotos/BP_InstantPhotoCamera_Cool.BP_InstantPhotoCamera_Cool_C"))
        (if (Variables|/Game/Lens/Lens03/CameraPhotos/BP_InstantPhotoCamera_Cool.BP_InstantPhotoCamera_Cool_C|GetphotoTaken01 _returnvalue)
          (if (Variables|/Game/Lens/Lens03/CameraPhotos/BP_InstantPhotoCamera_Cool.BP_InstantPhotoCamera_Cool_C|GetphotoTaken02 _returnvalue)
            (if (Variables|/Game/Lens/Lens03/CameraPhotos/BP_InstantPhotoCamera_Cool.BP_InstantPhotoCamera_Cool_C|GetphotoTaken03 _returnvalue)
              (if (not (Variables|/Game/Lens/Lens03/CameraPhotos/BP_InstantPhotoCamera_Cool.BP_InstantPhotoCamera_Cool_C|GetphotoTaken04 _returnvalue))
                (Default|TakePhoto04 _returnvalue)
                (bind _returnvalue_2 (Actor|GetActorOfClass "/Game/Lens/Lens03/CameraPhotos/BP_Polaroid04.BP_Polaroid04_C"))
                (Rendering|SetActorHiddenInGame _returnvalue_2 false)
                (bind _returnvalue_3 (Actor|GetActorOfClass "/Game/Lens/Lens03/CameraPhotos/BP_InstantPhotoCamera_Cool.BP_InstantPhotoCamera_Cool_C"))
                (Transformation|SetActorTransform _returnvalue_2 (Math|Transform|MakeTransform (.location (Transformation|GetWorldTransform (Variables|/Game/Lens/Lens03/CameraPhotos/BP_InstantPhotoCamera_Cool.BP_InstantPhotoCamera_Cool_C|GetArrow _returnvalue_3))) (.rotation (Transformation|GetWorldTransform (Variables|/Game/Lens/Lens03/CameraPhotos/BP_InstantPhotoCamera_Cool.BP_InstantPhotoCamera_Cool_C|GetArrow _returnvalue_3))) "0.065000,0.065000,0.065000"))
                (Default|SetGrabEnabled (Variables|/Game/Lens/Lens03/CameraPhotos/BP_Polaroid04.BP_Polaroid04_C|GetComp_Grab _returnvalue_2) true)
                (Collision|SetActorEnableCollision _returnvalue_2 true))
              (else
                (Default|TakePhoto03 _returnvalue)
                (bind _returnvalue_4 (Actor|GetActorOfClass "/Game/Lens/Lens03/CameraPhotos/BP_Polaroid03.BP_Polaroid03_C"))
                (Rendering|SetActorHiddenInGame _returnvalue_4 false)
                (bind _returnvalue_5 (Actor|GetActorOfClass "/Game/Lens/Lens03/CameraPhotos/BP_InstantPhotoCamera_Cool.BP_InstantPhotoCamera_Cool_C"))
                (Transformation|SetActorTransform _returnvalue_4 (Math|Transform|MakeTransform (.location (Transformation|GetWorldTransform (Variables|/Game/Lens/Lens03/CameraPhotos/BP_InstantPhotoCamera_Cool.BP_InstantPhotoCamera_Cool_C|GetArrow _returnvalue_5))) (.rotation (Transformation|GetWorldTransform (Variables|/Game/Lens/Lens03/CameraPhotos/BP_InstantPhotoCamera_Cool.BP_InstantPhotoCamera_Cool_C|GetArrow _returnvalue_5))) "0.065000,0.065000,0.065000"))
                (Default|SetGrabEnabled (Variables|/Game/Lens/Lens03/CameraPhotos/BP_Polaroid03.BP_Polaroid03_C|GetComp_Grab _returnvalue_4) true)
                (Collision|SetActorEnableCollision _returnvalue_4 true)))
            (else
              (Default|TakePhoto02 _returnvalue)
              (bind _returnvalue_6 (Actor|GetActorOfClass "/Game/Lens/Lens03/CameraPhotos/BP_Polaroid02.BP_Polaroid02_C"))
              (Rendering|SetActorHiddenInGame _returnvalue_6 false)
              (bind _returnvalue_7 (Actor|GetActorOfClass "/Game/Lens/Lens03/CameraPhotos/BP_InstantPhotoCamera_Cool.BP_InstantPhotoCamera_Cool_C"))
              (Transformation|SetActorTransform _returnvalue_6 (Math|Transform|MakeTransform (.location (Transformation|GetWorldTransform (Variables|/Game/Lens/Lens03/CameraPhotos/BP_InstantPhotoCamera_Cool.BP_InstantPhotoCamera_Cool_C|GetArrow _returnvalue_7))) (.rotation (Transformation|GetWorldTransform (Variables|/Game/Lens/Lens03/CameraPhotos/BP_InstantPhotoCamera_Cool.BP_InstantPhotoCamera_Cool_C|GetArrow _returnvalue_7))) "0.065000,0.065000,0.065000"))
              (Default|SetGrabEnabled (Variables|/Game/Lens/Lens03/CameraPhotos/BP_Polaroid02.BP_Polaroid02_C|GetComp_Grab _returnvalue_6) true)
              (Collision|SetActorEnableCollision _returnvalue_6 true)))
          (else
            (Default|TakePhoto01 _returnvalue)
            (bind _returnvalue_8 (Actor|GetActorOfClass "/Game/Lens/Lens03/CameraPhotos/BP_Polaroid01.BP_Polaroid01_C"))
            (Rendering|SetActorHiddenInGame _returnvalue_8 false)
            (bind _returnvalue_9 (Actor|GetActorOfClass "/Game/Lens/Lens03/CameraPhotos/BP_InstantPhotoCamera_Cool.BP_InstantPhotoCamera_Cool_C"))
            (Transformation|SetActorTransform _returnvalue_8 (Math|Transform|MakeTransform (.location (Transformation|GetWorldTransform (Variables|/Game/Lens/Lens03/CameraPhotos/BP_InstantPhotoCamera_Cool.BP_InstantPhotoCamera_Cool_C|GetArrow _returnvalue_9))) (.rotation (Transformation|GetWorldTransform (Variables|/Game/Lens/Lens03/CameraPhotos/BP_InstantPhotoCamera_Cool.BP_InstantPhotoCamera_Cool_C|GetArrow _returnvalue_9))) "0.065000,0.065000,0.065000"))
            (Default|SetGrabEnabled (Variables|/Game/Lens/Lens03/CameraPhotos/BP_Polaroid01.BP_Polaroid01_C|GetComp_Grab _returnvalue_8) true)
            (Collision|SetActorEnableCollision _returnvalue_8 true))))
      (:then_1
        (Utilities|FlowControl|Delay 0.2)
        (Default|Toggle (Variables|Default|GetComp_Switch))))))

(event EventBeginPlay
  (bind _returnvalue (Actor|GetActorOfClass "/Game/Lens/Lens03/CameraPhotos/BP_Polaroid01.BP_Polaroid01_C"))
  (bind _returnvalue_2 (Actor|GetActorOfClass "/Game/Lens/Lens03/CameraPhotos/BP_Polaroid02.BP_Polaroid02_C"))
  (bind _returnvalue_3 (Actor|GetActorOfClass "/Game/Lens/Lens03/CameraPhotos/BP_Polaroid03.BP_Polaroid03_C"))
  (bind _returnvalue_4 (Actor|GetActorOfClass "/Game/Lens/Lens03/CameraPhotos/BP_Polaroid04.BP_Polaroid04_C"))
  (Rendering|SetActorHiddenInGame _returnvalue true)
  (Default|SetGrabEnabled (Variables|/Game/Lens/Lens03/CameraPhotos/BP_Polaroid04.BP_Polaroid04_C|GetComp_Grab _returnvalue_4) false)
  (Collision|SetActorEnableCollision _returnvalue false))

(fn ConstructionScript)