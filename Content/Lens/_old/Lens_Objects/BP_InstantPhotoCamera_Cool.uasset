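; Instant photo camera with four photo slots, each backed by its own scene capture component.
; Each TakePhoto function freezes a capture into a new render target in the Reel, exports a player-named PNG and uploads it through HttpSenderActor.
; Outside Lens_Tutorial, SavePhotos reports camera transform and time to BP_GameManager_03, then writes and uploads a text log.
; RemovePhoto clears a slot and restores live capture to the shared render target.
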(event EventBeginPlay)

(fn ConstructionScript)

(fn TakePhoto01
  (bind _returnvalue (Class|KismetSystemLibrary|GetProjectSavedDirectory))
  (bind _scenecapturecomponent2d01 (Variables|Default|GetSceneCaptureComponent2D01))
  (bind _returnvalue_2 (Utilities|String|Append _returnvalue "/Data/Photos"))
  (bind _result (Math|Integer|IncrementInt (Variables|Default|GettimesPhotoTaken01))
    (:%20%20
      (bind _asbp_game_instance_main (Utilities|Casting|CastToBP_GameInstance_Main (Game|GetGameInstance)))
      (bind _returnvalue_3 (Rendering|CreateRenderTarget2D 256 256 "RTF_RGBA8"))
      (bind _output_get (Variables|/Script/Engine.SceneCaptureComponent2D|SetTextureTarget _scenecapturecomponent2d01 _returnvalue_3))
      (Rendering|SceneCapture|CaptureScene _scenecapturecomponent2d01 :!class /Script/Engine.SceneCaptureComponent2D)
      (Rendering|ExportRenderTarget _output_get _returnvalue_2 (Utilities|String|Append "photo_" (Variables|/Game/AFCore/Blueprints/Game/BP_GameInstance_Main.BP_GameInstance_Main_C|GetplayerName _asbp_game_instance_main) "_" "01" "_" (Utilities|String|ToString(Integer) _result) ".png"))
      (bind _returnvalue_4 (Actor|GetActorOfClass "/Script/TheVirtualCode.HttpSenderActor"))
      (Class|HttpSenderActor|SendPngFile _returnvalue_4 (Utilities|String|Append _returnvalue_2 "/" (Utilities|String|Append "photo_" (Variables|/Game/AFCore/Blueprints/Game/BP_GameInstance_Main.BP_GameInstance_Main_C|GetplayerName _asbp_game_instance_main) "_" "01" "_" (Utilities|String|ToString(Integer) _result) ".png")))
      (Variables|/Script/Engine.SceneCaptureComponent|SetbCaptureEveryFrame _scenecapturecomponent2d01 false)
      (Utilities|Array|SetArrayElem (Variables|Default|Getreel) 0 _returnvalue_3 true)
      (Variables|Default|SetphotoTaken01 true)
      (CallFunction|SavePhotos 1)
      (return true))))

(fn TakePhoto02
  (bind _returnvalue (Class|KismetSystemLibrary|GetProjectSavedDirectory))
  (bind _scenecapturecomponent2d02 (Variables|Default|GetSceneCaptureComponent2D02))
  (bind _returnvalue_2 (Utilities|String|Append _returnvalue "/Data/Photos"))
  (bind _result (Math|Integer|IncrementInt (Variables|Default|GettimesPhotoTaken02))
    (:%20%20
      (bind _asbp_game_instance_main (Utilities|Casting|CastToBP_GameInstance_Main (Game|GetGameInstance)))
      (bind _returnvalue_3 (Rendering|CreateRenderTarget2D 256 256 "RTF_RGBA8"))
      (bind _output_get (Variables|/Script/Engine.SceneCaptureComponent2D|SetTextureTarget _scenecapturecomponent2d02 _returnvalue_3))
      (Rendering|SceneCapture|CaptureScene _scenecapturecomponent2d02 :!class /Script/Engine.SceneCaptureComponent2D)
      (Rendering|ExportRenderTarget _output_get _returnvalue_2 (Utilities|String|Append "photo_" (Variables|/Game/AFCore/Blueprints/Game/BP_GameInstance_Main.BP_GameInstance_Main_C|GetplayerName _asbp_game_instance_main) "_" "02" "_" (Utilities|String|ToString(Integer) _result) ".png"))
      (bind _returnvalue_4 (Actor|GetActorOfClass "/Script/TheVirtualCode.HttpSenderActor"))
      (Class|HttpSenderActor|SendPngFile _returnvalue_4 (Utilities|String|Append _returnvalue_2 "/" (Utilities|String|Append "photo_" (Variables|/Game/AFCore/Blueprints/Game/BP_GameInstance_Main.BP_GameInstance_Main_C|GetplayerName _asbp_game_instance_main) "_" "02" "_" (Utilities|String|ToString(Integer) _result) ".png")))
      (Variables|/Script/Engine.SceneCaptureComponent|SetbCaptureEveryFrame _scenecapturecomponent2d02 false)
      (Utilities|Array|SetArrayElem (Variables|Default|Getreel) 1 _returnvalue_3 true)
      (Variables|Default|SetphotoTaken02 true)
      (CallFunction|SavePhotos 2)
      (return true))))

(fn TakePhoto03
  (bind _returnvalue (Class|KismetSystemLibrary|GetProjectSavedDirectory))
  (bind _scenecapturecomponent2d03 (Variables|Default|GetSceneCaptureComponent2D03))
  (bind _returnvalue_2 (Utilities|String|Append _returnvalue "/Data/Photos"))
  (bind _result (Math|Integer|IncrementInt (Variables|Default|GettimesPhotoTaken03))
    (:%20%20
      (bind _asbp_game_instance_main (Utilities|Casting|CastToBP_GameInstance_Main (Game|GetGameInstance)))
      (bind _returnvalue_3 (Rendering|CreateRenderTarget2D 256 256 "RTF_RGBA8"))
      (bind _output_get (Variables|/Script/Engine.SceneCaptureComponent2D|SetTextureTarget _scenecapturecomponent2d03 _returnvalue_3))
      (Rendering|SceneCapture|CaptureScene _scenecapturecomponent2d03 :!class /Script/Engine.SceneCaptureComponent2D)
      (Rendering|ExportRenderTarget _output_get _returnvalue_2 (Utilities|String|Append "photo_" (Variables|/Game/AFCore/Blueprints/Game/BP_GameInstance_Main.BP_GameInstance_Main_C|GetplayerName _asbp_game_instance_main) "_" "03" "_" (Utilities|String|ToString(Integer) _result) ".png"))
      (bind _returnvalue_4 (Actor|GetActorOfClass "/Script/TheVirtualCode.HttpSenderActor"))
      (Class|HttpSenderActor|SendPngFile _returnvalue_4 (Utilities|String|Append _returnvalue_2 "/" (Utilities|String|Append "photo_" (Variables|/Game/AFCore/Blueprints/Game/BP_GameInstance_Main.BP_GameInstance_Main_C|GetplayerName _asbp_game_instance_main) "_" "03" "_" (Utilities|String|ToString(Integer) _result) ".png")))
      (Variables|/Script/Engine.SceneCaptureComponent|SetbCaptureEveryFrame _scenecapturecomponent2d03 false)
      (Utilities|Array|SetArrayElem (Variables|Default|Getreel) 2 _returnvalue_3 true)
      (Variables|Default|SetphotoTaken03 true)
      (CallFunction|SavePhotos 3)
      (return true))))

(fn TakePhoto04
  (bind _returnvalue (Class|KismetSystemLibrary|GetProjectSavedDirectory))
  (bind _scenecapturecomponent2d04 (Variables|Default|GetSceneCaptureComponent2D04))
  (bind _returnvalue_2 (Utilities|String|Append _returnvalue "/Data/Photos"))
  (bind _result (Math|Integer|IncrementInt (Variables|Default|GettimesPhotoTaken04))
    (:%20%20
      (bind _asbp_game_instance_main (Utilities|Casting|CastToBP_GameInstance_Main (Game|GetGameInstance)))
      (bind _returnvalue_3 (Rendering|CreateRenderTarget2D 256 256 "RTF_RGBA8"))
      (bind _output_get (Variables|/Script/Engine.SceneCaptureComponent2D|SetTextureTarget _scenecapturecomponent2d04 _returnvalue_3))
      (Rendering|SceneCapture|CaptureScene _scenecapturecomponent2d04 :!class /Script/Engine.SceneCaptureComponent2D)
      (Rendering|ExportRenderTarget _output_get _returnvalue_2 (Utilities|String|Append "photo_" (Variables|/Game/AFCore/Blueprints/Game/BP_GameInstance_Main.BP_GameInstance_Main_C|GetplayerName _asbp_game_instance_main) "_" "04" "_" (Utilities|String|ToString(Integer) _result) ".png"))
      (bind _returnvalue_4 (Actor|GetActorOfClass "/Script/TheVirtualCode.HttpSenderActor"))
      (Class|HttpSenderActor|SendPngFile _returnvalue_4 (Utilities|String|Append _returnvalue_2 "/" (Utilities|String|Append "photo_" (Variables|/Game/AFCore/Blueprints/Game/BP_GameInstance_Main.BP_GameInstance_Main_C|GetplayerName _asbp_game_instance_main) "_" "04" "_" (Utilities|String|ToString(Integer) _result) ".png")))
      (Variables|/Script/Engine.SceneCaptureComponent|SetbCaptureEveryFrame _scenecapturecomponent2d04 false)
      (Utilities|Array|SetArrayElem (Variables|Default|Getreel) 3 _returnvalue_3 true)
      (Variables|Default|SetphotoTaken04 true)
      (CallFunction|SavePhotos 4)
      (return true))))

(fn SaveLocationRotationPawn
  (params (readyToSave :type Boolean))
  (bind _returnvalue (Game|GetPlayerCharacter 0))
  (if readyToSave
    (bind _asbp_pawn_vr_hands (Utilities|Casting|CastToBP_Pawn_VR_Hands _returnvalue)
      (:then
        (return (Math|Transform|MakeTransform (Transformation|GetActorLocation _asbp_pawn_vr_hands) (Transformation|GetActorRotation _asbp_pawn_vr_hands))))
      (:CastFailed
        (bind _asbp_pawn_desktop_hands (Utilities|Casting|CastToBP_Pawn_Desktop_Hands _returnvalue))
        (return (Math|Transform|MakeTransform (Transformation|GetActorLocation _asbp_pawn_desktop_hands) (Transformation|GetActorRotation _asbp_pawn_desktop_hands)))))))

(fn SavePhotos
  (params (photo :type Integer))
  (switch int photo
    (:1
      (bind _returnvalue (Game|GetCurrentLevelName true))
      (if (Utilities|Enum|NotEqual(Enum) _returnvalue "Lens_Tutorial")
        (Variables|Default|SetcaptureTime (Utilities|Time|GetGameTimeinSeconds))
        (bind _pawnlocrot (CallFunction|SaveLocationRotationCamera true))
        (bind _returnvalue_2 (Utilities|Array|Add (Variables|Default|GetpawnLocRot) _pawnlocrot))
        (bind _returnvalue_3 (Actor|GetActorOfClass "/Game/Lens/Lens03/BP/BP_GameManager_03.BP_GameManager_03_C"))
        (Default|PhotoTaken _returnvalue_3 (.Location (Math|Transform|BreakTransform _pawnlocrot)) (.Rotation (Math|Transform|BreakTransform _pawnlocrot)) (Variables|Default|GetcaptureTime))
        (CallFunction|CollectDataOfTakenPhotos _returnvalue_2 (Variables|Default|GetcaptureTime))
        (CallFunction|SaveDataOfTakenPhotos :!label _label)))
    (:2
      (bind _returnvalue_4 (Game|GetCurrentLevelName true))
      (if (Utilities|Enum|NotEqual(Enum) _returnvalue_4 "Lens_Tutorial")
        (Variables|Default|SetcaptureTime (Utilities|Time|GetGameTimeinSeconds))
        (bind _pawnlocrot_2 (CallFunction|SaveLocationRotationCamera true))
        (bind _returnvalue_5 (Utilities|Array|Add (Variables|Default|GetpawnLocRot) _pawnlocrot_2))
        (bind _returnvalue_6 (Actor|GetActorOfClass "/Game/Lens/Lens03/BP/BP_GameManager_03.BP_GameManager_03_C"))
        (Default|PhotoTaken _returnvalue_6 (.Location (Math|Transform|BreakTransform _pawnlocrot_2)) (.Rotation (Math|Transform|BreakTransform _pawnlocrot_2)) (Variables|Default|GetcaptureTime))
        (CallFunction|CollectDataOfTakenPhotos _returnvalue_5 (Variables|Default|GetcaptureTime))
        (goto _label)))
    (:3
      (bind _returnvalue_7 (Game|GetCurrentLevelName true))
      (if (Utilities|Enum|NotEqual(Enum) _returnvalue_7 "Lens_Tutorial")
        (Variables|Default|SetcaptureTime (Utilities|Time|GetGameTimeinSeconds))
        (bind _pawnlocrot_3 (CallFunction|SaveLocationRotationCamera true))
        (bind _returnvalue_8 (Utilities|Array|Add (Variables|Default|GetpawnLocRot) _pawnlocrot_3))
        (bind _returnvalue_9 (Actor|GetActorOfClass "/Game/Lens/Lens03/BP/BP_GameManager_03.BP_GameManager_03_C"))
        (Default|PhotoTaken _returnvalue_9 (.Location (Math|Transform|BreakTransform _pawnlocrot_3)) (.Rotation (Math|Transform|BreakTransform _pawnlocrot_3)) (Variables|Default|GetcaptureTime))
        (CallFunction|CollectDataOfTakenPhotos _returnvalue_8 (Variables|Default|GetcaptureTime))
        (goto _label)))
    (:4
      (bind _returnvalue_10 (Game|GetCurrentLevelName true))
      (if (Utilities|Enum|NotEqual(Enum) _returnvalue_10 "Lens_Tutorial")
        (Variables|Default|SetcaptureTime (Utilities|Time|GetGameTimeinSeconds))
        (bind _pawnlocrot_4 (CallFunction|SaveLocationRotationCamera true))
        (bind _returnvalue_11 (Utilities|Array|Add (Variables|Default|GetpawnLocRot) _pawnlocrot_4))
        (bind _returnvalue_12 (Actor|GetActorOfClass "/Game/Lens/Lens03/BP/BP_GameManager_03.BP_GameManager_03_C"))
        (Default|PhotoTaken _returnvalue_12 (.Location (Math|Transform|BreakTransform _pawnlocrot_4)) (.Rotation (Math|Transform|BreakTransform _pawnlocrot_4)) (Variables|Default|GetcaptureTime))
        (CallFunction|CollectDataOfTakenPhotos _returnvalue_11 (Variables|Default|GetcaptureTime))
        (goto _label)))))

(fn ClearPhoto
  (params (index :type Integer))
  (Utilities|Array|SetArrayElem (Variables|Default|Getreel) index (Variables|Default|GettextureRenderNone))
  (Utilities|Array|SetArrayElem :TargetArray (Variables|Default|GetpawnLocRot) :Index index))

(fn RemovePhoto
  (params (photoToRemove :type Integer))
  (bind _scenecapturecomponent2d01 (Variables|Default|GetSceneCaptureComponent2D01))
  (bind _scenecapturecomponent2d02 (Variables|Default|GetSceneCaptureComponent2D02))
  (bind _scenecapturecomponent2d03 (Variables|Default|GetSceneCaptureComponent2D03))
  (bind _scenecapturecomponent2d04 (Variables|Default|GetSceneCaptureComponent2D04))
  (switch int photoToRemove
    (:0
      (CallFunction|ClearPhoto photoToRemove)
      (Variables|Default|SetphotoTaken01 false)
      (Variables|/Script/Engine.SceneCaptureComponent|SetbCaptureEveryFrame _scenecapturecomponent2d01 true)
      (Variables|/Script/Engine.SceneCaptureComponent2D|SetTextureTarget _scenecapturecomponent2d01 "/Game/Lens/Lens03/CameraPhotos/Texture_Photos/RT_InstantPhoto01.RT_InstantPhoto01"))
    (:1
      (CallFunction|ClearPhoto photoToRemove)
      (Variables|Default|SetphotoTaken02 false)
      (Variables|/Script/Engine.SceneCaptureComponent|SetbCaptureEveryFrame _scenecapturecomponent2d02 true)
      (Variables|/Script/Engine.SceneCaptureComponent2D|SetTextureTarget _scenecapturecomponent2d02 "/Game/Lens/Lens03/CameraPhotos/Texture_Photos/RT_InstantPhoto01.RT_InstantPhoto01"))
    (:2
      (CallFunction|ClearPhoto photoToRemove)
      (Variables|Default|SetphotoTaken03 false)
      (Variables|/Script/Engine.SceneCaptureComponent|SetbCaptureEveryFrame _scenecapturecomponent2d03 true)
      (Variables|/Script/Engine.SceneCaptureComponent2D|SetTextureTarget _scenecapturecomponent2d03 "/Game/Lens/Lens03/CameraPhotos/Texture_Photos/RT_InstantPhoto01.RT_InstantPhoto01"))
    (:3
      (CallFunction|ClearPhoto photoToRemove)
      (Variables|Default|SetphotoTaken04 false)
      (Variables|/Script/Engine.SceneCaptureComponent|SetbCaptureEveryFrame _scenecapturecomponent2d04 true)
      (Variables|/Script/Engine.SceneCaptureComponent2D|SetTextureTarget _scenecapturecomponent2d04 "/Game/Lens/Lens03/CameraPhotos/Texture_Photos/RT_InstantPhoto01.RT_InstantPhoto01"))))

(fn CollectDataOfTakenPhotos
  (params (index :type Integer) (captureTime :type Float%20%28double-precision%29))
  (bind _phototakenandpawnlocrot (Variables|Default|GetphotoTakenANDpawnLocRot))
  (for (_array_element _array_index) (Variables|Default|Getreel)
    (if (== _array_index index)
      (Utilities|Array|Add (Variables|Default|GetphotoTakenANDpawnLocRot) (Utilities|GetDisplayName _array_element))
      (for (_array_element_2 _array_index_2) (Variables|Default|GetpawnLocRot)
        (if (== _array_index_2 index)
          (Utilities|Array|Add _phototakenandpawnlocrot (Utilities|String|ToString(Transform) _array_element_2))
          (Utilities|Array|Add _phototakenandpawnlocrot (Utilities|String|Append "Time: " (Utilities|String|ToString(Float) captureTime))))))))

(fn SaveDataOfTakenPhotos
  (bind _returnvalue (Class|KismetSystemLibrary|GetProjectSavedDirectory))
  (bind _returnvalue_2 (Math|DateTime|Now))
  (bind _returnvalue_3 (Utilities|String|Append _returnvalue "/Data"))
  ;[1 1 1] save the data from photo
  (bind _asbp_game_instance_main (Utilities|Casting|CastToBP_GameInstance_Main (Game|GetGameInstance)))
  (Class|VictoryBPFunctionLibrary|FileIOSaveStringArraytoFile _returnvalue_3 (Utilities|String|Append "EVL_" (Utilities|String|ToString(Integer) (.year _returnvalue_2)) (Utilities|String|ToString(Integer) (.month _returnvalue_2)) (Utilities|String|ToString(Integer) (.day _returnvalue_2)) (Utilities|String|ToString(Integer) (.hour _returnvalue_2)) (Utilities|String|ToString(Integer) (.minute _returnvalue_2)) (Utilities|String|ToString(Integer) (.second _returnvalue_2)) "_DataPhotoWhereTook_" (Variables|/Game/AFCore/Blueprints/Game/BP_GameInstance_Main.BP_GameInstance_Main_C|GetplayerName _asbp_game_instance_main) ".txt") (Variables|Default|GetphotoTakenANDpawnLocRot) true true)
  (bind _returnvalue_4 (Actor|GetActorOfClass "/Script/TheVirtualCode.HttpSenderActor"))
  (Class|HttpSenderActor|SendTxtFile _returnvalue_4 (Utilities|String|Append _returnvalue_3 "/" (Utilities|String|Append "EVL_" (Utilities|String|ToString(Integer) (.year _returnvalue_2)) (Utilities|String|ToString(Integer) (.month _returnvalue_2)) (Utilities|String|ToString(Integer) (.day _returnvalue_2)) (Utilities|String|ToString(Integer) (.hour _returnvalue_2)) (Utilities|String|ToString(Integer) (.minute _returnvalue_2)) (Utilities|String|ToString(Integer) (.second _returnvalue_2)) "_DataPhotoWhereTook_" (Variables|/Game/AFCore/Blueprints/Game/BP_GameInstance_Main.BP_GameInstance_Main_C|GetplayerName _asbp_game_instance_main) ".txt"))))

(fn SaveLocationRotationCamera
  (params (readyToSave :type Boolean))
  (bind _camera (Variables|Default|GetCamera))
  (if readyToSave
    (return (Math|Transform|MakeTransform (Transformation|GetWorldLocation _camera) (Transformation|GetWorldRotation _camera)))))